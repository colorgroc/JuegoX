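; Vela_BP is a candle with a point light that flickers and a particle system, likely the flame.
; On BeginPlay it picks random min and max intensities and a random timeline play rate, then a timeline interpolates the light between them so instances vary.
; SetEnabled, also run from the construction script, toggles light and particle visibility and turns off the mesh's shadow casting while enabled.
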(event EventBeginPlay
  (Variables|Default|SetMaxIntensity (Math|Random|RandomFloatinRange (Variables|Default|GetMinimoDelMaximo) (Variables|Default|GetMaximoDelMaximo)))
  (Variables|Default|SetMinIntensity (Math|Random|RandomFloatinRange (Variables|Default|GetMinimoDelMinimo) (Variables|Default|GetMaximoDelMinimo)))
  (Components|Timeline|SetPlayRate (Variables|Default|GetTimeline_0) (Math|Random|RandomFloatinRange 0.8 1.2))
  (bind _intensity (Timeline|Timeline_0 Play)
    (:Update
      (Rendering|Components|Light|SetIntensity (Variables|Default|GetPointLight) (Math|Float|Lerp (Variables|Default|GetMinIntensity) (Variables|Default|GetMaxIntensity) _intensity)))))

(fn ConstructionScript
  (CallFunction|SetEnabled (Variables|Default|GetEnabled)))

(fn SetEnabled
  (params (Enabled :type Boolean))
  (bind _output_get (Variables|Default|SetEnabled Enabled))
  (Rendering|SetVisibility (Variables|Default|GetPointLight) _output_get false)
  (Rendering|SetVisibility (Variables|Default|GetParticleSystem) _output_get false)
  (Rendering|SetCastShadow (Variables|Default|GetStaticMesh) (not _output_get)))