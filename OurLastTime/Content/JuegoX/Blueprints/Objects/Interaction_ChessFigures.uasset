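; Interactable chess figure that highlights its mesh while the player is playing chess.
; Each tick, if interaction is activated, it reads PlayerPlayingChess from the FirstPersonCharacter, looked up by class every time.
; When both conditions hold, it enables custom depth rendering and switches the stencil value according to focus.
; Otherwise it disables custom depth.
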(event EventBeginPlay
  (|CallParentFunction))

(event EventTick
  (params (DeltaSeconds :type Float%20%28single-precision%29))
  (bind _mesh (Variables|Default|GetMesh))
  (if (Variables|Default|GetInteraction_Activated)
    (bind _bool (CallFunction|BoolCheck))
    (if _bool
      (Rendering|SetRenderCustomDepth (Variables|Default|GetMesh) true)
      (if (Variables|Default|GetisFocused?)
        (Rendering|SetCustomDepthStencilValue _mesh 2)
        (else
          (Rendering|SetCustomDepthStencilValue _mesh 1)))
      (else
        (Rendering|SetRenderCustomDepth (Variables|Default|GetMesh) false :!label _label)))
    (else
      (goto _label))))

(fn BoolCheck
  (bind _returnvalue (Actor|GetActorOfClass "/Game/FirstPersonBP/Blueprints/FirstPersonCharacter.FirstPersonCharacter_C"))
  (return (Variables|/Game/FirstPersonBP/Blueprints/FirstPersonCharacter.FirstPersonCharacter_C|GetPlayer%20Playing%20Chess _returnvalue)))