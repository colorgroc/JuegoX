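; Pickup object that the player can inspect, then collect into the GameInstance inventory by its Type.
; It can attach to a container's mesh (LugarDondeEstaGuardada) and refresh its stored interactable transform when that container's finished event fires.
; Interacting hides the collect/drop HUD, ends inspection and adds the item.
; At interaction end, small items such as keys or cassettes are destroyed, while body parts are only hidden with their collision profile changed.
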(event Custom|End_Of_interaction
  (bind _mesh (Variables|Character|GetMesh))
  (switch Utilities|FlowControl|Switch|SwitchonEnum_Inventory_Items (Variables|Default|Gettype)
    (:NewEnumerator0
      (Actor|DestroyActor :!label _label))
    (:NewEnumerator10
      (goto _label))
    (:NewEnumerator1
      (goto _label))
    (:NewEnumerator2
      (goto _label))
    (:NewEnumerator3
      (goto _label))
    (:NewEnumerator4
      (goto _label))
    (:NewEnumerator5
      (Collision|SetCollisionProfileName _mesh "NoColiision" :!class /Script/Engine.PrimitiveComponent :!label _label_2)
      (Rendering|SetVisibility _mesh false true))
    (:NewEnumerator6
      (goto _label_2))
    (:NewEnumerator7
      (goto _label_2))
    (:NewEnumerator8
      (goto _label_2))
    (:NewEnumerator9
      (goto _label_2))))

(event Custom|Has%20item%20to%20true)

(event Custom|Update%20Positions
  (Variables|/Game/JuegoX/Blueprints/Objects/Interactable.Interactable_C|SetinitialRot (Variables|Default|GetInteractable) (Transformation|GetActorRotation))
  (Variables|/Game/JuegoX/Blueprints/Objects/Interactable.Interactable_C|SetinitialPos (Variables|Default|GetInteractable) (Transformation|GetActorLocation)))

(event EventTick
  (params (DeltaSeconds :type Float%20%28single-precision%29))
  (Utilities|IsValid (Variables|Savedinaclosed|GetlugarDondeEstaGuardada)
    (:Is%20Valid
      (EventDispatchers|BindEventtoFinished (Variables|Savedinaclosed|GetlugarDondeEstaGuardada) (delegate Custom|Update%20Positions)))
    (:Is%20Not%20Valid
      (if (and (Utilities|Enum|Equal(Enum) (Variables|Default|Gettype) "NewEnumerator10") (Variables|/Game/JuegoX/Blueprints/Objects/Interactable.Interactable_C|GetfadeE (Variables|Default|GetInteractable)))
        (CallFunction|UpdatePositions))))
  (|CallParentFunction DeltaSeconds))

(event EventInteract
  (CallFunction|HideHUD)
  (CallFunction|HasItemtoTrue)
  (Variables|/Game/JuegoX/Blueprints/Objects/Interactable.Interactable_C|SetisInspectingIt (Variables|Default|GetInteractable) false)
  (Variables|/Game/FirstPersonBP/Blueprints/FirstPersonCharacter.FirstPersonCharacter_C|SetplayerInspectingObject (Variables|Default|Getplayer) false)
  (Variables|/Game/JuegoX/Blueprints/Objects/Interactable.Interactable_C|SetinteractionActivated (Variables|Default|GetInteractable) false)
  (Default|AddItem (Variables|/Game/JuegoX/Blueprints/MyGameInstance.MyGameInstance_C|GetInventory (Variables|Default|GetGameInstance)) (Variables|Default|Gettype))
  (CallFunction|EndOfInteraction))

(event EventBeginPlay
  (bind _lugardondeestaguardada (Variables|Savedinaclosed|GetlugarDondeEstaGuardada))
  (|CallParentFunction)
  (Utilities|IsValid _lugardondeestaguardada
    (:Is%20Valid
      (Transformation|AttachComponentToComponent (Variables|/Game/JuegoX/Blueprints/Objects/Interactable_Static/Dressers/OBJ_Furniture.OBJ_Furniture_C|GetMesh _lugardondeestaguardada) "None" "KeepWorld" "KeepWorld" "KeepWorld" true))))

(event EventShowHUD
  (Default|PlayINControls2 (Variables|Default|GetGameInstance) "collect" "drop"))

(event EventHideHUD
  (Default|PlayOUTControls2 (Variables|Default|GetGameInstance)))

(fn ConstructionScript
  (|CallParentFunction))