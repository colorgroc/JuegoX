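; Base interactable world object that the first-person player can inspect up close, with empty Interact and HUD-text hooks, apparently for children to override.
; Tick enables input only while interaction is activated and the object is focused or inspected, so Inspect toggles inspection and Interact works during it.
; A timeline lerps the object to a point before the camera and reverses it back, while GameInstance handles HUD prompts and gamepad/keyboard detection.
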(event Custom|Set_Initial_grab%20spot)

(event Custom|Inspection
  (if (Variables|/Game/JuegoX/Blueprints/Objects/Interactable.Interactable_C|GetisInspectingIt (Variables|Default|GetInteractable))
    (CallFunction|EndInspection)
    (else
      (Utilities|FlowControl|Sequence
        (:then_0
          ;[1 1 1] Sound being played
          (Class|FMODBlueprintStatics|PlayEvent2D (Variables|Default|GetFMOD_Sound)))
        (:then_1
          (CallFunction|BeginInspection))))))

(event Custom|DemianKey_Glasses)

(event Custom|HUD%20Text%20Object%20Play%20IN)

(event Custom|EndInspection
  (Variables|/Game/FirstPersonBP/Blueprints/FirstPersonCharacter.FirstPersonCharacter_C|SetObjetoInspeccionandose (Variables|Default|Getplayer) 0)
  (CallFunction|HideHUD)
  (CallFunction|HUDTextObjectPlayOUT)
  (Variables|/Game/JuegoX/Blueprints/Objects/Interactable.Interactable_C|SetisInspectingIt (Variables|Default|GetInteractable) false)
  (Variables|/Game/FirstPersonBP/Blueprints/FirstPersonCharacter.FirstPersonCharacter_C|SetplayerInspectingObject (Variables|Default|Getplayer) false)
  (bind (_direction _move_object) (Timeline|inpection%20Timeline Reverse)
    (:Update
      (CallFunction|UpdateLocation _move_object))
    (:Finished
      (if (Utilities|Enum|Equal(Enum) _direction "Backward")
        (Variables|/Game/JuegoX/Blueprints/Objects/Interactable.Interactable_C|SetfadeE (Variables|Default|GetInteractable) true)
        (CallFunction|HideHUD)
        (CallFunction|HUDTextObjectPlayOUT)))))

(event Custom|HUD%20Text%20Object%20Play%20OUT)

(event Custom|BeginInspection
  (Utilities|FlowControl|Sequence
    (:then_0
      (CallFunction|ShowHUD)
      (CallFunction|HUDTextObjectPlayIN))
    (:then_1
      (CallFunction|InspectionView)
      (Variables|/Game/JuegoX/Blueprints/Objects/Interactable.Interactable_C|SetisInspectingIt (Variables|Default|GetInteractable) true)
      (Variables|/Game/FirstPersonBP/Blueprints/FirstPersonCharacter.FirstPersonCharacter_C|SetplayerInspectingObject (Variables|Default|Getplayer) true)
      (Variables|/Game/JuegoX/Blueprints/Objects/Interactable.Interactable_C|SetfadeE (Variables|Default|GetInteractable) false)
      (bind (_direction _move_object) (Timeline|inpection%20Timeline Play)
        (:Update
          (CallFunction|UpdateLocation _move_object))
        (:Finished
          (if (Utilities|Enum|Equal(Enum) _direction "Backward")
            (Variables|/Game/JuegoX/Blueprints/Objects/Interactable.Interactable_C|SetfadeE (Variables|Default|GetInteractable) true)
            (CallFunction|HideHUD)
            (CallFunction|HUDTextObjectPlayOUT)))))))

(event EventBeginPlay
  (Variables|/Game/JuegoX/Blueprints/Objects/Interactable.Interactable_C|SetfadeE (Variables|Default|GetInteractable) true)
  (bind _returnvalue (Actor|GetActorOfClass "/Game/FirstPersonBP/Blueprints/FirstPersonCharacter.FirstPersonCharacter_C"))
  (bind _output_get (Variables|Default|Setplayer _returnvalue))
  (Variables|/Game/JuegoX/Blueprints/Objects/Interactable.Interactable_C|Setplayer (Variables|Default|GetInteractable) _output_get)
  (bind _asmy_game_instance (Utilities|Casting|CastToMyGameInstance (Game|GetGameInstance)))
  (Variables|Default|SetGameInstance _asmy_game_instance)
  (Variables|/Game/JuegoX/Blueprints/Objects/Interactable.Interactable_C|SetinitialRot (Variables|Default|GetInteractable) (Transformation|GetActorRotation))
  (Variables|/Game/JuegoX/Blueprints/Objects/Interactable.Interactable_C|SetinitialPos (Variables|Default|GetInteractable) (Transformation|GetActorLocation)))

(event EventTick
  (params (DeltaSeconds :type Float%20%28single-precision%29))
  (bind _returnvalue (Game|GetPlayerController 0))
  (if (Variables|/Game/JuegoX/Blueprints/Objects/Interactable.Interactable_C|GetinteractionActivated (Variables|Default|GetInteractable))
    (if (Variables|/Game/JuegoX/Blueprints/Objects/Interactable.Interactable_C|GetisInspectingIt (Variables|Default|GetInteractable))
      (Input|EnableInput _returnvalue :!label _label)
      (elif (Variables|/Game/JuegoX/Blueprints/Objects/Interactable.Interactable_C|GetisFocused? (Variables|Default|GetInteractable))
        (goto _label)
        (else
          (Input|DisableInput _returnvalue :!label _label_2))))
    (else
      (goto _label_2))))

(event Input|ActionEvents|InputActionInteract
  (params (Key :type Key%20Structure :default "None"))
  (:Pressed
    (Utilities|FlowControl|Sequence
      (:then_0
        (Default|CheckInput (Variables|Default|GetGameInstance) Key))
      (:then_1
        (if (Variables|/Game/JuegoX/Blueprints/Objects/Interactable.Interactable_C|GetisInspectingIt (Variables|Default|GetInteractable))
          (CallFunction|Interact))))))

(event Input|ActionEvents|InputActionInspect
  (params (Key :type Key%20Structure :default "None"))
  (:Pressed
    (Utilities|FlowControl|Sequence
      (:then_0
        (Default|CheckInput (Variables|Default|GetGameInstance) Key))
      (:then_1
        (CallFunction|Inspection)))))

(fn ConstructionScript
  (Variables|/Game/JuegoX/Blueprints/Objects/Interactable.Interactable_C|SetMesh (Variables|Default|GetInteractable) (Variables|Default|GetMesh))
  (Variables|/Game/JuegoX/Blueprints/Objects/Interactable.Interactable_C|SetBillboard (Variables|Default|GetInteractable) (Variables|Default|GetBillboard))
  (Variables|Default|SetinspectionDistance 4e+01)
  (Variables|/Game/JuegoX/Blueprints/Objects/Interactable.Interactable_C|SetAperture_Focus (Variables|Default|GetInteractable) 1.0))

(fn Interact)

(fn UpdateLocation
  (params (timeline%20Value :type Float%20%28single-precision%29))
  (bind _interactable (Variables|Default|GetInteractable))
  (Transformation|SetActorLocationAndRotation (Math|Vector|Lerp(Vector) (Variables|/Game/JuegoX/Blueprints/Objects/Interactable.Interactable_C|GetinitialPos _interactable) (Variables|/Game/JuegoX/Blueprints/Objects/Interactable.Interactable_C|GetinspectionPoint _interactable) timeline%20Value) (Math|Rotator|Lerp(Rotator) (Variables|/Game/JuegoX/Blueprints/Objects/Interactable.Interactable_C|GetinitialRot _interactable) (Transformation|GetActorRotation) timeline%20Value true) true))

(fn InspectionView
  (bind _player (Variables|Default|Getplayer))
  (bind _firstpersoncamera (Variables|/Game/FirstPersonBP/Blueprints/FirstPersonCharacter.FirstPersonCharacter_C|GetFirstPersonCamera _player))
  (Variables|/Game/JuegoX/Blueprints/Objects/Interactable.Interactable_C|SetinspectionPoint (Variables|Default|GetInteractable) (+ (Transformation|GetWorldLocation _firstpersoncamera) (* (Math|Vector|GetForwardVector (Transformation|GetWorldRotation _firstpersoncamera)) (Variables|Default|GetinspectionDistance)))))

(fn ShowHUD
  (bind _gameinstance (Variables|Default|GetGameInstance))
  (Default|PlayINControls1 (Variables|Default|GetGameInstance) "drop")
  (if (Variables|/Game/JuegoX/Blueprints/MyGameInstance.MyGameInstance_C|GetHas_Glasses? _gameinstance)
    (Default|PlayOUTGlasses _gameinstance)))

(fn HideHUD
  (bind _gameinstance (Variables|Default|GetGameInstance))
  (bind _gameinstance_2 (Variables|Default|GetGameInstance))
  (Default|PlayOUTControls1 _gameinstance)
  (Default|PlayOUTControls2 _gameinstance)
  (Default|PlayOUTControls3 _gameinstance)
  (if (Variables|/Game/JuegoX/Blueprints/MyGameInstance.MyGameInstance_C|GetHas_Glasses? _gameinstance_2)
    (Default|PlayINGlasses _gameinstance_2)))

(fn SetIntensityLight
  (Variables|/Game/FirstPersonBP/Blueprints/FirstPersonCharacter.FirstPersonCharacter_C|SetlightIntensity (Variables|Default|Getplayer) 1e+02))