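; Interactable component that highlights its owner and shows an interaction prompt for the first-person player.
; Tick sets a custom-depth stencil outline by focus, distance and player inspection state, using separate values for nearby and focused objects.
; A looping timer blinks the glow of nearby important objects while unfocused.
; ShowE toggles up to two billboards by focus and inspection state, swapping keyboard and gamepad sprites.
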(event EventBeginPlay
  (bind _returnvalue (Components|GetOwner))
  (bind _returnvalue_2 (Transformation|GetActorRotation _returnvalue))
  (Variables|Inspection|SetisFocused? false)
  (Variables|Inspection|SetisInspectingIt false)
  (Variables|Default|SetinitialPos (Transformation|GetActorLocation (Components|GetOwner)))
  (Variables|Default|SetinitialRot (Transformation|GetActorRotation (Components|GetOwner)))
  (Variables|Default|SetInitial%20Right%20Vector (Math|Vector|GetRightVector _returnvalue_2))
  (Variables|Default|Setinitial%20up%20vector (Math|Vector|GetUpVector _returnvalue_2))
  (Utilities|IsValid (Variables|Default|GetMesh) :!label _label
    (:Is%20Valid
      (bind _returnvalue_3 (Actor|GetActorOfClass "/Game/FirstPersonBP/Blueprints/FirstPersonCharacter.FirstPersonCharacter_C"))
      (Variables|Default|Setplayer _returnvalue_3)
      (if (Variables|Highlight|GetisImportant?)
        (Utilities|Time|SetTimerbyFunctionName 0 "importantObject" 0.4 true)))
    (:Is%20Not%20Valid
      (Utilities|FlowControl|Delay 0.2)
      (goto _label))))

(event EventTick
  (params (DeltaSeconds :type Float%20%28single-precision%29))
  (bind _billboard_2 (Variables|Default|GetBillboard_2))
  (bind _billboard (Variables|Default|GetBillboard))
  (Utilities|IsValid (Variables|Default|GetMesh)
    (:Is%20Valid
      (if (Variables|Interaction|GetinteractionActivated)
        (CallFunction|ShowE)
        (if (Variables|/Game/FirstPersonBP/Blueprints/FirstPersonCharacter.FirstPersonCharacter_C|GetplayerInspectingObject (Variables|Default|Getplayer))
          (CallFunction|RenderOutline false)
          (elif (Variables|Inspection|GetisFocused?)
            (if (Variables|Default|GetfadeE)
              (CallFunction|RenderOutline true 2))
            (elif (not (Variables|Highlight|GetisImportant?))
              (if (Variables|/Game/FirstPersonBP/Blueprints/FirstPersonCharacter.FirstPersonCharacter_C|GetplayerInpectingMapa (Variables|Default|Getplayer))
                (CallFunction|RenderOutline false)
                (else
                  (Math|Float|CompareFloat (Transformation|GetDistanceTo (Components|GetOwner) (Pawn|GetControlledPawn (Game|GetPlayerController 0))) (Variables|Highlight|GetDistance%20to%20Glow)
                    (:>
                      (CallFunction|RenderOutline false))
                    (:==
                      (CallFunction|RenderOutline true 1 :!label _label))
                    (:<
                      (goto _label))))))))
        (else
          (CallFunction|RenderOutline false)
          (Variables|Inspection|SetisFocused? false)
          (Rendering|SetVisibility _billboard false false)
          (Utilities|ChangeBillboard _billboard
            (:Output
              (Utilities|IsValid _billboard_2
                (:Is%20Valid
                  (Rendering|SetVisibility _billboard_2 false false)
                  (Utilities|ChangeBillboard _billboard_2))))))))
    (:Is%20Not%20Valid
      (Variables|Inspection|SetisFocused? false))))

(fn ImportantObject
  (Utilities|IsValid (Variables|Default|GetMesh)
    (:Is%20Valid
      (if (not (Variables|Inspection|GetisFocused?))
        (Math|Float|CompareFloat (Transformation|GetDistanceTo (Components|GetOwner) (Game|GetPlayerCharacter 0)) (Variables|Highlight|GetDistance%20to%20Glow)
          (:>
            (CallFunction|RenderOutline false :!label _label)
            (Variables|Highlight|Settimer 0)
            (Variables|Default|SetnotHighlighting true))
          (:==
            (if (> (Variables|Highlight|Gettimer) 1) :!label _label_2
              (goto _label)
              (else
                (CallFunction|RenderOutline true 1)
                (Math|Integer|IncrementInt (Variables|Highlight|Gettimer)
                  (:%20%20
                    (Variables|Default|SetnotHighlighting false))))))
          (:<
            (goto _label_2)))))))

(fn ShowE
  (bind _billboard (Variables|Default|GetBillboard))
  (bind _billboard_2 (Variables|Default|GetBillboard))
  (bind _billboard_3 (Variables|Default|GetBillboard))
  (bind _billboard_2 (Variables|Default|GetBillboard_2))
  (bind _billboard_4 (Variables|Default|GetBillboard))
  (bind _billboard_2_2 (Variables|Default|GetBillboard_2))
  (bind _billboard_2_3 (Variables|Default|GetBillboard_2))
  (bind _billboard_2_4 (Variables|Default|GetBillboard_2))
  (if (and (Variables|Inspection|GetisFocused?) (Variables|Interaction|GetinteractionActivated))
    (if (Variables|Default|Getis%20a%20nonInspectionable%20Object?)
      (Rendering|SetVisibility _billboard true false)
      (Utilities|ChangeBillboard _billboard
        (:Output
          (Utilities|IsValid _billboard_2_4
            (:Is%20Valid
              (Rendering|SetVisibility _billboard_2_4 true false)
              (Utilities|ChangeBillboard _billboard_2_4)))))
      (elif (Variables|Inspection|GetisInspectingIt)
        (Rendering|SetVisibility _billboard_2 false false)
        (Utilities|ChangeBillboard _billboard_2
          (:Output
            (Utilities|IsValid _billboard_2_3
              (:Is%20Valid
                (Rendering|SetVisibility _billboard_2_3 false false)
                (Utilities|ChangeBillboard _billboard_2_3)))))
        (elif (Variables|Default|GetfadeE)
          (Rendering|SetVisibility _billboard_3 true false)
          (Utilities|ChangeBillboard _billboard_3
            (:Output
              (Utilities|IsValid _billboard_2_2
                (:Is%20Valid
                  (Rendering|SetVisibility _billboard_2_2 true false)
                  (Utilities|ChangeBillboard _billboard_2_2))))))))
    (else
      (Rendering|SetVisibility _billboard_4 false false)
      (Utilities|ChangeBillboard _billboard_4
        (:Output
          (Utilities|IsValid _billboard_2
            (:Is%20Valid
              (Rendering|SetVisibility _billboard_2 false false)
              (Utilities|ChangeBillboard _billboard_2))))))))

(fn RenderOutline
  (params (Outline? :type Boolean) (Type%20of%20outline :type Integer))
  (Rendering|SetRenderCustomDepth (Variables|Default|GetMesh) Outline?)
  (for _array_element (Variables|Default|GetArray_Extra_Meshes)
    (Rendering|SetRenderCustomDepth _array_element Outline?))
  (if Outline?
    (Rendering|SetCustomDepthStencilValue (Variables|Default|GetMesh) Type%20of%20outline)
    (for _array_element_2 (Variables|Default|GetArray_Extra_Meshes)
      (Rendering|SetCustomDepthStencilValue _array_element_2 Type%20of%20outline))))

(fn BlinkOutline
  (Utilities|IsValid (Variables|Default|GetMesh)
    (:Is%20Valid
      (if (Variables|Inspection|GetisFocused?)
        (if (> (Variables|Highlight|Gettimer) 1)
          (CallFunction|RenderOutline false)
          (Variables|Highlight|Settimer 0)
          (else
            (CallFunction|RenderOutline true 2)
            (Math|Integer|IncrementInt (Variables|Highlight|Gettimer))))))))