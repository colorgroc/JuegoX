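; Interactable chess square that highlights while the player is playing chess.
; On BeginPlay it creates a dynamic white or black material instance based on the mesh's current material.
; Each Tick it reads PlayerPlayingChess from the FirstPersonCharacter.
; When playing and Glowing, it enables custom depth and sets stencil, glow and overlay color by focus state; otherwise it clears both depth and glow.
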(event EventBeginPlay
  (bind _mesh (Variables|Default|GetMesh))
  (|CallParentFunction)
  (if (== (Rendering|Material|GetMaterial (Variables|Default|GetMesh) 0) "/Game/Materiales/Zeus/Zeus_FichasBlancas_Mat_Inst.Zeus_FichasBlancas_Mat_Inst")
    (bind _returnvalue (Rendering|Material|CreateDynamicMaterialInstance _mesh 0 "/Game/Materiales/Zeus/Zeus_FichasBlancas_Mat_Inst.Zeus_FichasBlancas_Mat_Inst" "None" :!class /Script/Engine.PrimitiveComponent))
    (Variables|Default|Setmaterial _returnvalue)
    (else
      (bind _returnvalue_2 (Rendering|Material|CreateDynamicMaterialInstance _mesh 0 "/Game/Materiales/Zeus/Zeus_FichasNegras_Mat_Inst.Zeus_FichasNegras_Mat_Inst" "None" :!class /Script/Engine.PrimitiveComponent))
      (Variables|Default|Setmaterial _returnvalue_2))))

(event EventTick
  (params (DeltaSeconds :type Float%20%28single-precision%29))
  (bind _mesh (Variables|Default|GetMesh))
  (bind _material (Variables|Default|Getmaterial))
  (bind _bool (CallFunction|BoolCheck))
  (if _bool
    (if (Variables|Default|GetGlowing)
      (Rendering|SetRenderCustomDepth (Variables|Default|GetMesh) true)
      (if (Variables|Default|GetisFocused?)
        (Rendering|SetCustomDepthStencilValue _mesh 2)
        (Rendering|Material|SetScalarParameterValue _material "Glow" 0.3 :!class /Script/Engine.MaterialInstanceDynamic)
        (Rendering|Material|SetVectorParameterValue _material "OverlayColor" "(R=1.000000,G=0.372549,B=0.000000,A=1.000000)" :!class /Script/Engine.MaterialInstanceDynamic)
        (else
          (Rendering|SetCustomDepthStencilValue _mesh 1)
          (Rendering|Material|SetScalarParameterValue _material "Glow" 0.3 :!class /Script/Engine.MaterialInstanceDynamic)
          (Rendering|Material|SetVectorParameterValue _material "OverlayColor" "(R=1.000000,G=0.878431,B=0.709804,A=1.000000)" :!class /Script/Engine.MaterialInstanceDynamic)))
      (else
        (Rendering|SetRenderCustomDepth (Variables|Default|GetMesh) false :!label _label)
        (Rendering|Material|SetScalarParameterValue (Variables|Default|Getmaterial) "Glow" 0.0 :!class /Script/Engine.MaterialInstanceDynamic)))
    (else
      (goto _label))))

(fn BoolCheck
  (bind _returnvalue (Actor|GetActorOfClass "/Game/FirstPersonBP/Blueprints/FirstPersonCharacter.FirstPersonCharacter_C"))
  (return (Variables|/Game/FirstPersonBP/Blueprints/FirstPersonCharacter.FirstPersonCharacter_C|GetPlayer%20Playing%20Chess _returnvalue)))