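; Corridor prop Blueprint that makes stacked boxes appear to fall when the box trigger is overlapped.
; A one-shot overlap swaps five placed meshes for five fallen ones by toggling visibility and collision, without animation or simulation.
; It also sets the Box component to block all, sets and prints the SeHanCaido flag, and destroys the trigger.
; Overlapping the sound trigger afterwards only destroys that trigger; no sound plays in this graph.
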(event OnComponentBeginOverlap(Trigger_Boxes)
  (params (OverlappedComponent :type Primitive%20Component%20Object%20Reference) (OtherActor :type Actor%20Object%20Reference) (OtherComp :type Primitive%20Component%20Object%20Reference) (OtherBodyIndex :type Integer) (bFromSweep :type Boolean) (SweepResult :type Hit%20Result%20Structure%20%28by%20ref%29))
  (bind _cajacolocada_05 (Variables|Default|GetCajaColocada_05))
  (bind _cajatirada_01 (Variables|Default|GetCajaTirada_01))
  (bind _cajatirada_02 (Variables|Default|GetCajaTirada_02))
  (bind _cajatirada_03 (Variables|Default|GetCajaTirada_03))
  (bind _cajatirada_04 (Variables|Default|GetCajaTirada_04))
  (bind _cajacolocada_01 (Variables|Default|GetCajaColocada_01))
  (bind _cajatirada_05 (Variables|Default|GetCajaTirada_05))
  (bind _cajacolocada_02 (Variables|Default|GetCajaColocada_02))
  (bind _cajacolocada_03 (Variables|Default|GetCajaColocada_03))
  (bind _cajacolocada_04 (Variables|Default|GetCajaColocada_04))
  (Utilities|FlowControl|DoOnce false
    (:Completed
      (Utilities|FlowControl|Sequence
        (:then_0
          (Development|SetHiddeninGame _cajacolocada_01 true false)
          (Development|SetHiddeninGame _cajacolocada_02 true false)
          (Development|SetHiddeninGame _cajacolocada_03 true false)
          (Development|SetHiddeninGame _cajacolocada_04 true false)
          (Development|SetHiddeninGame _cajacolocada_05 true false)
          (Development|SetHiddeninGame _cajatirada_01 false false)
          (Development|SetHiddeninGame _cajatirada_02 false false)
          (Development|SetHiddeninGame _cajatirada_03 false false)
          (Development|SetHiddeninGame _cajatirada_04 false false)
          (Development|SetHiddeninGame _cajatirada_05 false false)
          (Collision|SetCollisionProfileName (Variables|Default|GetBox) "BlockAll" :!class /Script/Engine.PrimitiveComponent)
          (bind _output_get (Variables|Default|SetSeHanCaido true))
          (Development|PrintString (Utilities|String|ToString(Boolean) _output_get) true true "(R=0.000000,G=1.000000,B=0.081434,A=1.000000)")
          (Components|DestroyComponent (Variables|Default|GetTrigger_Boxes)))
        (:then_1
          (Collision|SetCollisionEnabled _cajacolocada_01 "NoCollision")
          (Collision|SetCollisionEnabled _cajacolocada_02 "NoCollision")
          (Collision|SetCollisionEnabled _cajacolocada_03 "NoCollision")
          (Collision|SetCollisionEnabled _cajacolocada_04 "NoCollision")
          (Collision|SetCollisionEnabled _cajacolocada_05 "NoCollision")
          (Collision|SetCollisionEnabled _cajatirada_01 "QueryAndPhysics")
          (Collision|SetCollisionEnabled _cajatirada_02 "QueryAndPhysics")
          (Collision|SetCollisionEnabled _cajatirada_03 "QueryAndPhysics")
          (Collision|SetCollisionEnabled _cajatirada_04 "QueryAndPhysics")
          (Collision|SetCollisionEnabled _cajatirada_05 "QueryAndPhysics"))))))

(event OnComponentBeginOverlap(Trigger_Sound)
  (params (OverlappedComponent :type Primitive%20Component%20Object%20Reference) (OtherActor :type Actor%20Object%20Reference) (OtherComp :type Primitive%20Component%20Object%20Reference) (OtherBodyIndex :type Integer) (bFromSweep :type Boolean) (SweepResult :type Hit%20Result%20Structure%20%28by%20ref%29))
  (if (Variables|Default|GetSeHanCaido)
    (Components|DestroyComponent (Variables|Default|GetTrigger_Sound))))

(fn ConstructionScript)