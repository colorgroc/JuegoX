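; TV_Zeus is a proximity-triggered television that switches on to static noise while the first-person player character is nearby.
; Entering its sphere swaps the screen material slot to static, reveals a rect light and spawns a static sound at the TV, keeping a reference to it.
; Leaving restores the off material, hides the light, then stops and clears the stored sound.
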(event OnComponentBeginOverlap(Sphere)
  (params (OverlappedComponent :type Primitive%20Component%20Object%20Reference) (OtherActor :type Actor%20Object%20Reference) (OtherComp :type Primitive%20Component%20Object%20Reference) (OtherBodyIndex :type Integer) (bFromSweep :type Boolean) (SweepResult :type Hit%20Result%20Structure%20%28by%20ref%29))
  (bind _tv (Variables|Default|GetTV))
  (Utilities|Casting|CastToFirstPersonCharacter OtherActor)
  (Rendering|Material|SetMaterial (Variables|Default|GetTV) 1 "/Game/Materiales/StaticNoise_Mat_Inst.StaticNoise_Mat_Inst")
  (Development|SetHiddeninGame (Variables|Default|GetRectLight) false false)
  (bind _returnvalue (Audio|SpawnSoundatLocation "/Game/Soniditos/StaticNoise_Snd.StaticNoise_Snd" (Transformation|GetWorldLocation _tv) (Transformation|GetWorldRotation _tv) 1.0 1.0 0.0 0 0))
  (Variables|Default|Setsound _returnvalue))

(event OnComponentEndOverlap(Sphere)
  (params (OverlappedComponent :type Primitive%20Component%20Object%20Reference) (OtherActor :type Actor%20Object%20Reference) (OtherComp :type Primitive%20Component%20Object%20Reference) (OtherBodyIndex :type Integer))
  (Utilities|Casting|CastToFirstPersonCharacter OtherActor)
  (Rendering|Material|SetMaterial (Variables|Default|GetTV) 1 "/Game/Materiales/TV_OFF_Mat_Inst.TV_OFF_Mat_Inst")
  (Development|SetHiddeninGame (Variables|Default|GetRectLight) true false)
  (Utilities|IsValid (Variables|Default|Getsound)
    (:Is%20Valid
      (Audio|Components|Audio|Stop (Variables|Default|Getsound))
      (Variables|Default|Setsound 0))))

(fn ConstructionScript)