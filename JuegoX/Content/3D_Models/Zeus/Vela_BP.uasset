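; Candle (Vela) prop Blueprint with a mesh, particle system and point light whose intensity varies to suggest flicker.
; On BeginPlay it randomizes minimum and maximum intensity and timeline play rate, so each instance differs.
; A timeline curve interpolates the light intensity between those bounds.
; The construction script applies the Enabled flag through SetEnabled, toggling light and particle visibility and disabling mesh shadow casting while lit.
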(event EventBeginPlay
  (Variables|Default|SetMaxIntensity (Math|Random|RandomFloatinRange 5e+02 7e+02))
  (Variables|Default|SetMinIntensity (Math|Random|RandomFloatinRange 1e+02 3e+02))
  (Components|Timeline|SetPlayRate (Variables|Default|GetTimeline_0) (Math|Random|RandomFloatinRange 0.8 1.2))
  (bind _intensity (Timeline|Timeline_0 Play)
    (:Update
      (Rendering|Components|Light|SetIntensity (Variables|Default|GetPointLight) (Math|Float|Lerp (Variables|Default|GetMinIntensity) (Variables|Default|GetMaxIntensity) _intensity)))))

(fn ConstructionScript
  (CallFunction|SetEnabled (Variables|Default|GetEnabled)))

(fn SetEnabled
  (params (Enabled :type Boolean))
  (bind _output_get (Variables|Default|SetEnabled Enabled))
  (Rendering|SetVisibility (Variables|Default|GetPointLight) _output_get false)
  (Rendering|SetVisibility (Variables|Default|GetParticleSystem) _output_get false)
  (Rendering|SetCastShadow (Variables|Default|GetStaticMesh) (not _output_get)))