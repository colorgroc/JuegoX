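; OpenedDiary is the open state of an inspectable diary, from which the player can tear a page (ArrancoPagina).
; It accepts input only while focused or inspected; its Interact function also spawns an Avion at the player's inspection view.
; Pressing Inspect swaps it for a Diario actor, linked to the Sillon, and a timeline lerps that back to its initial transform.
; It then re-enables Sillon interaction and destroys itself.
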(event EventTick
  (params (DeltaSeconds :type Float%20%28single-precision%29))
  (bind _returnvalue (Game|GetPlayerController 0))
  (if (Variables|/Game/JuegoX/Blueprints/Objects/Interactable.Interactable_C|GetisInspectingIt (Variables|Default|GetInteractuable))
    (Input|EnableInput _returnvalue :!label _label)
    (elif (Variables|/Game/JuegoX/Blueprints/Objects/Interactable.Interactable_C|GetisFocused? (Variables|Default|GetInteractuable))
      (goto _label)
      (else
        (Input|DisableInput _returnvalue)))))

(event EventBeginPlay
  (bind _asfirst_person_character (Utilities|Casting|CastToFirstPersonCharacter (Game|GetPlayerCharacter 0)))
  (Variables|Default|Setplayer _asfirst_person_character))

(event Input|ActionEvents|InputActionInteract
  (params (Key :type Key%20Structure :default "None"))
  (:Pressed
    (if (Variables|/Game/JuegoX/Blueprints/Objects/Interactable.Interactable_C|GetisFocused? (Variables|Default|GetInteractuable))
      (Variables|/Game/FirstPersonBP/Blueprints/FirstPersonCharacter.FirstPersonCharacter_C|SetArrancoPagina? (Variables|Default|Getplayer) true))))

(event Input|ActionEvents|InputActionInspect
  (params (Key :type Key%20Structure :default "None"))
  (bind _returnvalue (Transformation|GetActorLocation))
  (:Pressed
    (bind _returnvalue_2 (Game|SpawnActorfromClass "/Game/JuegoX/Blueprints/Objects/Diario.Diario_C" (Math|Transform|MakeTransform _returnvalue (Transformation|GetActorRotation) "0.500000,0.500000,0.500000") "AlwaysSpawn" 0 0))
    (Variables|/Game/JuegoX/Blueprints/Objects/Interactable.Interactable_C|SetinitialPos (Variables|/Game/JuegoX/Blueprints/Objects/Diario.Diario_C|GetInteractuable _returnvalue_2) (Variables|Default|GetinitialPoint))
    (Variables|/Game/JuegoX/Blueprints/Objects/Interactable.Interactable_C|SetinitialRot (Variables|/Game/JuegoX/Blueprints/Objects/Diario.Diario_C|GetInteractuable _returnvalue_2) (Variables|Default|GetinitialRot))
    (Variables|/Game/JuegoX/Blueprints/Objects/Diario.Diario_C|SetinspectionPos _returnvalue_2 _returnvalue)
    (Variables|/Game/JuegoX/Blueprints/Objects/Diario.Diario_C|SetSillon _returnvalue_2 (Variables|DondeSeGuarda|GetSillon))
    (Variables|/Game/JuegoX/Blueprints/Objects/Sillon.Sillon_C|SetDiario (Variables|DondeSeGuarda|GetSillon) _returnvalue_2)
    (Components|DestroyComponent (Variables|Default|GetMesh))
    (Variables|/Game/JuegoX/Blueprints/Objects/Interactable.Interactable_C|SetisInspectingIt (Variables|/Game/JuegoX/Blueprints/Objects/Diario.Diario_C|GetInteractuable _returnvalue_2) false)
    (Variables|/Game/FirstPersonBP/Blueprints/FirstPersonCharacter.FirstPersonCharacter_C|SetplayerIsReading? (Variables|Default|Getplayer) false)
    (bind _move_object (Timeline|Inspect Play)
      (:Update
        (bind _output_get (Variables|Default|SetMovedObject _move_object))
        (Transformation|SetActorLocationAndRotation _returnvalue_2 (Math|Vector|Lerp(Vector) (Transformation|GetActorLocation _returnvalue_2) (Variables|Default|GetinitialPoint) _output_get) (Math|Rotator|Lerp(Rotator) (Transformation|GetActorRotation _returnvalue_2) (Variables|Default|GetinitialRot) _output_get)))
      (:Finished
        (if (Utilities|IsValid (Variables|DondeSeGuarda|GetSillon))
          (Variables|/Game/JuegoX/Blueprints/Objects/Interactable.Interactable_C|SetinteractionActivated (Variables|/Game/JuegoX/Blueprints/Objects/Sillon.Sillon_C|GetInteractuable (Variables|DondeSeGuarda|GetSillon)) true)
          (Actor|DestroyActor))))))

(fn ConstructionScript)

(fn Interact
  (bind _player (Variables|Default|Getplayer))
  (Development|PrintString "opened diary")
  (Variables|/Game/FirstPersonBP/Blueprints/FirstPersonCharacter.FirstPersonCharacter_C|SetArrancoPagina? (Variables|Default|Getplayer) true)
  (Game|SpawnActorfromClass "/Game/JuegoX/Blueprints/Objects/Avion.Avion_C" (Math|Transform|MakeTransform (Transformation|GetWorldLocation (Variables|/Game/FirstPersonBP/Blueprints/FirstPersonCharacter.FirstPersonCharacter_C|GetInpectionViewBig _player)) (Transformation|GetWorldRotation (Variables|/Game/FirstPersonBP/Blueprints/FirstPersonCharacter.FirstPersonCharacter_C|GetFirstPersonCamera _player))) "AlwaysSpawn" 0 0))