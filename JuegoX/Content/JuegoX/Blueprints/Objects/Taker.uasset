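; Pickup actor for the Taker item, which the player can inspect and collect.
; Tick drives an outline material by distance and focus from its Interactuable state, enables input when focused, and keeps a saved item attached to its storage object.
; Inspect toggles a timeline that moves it between its resting spot and the player's inspection point.
; Interacting during inspection sets HasTaker on the game instance, shows the inventory HUD icon and destroys the actor.
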(event Custom|EndInspection
  (bind _interactuable (Variables|Default|GetInteractuable))
  (CallFunction|HideControls)
  (Variables|/Game/JuegoX/Blueprints/Objects/Interactable.Interactable_C|SetisInspectingIt (Variables|Default|GetInteractuable) false)
  (Variables|/Game/FirstPersonBP/Blueprints/FirstPersonCharacter.FirstPersonCharacter_C|SetplayerInspectingObject (Variables|Default|Getplayer) false)
  (bind _move_object (Timeline|Inspect Reverse)
    (:Update
      (bind _output_get (Variables|Default|SetMovedObject _move_object))
      (Transformation|SetActorLocationAndRotation (Math|Vector|Lerp(Vector) (Variables|/Game/JuegoX/Blueprints/Objects/Interactable.Interactable_C|GetinitialPos _interactuable) (Variables|/Game/JuegoX/Blueprints/Objects/Interactable.Interactable_C|GetinspectionPoint _interactuable) _output_get) (Math|Rotator|Lerp(Rotator) (Variables|/Game/JuegoX/Blueprints/Objects/Interactable.Interactable_C|GetinitialRot _interactuable) (Transformation|GetActorRotation) _output_get)))))

(event EventTick
  (params (DeltaSeconds :type Float%20%28single-precision%29))
  (bind _returnvalue (Game|GetPlayerController 0))
  (bind _materialhighlight (Variables|Default|GetMaterialHighlight))
  (bind _materialhighlight_2 (Variables|Default|GetMaterialHighlight))
  (if (Variables|/Game/JuegoX/Blueprints/Objects/Interactable.Interactable_C|GetisInspectingIt (Variables|Default|GetInteractuable))
    (Rendering|Material|SetScalarParameterValue _materialhighlight_2 "Scale" 0.0 :!class /Script/Engine.MaterialInstanceDynamic)
    (Input|EnableInput _returnvalue :!label _label)
    (Rendering|SetVisibility (Variables|Default|GetWidget) true false)
    (Transformation|SetWorldRotation (Variables|Default|GetTextRender) (Math|Rotator|FindLookatRotation (Transformation|GetActorLocation) (Transformation|GetActorLocation (Variables|Default|Getplayer))) false false)
    (else
      (if (Variables|Default|GetitsSaved?)
        (Transformation|SetActorLocation (Transformation|GetWorldLocation (Variables|Default|GetWhatToFollow)) false false))
      (Variables|/Game/JuegoX/Blueprints/Objects/Interactable.Interactable_C|SetinitialPos (Variables|Default|GetInteractuable) (Transformation|GetActorLocation))
      (if (Variables|/Game/JuegoX/Blueprints/Objects/Interactable.Interactable_C|GetisFocused? (Variables|Default|GetInteractuable))
        (Rendering|Material|SetScalarParameterValue _materialhighlight_2 "Scale" 0.5 :!class /Script/Engine.MaterialInstanceDynamic)
        (Rendering|Material|SetVectorParameterValue _materialhighlight_2 "Color" "(R=1.000000,G=0.000000,B=0.000000,A=1.000000)" :!class /Script/Engine.MaterialInstanceDynamic)
        (goto _label)
        (else
          (Input|DisableInput _returnvalue)
          (Math|Float|CompareFloat (Transformation|GetDistanceTo (Variables|Default|Getplayer)) (Variables|/Game/JuegoX/Blueprints/Objects/Interactable.Interactable_C|GetDistance%20to%20Glow (Variables|Default|GetInteractuable))
            (:>
              (Rendering|Material|SetScalarParameterValue _materialhighlight "Scale" 0.0 :!class /Script/Engine.MaterialInstanceDynamic))
            (:==
              (Rendering|Material|SetScalarParameterValue _materialhighlight "Scale" 0.5 :!class /Script/Engine.MaterialInstanceDynamic :!label _label_2))
            (:<
              (goto _label_2)))
          (Rendering|Material|SetVectorParameterValue _materialhighlight "Color" "(R=1.000000,G=1.000000,B=1.000000,A=1.000000)" :!class /Script/Engine.MaterialInstanceDynamic)
          (Rendering|SetVisibility (Variables|Default|GetWidget) false false))))))

(event EventBeginPlay
  (bind _lugardondeestaguardada (Variables|DondeSeGuarda|GetLugarDondeEstaGuardada))
  (if (Variables|Default|GetitsSaved?)
    (if (Utilities|IsValid _lugardondeestaguardada)
      (Variables|Default|SetWhatToFollow (Variables|/Game/JuegoX/Blueprints/Objects/Cajon_Mesa.Cajon_Mesa_C|GetObjetoInterno _lugardondeestaguardada))
      (bind _asfirst_person_character (Utilities|Casting|CastToFirstPersonCharacter (Game|GetPlayerCharacter 0) :!label _label))
      (Variables|Default|Setplayer _asfirst_person_character)
      (bind _returnvalue (Rendering|Material|CreateDynamicMaterialInstance (Variables|Default|GetDuplicated) 0 "/Game/JuegoX/Materials/Outline_ObjectsHided.Outline_ObjectsHided" "None" :!class /Script/Engine.PrimitiveComponent))
      (Variables|Default|SetMaterialHighlight _returnvalue))
    (else
      (goto _label))))

(event Input|ActionEvents|InputActionInteract
  (params (Key :type Key%20Structure :default "None"))
  (:Pressed
    (if (Variables|/Game/JuegoX/Blueprints/Objects/Interactable.Interactable_C|GetisInspectingIt (Variables|Default|GetInteractuable))
      (CallFunction|Interact))))

(event Input|ActionEvents|InputActionInspect
  (params (Key :type Key%20Structure :default "None"))
  (bind _interactuable (Variables|Default|GetInteractuable))
  (bind _interactuable_2 (Variables|Default|GetInteractuable))
  (:Pressed
    (if (Variables|/Game/JuegoX/Blueprints/Objects/Interactable.Interactable_C|GetisInspectingIt _interactuable)
      (CallFunction|EndInspection)
      (else
        (Utilities|FlowControl|Sequence
          (:then_0
            (CallFunction|ShowControls))
          (:then_1
            (Variables|/Game/JuegoX/Blueprints/Objects/Interactable.Interactable_C|SetinspectionPoint _interactuable (Transformation|GetWorldLocation (Variables|/Game/FirstPersonBP/Blueprints/FirstPersonCharacter.FirstPersonCharacter_C|GetInpectionView (Variables|Default|Getplayer))))
            (Variables|/Game/JuegoX/Blueprints/Objects/Interactable.Interactable_C|SetisInspectingIt _interactuable true)
            (Variables|/Game/FirstPersonBP/Blueprints/FirstPersonCharacter.FirstPersonCharacter_C|SetplayerInspectingObject (Variables|Default|Getplayer) true)
            (bind _move_object (Timeline|Inspect Play)
              (:Update
                (bind _output_get (Variables|Default|SetMovedObject _move_object))
                (Transformation|SetActorLocationAndRotation (Math|Vector|Lerp(Vector) (Variables|/Game/JuegoX/Blueprints/Objects/Interactable.Interactable_C|GetinitialPos _interactuable_2) (Variables|/Game/JuegoX/Blueprints/Objects/Interactable.Interactable_C|GetinspectionPoint _interactuable_2) _output_get) (Math|Rotator|Lerp(Rotator) (Variables|/Game/JuegoX/Blueprints/Objects/Interactable.Interactable_C|GetinitialRot _interactuable_2) (Transformation|GetActorRotation) _output_get))))))))))

(fn ConstructionScript)

(fn Interact
  (bind _asmy_game_instance (Utilities|Casting|CastToMyGameInstance (Game|GetGameInstance)))
  (Variables|/Game/JuegoX/Blueprints/MyGameInstance.MyGameInstance_C|SetHas_Taker? _asmy_game_instance true)
  (Variables|/Game/JuegoX/Blueprints/Objects/Interactable.Interactable_C|SetisInspectingIt (Variables|Default|GetInteractuable) false)
  (bind _asfirst_person_character (Utilities|Casting|CastToFirstPersonCharacter (Game|GetPlayerCharacter 0)))
  (Variables|/Game/FirstPersonBP/Blueprints/FirstPersonCharacter.FirstPersonCharacter_C|SetplayerInspectingObject _asfirst_person_character false)
  (CallFunction|Inventory)
  (CallFunction|HideControls)
  (Actor|DestroyActor))

(fn Inventory
  (bind _player (Variables|Default|Getplayer))
  (bind _inventoryhud (Variables|/Game/FirstPersonBP/Blueprints/FirstPersonCharacter.FirstPersonCharacter_C|GetInventoryHUD _player))
  (Appearance|SetBrushfromTexture (Variables|/Game/JuegoX/UI/HUD/WB_Inventory.WB_Inventory_C|GetItem _inventoryhud) "/Game/JuegoX/Sprites/inventario/taker.taker" true)
  (UserInterface|Viewport|AddtoViewport _inventoryhud 0))

(fn ShowControls
  (bind _player (Variables|Default|Getplayer))
  (if (Utilities|IsValid (Variables|/Game/FirstPersonBP/Blueprints/FirstPersonCharacter.FirstPersonCharacter_C|GetWB_PickUp _player))
    _
    (else
      (bind _returnvalue (UserInterface|CreateWidget "/Game/JuegoX/UI/HUD/WB_PickUp.WB_PickUp_C" (Game|GetPlayerController 0)))
      (Variables|/Game/FirstPersonBP/Blueprints/FirstPersonCharacter.FirstPersonCharacter_C|SetWB_PickUp _player _returnvalue)))
  (UserInterface|Viewport|AddtoViewport (Variables|/Game/FirstPersonBP/Blueprints/FirstPersonCharacter.FirstPersonCharacter_C|GetWB_PickUp _player) 0))

(fn HideControls
  (bind _player (Variables|Default|Getplayer))
  (bind _inventoryhud (Variables|/Game/FirstPersonBP/Blueprints/FirstPersonCharacter.FirstPersonCharacter_C|GetInventoryHUD _player))
  (bind _controls_2_anim (Variables|/Game/JuegoX/UI/HUD/WB_Inventory.WB_Inventory_C|GetControls_2_Anim _inventoryhud))
  (UserInterface|Animation|PlayAnimation _inventoryhud _controls_2_anim 0.0 1 "Reverse" 6.0)
  (Class|UserWidget|BindtoAnimationFinished _inventoryhud _controls_2_anim (EventDispatchers|CreateEvent :!event SetVisibility))
  (Class|UserWidget|UnbindfromAnimationFinished _inventoryhud _controls_2_anim (EventDispatchers|CreateEvent :!event SetVisibility)))

(fn SetVisibility
  (Widget|SetVisibility (Variables|/Game/JuegoX/UI/HUD/WB_Inventory.WB_Inventory_C|GetLegend_Two (Variables|/Game/FirstPersonBP/Blueprints/FirstPersonCharacter.FirstPersonCharacter_C|GetInventoryHUD (Variables|Default|Getplayer))) "Hidden"))