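; Interactable glasses prop that toggles a hidden key on the decorative masks actor by lowering or retracting its cable.
; It starts hidden and non-interactive, with GlassesOn and GlassesOff events switching visibility, collision and interaction.
; Tick enables input only while focused or inspected.
; Inspect toggles the key's visibility and interactability, plays the mask sequence forward or backward, and drives cable length through a reversible timeline.
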(event Custom|Play%20Reverse_Cable
  (bind _cable (Timeline|Cable_Key_Timeline ReverseFromEnd)
    (:Update
      (Variables|/Script/CableComponent.CableComponent|SetCableLength (Variables|/Script/CableComponent.CableActor|GetCableComponent (Variables|/Game/JuegoX/Blueprints/Objects/OBJ_Decorative_Masks.OBJ_Decorative_Masks_C|GetCable (Variables|Default|GetMask))) (Math|Float|Lerp (Variables|Default|GetCableLenghtHided) (Variables|Default|GetCableLenghtDesplegated) _cable)))))

(event Custom|Play_Cable
  (bind _cable (Timeline|Cable_Key_Timeline PlayFromStart)
    (:Update
      (Variables|/Script/CableComponent.CableComponent|SetCableLength (Variables|/Script/CableComponent.CableActor|GetCableComponent (Variables|/Game/JuegoX/Blueprints/Objects/OBJ_Decorative_Masks.OBJ_Decorative_Masks_C|GetCable (Variables|Default|GetMask))) (Math|Float|Lerp (Variables|Default|GetCableLenghtHided) (Variables|Default|GetCableLenghtDesplegated) _cable)))))

(event Custom|GlassesOff
  (Rendering|SetVisibility (Variables|Default|GetMesh) false false)
  (Collision|SetCollisionProfileName (Variables|Default|GetMesh) "NoCollision" :!class /Script/Engine.PrimitiveComponent)
  (Variables|/Game/JuegoX/Blueprints/Objects/Interactable.Interactable_C|SetinteractionActivated (Variables|Default|GetInteractable) false))

(event Custom|GlassesOn
  (Rendering|SetVisibility (Variables|Default|GetMesh) true false)
  (Collision|SetCollisionProfileName (Variables|Default|GetMesh) "BlockAllDynamic" :!class /Script/Engine.PrimitiveComponent)
  (Variables|/Game/JuegoX/Blueprints/Objects/Interactable.Interactable_C|SetinteractionActivated (Variables|Default|GetInteractable) true))

(event EventBeginPlay
  (CallFunction|GlassesOff)
  (bind _returnvalue (Actor|GetActorOfClass "/Game/JuegoX/Blueprints/Objects/OBJ_Decorative_Masks.OBJ_Decorative_Masks_C"))
  (Variables|Default|SetMask _returnvalue)
  (Variables|Default|SetCableLenghtDesplegated (Variables|/Script/CableComponent.CableComponent|GetCableLength (Variables|/Script/CableComponent.CableActor|GetCableComponent (Variables|/Game/JuegoX/Blueprints/Objects/OBJ_Decorative_Masks.OBJ_Decorative_Masks_C|GetCable (Variables|Default|GetMask)))))
  (bind _output_get (Variables|Default|SetCableLenghtHided 0.0))
  (Variables|/Script/CableComponent.CableComponent|SetCableLength (Variables|/Script/CableComponent.CableActor|GetCableComponent (Variables|/Game/JuegoX/Blueprints/Objects/OBJ_Decorative_Masks.OBJ_Decorative_Masks_C|GetCable (Variables|Default|GetMask))) _output_get)
  (bind _asfirst_person_character (Utilities|Casting|CastToFirstPersonCharacter (Game|GetPlayerCharacter 0)))
  (bind _output_get_2 (Variables|Default|SetPlayer _asfirst_person_character))
  (Variables|/Game/JuegoX/Blueprints/Objects/Interactable.Interactable_C|Setplayer (Variables|Default|GetInteractable) _output_get_2)
  (if (Utilities|IsValid (Variables|/Game/JuegoX/Blueprints/Objects/OBJ_Decorative_Masks.OBJ_Decorative_Masks_C|Getkey (Variables|Default|GetMask)))
    (Rendering|SetVisibility (Variables|/Game/JuegoX/Blueprints/Objects/OBJ_Cigarros_InteractuableParent.OBJ_Cigarros_InteractuableParent_C|GetMesh (Variables|/Game/JuegoX/Blueprints/Objects/OBJ_Decorative_Masks.OBJ_Decorative_Masks_C|Getkey (Variables|Default|GetMask))) false true)
    (Variables|/Game/JuegoX/Blueprints/Objects/Interactable.Interactable_C|SetinteractionActivated (Variables|/Game/JuegoX/Blueprints/Objects/OBJ_Cigarros_InteractuableParent.OBJ_Cigarros_InteractuableParent_C|GetInteractable (Variables|/Game/JuegoX/Blueprints/Objects/OBJ_Decorative_Masks.OBJ_Decorative_Masks_C|Getkey (Variables|Default|GetMask))) false)))

(event Collision|EventActorBeginOverlap
  (params (OtherActor :type Actor%20Object%20Reference)))

(event EventTick
  (params (DeltaSeconds :type Float%20%28single-precision%29))
  (bind _returnvalue (Game|GetPlayerController 0))
  (if (Variables|/Game/JuegoX/Blueprints/Objects/Interactable.Interactable_C|GetinteractionActivated (Variables|Default|GetInteractable))
    (if (Variables|/Game/JuegoX/Blueprints/Objects/Interactable.Interactable_C|GetisInspectingIt (Variables|Default|GetInteractable))
      (Input|EnableInput _returnvalue :!label _label)
      (elif (Variables|/Game/JuegoX/Blueprints/Objects/Interactable.Interactable_C|GetisFocused? (Variables|Default|GetInteractable))
        (goto _label)
        (else
          (Input|DisableInput _returnvalue))))))

(event Input|ActionEvents|InputActionInspect
  (params (Key :type Key%20Structure :default "None"))
  (:Pressed
    (if (Variables|/Game/JuegoX/Blueprints/Objects/Interactable.Interactable_C|GetinteractionActivated (Variables|Default|GetInteractable))
      (if (Variables|/Game/JuegoX/Blueprints/Objects/Interactable.Interactable_C|GetinteractionActivated (Variables|/Game/JuegoX/Blueprints/Objects/OBJ_Cigarros_InteractuableParent.OBJ_Cigarros_InteractuableParent_C|GetInteractable (Variables|/Game/JuegoX/Blueprints/Objects/OBJ_Decorative_Masks.OBJ_Decorative_Masks_C|Getkey (Variables|Default|GetMask))))
        (if (Utilities|IsValid (Variables|/Game/JuegoX/Blueprints/Objects/OBJ_Decorative_Masks.OBJ_Decorative_Masks_C|Getkey (Variables|Default|GetMask)))
          (Rendering|SetVisibility (Variables|/Game/JuegoX/Blueprints/Objects/OBJ_Cigarros_InteractuableParent.OBJ_Cigarros_InteractuableParent_C|GetMesh (Variables|/Game/JuegoX/Blueprints/Objects/OBJ_Decorative_Masks.OBJ_Decorative_Masks_C|Getkey (Variables|Default|GetMask))) false true)
          (Variables|/Game/JuegoX/Blueprints/Objects/Interactable.Interactable_C|SetinteractionActivated (Variables|/Game/JuegoX/Blueprints/Objects/OBJ_Cigarros_InteractuableParent.OBJ_Cigarros_InteractuableParent_C|GetInteractable (Variables|/Game/JuegoX/Blueprints/Objects/OBJ_Decorative_Masks.OBJ_Decorative_Masks_C|Getkey (Variables|Default|GetMask))) false)
          (Class|MovieSceneSequencePlayer|PlayReverse (Variables|/Script/ActorSequence.ActorSequenceComponent|GetSequencePlayer (Variables|/Game/JuegoX/Blueprints/Objects/OBJ_Decorative_Masks.OBJ_Decorative_Masks_C|GetAnim (Variables|Default|GetMask))))
          (CallFunction|PlayReverseCable))
        (elif (Utilities|IsValid (Variables|/Game/JuegoX/Blueprints/Objects/OBJ_Decorative_Masks.OBJ_Decorative_Masks_C|Getkey (Variables|Default|GetMask)))
          (Rendering|SetVisibility (Variables|/Game/JuegoX/Blueprints/Objects/OBJ_Cigarros_InteractuableParent.OBJ_Cigarros_InteractuableParent_C|GetMesh (Variables|/Game/JuegoX/Blueprints/Objects/OBJ_Decorative_Masks.OBJ_Decorative_Masks_C|Getkey (Variables|Default|GetMask))) true true)
          (Variables|/Game/JuegoX/Blueprints/Objects/Interactable.Interactable_C|SetinteractionActivated (Variables|/Game/JuegoX/Blueprints/Objects/OBJ_Cigarros_InteractuableParent.OBJ_Cigarros_InteractuableParent_C|GetInteractable (Variables|/Game/JuegoX/Blueprints/Objects/OBJ_Decorative_Masks.OBJ_Decorative_Masks_C|Getkey (Variables|Default|GetMask))) true)
          (Sequencer|Player|Play (Variables|/Script/ActorSequence.ActorSequenceComponent|GetSequencePlayer (Variables|/Game/JuegoX/Blueprints/Objects/OBJ_Decorative_Masks.OBJ_Decorative_Masks_C|GetAnim (Variables|Default|GetMask))) :!class /Script/MovieScene.MovieSceneSequencePlayer)
          (CallFunction|PlayCable))))))

(fn ConstructionScript
  (Variables|/Game/JuegoX/Blueprints/Objects/Interactable.Interactable_C|SetMesh (Variables|Default|GetInteractable) (Variables|Default|GetMesh))
  (Variables|/Game/JuegoX/Blueprints/Objects/Interactable.Interactable_C|SetText (Variables|Default|GetInteractable) (Variables|Default|GetTextRender)))