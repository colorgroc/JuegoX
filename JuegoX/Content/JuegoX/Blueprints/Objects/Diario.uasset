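; Closed diary that the player can inspect while in reading mode, tied to the Sillon (armchair) actor.
; Tick drives a dynamic outline material, white when within glow range and red when focused, and toggles input, visibility of the prompt widget and its player-facing text.
; Inspect runs a timeline moving the diary to the Sillon's book point, shows HUD controls, then swaps it for a spawned OpenedDiary and disables Sillon interaction.
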(event EventTick
  (params (DeltaSeconds :type Float%20%28single-precision%29))
  (bind _returnvalue (Game|GetPlayerController 0))
  (bind _materialhighlight (Variables|Default|GetMaterialHighlight))
  (bind _materialhighlight_2 (Variables|Default|GetMaterialHighlight))
  (if (Variables|/Game/FirstPersonBP/Blueprints/FirstPersonCharacter.FirstPersonCharacter_C|GetplayerIsReading? (Variables|Default|Getplayer))
    (if (Variables|/Game/JuegoX/Blueprints/Objects/Interactable.Interactable_C|GetisInspectingIt (Variables|Default|GetInteractuable))
      (Rendering|Material|SetScalarParameterValue _materialhighlight_2 "Scale" 0.0 :!class /Script/Engine.MaterialInstanceDynamic)
      (Input|EnableInput _returnvalue :!label _label)
      (Rendering|SetVisibility (Variables|Default|GetWidget) true false)
      (Transformation|SetWorldRotation (Variables|Default|GetTextRender) (Math|Rotator|FindLookatRotation (Transformation|GetActorLocation) (Transformation|GetActorLocation (Variables|Default|Getplayer))) false false)
      (elif (Variables|/Game/JuegoX/Blueprints/Objects/Interactable.Interactable_C|GetisFocused? (Variables|Default|GetInteractuable))
        (Rendering|Material|SetScalarParameterValue _materialhighlight_2 "Scale" 0.5 :!class /Script/Engine.MaterialInstanceDynamic)
        (Rendering|Material|SetVectorParameterValue _materialhighlight_2 "Color" "(R=1.000000,G=0.000000,B=0.000000,A=1.000000)" :!class /Script/Engine.MaterialInstanceDynamic)
        (goto _label)
        (else
          (Input|DisableInput _returnvalue)
          (Math|Float|CompareFloat (Transformation|GetDistanceTo (Variables|Default|Getplayer)) (Variables|/Game/JuegoX/Blueprints/Objects/Interactable.Interactable_C|GetDistance%20to%20Glow (Variables|Default|GetInteractuable))
            (:>
              (Rendering|Material|SetScalarParameterValue _materialhighlight "Scale" 0.0 :!class /Script/Engine.MaterialInstanceDynamic :!label _label_2))
            (:==
              (Rendering|Material|SetScalarParameterValue _materialhighlight "Scale" 0.5 :!class /Script/Engine.MaterialInstanceDynamic :!label _label_3))
            (:<
              (goto _label_3)))
          (Rendering|Material|SetVectorParameterValue _materialhighlight "Color" "(R=1.000000,G=1.000000,B=1.000000,A=1.000000)" :!class /Script/Engine.MaterialInstanceDynamic)
          (Rendering|SetVisibility (Variables|Default|GetWidget) false false))))
    (else
      (goto _label_2))))

(event EventBeginPlay
  (bind _asfirst_person_character (Utilities|Casting|CastToFirstPersonCharacter (Game|GetPlayerCharacter 0)))
  (Variables|Default|Setplayer _asfirst_person_character)
  (bind _returnvalue (Rendering|Material|CreateDynamicMaterialInstance (Variables|Default|GetDuplicated) 0 "/Game/JuegoX/Materials/Outline_ObjectsHided.Outline_ObjectsHided" "None" :!class /Script/Engine.PrimitiveComponent))
  (Variables|Default|SetMaterialHighlight _returnvalue))

(event Input|ActionEvents|InputActionInspect
  (params (Key :type Key%20Structure))
  (bind _interactuable (Variables|Default|GetInteractuable))
  (bind _interactuable_2 (Variables|Default|GetInteractuable))
  (:Pressed
    (if (Variables|/Game/JuegoX/Blueprints/Objects/Interactable.Interactable_C|GetinteractionActivated (Variables|Default|GetInteractuable))
      (if (not (Variables|/Game/JuegoX/Blueprints/Objects/Interactable.Interactable_C|GetisInspectingIt _interactuable))
        (Variables|/Game/JuegoX/Blueprints/Objects/Interactable.Interactable_C|SetinspectionPoint _interactuable (Transformation|GetWorldLocation (Variables|/Game/JuegoX/Blueprints/Objects/Sillon.Sillon_C|GetBook (Variables|DondeSeGuarda|GetSillon))))
        (Variables|/Game/JuegoX/Blueprints/Objects/Interactable.Interactable_C|SetisInspectingIt _interactuable true)
        (bind _move_object (Timeline|Inspect Play)
          (:Update
            (bind _output_get (Variables|Default|SetMovedObject _move_object))
            (Transformation|SetActorLocationAndRotation (Math|Vector|Lerp(Vector) (Variables|/Game/JuegoX/Blueprints/Objects/Interactable.Interactable_C|GetinitialPos _interactuable_2) (Variables|/Game/JuegoX/Blueprints/Objects/Interactable.Interactable_C|GetinspectionPoint _interactuable_2) _output_get) (Math|Rotator|Lerp(Rotator) (Variables|/Game/JuegoX/Blueprints/Objects/Interactable.Interactable_C|GetinitialRot _interactuable_2) (Transformation|GetActorRotation) _output_get)))
          (:Finished
            (CallFunction|ShowControls)
            (CallFunction|Interact)))))))

(fn ConstructionScript)

(fn Interact
  (bind _interactuable (Variables|Default|GetInteractuable))
  (Variables|/Game/JuegoX/Blueprints/Objects/Interactable.Interactable_C|SetisInspectingIt (Variables|Default|GetInteractuable) false)
  (bind _returnvalue (Game|SpawnActorfromClass "/Game/JuegoX/Blueprints/Objects/OpenedDiary.OpenedDiary_C" (Math|Transform|MakeTransform (Transformation|GetActorLocation) (Math|Rotator|MakeRotator (.Roll (Math|Rotator|BreakRotator (Transformation|GetActorRotation (Variables|DondeSeGuarda|GetSillon)))) 3e+01 (.Yaw (Math|Rotator|BreakRotator (Transformation|GetActorRotation (Variables|DondeSeGuarda|GetSillon))))) (LocalVariables|GetdiaryScale)) "AlwaysSpawn" 0 0))
  (Variables|/Game/JuegoX/Blueprints/Objects/OpenedDiary.OpenedDiary_C|SetinitialPoint _returnvalue (Variables|/Game/JuegoX/Blueprints/Objects/Interactable.Interactable_C|GetinitialPos _interactuable))
  (Variables|/Game/JuegoX/Blueprints/Objects/OpenedDiary.OpenedDiary_C|SetinitialRot _returnvalue (Variables|/Game/JuegoX/Blueprints/Objects/Interactable.Interactable_C|GetinitialRot _interactuable))
  (Variables|/Game/JuegoX/Blueprints/Objects/OpenedDiary.OpenedDiary_C|SetSillon _returnvalue (Variables|DondeSeGuarda|GetSillon))
  (Variables|/Game/JuegoX/Blueprints/Objects/Interactable.Interactable_C|SetinteractionActivated (Variables|/Game/JuegoX/Blueprints/Objects/Sillon.Sillon_C|GetInteractuable (Variables|DondeSeGuarda|GetSillon)) false)
  (Actor|DestroyActor))

(fn ShowControls
  (bind _player (Variables|Default|Getplayer))
  (if (Utilities|IsValid (Variables|/Game/FirstPersonBP/Blueprints/FirstPersonCharacter.FirstPersonCharacter_C|GetInventoryHUD _player))
    _
    (else
      (bind _returnvalue (UserInterface|CreateWidget "/Game/JuegoX/UI/HUD/WB_Inventory.WB_Inventory_C" (Game|GetPlayerController 0)))
      (Variables|/Game/FirstPersonBP/Blueprints/FirstPersonCharacter.FirstPersonCharacter_C|SetInventoryHUD _player _returnvalue)))
  (Rendering|Components|TextRender|SetText (Variables|/Game/JuegoX/UI/HUD/WB_Inventory.WB_Inventory_C|GetT_Drop (Variables|/Game/FirstPersonBP/Blueprints/FirstPersonCharacter.FirstPersonCharacter_C|GetInventoryHUD _player)) "to drop")
  (Rendering|Components|TextRender|SetText (Variables|/Game/JuegoX/UI/HUD/WB_Inventory.WB_Inventory_C|GetT_Action (Variables|/Game/FirstPersonBP/Blueprints/FirstPersonCharacter.FirstPersonCharacter_C|GetInventoryHUD _player)) "to open")
  (if (Variables|/Game/JuegoX/Blueprints/MyGameInstance.MyGameInstance_C|GetHas_Key? (Variables|/Game/FirstPersonBP/Blueprints/FirstPersonCharacter.FirstPersonCharacter_C|GetgameInstance _player))
    (Widget|SetVisibility (Variables|/Game/JuegoX/UI/HUD/WB_Inventory.WB_Inventory_C|GetInventory (Variables|/Game/FirstPersonBP/Blueprints/FirstPersonCharacter.FirstPersonCharacter_C|GetInventoryHUD _player)) "Visible")
    (if (UserInterface|Viewport|IsinViewport (Variables|/Game/FirstPersonBP/Blueprints/FirstPersonCharacter.FirstPersonCharacter_C|GetInventoryHUD _player)) :!label _label
      _
      (else
        (UserInterface|Viewport|AddtoViewport (Variables|/Game/FirstPersonBP/Blueprints/FirstPersonCharacter.FirstPersonCharacter_C|GetInventoryHUD _player) 0)))
    (UserInterface|Animation|PlayAnimation (Variables|/Game/FirstPersonBP/Blueprints/FirstPersonCharacter.FirstPersonCharacter_C|GetInventoryHUD _player) (Variables|/Game/JuegoX/UI/HUD/WB_Inventory.WB_Inventory_C|GetControls_2_Anim (Variables|/Game/FirstPersonBP/Blueprints/FirstPersonCharacter.FirstPersonCharacter_C|GetInventoryHUD _player)) 0.0 1 "Forward" 4.0)
    (else
      (Utilities|FlowControl|Sequence
        (:then_0
          (Widget|SetVisibility (Variables|/Game/JuegoX/UI/HUD/WB_Inventory.WB_Inventory_C|GetInventory (Variables|/Game/FirstPersonBP/Blueprints/FirstPersonCharacter.FirstPersonCharacter_C|GetInventoryHUD _player)) "Hidden"))
        (:then_1
          (Widget|SetVisibility (Variables|/Game/JuegoX/UI/HUD/WB_Inventory.WB_Inventory_C|GetLegend_Two (Variables|/Game/FirstPersonBP/Blueprints/FirstPersonCharacter.FirstPersonCharacter_C|GetInventoryHUD _player)) "Visible"))
        (:then_2
          (Widget|SetVisibility (Variables|/Game/JuegoX/UI/HUD/WB_Inventory.WB_Inventory_C|GetLegend_Four (Variables|/Game/FirstPersonBP/Blueprints/FirstPersonCharacter.FirstPersonCharacter_C|GetInventoryHUD _player)) "Hidden")
          (goto _label))))))

(fn HideControls
  (bind _player (Variables|Default|Getplayer))
  (bind _inventoryhud (Variables|/Game/FirstPersonBP/Blueprints/FirstPersonCharacter.FirstPersonCharacter_C|GetInventoryHUD _player))
  (bind _controls_2_anim (Variables|/Game/JuegoX/UI/HUD/WB_Inventory.WB_Inventory_C|GetControls_2_Anim _inventoryhud))
  (UserInterface|Animation|PlayAnimation _inventoryhud _controls_2_anim 0.0 1 "Reverse" 6.0)
  (Class|UserWidget|BindtoAnimationFinished _inventoryhud _controls_2_anim (EventDispatchers|CreateEvent :!event SetVisibility))
  (Class|UserWidget|UnbindfromAnimationFinished _inventoryhud _controls_2_anim (EventDispatchers|CreateEvent :!event SetVisibility)))

(fn SetVisibility
  (Widget|SetVisibility (Variables|/Game/JuegoX/UI/HUD/WB_Inventory.WB_Inventory_C|GetLegend_Two (Variables|/Game/FirstPersonBP/Blueprints/FirstPersonCharacter.FirstPersonCharacter_C|GetInventoryHUD (Variables|Default|Getplayer))) "Hidden"))