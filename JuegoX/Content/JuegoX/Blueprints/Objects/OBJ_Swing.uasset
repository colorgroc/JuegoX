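; Interactable playground swing puzzle that opens a trapdoor (Trampilla) once the swing's pitch reaches FinalAngle.
; Inspect toggles the swing camera, and alternating MouseY input drives SwingTimeline to lerp actor pitch through growing, capped forward and backward steps.
; Wrong-direction input, a second without input or leaving triggers Swing_Fail, which plays forward and in reverse, shrinking the steps until the swing stops.
; Tick enables input only while focused or inspected.
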(event Custom|Fail%20Init
  (params (Can%20Go%20Forward? :type Boolean))
  (bind _returnvalue (Transformation|GetActorRotation))
  ;[1 1 1] Swing when fail
  (Variables|Default|SetCan%20Swing? false)
  (if Can%20Go%20Forward?
    (Utilities|InitAPositiveSetUp
      (:Continue
        (bind (_direction _y) (Timeline|Swing_Fail PlayFromStart)
          (:Update
            (Transformation|SetActorRotation (Math|Rotator|MakeRotator (.roll _returnvalue) (Math|Float|Lerp (Variables|Default|GetA) (Variables|Default|GetB) _y) (.yaw _returnvalue))))
          (:Finished
            (if (Utilities|Enum|Equal(Enum) _direction "Forward")
              (Variables|Default|SetCan%20Go%20Forward? (not Can%20Go%20Forward?))
              ;;[1 1 1] time to let the player interact
              (Variables|Default|SetCan%20Swing? true)
              (Utilities|FlowControl|Delay 0.1)
              (CallFunction|FailEnd)
              (else
                (bind _output_get (Variables|Default|SetCan%20Go%20Forward? Can%20Go%20Forward?))
                (Variables|Default|SetCan%20Swing? true)
                (Utilities|FlowControl|Delay 0.1)
                (CallFunction|FailInit _output_get)))))))
    (else
      (Utilities|InitANegativeSetUp
        (:Continue
          (Timeline|Swing_Fail PlayFromStart))))))

(event Custom|Fail%20End
  (bind _returnvalue (Transformation|GetActorRotation))
  ;[1 1 1] Swing when fail
  (Variables|Default|SetCan%20Swing? false)
  (if (stale Custom|Fail%20Init Can%20Go%20Forward?)
    (Utilities|EndAPositiveSetUp
      (:Continue
        (bind (_direction _y) (Timeline|Swing_Fail ReverseFromEnd)
          (:Update
            (Transformation|SetActorRotation (Math|Rotator|MakeRotator (.roll _returnvalue) (Math|Float|Lerp (Variables|Default|GetA) (Variables|Default|GetB) _y) (.yaw _returnvalue))))
          (:Finished
            (if (Utilities|Enum|Equal(Enum) _direction "Forward")
              (Variables|Default|SetCan%20Go%20Forward? (not (stale Custom|Fail%20Init Can%20Go%20Forward?)))
              ;;[1 1 1] time to let the player interact
              (Variables|Default|SetCan%20Swing? true)
              (Utilities|FlowControl|Delay 0.1)
              (CallFunction|FailEnd)
              (else
                (bind _output_get (Variables|Default|SetCan%20Go%20Forward? (stale Custom|Fail%20Init Can%20Go%20Forward?)))
                (Variables|Default|SetCan%20Swing? true)
                (Utilities|FlowControl|Delay 0.1)
                (CallFunction|FailInit _output_get)))))))
    (else
      (Utilities|EndANegativeSetUp
        (:Continue
          (Timeline|Swing_Fail ReverseFromEnd))))))

(event Custom|Swing_Begin
  (params (Can%20Go%20Forward? :type Boolean))
  (bind _returnvalue (Transformation|GetActorRotation))
  (bind _forward (Variables|Default|Getforward))
  (bind _backguard (Variables|Default|Getbackguard))
  ;[1 1 1] Normal swing
  (bind _output_get (Variables|Default|Setiniti%20position (.pitch (Transformation|GetActorRotation))))
  (if Can%20Go%20Forward?
    (Variables|Default|Setfinal%20position (* (Variables|Default|Getforward) (Variables|Default|Getsteps)))
    (else
      (Variables|Default|Setfinal%20position (* (Variables|Default|Getbackguard) (Variables|Default|Getsteps)))))
  (Variables|Default|SetCan%20Swing? false)
  (bind (_direction _y) (Timeline|Swing%20Timeline PlayFromStart)
    (:Update
      (Transformation|SetActorRotation (Math|Rotator|MakeRotator (.roll _returnvalue) (Math|Float|Lerp (Variables|Default|Getiniti%20position) (Variables|Default|Getfinal%20position) _y) (.yaw _returnvalue))))
    (:Finished
      (if (Utilities|Enum|Equal(Enum) _direction "Forward")
        (if Can%20Go%20Forward?
          (Math|Integer|DecrementInt _backguard
            (:%20%20
              (Utilities|<=or>= _backguard -3 true false)
              (Variables|Default|SetCan%20Go%20Forward? true)))
          (else
            (Math|Integer|IncrementInt _forward
              (:%20%20
                (Utilities|<=or>= _forward 3 false true)
                (Variables|Default|SetCan%20Go%20Forward? false))))))
      (Variables|Default|SetCan%20Swing? true)
      (Variables|Default|Settimer 0.0))))

(event Custom|Swing_End
  (bind _returnvalue (Transformation|GetActorRotation))
  (bind _forward (Variables|Default|Getforward))
  (bind _backguard (Variables|Default|Getbackguard))
  ;[1 1 1] Normal swing
  (Variables|Default|SetCan%20Swing? false)
  (bind (_direction _y) (Timeline|Swing%20Timeline ReverseFromEnd)
    (:Update
      (Transformation|SetActorRotation (Math|Rotator|MakeRotator (.roll _returnvalue) (Math|Float|Lerp (Variables|Default|Getiniti%20position) (Variables|Default|Getfinal%20position) _y) (.yaw _returnvalue))))
    (:Finished
      (if (Utilities|Enum|Equal(Enum) _direction "Forward")
        (if (stale Custom|Swing_Begin Can%20Go%20Forward?)
          (Math|Integer|DecrementInt _backguard
            (:%20%20
              (Utilities|<=or>= _backguard -3 true false)
              (Variables|Default|SetCan%20Go%20Forward? true)))
          (else
            (Math|Integer|IncrementInt _forward
              (:%20%20
                (Utilities|<=or>= _forward 3 false true)
                (Variables|Default|SetCan%20Go%20Forward? false))))))
      (Variables|Default|SetCan%20Swing? true)
      (Variables|Default|Settimer 0.0))))

(event Custom|stopSwing
  (bind _returnvalue (Transformation|GetActorRotation))
  ;[1 1 1] Swing when fail
  (Variables|Default|SetCan%20Swing? true)
  (Variables|Default|SetinitialSwing true)
  (Variables|Default|Settimer 0.0)
  (Variables|Default|Setfailed false)
  (Variables|Default|SetB 0.0)
  (Variables|Default|SetA 0.0)
  (bind (_direction _y) (Timeline|Swing_Fail Stop)
    (:Update
      (Transformation|SetActorRotation (Math|Rotator|MakeRotator (.roll _returnvalue) (Math|Float|Lerp (Variables|Default|GetA) (Variables|Default|GetB) _y) (.yaw _returnvalue))))
    (:Finished
      (if (Utilities|Enum|Equal(Enum) _direction "Forward")
        (Variables|Default|SetCan%20Go%20Forward? (not (stale Custom|Fail%20Init Can%20Go%20Forward?)))
        ;;[1 1 1] time to let the player interact
        (Variables|Default|SetCan%20Swing? true)
        (Utilities|FlowControl|Delay 0.1)
        (CallFunction|FailEnd)
        (else
          (bind _output_get (Variables|Default|SetCan%20Go%20Forward? (stale Custom|Fail%20Init Can%20Go%20Forward?)))
          (Variables|Default|SetCan%20Swing? true)
          (Utilities|FlowControl|Delay 0.1)
          (CallFunction|FailInit _output_get))))))

(event EventBeginPlay
  (Variables|/Game/JuegoX/Blueprints/Objects/Interactable.Interactable_C|SetMesh (Variables|Default|GetInteractable) (Variables|Default|GetMesh))
  (Variables|/Game/JuegoX/Blueprints/Objects/Interactable.Interactable_C|SetText (Variables|Default|GetInteractable) (Variables|Default|GetTextRender))
  (Variables|/Game/JuegoX/Blueprints/Objects/Interactable.Interactable_C|SetinitialRot (Variables|Default|GetInteractable) (Transformation|GetWorldRotation (Variables|Default|GetDefaultSceneRoot)))
  (Variables|/Game/JuegoX/Blueprints/Objects/Interactable.Interactable_C|SetfadeE (Variables|Default|GetInteractable) true)
  (bind _asfirst_person_character (Utilities|Casting|CastToFirstPersonCharacter (Game|GetPlayerCharacter 0)))
  (bind _output_get (Variables|Default|Setplayer _asfirst_person_character))
  (Variables|/Game/JuegoX/Blueprints/Objects/Interactable.Interactable_C|Setplayer (Variables|Default|GetInteractable) _output_get)
  (Variables|/Game/JuegoX/Blueprints/Objects/Interactable.Interactable_C|Setis%20a%20nonInspectionable%20Object? (Variables|Default|GetInteractable) true)
  (Variables|Default|SetSwinging false)
  (bind _asmy_game_instance (Utilities|Casting|CastToMyGameInstance (Game|GetGameInstance)))
  (Variables|Default|SetGame%20Instance _asmy_game_instance))

(event Collision|EventActorBeginOverlap
  (params (OtherActor :type Actor%20Object%20Reference)))

(event EventTick
  (params (DeltaSeconds :type Float%20%28single-precision%29))
  (bind _returnvalue (Game|GetPlayerController 0))
  (if (Variables|/Game/JuegoX/Blueprints/Objects/Interactable.Interactable_C|GetisInspectingIt (Variables|Default|GetInteractable))
    (Input|EnableInput _returnvalue :!label _label)
    (elif (Variables|/Game/JuegoX/Blueprints/Objects/Interactable.Interactable_C|GetisFocused? (Variables|Default|GetInteractable))
      (goto _label)
      (else
        (Input|DisableInput _returnvalue)))))

(event Input|ActionEvents|InputActionInspect
  (params (Key :type Key%20Structure :default "None"))
  (:Pressed
    (if (Variables|/Game/JuegoX/Blueprints/Objects/Interactable.Interactable_C|GetinteractionActivated (Variables|Default|GetInteractable))
      (if (Variables|Default|GetSwinging)
        (Variables|Default|SetSwinging false)
        (Variables|/Game/FirstPersonBP/Blueprints/FirstPersonCharacter.FirstPersonCharacter_C|SetwakeUp (Variables|Default|GetPlayer) false)
        (bind _output_get (Variables|Default|SetA (.pitch (Transformation|GetActorRotation))))
        (CallFunction|FailInit (> _output_get 0.0))
        (Game|Player|SetViewTargetwithBlend (Game|GetPlayerController 0) (Game|GetPlayerCharacter 0) 0.0 "VTBlend_Linear" 1.0 false)
        (Utilities|FlowControl|Delay 0.2)
        (else
          (Variables|Default|SetSwinging true)
          (Variables|/Game/FirstPersonBP/Blueprints/FirstPersonCharacter.FirstPersonCharacter_C|SetwakeUp (Variables|Default|GetPlayer) true)
          (Game|Player|SetViewTargetwithBlend (Game|GetPlayerController 0) (Variables|Default|GetCamera) 0.0 "VTBlend_Linear" 1.0 false)
          (Utilities|FlowControl|Delay 0.2))))))

(event Input|MouseEvents|MouseY
  (params (AxisValue :type Float%20%28single-precision%29))
  (if (Variables|Default|GetSwinging)
    (if (Variables|Default|GetCan%20Swing?)
      (Variables|Default|SetswingValue AxisValue)
      (CallFunction|Swing))))

(fn ConstructionScript)

(fn Swing
  (bind _trampilla (Variables|Default|GetTrampilla))
  (if (Math|Float|NearlyEqual(Float) (.pitch (Transformation|GetWorldRotation (Variables|Default|GetDefaultSceneRoot))) (LocalVariables|GetFinal%20angle) 1.0)
    ;[1 1 1] puzzle completado
    (Utilities|FlowControl|DoOnce false
      (:Completed
        (Variables|/Game/JuegoX/Blueprints/MyGameInstance.MyGameInstance_C|SetTrampillaAbierta? (Variables|Default|GetGame%20Instance) true)
        (Audio|PlaySound2D (Variables|/Game/JuegoX/Blueprints/Objects/OBJ_Trampilla.OBJ_Trampilla_C|GetSound _trampilla) 1.0 1.0 0.0 0 _trampilla)
        (Sequencer|Player|Play (Variables|/Script/ActorSequence.ActorSequenceComponent|GetSequencePlayer (Variables|/Game/JuegoX/Blueprints/Objects/OBJ_Trampilla.OBJ_Trampilla_C|GetAnim (Variables|Default|GetTrampilla))) :!class /Script/MovieScene.MovieSceneSequencePlayer)))
    (elif (and (Math|Float|NearlyEqual(Float) (Variables|Default|GetswingValue) 0.0 1e-06) (Variables|Default|GetCan%20Swing?))
      (Utilities|+= (Variables|Default|Gettimer) (Utilities|Time|GetWorldDeltaSeconds)
        (:Outputs
          (if (and (>= (Variables|Default|Gettimer) 1.0) (not (Variables|Default|Getfailed)))
            (Variables|Default|Setfailed true)
            (bind _output_get (Variables|Default|SetA (.pitch (Transformation|GetActorRotation))))
            (CallFunction|FailInit (> _output_get 0.0)))))
      (else
        (Variables|Default|Settimer 0.0)
        (Variables|Default|Setfailed false)
        (if (Audio|Components|Audio|IsPlaying (Variables|Default|GetSwing_Fail))
          (CallFunction|StopSwing))
        (if (Variables|Default|GetinitialSwing)
          ;[1 1 1] initial
          (Variables|Default|SetinitialSwing false)
          (Variables|Default|Setforward 1)
          (Variables|Default|Setbackguard -1)
          (Math|Float|CompareFloat (Variables|Default|GetswingValue) 0.0
            (:>
              (CallFunction|SwingBegin false))
            (:<
              (CallFunction|SwingBegin true)))
          (else
            (Math|Float|CompareFloat (Variables|Default|GetswingValue) 0.0
              (:>
                (if (Variables|Default|GetCan%20Go%20Forward?)
                  (CallFunction|SwingBegin false)
                  (else
                    ;[1 1 1] fail
                    (bind _output_get_2 (Variables|Default|SetA (.pitch (Transformation|GetActorRotation)) :!label _label))
                    (CallFunction|FailInit (> _output_get_2 0.0)))))
              (:<
                (if (Variables|Default|GetCan%20Go%20Forward?)
                  (goto _label)
                  (else
                    (CallFunction|SwingBegin true)))))))))))

(fn FloatRange
  (params (Var%20Inc :type Integer%20%28by%20ref%29) (isNegative? :type Boolean)))

(fn NumOfSteps
  (Math|Integer|CompareInt 0))