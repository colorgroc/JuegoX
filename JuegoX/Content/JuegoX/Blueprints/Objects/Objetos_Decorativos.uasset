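; Decorative prop that the player can inspect, bringing it to a view point and back.
; Tick enables input while Interactuable reports focus or inspection.
; Inspect toggles a timeline that moves the actor and the controls widget, with tags choosing a farther "Big" view point or "Seal" scream.
; "Polaroid" props also straighten, double in size and use a duplicate-mesh outline, red when focused and white within glow distance.
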(event Custom|EndInspection
  (bind _interactuable (Variables|Default|GetInteractuable))
  (bind _init_scale (Variables|Default|Getinit%20scale))
  (CallFunction|HideControls)
  (Variables|/Game/JuegoX/Blueprints/Objects/Interactable.Interactable_C|SetisInspectingIt (Variables|Default|GetInteractuable) false)
  (Variables|/Game/FirstPersonBP/Blueprints/FirstPersonCharacter.FirstPersonCharacter_C|SetplayerInspectingObject (Variables|Default|Getplayer) false)
  (bind _move_object (Timeline|Inspect Reverse)
    (:Update
      (bind _output_get (Variables|Default|SetMovedObject _move_object))
      ;[1 1 1] Si es una Polaroid
      (if (Actor|ActorHasTag "Polaroid")
        (Variables|Default|Setrotation "0.000000, 0, 0") ; Rotacion pa que mire enfrente bien
        (Transformation|SetActorLocation (Math|Vector|Lerp(Vector) (Variables|/Game/JuegoX/Blueprints/Objects/Interactable.Interactable_C|GetinitialPos _interactuable) (Variables|/Game/JuegoX/Blueprints/Objects/Interactable.Interactable_C|GetinspectionPoint _interactuable) _output_get) false false)
        (Transformation|SetActorRotation (Math|Rotator|Lerp(Rotator) (Variables|/Game/JuegoX/Blueprints/Objects/Interactable.Interactable_C|GetinitialRot _interactuable) (Variables|Default|Getrotation) _output_get))
        (Transformation|SetActorScale3D (Math|Vector|Lerp(Vector) _init_scale (* _init_scale 2.0) _output_get))
        (else
          (Variables|Default|Setrotation (Transformation|GetActorRotation))
          (Transformation|SetActorLocationAndRotation (Math|Vector|Lerp(Vector) (Variables|/Game/JuegoX/Blueprints/Objects/Interactable.Interactable_C|GetinitialPos _interactuable) (Variables|/Game/JuegoX/Blueprints/Objects/Interactable.Interactable_C|GetinspectionPoint _interactuable) _output_get) (Math|Rotator|Lerp(Rotator) (Variables|/Game/JuegoX/Blueprints/Objects/Interactable.Interactable_C|GetinitialRot _interactuable) (Variables|Default|Getrotation) _output_get) true))))))

(event EventTick
  (params (DeltaSeconds :type Float%20%28single-precision%29))
  (bind _returnvalue (Actor|ActorHasTag "Polaroid"))
  (bind _returnvalue_2 (Game|GetPlayerController 0))
  (bind _materialhighlight (Variables|Default|GetMaterialHighlight))
  (bind _materialhighlight_2 (Variables|Default|GetMaterialHighlight))
  (if (Variables|/Game/JuegoX/Blueprints/Objects/Interactable.Interactable_C|GetisInspectingIt (Variables|Default|GetInteractuable))
    (if _returnvalue
      (Rendering|Material|SetScalarParameterValue _materialhighlight_2 "Scale" 0.0 :!class /Script/Engine.MaterialInstanceDynamic))
    (Input|EnableInput _returnvalue_2 :!label _label)
    (elif (Variables|/Game/JuegoX/Blueprints/Objects/Interactable.Interactable_C|GetisFocused? (Variables|Default|GetInteractuable))
      (if _returnvalue
        (Rendering|Material|SetScalarParameterValue _materialhighlight_2 "Scale" 0.5 :!class /Script/Engine.MaterialInstanceDynamic)
        (Rendering|Material|SetVectorParameterValue _materialhighlight_2 "Color" "(R=1.000000,G=0.000000,B=0.000000,A=1.000000)" :!class /Script/Engine.MaterialInstanceDynamic)
        (goto _label)
        (else
          (goto _label)))
      (elif _returnvalue
        (Input|DisableInput _returnvalue_2)
        (Math|Float|CompareFloat (Transformation|GetDistanceTo (Variables|Default|Getplayer)) (Variables|/Game/JuegoX/Blueprints/Objects/Interactable.Interactable_C|GetDistance%20to%20Glow (Variables|Default|GetInteractuable))
          (:>
            (Rendering|Material|SetScalarParameterValue _materialhighlight "Scale" 0.0 :!class /Script/Engine.MaterialInstanceDynamic))
          (:==
            (Rendering|Material|SetScalarParameterValue _materialhighlight "Scale" 0.5 :!class /Script/Engine.MaterialInstanceDynamic :!label _label_2))
          (:<
            (goto _label_2)))
        (Rendering|Material|SetVectorParameterValue _materialhighlight "Color" "(R=1.000000,G=1.000000,B=1.000000,A=1.000000)" :!class /Script/Engine.MaterialInstanceDynamic)
        (else
          (Input|DisableInput _returnvalue_2))))))

(event EventBeginPlay
  (bind _mesh (Variables|Default|GetMesh))
  (if (Actor|ActorHasTag "Polaroid")
    (bind _returnvalue (AddComponent|AddStaticMeshComponent true (Transformation|GetWorldTransform _mesh)))
    (Transformation|AttachComponentToComponent _returnvalue _mesh "None" "KeepRelative" "KeepRelative" "KeepRelative" true)
    (Components|StaticMesh|SetStaticMesh _returnvalue (Variables|/Script/Engine.StaticMeshComponent|GetStaticMesh _mesh))
    (Rendering|Material|SetMaterial _returnvalue 0 (Rendering|Material|GetMaterial _mesh 0))
    (bind _returnvalue_2 (Rendering|Material|CreateDynamicMaterialInstance _returnvalue 0 "/Game/JuegoX/Materials/Outline_ObjectsHided.Outline_ObjectsHided" "None" :!class /Script/Engine.PrimitiveComponent))
    (Variables|Default|SetMaterialHighlight _returnvalue_2))
  (bind _asfirst_person_character (Utilities|Casting|CastToFirstPersonCharacter (Game|GetPlayerCharacter 0)))
  (Variables|Default|Setplayer _asfirst_person_character)
  (if (Actor|ActorHasTag "Polaroid")
    (Variables|Default|Setinit%20scale (Transformation|GetActorScale3D))))

(event Input|ActionEvents|InputActionInspect
  (params (Key :type Key%20Structure :default "None"))
  (bind _player (Variables|Default|Getplayer))
  (bind _interactuable (Variables|Default|GetInteractuable))
  (bind _interactuable_2 (Variables|Default|GetInteractuable))
  (bind _init_scale (Variables|Default|Getinit%20scale))
  (:Pressed
    (if (Variables|/Game/JuegoX/Blueprints/Objects/Interactable.Interactable_C|GetisInspectingIt _interactuable_2)
      (CallFunction|EndInspection)
      (else
        (Utilities|FlowControl|Sequence
          (:then_0
            (CallFunction|ShowControls))
          (:then_1
            (if (Actor|ActorHasTag "Seal")
              (Audio|PlaySound2D "/Game/Soniditos/435851__dersuperanton__hello-scream-male-loud.435851__dersuperanton__hello-scream-male-loud" 1.0 1.0 0.0 0 0)))
          (:then_2
            (if (Actor|ActorHasTag "Big")
              (Variables|/Game/JuegoX/Blueprints/Objects/Interactable.Interactable_C|SetinspectionPoint _interactuable_2 (Transformation|GetWorldLocation (Variables|/Game/FirstPersonBP/Blueprints/FirstPersonCharacter.FirstPersonCharacter_C|GetInpectionViewBig _player)))
              (else
                (Variables|/Game/JuegoX/Blueprints/Objects/Interactable.Interactable_C|SetinspectionPoint _interactuable_2 (Transformation|GetWorldLocation (Variables|/Game/FirstPersonBP/Blueprints/FirstPersonCharacter.FirstPersonCharacter_C|GetInpectionView _player)))))
            (Variables|/Game/JuegoX/Blueprints/Objects/Interactable.Interactable_C|SetisInspectingIt _interactuable_2 true)
            (Variables|/Game/FirstPersonBP/Blueprints/FirstPersonCharacter.FirstPersonCharacter_C|SetplayerInspectingObject (Variables|Default|Getplayer) true)
            (bind _move_object (Timeline|Inspect Play)
              (:Update
                (bind _output_get (Variables|Default|SetMovedObject _move_object))
                ;[1 1 1] Si es una Polaroid
                (if (Actor|ActorHasTag "Polaroid")
                  (Variables|Default|Setrotation "0.000000, 0, 0") ; Rotacion pa que mire enfrente bien
                  (Transformation|SetActorLocation (Math|Vector|Lerp(Vector) (Variables|/Game/JuegoX/Blueprints/Objects/Interactable.Interactable_C|GetinitialPos _interactuable) (Variables|/Game/JuegoX/Blueprints/Objects/Interactable.Interactable_C|GetinspectionPoint _interactuable) _output_get) false false)
                  (Transformation|SetActorRotation (Math|Rotator|Lerp(Rotator) (Variables|/Game/JuegoX/Blueprints/Objects/Interactable.Interactable_C|GetinitialRot _interactuable) (Variables|Default|Getrotation) _output_get))
                  (Transformation|SetActorScale3D (Math|Vector|Lerp(Vector) _init_scale (* _init_scale 2.0) _output_get))
                  (else
                    (Variables|Default|Setrotation (Transformation|GetActorRotation))
                    (Transformation|SetActorLocationAndRotation (Math|Vector|Lerp(Vector) (Variables|/Game/JuegoX/Blueprints/Objects/Interactable.Interactable_C|GetinitialPos _interactuable) (Variables|/Game/JuegoX/Blueprints/Objects/Interactable.Interactable_C|GetinspectionPoint _interactuable) _output_get) (Math|Rotator|Lerp(Rotator) (Variables|/Game/JuegoX/Blueprints/Objects/Interactable.Interactable_C|GetinitialRot _interactuable) (Variables|Default|Getrotation) _output_get) true)))))))))))

(fn ConstructionScript)

(fn ShowControls
  (bind _player (Variables|Default|Getplayer))
  (if (Utilities|IsValid (Variables|/Game/FirstPersonBP/Blueprints/FirstPersonCharacter.FirstPersonCharacter_C|GetWB_NoPickUp (Variables|Default|Getplayer)))
    _
    (else
      (bind _returnvalue (UserInterface|CreateWidget "/Game/JuegoX/UI/HUD/WB_NoPickUp_Objects.WB_NoPickUp_Objects_C" (Game|GetPlayerController 0)))
      (Variables|/Game/FirstPersonBP/Blueprints/FirstPersonCharacter.FirstPersonCharacter_C|SetWB_NoPickUp _player _returnvalue)))
  (UserInterface|Viewport|AddtoViewport (Variables|/Game/FirstPersonBP/Blueprints/FirstPersonCharacter.FirstPersonCharacter_C|GetWB_NoPickUp _player) 0))

(fn HideControls
  (Widget|RemovefromParent (Variables|/Game/FirstPersonBP/Blueprints/FirstPersonCharacter.FirstPersonCharacter_C|GetWB_NoPickUp (Variables|Default|Getplayer))))