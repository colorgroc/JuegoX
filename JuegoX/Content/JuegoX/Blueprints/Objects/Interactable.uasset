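; Actor component for interactable objects that drives highlighting of the owner's static mesh through custom depth and stencil values.
; Every tick it reads the first-person character's state, hiding the highlight while the player is frozen.
; A focused object gets its own stencil value; unfocused, non-important ones glow within a set distance unless the player is inspecting the map.
; Unfocused objects flagged important keep their current depth state.
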(event EventBeginPlay
  (Variables|Default|SetisFocused? false)
  (Variables|Default|SetisInspectingIt false)
  (Variables|Default|SetMesh (Actor|GetComponentbyClass (Components|GetOwner) "/Script/Engine.StaticMeshComponent")))

(event EventTick
  (params (DeltaSeconds :type Float%20%28single-precision%29))
  (bind _returnvalue (Game|GetPlayerCharacter 0))
  (bind _mesh (Variables|Default|GetMesh))
  (bind _mesh_2 (Variables|Default|GetMesh))
  (bind _asfirst_person_character (Utilities|Casting|CastToFirstPersonCharacter _returnvalue))
  (if (Variables|/Game/FirstPersonBP/Blueprints/FirstPersonCharacter.FirstPersonCharacter_C|GetplayerFrozen _asfirst_person_character)
    (Rendering|SetRenderCustomDepth _mesh false :!label _label)
    (Rendering|SetCustomDepthStencilValue _mesh 1 :!label _label_2)
    (elif (Variables|Default|GetisFocused?)
      (Rendering|SetRenderCustomDepth _mesh_2 true)
      (Rendering|SetCustomDepthStencilValue _mesh_2 2)
      (elif (not (Variables|Highlight|GetisImportant?))
        (if (Variables|/Game/FirstPersonBP/Blueprints/FirstPersonCharacter.FirstPersonCharacter_C|GetplayerInpectingMapa _asfirst_person_character)
          (Rendering|SetRenderCustomDepth _mesh_2 false)
          (else
            (Math|Float|CompareFloat (Transformation|GetDistanceTo (Components|GetOwner) _returnvalue) (Variables|Highlight|GetDistance%20to%20Glow)
              (:>
                (goto _label))
              (:==
                _)
              (:<
                _))
            (Rendering|SetRenderCustomDepth _mesh true)
            (goto _label_2)))))))