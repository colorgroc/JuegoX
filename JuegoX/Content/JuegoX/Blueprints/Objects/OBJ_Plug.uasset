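; OBJ_Plug is an interactable power plug that the player connects to the radio cassette with a cable item.
; Its Interactable component starts disabled; once activated, focus gates input, and Inspect checks the GameInstance's cable flags.
; If the radio's cable is out, its end snaps to the plug, the connection is recorded and the inventory cable hides.
; Otherwise the plug toggles its own runtime-created cable component trailing to the player.
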(event EventTick
  (params (DeltaSeconds :type Float%20%28single-precision%29))
  (bind _returnvalue (Game|GetPlayerController 0))
  (if (Variables|/Game/JuegoX/Blueprints/Objects/Interactable.Interactable_C|GetinteractionActivated (Variables|Default|GetInteractable))
    (if (Variables|/Game/JuegoX/Blueprints/Objects/Interactable.Interactable_C|GetisFocused? (Variables|Default|GetInteractable))
      (Input|EnableInput _returnvalue)
      (else
        (Input|DisableInput _returnvalue)))))

(event EventBeginPlay
  (bind _asfirst_person_character (Utilities|Casting|CastToFirstPersonCharacter (Game|GetPlayerCharacter 0)))
  (bind _output_get (Variables|Default|Setplayer _asfirst_person_character))
  (Variables|/Game/JuegoX/Blueprints/Objects/Interactable.Interactable_C|Setplayer (Variables|Default|GetInteractable) _output_get)
  (bind _asmy_game_instance (Utilities|Casting|CastToMyGameInstance (Game|GetGameInstance)))
  (Variables|Default|SetGameInstance _asmy_game_instance))

(event Input|ActionEvents|InputActionInspect
  (params (Key :type Key%20Structure :default "None"))
  (:Pressed
    (if (Variables|/Game/JuegoX/Blueprints/Objects/Interactable.Interactable_C|GetinteractionActivated (Variables|Default|GetInteractable))
      (CallFunction|Inspection))))

(fn ConstructionScript
  (Variables|Default|SetSound 0)
  (Variables|/Game/JuegoX/Blueprints/Objects/Interactable.Interactable_C|SetMesh (Variables|Default|GetInteractable) (Variables|Default|GetMesh))
  (Variables|/Game/JuegoX/Blueprints/Objects/Interactable.Interactable_C|SetText (Variables|Default|GetInteractable) (Variables|Default|GetTextRender))
  (Variables|/Game/JuegoX/Blueprints/Objects/Interactable.Interactable_C|Setis%20a%20nonInspectionable%20Object? (Variables|Default|GetInteractable) true)
  (bind _returnvalue (Actor|GetActorOfClass "/Game/JuegoX/Blueprints/Objects/OBJ_RadioCassette.OBJ_RadioCassette_C"))
  (Variables|Default|SetObject _returnvalue)
  (Variables|/Game/JuegoX/Blueprints/Objects/Interactable.Interactable_C|SetinteractionActivated (Variables|Default|GetInteractable) false))

(fn Inspection
  (if (not (Variables|/Game/JuegoX/Blueprints/MyGameInstance.MyGameInstance_C|GetCable_Connected? (Variables|Default|GetGameInstance)))
    (if (Variables|/Game/JuegoX/Blueprints/MyGameInstance.MyGameInstance_C|GetHas_Cable? (Variables|Default|GetGameInstance))
      (CallFunction|ConnectwithCable))))

(fn ConnectwithCable
  (if (Variables|/Game/JuegoX/Blueprints/Objects/OBJ_RadioCassette.OBJ_RadioCassette_C|GetCableConnected (Variables|Default|GetObject))
    (Variables|/Script/CableComponent.CableComponent|SetbAttachEnd (Variables|/Game/JuegoX/Blueprints/Objects/OBJ_RadioCassette.OBJ_RadioCassette_C|GetCable (Variables|Default|GetObject)) true)
    (Class|CableComponent|SetAttachEndto (Variables|/Game/JuegoX/Blueprints/Objects/OBJ_RadioCassette.OBJ_RadioCassette_C|GetCable (Variables|Default|GetObject)) self "None" "None")
    (Variables|/Script/CableComponent.CableComponent|SetEndLocation (Variables|/Game/JuegoX/Blueprints/Objects/OBJ_RadioCassette.OBJ_RadioCassette_C|GetCable (Variables|Default|GetObject)) "0, 0, 0")
    (Variables|Default|SetCableConnected true)
    (Variables|/Game/JuegoX/Blueprints/MyGameInstance.MyGameInstance_C|SetCable_Connected? (Variables|Default|GetGameInstance) true)
    (bind _returnvalue (Actor|GetActorOfClass "/Game/JuegoX/Blueprints/Objects/OBJ_Cable_KeyChild.OBJ_Cable_KeyChild_C"))
    (Default|HideInventory _returnvalue)
    (elif (Variables|Default|GetCableConnected)
      (Utilities|IsValid (Variables|Default|GetCable)
        (:Is%20Valid
          (Components|DestroyComponent (Variables|Default|GetCable))
          (Variables|Default|SetCableConnected false)))
      (else
        (bind _returnvalue_2 (AddComponent|AddCableComponent false (Variables|Default|GetTransform)))
        (Variables|Default|SetCable _returnvalue_2)
        (Variables|/Script/CableComponent.CableComponent|SetbAttachEnd (Variables|Default|GetCable) true)
        (Class|CableComponent|SetAttachEndto (Variables|Default|GetCable) (Variables|Default|Getplayer) "None" "None")
        (Variables|/Script/CableComponent.CableComponent|SetCableWidth (Variables|Default|GetCable) 3.0)
        (Variables|/Script/CableComponent.CableComponent|SetbEnableCollision (Variables|Default|GetCable) true)
        (Variables|Default|SetCableConnected true)))))