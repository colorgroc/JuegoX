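; Interactable child Blueprint for a saved compass object, attached at BeginPlay to the mesh of the place where it is stored.
; A duplicate of its mesh, set in the construction script, carries a dynamic hidden-object outline material.
; Each Tick drives that outline: hidden while inspected, red when focused, otherwise white within glow distance of the player.
; Input is enabled only while inspected or focused, and ConnectWithCable is empty.
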(event EventTick
  (params (DeltaSeconds :type Float%20%28single-precision%29))
  (bind _returnvalue (Game|GetPlayerController 0))
  (bind _materialhighlight (Variables|Default|GetmaterialHighlight))
  (bind _materialhighlight_2 (Variables|Default|GetmaterialHighlight))
  (if (Variables|/Game/JuegoX/Blueprints/Objects/Interactable.Interactable_C|GetisInspectingIt (Variables|Default|GetInteractable))
    (Rendering|Material|SetScalarParameterValue _materialhighlight "Scale" 0.0 :!class /Script/Engine.MaterialInstanceDynamic)
    (Input|EnableInput _returnvalue :!label _label)
    (elif (Variables|/Game/JuegoX/Blueprints/Objects/Interactable.Interactable_C|GetisFocused? (Variables|Default|GetInteractable))
      (Rendering|Material|SetScalarParameterValue _materialhighlight "Scale" 0.5 :!class /Script/Engine.MaterialInstanceDynamic)
      (Rendering|Material|SetVectorParameterValue _materialhighlight "Color" "(R=1.000000,G=0.000000,B=0.000000,A=1.000000)" :!class /Script/Engine.MaterialInstanceDynamic)
      (goto _label)
      (else
        (Input|DisableInput _returnvalue)
        (Math|Float|CompareFloat (Transformation|GetDistanceTo (Variables|Default|Getplayer)) (Variables|/Game/JuegoX/Blueprints/Objects/Interactable.Interactable_C|GetDistance%20to%20Glow (Variables|Default|GetInteractable))
          (:>
            (Rendering|Material|SetScalarParameterValue _materialhighlight_2 "Scale" 0.0 :!class /Script/Engine.MaterialInstanceDynamic))
          (:==
            (Rendering|Material|SetScalarParameterValue _materialhighlight_2 "Scale" 0.5 :!class /Script/Engine.MaterialInstanceDynamic :!label _label_2))
          (:<
            (goto _label_2)))
        (Rendering|Material|SetVectorParameterValue _materialhighlight_2 "Color" "(R=1.000000,G=1.000000,B=1.000000,A=1.000000)" :!class /Script/Engine.MaterialInstanceDynamic)))))

(event EventBeginPlay
  (|CallParentFunction)
  (bind _returnvalue (Rendering|Material|CreateDynamicMaterialInstance (Variables|Default|GetDuplicated) 0 "/Game/JuegoX/Materials/Outline_ObjectsHided.Outline_ObjectsHided" "None" :!class /Script/Engine.PrimitiveComponent))
  (Variables|Default|SetmaterialHighlight _returnvalue)
  (Transformation|AttachComponentToComponent (Variables|/Game/JuegoX/Blueprints/Objects/Interactable_Static/Dressers/OBJ_Dresser_DrawerParent.OBJ_Dresser_DrawerParent_C|GetMesh (Variables|Default|GetlugarDondeEstaGuardada)) "None" "KeepWorld" "KeepWorld" "KeepWorld" true))

(fn ConstructionScript
  (|CallParentFunction)
  (Components|StaticMesh|SetStaticMesh (Variables|Default|GetDuplicated) (Variables|/Script/Engine.StaticMeshComponent|GetStaticMesh (Variables|Character|GetMesh))))

(fn ConnectwithCable)