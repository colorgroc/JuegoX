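; Opened, readable diary that shows five pages of Spanish story text, then spawns a paper plane for the player.
; Tick gates interaction and input by focus, inspection and paper-plane state; each Interact advances a page in DialogueWidget.
; Inspect, or GameInstance.DiaryCompleted, closes it by spawning a closed OBJ_Diary_Parent and lerping that back to its initial transform on a timeline.
; It then re-enables the Sillon (armchair), resets DiaryCompleted and destroys itself.
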(event Custom|CloseDiary
  (if (not (Variables|/Game/FirstPersonBP/Blueprints/FirstPersonCharacter.FirstPersonCharacter_C|GethacerAvionDePapel? (Variables|Default|Getplayer)))
    (bind _returnvalue (Game|SpawnActorfromClass "/Game/JuegoX/Blueprints/Objects/OBJ_Diary_Parent.OBJ_Diary_Parent_C" (Math|Transform|MakeTransform (Transformation|GetActorLocation) (Transformation|GetActorRotation) "1.000000,1.000000,1.000000") "AlwaysSpawn" 0 0))
    (Variables|Default|SetDiarioCerrado _returnvalue)
    (Variables|/Game/JuegoX/Blueprints/Objects/Interactable.Interactable_C|SetinitialPos (Variables|/Game/JuegoX/Blueprints/Objects/OBJ_Diary_Parent.OBJ_Diary_Parent_C|GetInteractuable (Variables|Default|GetDiarioCerrado)) (Variables|Default|GetinitialPoint))
    (Variables|/Game/JuegoX/Blueprints/Objects/Interactable.Interactable_C|SetinitialRot (Variables|/Game/JuegoX/Blueprints/Objects/OBJ_Diary_Parent.OBJ_Diary_Parent_C|GetInteractuable (Variables|Default|GetDiarioCerrado)) (Variables|Default|GetinitialRot))
    (Variables|/Game/JuegoX/Blueprints/Objects/OBJ_Diary_Parent.OBJ_Diary_Parent_C|SetinspectionPos (Variables|Default|GetDiarioCerrado) (Transformation|GetActorLocation))
    (Variables|/Game/JuegoX/Blueprints/Objects/OBJ_Diary_Parent.OBJ_Diary_Parent_C|SetSillon (Variables|Default|GetDiarioCerrado) (Variables|Default|GetSillon))
    (Variables|/Game/JuegoX/Blueprints/Objects/Sillon.Sillon_C|SetDiario (Variables|Default|GetSillon) (Variables|Default|GetDiarioCerrado))
    (Components|DestroyComponent (Variables|Character|GetMesh))
    (Variables|/Game/JuegoX/Blueprints/Objects/Interactable.Interactable_C|SetisInspectingIt (Variables|/Game/JuegoX/Blueprints/Objects/OBJ_Diary_Parent.OBJ_Diary_Parent_C|GetInteractuable (Variables|Default|GetDiarioCerrado)) false)
    (bind _move_object (Timeline|CloseDiary_Timeline Play)
      (:Update
        (Transformation|SetActorLocationAndRotation (Variables|Default|GetDiarioCerrado) (Math|Vector|Lerp(Vector) (Transformation|GetActorLocation (Variables|Default|GetDiarioCerrado)) (Variables|Default|GetinitialPoint) _move_object) (Math|Rotator|Lerp(Rotator) (Transformation|GetActorRotation (Variables|Default|GetDiarioCerrado)) (Variables|Default|GetinitialRot) _move_object)))
      (:Finished
        (CallFunction|FinishUpdate)))))

(event Custom|FinishUpdate
  (if (Utilities|IsValid (Variables|Default|GetSillon))
    (Variables|/Game/JuegoX/Blueprints/Objects/Interactable.Interactable_C|SetinteractionActivated (Variables|/Game/JuegoX/Blueprints/Objects/Sillon.Sillon_C|GetInteractuable (Variables|Default|GetSillon)) true)
    (Variables|Default|SetPage 0)
    (CallFunction|HideControls)
    (Variables|/Game/JuegoX/Blueprints/MyGameInstance.MyGameInstance_C|Setdiary_completed (Variables|Default|GetgameInstance) false)
    (Actor|DestroyActor)))

(event EventTick
  (params (DeltaSeconds :type Float%20%28single-precision%29))
  (bind _returnvalue (Game|GetPlayerController 0))
  (if (Variables|/Game/JuegoX/Blueprints/MyGameInstance.MyGameInstance_C|Getdiary_completed (Variables|Default|GetgameInstance))
    (Utilities|FlowControl|DoOnce false
      (:Completed
        (CallFunction|CloseDiary)))
    (elif (Variables|/Game/JuegoX/Blueprints/Objects/Interactable.Interactable_C|GetisInspectingIt (Variables|Default|GetInteractuable))
      (Input|EnableInput _returnvalue :!label _label)
      (else
        (if (Variables|/Game/FirstPersonBP/Blueprints/FirstPersonCharacter.FirstPersonCharacter_C|GethacerAvionDePapel? (Variables|Default|Getplayer))
          (Variables|/Game/JuegoX/Blueprints/Objects/Interactable.Interactable_C|SetinteractionActivated (Variables|Default|GetInteractuable) false)
          (else
            (Variables|/Game/JuegoX/Blueprints/Objects/Interactable.Interactable_C|SetinteractionActivated (Variables|Default|GetInteractuable) true)
            (if (Variables|/Game/JuegoX/Blueprints/Objects/Interactable.Interactable_C|GetisFocused? (Variables|Default|GetInteractuable))
              (goto _label)
              (else
                _))))
        (Input|DisableInput _returnvalue)))))

(event EventBeginPlay
  (|CallParentFunction)
  (bind _returnvalue (UserInterface|CreateWidget "/Game/JuegoX/UI/Dialogue/DialogueWidget.DialogueWidget_C" (Game|GetPlayerController 0)))
  (bind _output_get (Variables|Default|SetDialogueWidget _returnvalue))
  (UserInterface|Viewport|AddtoViewport _output_get 0)
  (bind _asmy_game_instance (Utilities|Casting|CastToMyGameInstance (Game|GetGameInstance)))
  (Variables|Default|SetgameInstance _asmy_game_instance))

(event EventInteract
  (if (not (Variables|/Game/FirstPersonBP/Blueprints/FirstPersonCharacter.FirstPersonCharacter_C|GethacerAvionDePapel? (Variables|Default|Getplayer)))
    (if (not (Variables|/Game/FirstPersonBP/Blueprints/FirstPersonCharacter.FirstPersonCharacter_C|GetthrowingPaperPlane (Variables|Default|Getplayer)))
      (if (Variables|/Game/JuegoX/Blueprints/Objects/Interactable.Interactable_C|GetisFocused? (Variables|Default|GetInteractuable))
        (CallFunction|CheckPage)))))

(event EventInspect
  (CallFunction|CloseDiary))

(fn ConstructionScript
  (Variables|Default|Setsound 0))

(fn CheckPage
  (bind _player (Variables|Default|Getplayer))
  (bind _page (Variables|Default|GetPage))
  (if (>= _page (Variables|Default|GetnumOfPages))
    (if (not (Variables|/Game/FirstPersonBP/Blueprints/FirstPersonCharacter.FirstPersonCharacter_C|GethacerAvionDePapel? (Variables|Default|Getplayer)))
      (Utilities|FlowControl|Sequence
        (:then_0
          (CallFunction|HideControls))
        (:then_1
          (Variables|/Game/FirstPersonBP/Blueprints/FirstPersonCharacter.FirstPersonCharacter_C|SethacerAvionDePapel? (Variables|Default|Getplayer) true)
          (if (Utilities|IsValid (Variables|Default|GetDialogueWidget))
            (Widget|RemovefromParent (Variables|Default|GetDialogueWidget))
            (Variables|Default|SetDialogueWidget 0))
          (Audio|PlaySound2D "/Game/Soniditos/468134__aquafeniz__remove-sheet.468134__aquafeniz__remove-sheet" 1.0 1.0 0.0 0 0)
          (Game|SpawnActorfromClass "/Game/JuegoX/Blueprints/Objects/Avion.Avion_C" (Math|Transform|MakeTransform (Transformation|GetWorldLocation (Variables|/Game/FirstPersonBP/Blueprints/FirstPersonCharacter.FirstPersonCharacter_C|GetInpectionAvion _player)) (Transformation|GetWorldRotation (Variables|/Game/FirstPersonBP/Blueprints/FirstPersonCharacter.FirstPersonCharacter_C|GetFirstPersonCamera _player))) "AlwaysSpawn" 0 0))))
    (else
      (Math|Integer|IncrementInt _page
        (:%20%20
          (switch int _page
            (:1
              ;[1 1 1] Mostrar texto en pantalla segun page
              (Development|PrintString "Pagina 1" true true "(R=0.000000,G=0.362427,B=1.000000,A=1.000000)")
              (Variables|/Game/JuegoX/UI/Dialogue/DialogueWidget.DialogueWidget_C|SetDialogueText (Variables|Default|GetDialogueWidget) "Siempre tuve muy claro que viajaría a mil lugares, y conocería a muchas personas durante el trayecto. Que cogiera un avión hacia Suecia y empezara allí mi nueva vida como enfermera, era solo cuestión de tiempo."))
            (:2
              (Development|PrintString "Pagina 2" true true "(R=0.000000,G=0.362427,B=1.000000,A=1.000000)")
              (Variables|/Game/JuegoX/UI/Dialogue/DialogueWidget.DialogueWidget_C|SetDialogueText (Variables|Default|GetDialogueWidget) "Mi avión llevaba programado desde que decidí estudiar medicina. Podía ver, como si de un reloj a toda prisa se tratara, el tiempo que me quedaba a vuestro lado. Lo que nos une a los 4 es mucho más que un simple vínculo… Y lo sabéis. "))
            (:3
              (Development|PrintString "Pagina 3" true true "(R=0.000000,G=0.362427,B=1.000000,A=1.000000)")
              (Variables|/Game/JuegoX/UI/Dialogue/DialogueWidget.DialogueWidget_C|SetDialogueText (Variables|Default|GetDialogueWidget) "Ni siquiera hablamos mucho sobre el tema… Estaba claro que nos daba miedo comentarlo. Solo sé que si estábamos lejos de aquí, nuestras vidas volvían a ser normales.Ya casi no recuerdo nada. No me queda tiempo, Nate. "))
            (:4
              (Development|PrintString "Pagina 4" true true "(R=0.000000,G=0.362427,B=1.000000,A=1.000000)")
              (Variables|/Game/JuegoX/UI/Dialogue/DialogueWidget.DialogueWidget_C|SetDialogueText (Variables|Default|GetDialogueWidget) "Todo esto me está destrozando. Hubiera dado lo que fuera por utilizar eso que todos sabemos... Y volver contigo a ese lugar fantástico que tanto nos gusta, para siempre."))
            (:5
              (Development|PrintString "Pagina 5")
              (Variables|/Game/JuegoX/UI/Dialogue/DialogueWidget.DialogueWidget_C|SetDialogueText (Variables|Default|GetDialogueWidget) " ¿Recuerdas ese lugar? 3 ciudades clave darán con sus coordenadas… Recuerda eso. Y si no lo recuerdas, lo tendrás aquí escrito. Para ti. Para siempre.")))
          (Audio|PlaySound2D "/Game/Soniditos/63318__flag2__page-turn-please-turn-over-pto-paper-turn-over.63318__flag2__page-turn-please-turn-over-pto-paper-turn-over" 1.0 1.0 0.0 0 0))))))