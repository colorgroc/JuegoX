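; Interactable object that can be stored inside another actor, with outline highlighting and inspection support.
; It attaches to its storage actor on BeginPlay and re-records its initial transform when that actor's Finished event fires.
; A duplicate mesh carries a dynamic outline material, updated on Tick: white within glow distance, red when focused, hidden while inspected.
; Tick also toggles input and swaps keyboard/gamepad prompt icons during inspection.
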(event Custom|Event
  (Variables|/Game/JuegoX/Blueprints/Objects/Interactable.Interactable_C|SetinitialRot (Variables|Default|GetInteractable) (Transformation|GetActorRotation))
  (Variables|/Game/JuegoX/Blueprints/Objects/Interactable.Interactable_C|SetinitialPos (Variables|Default|GetInteractable) (Transformation|GetActorLocation)))

(event EventTick
  (params (DeltaSeconds :type Float%20%28single-precision%29))
  (bind _returnvalue (Game|GetPlayerController 0))
  (bind _materialhighlight (Variables|Default|GetmaterialHighlight))
  (bind _materialhighlight_2 (Variables|Default|GetmaterialHighlight))
  (Utilities|IsValid (Variables|Default|GetlugarDondeEstaGuardada)
    (:Is%20Valid
      (EventDispatchers|BindEventtoFinished (Variables|Default|GetlugarDondeEstaGuardada) (delegate Custom|Event)))
    (:Is%20Not%20Valid
      _))
  (if (Variables|/Game/JuegoX/Blueprints/Objects/Interactable.Interactable_C|GetisInspectingIt (Variables|Default|GetInteractable))
    (Rendering|Material|SetScalarParameterValue _materialhighlight "Scale" 0.0 :!class /Script/Engine.MaterialInstanceDynamic)
    (if (Variables|/Game/JuegoX/Blueprints/MyGameInstance.MyGameInstance_C|GetcontrolChanged? (Variables|Default|GetGameInstance))
      (Utilities|FlowControl|Sequence
        (:then_0
          (if (Variables|/Game/JuegoX/Blueprints/MyGameInstance.MyGameInstance_C|GetusingGamepad? (Variables|Default|GetGameInstance))
            (Variables|Default|SetTexture_E "/Game/JuegoX/UI/Sprites/Gamepad/redondaizquierda.redondaizquierda")
            (Variables|Default|SetTexture_LClick "/Game/JuegoX/UI/Sprites/Gamepad/redondabajo.redondabajo")
            (Variables|Default|SetTexture_RClick "/Game/JuegoX/UI/Sprites/Gamepad/redondaarriba.redondaarriba")
            (Variables|Default|SetTexture_Roll 0)
            (Variables|Default|SetTexture_Mouse 0)
            (else
              (Variables|Default|SetTexture_E "/Game/JuegoX/UI/Sprites/Keyboard/E.E")
              (Variables|Default|SetTexture_LClick "/Game/JuegoX/UI/Sprites/Keyboard/botonizquierda.botonizquierda")
              (Variables|Default|SetTexture_RClick "/Game/JuegoX/UI/Sprites/Keyboard/botonderecho.botonderecho")
              (Variables|Default|SetTexture_Roll 0)
              (Variables|Default|SetTexture_Mouse 0))))
        (:then_1
          (CallFunction|UpdateIcons))
        (:then_2
          (Variables|/Game/JuegoX/Blueprints/MyGameInstance.MyGameInstance_C|SetcontrolChanged? (Variables|Default|GetGameInstance) false))
        (:then_3
          (Input|EnableInput _returnvalue :!label _label)))
      (else
        (goto _label)))
    (elif (Variables|/Game/JuegoX/Blueprints/Objects/Interactable.Interactable_C|GetisFocused? (Variables|Default|GetInteractable))
      (Rendering|Material|SetScalarParameterValue _materialhighlight "Scale" 0.5 :!class /Script/Engine.MaterialInstanceDynamic)
      (Rendering|Material|SetVectorParameterValue _materialhighlight "Color" "(R=1.000000,G=0.000000,B=0.000000,A=1.000000)" :!class /Script/Engine.MaterialInstanceDynamic)
      (goto _label)
      (else
        (Input|DisableInput _returnvalue)
        (Math|Float|CompareFloat (Transformation|GetDistanceTo (Variables|Default|Getplayer)) (Variables|/Game/JuegoX/Blueprints/Objects/Interactable.Interactable_C|GetDistance%20to%20Glow (Variables|Default|GetInteractable))
          (:>
            (Rendering|Material|SetScalarParameterValue _materialhighlight_2 "Scale" 0.0 :!class /Script/Engine.MaterialInstanceDynamic))
          (:==
            (Rendering|Material|SetScalarParameterValue _materialhighlight_2 "Scale" 0.5 :!class /Script/Engine.MaterialInstanceDynamic :!label _label_2))
          (:<
            (goto _label_2)))
        (Rendering|Material|SetVectorParameterValue _materialhighlight_2 "Color" "(R=1.000000,G=1.000000,B=1.000000,A=1.000000)" :!class /Script/Engine.MaterialInstanceDynamic)))))

(event EventBeginPlay
  (bind _lugardondeestaguardada (Variables|Default|GetlugarDondeEstaGuardada))
  (|CallParentFunction)
  (bind _returnvalue (Rendering|Material|CreateDynamicMaterialInstance (Variables|Default|GetDuplicated) 0 "/Game/JuegoX/Materials/Outline_ObjectsHided.Outline_ObjectsHided" "None" :!class /Script/Engine.PrimitiveComponent))
  (Variables|Default|SetmaterialHighlight _returnvalue)
  (Utilities|IsValid _lugardondeestaguardada
    (:Is%20Valid
      (Transformation|AttachComponentToComponent (Variables|/Game/JuegoX/Blueprints/Objects/Interactable_Static/Dressers/OBJ_Furniture.OBJ_Furniture_C|GetMesh _lugardondeestaguardada) "None" "KeepWorld" "KeepWorld" "KeepWorld" true))))

(fn ConstructionScript
  (|CallParentFunction)
  (Components|StaticMesh|SetStaticMesh (Variables|Default|GetDuplicated) (Variables|/Script/Engine.StaticMeshComponent|GetStaticMesh (Variables|Character|GetMesh))))

(fn ConnectwithCable)