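; Parent door object that the player opens and closes with the Inspect input, optionally requiring a key.
; An Interactuable component gates input by focus, while OpenDoor toggles a sequence animation forward or in reverse with sounds.
; Locked doors check HasKey on MyGameInstance; first use clears the key from inventory and unlocks the door permanently.
; Without a key, it plays a locked sound and shows an animated hint on the player's HUD.
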(event Custom|Open%20Door
  (bind _anim (Variables|Default|GetAnim))
  (bind _sequenceplayer (Variables|/Script/ActorSequence.ActorSequenceComponent|GetSequencePlayer _anim))
  (if (Variables|/Game/JuegoX/Blueprints/Objects/Interactable.Interactable_C|GetisFocused? (Variables|Default|GetInteractuable))
    (if (Variables|Default|GetneedKey?)
      (bind _asmy_game_instance (Utilities|Casting|CastToMyGameInstance (Game|GetGameInstance)))
      (if (Variables|/Game/JuegoX/Blueprints/MyGameInstance.MyGameInstance_C|GetHas_Key? _asmy_game_instance)
        (Utilities|FlowControl|Sequence
          (:then_0
            (if (Variables|Default|GetisOpen?) :!label _label
              (Class|MovieSceneSequencePlayer|PlayReverse _sequenceplayer)
              (Variables|Default|SetisOpen? false)
              (Utilities|FlowControl|Delay 0.2)
              (Audio|PlaySound2D "/Game/Soniditos/411791__inspectorj__door-wooden-close-a-h1.411791__inspectorj__door-wooden-close-a-h1" 1.0 1.0 0.0 0 0)
              (else
                (Sequencer|Player|Play _sequenceplayer :!class /Script/MovieScene.MovieSceneSequencePlayer)
                (Variables|Default|SetisOpen? true)
                (Audio|PlaySound2D "/Game/Soniditos/398750__anthousai__door-open-01.398750__anthousai__door-open-01" 1.0 1.0 0.0 0 0))))
          (:then_1
            (Utilities|FlowControl|DoOnce false
              (:Completed
                (Default|HideInventory (Variables|Default|GetKey))
                (Variables|Default|SetneedKey? false)
                (bind _asmy_game_instance_2 (Utilities|Casting|CastToMyGameInstance (Game|GetGameInstance)))
                (Variables|/Game/JuegoX/Blueprints/MyGameInstance.MyGameInstance_C|SetHas_Key? _asmy_game_instance_2 false)))))
        (else
          (CallFunction|ShowHint "A key is needed!")
          (Audio|PlaySound2D "/Game/Soniditos/12739__leady__locked-door.12739__leady__locked-door" 1.0 1.0 0.0 0 0)))
      (else
        (goto _label)))))

(event EventTick
  (params (DeltaSeconds :type Float%20%28single-precision%29))
  (bind _returnvalue (Game|GetPlayerController 0))
  (if (Variables|/Game/JuegoX/Blueprints/Objects/Interactable.Interactable_C|GetisFocused? (Variables|Default|GetInteractuable))
    (Input|EnableInput _returnvalue)
    (else
      (Input|DisableInput _returnvalue))))

(event EventBeginPlay
  (Variables|Default|SetisOpen? false)
  (bind _asfirst_person_character (Utilities|Casting|CastToFirstPersonCharacter (Game|GetPlayerCharacter 0)))
  (bind _output_get (Variables|Default|Setplayer _asfirst_person_character))
  (Variables|/Game/JuegoX/Blueprints/Objects/Interactable.Interactable_C|Setplayer (Variables|Default|GetInteractuable) _output_get))

(event Input|ActionEvents|InputActionInspect
  (params (Key :type Key%20Structure :default "None"))
  (:Pressed
    (CallFunction|OpenDoor)))

(fn ConstructionScript
  (Variables|/Game/JuegoX/Blueprints/Objects/Interactable.Interactable_C|SetMesh (Variables|Default|GetInteractuable) (Variables|Default|GetMesh))
  (Variables|/Game/JuegoX/Blueprints/Objects/Interactable.Interactable_C|SetText (Variables|Default|GetInteractuable) (Variables|Default|GetTextRender))
  (Variables|/Game/JuegoX/Blueprints/Objects/Interactable.Interactable_C|Setis%20a%20nonInspectionable%20Object? (Variables|Default|GetInteractuable) true))

(fn Inventory
  (Default|HideInventory (Variables|Default|GetKey)))

(fn ShowHint
  (params (hint :type Text))
  (if (Utilities|IsValid (Variables|/Game/FirstPersonBP/Blueprints/FirstPersonCharacter.FirstPersonCharacter_C|GetHUD (Variables|Default|Getplayer)))
    _
    (else
      (bind _returnvalue (UserInterface|CreateWidget "/Game/JuegoX/UI/HUD/WB_HUD.WB_HUD_C" (Game|GetPlayerController 0)))
      (Variables|/Game/FirstPersonBP/Blueprints/FirstPersonCharacter.FirstPersonCharacter_C|SetHUD (Variables|Default|Getplayer) _returnvalue)))
  (Rendering|Components|TextRender|SetText (Variables|/Game/JuegoX/UI/HUD/WB_HUD.WB_HUD_C|GetHInt_Text (Variables|/Game/FirstPersonBP/Blueprints/FirstPersonCharacter.FirstPersonCharacter_C|GetHUD (Variables|Default|Getplayer))) hint)
  (if (UserInterface|Viewport|IsinViewport (Variables|/Game/FirstPersonBP/Blueprints/FirstPersonCharacter.FirstPersonCharacter_C|GetHUD (Variables|Default|Getplayer)))
    _
    (else
      (UserInterface|Viewport|AddtoViewport (Variables|/Game/FirstPersonBP/Blueprints/FirstPersonCharacter.FirstPersonCharacter_C|GetHUD (Variables|Default|Getplayer)) 0)))
  (Class|UserWidget|PlayAnimationForward (Variables|/Game/FirstPersonBP/Blueprints/FirstPersonCharacter.FirstPersonCharacter_C|GetHUD (Variables|Default|Getplayer)) (Variables|/Game/JuegoX/UI/HUD/WB_HUD.WB_HUD_C|GetHint_Anim (Variables|/Game/FirstPersonBP/Blueprints/FirstPersonCharacter.FirstPersonCharacter_C|GetHUD (Variables|Default|Getplayer))) 1.0))