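; Interactable gamepad prop, a child of an interactable base, that hands player control to a remote-control FlyingPawn plane.
; Construction caches the plane and starts with interaction deactivated; SetVariables sets the HUD prompts.
; Interacting while inspecting it switches "InvisiblePared"-tagged trigger boxes to BlockAllDynamic.
; If the plane is valid, it also swaps the control hints, possesses the plane and destroys the gamepad.
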(event EventBeginPlay
  (|CallParentFunction) ; This node is disabled and will not be called.\nDrag off pins to build functionality.
)

(event Collision|EventActorBeginOverlap
  (params (OtherActor :type Actor%20Object%20Reference)))

(event EventTick
  (params (DeltaSeconds :type Float%20%28single-precision%29))
  (|CallParentFunction DeltaSeconds) ; This node is disabled and will not be called.\nDrag off pins to build functionality.
)

(event EventInteract
  (if (Variables|/Game/JuegoX/Blueprints/Objects/Interactable.Interactable_C|GetinteractionActivated (Variables|Default|GetInteractable))
    (if (Variables|/Game/JuegoX/Blueprints/Objects/Interactable.Interactable_C|GetisInspectingIt (Variables|Default|GetInteractable))
      (Variables|/Game/JuegoX/Blueprints/Objects/Interactable.Interactable_C|SetisInspectingIt (Variables|Default|GetInteractable) false)
      (CallFunction|PlaneControl))))

(event EventSetVariables
  (bind _player (Variables|Default|Getplayer))
  (bind _hud (Variables|/Game/FirstPersonBP/Blueprints/FirstPersonCharacter.FirstPersonCharacter_C|GetHUD _player))
  (Rendering|Components|TextRender|SetText (Variables|/Game/JuegoX/UI/HUD/WB_HUD.WB_HUD_C|GetT_Drop _hud) "to drop")
  (Rendering|Components|TextRender|SetText (Variables|/Game/JuegoX/UI/HUD/WB_HUD.WB_HUD_C|GetT_Action _hud) "to pilot remote control plane")
  (Variables|Default|Setwidget_Anim (Variables|/Game/JuegoX/UI/HUD/WB_HUD.WB_HUD_C|GetControls_2_Anim _hud)))

(fn ConstructionScript
  (|CallParentFunction)
  (bind _returnvalue (Actor|GetActorOfClass "/Game/FlyingBP/Blueprints/FlyingPawn.FlyingPawn_C"))
  (Variables|Default|SetPlane _returnvalue)
  (Variables|/Game/JuegoX/Blueprints/Objects/Interactable.Interactable_C|SetinteractionActivated (Variables|Default|GetInteractable) false))

(fn PlaneControl
  (bind _outactors (Actor|GetAllActorswithTag "InvisiblePared"))
  (for _array_element _outactors
    (bind _astrigger_box (Utilities|Casting|CastToTriggerBox _array_element))
    (Collision|SetCollisionProfileName (Variables|/Script/Engine.TriggerBase|GetCollisionComponent _astrigger_box) "BlockAllDynamic" :!class /Script/Engine.PrimitiveComponent))
  (if (Utilities|IsValid (Variables|Default|GetPlane))
    (CallFunction|HideControls) ; Hide controller widget
    (CallFunction|ShowControlsPlane)
    (Components|DestroyComponent (Variables|Character|GetMesh))
    (Pawn|Possess (Game|GetPlayerController 0) (Variables|Default|GetPlane))
    (Actor|DestroyActor)))

(fn ShowControlsPlane
  (Variables|Default|Setwidget_Anim (Variables|/Game/JuegoX/UI/HUD/WB_HUD.WB_HUD_C|GetControls_4_Anim (Variables|/Game/FirstPersonBP/Blueprints/FirstPersonCharacter.FirstPersonCharacter_C|GetHUD (Variables|Default|Getplayer))))
  (if (UserInterface|Viewport|IsinViewport (Variables|/Game/FirstPersonBP/Blueprints/FirstPersonCharacter.FirstPersonCharacter_C|GetHUD (Variables|Default|Getplayer)))
    _
    (else
      (UserInterface|Viewport|AddtoViewport (Variables|/Game/FirstPersonBP/Blueprints/FirstPersonCharacter.FirstPersonCharacter_C|GetHUD (Variables|Default|Getplayer)) 0)))
  (Class|UserWidget|PlayAnimationForward (Variables|/Game/FirstPersonBP/Blueprints/FirstPersonCharacter.FirstPersonCharacter_C|GetHUD (Variables|Default|Getplayer)) (Variables|Default|Getwidget_Anim) 4.0))