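; Plane remote-control prop that, once the map puzzle is completed, can be inspected and used to pilot the Avion.
; Tick toggles its mesh visibility once, then enables input and shows the prompt while focused or inspected.
; Inspect moves it via timeline to one of the player's view points, chosen by the "Big" tag, and back.
; Interacting during inspection makes "InvisiblePared" trigger boxes blocking, swaps control widgets and possesses the Avion.
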(event Custom|EndInspection
  (bind _interactuable (Variables|Default|GetInteractuable))
  (CallFunction|HideControlsMando)
  (Variables|/Game/JuegoX/Blueprints/Objects/Interactable.Interactable_C|SetisInspectingIt (Variables|Default|GetInteractuable) false)
  (Variables|/Game/FirstPersonBP/Blueprints/FirstPersonCharacter.FirstPersonCharacter_C|SetplayerInspectingObject (Variables|Default|Getplayer) false)
  (bind _move_object (Timeline|Inspect Reverse)
    (:Update
      (bind _output_get (Variables|Default|SetMovedObject _move_object))
      (Transformation|SetActorLocationAndRotation (Math|Vector|Lerp(Vector) (Variables|/Game/JuegoX/Blueprints/Objects/Interactable.Interactable_C|GetinitialPos _interactuable) (Variables|/Game/JuegoX/Blueprints/Objects/Interactable.Interactable_C|GetinspectionPoint _interactuable) _output_get) (Math|Rotator|Lerp(Rotator) (Variables|/Game/JuegoX/Blueprints/Objects/Interactable.Interactable_C|GetinitialRot _interactuable) (Transformation|GetActorRotation) _output_get)))))

(event EventTick
  (params (DeltaSeconds :type Float%20%28single-precision%29))
  (bind _returnvalue (Game|GetPlayerController 0))
  (bind _gameinstance (Variables|Default|GetgameInstance))
  (bind _widget (Variables|Default|GetWidget))
  (if (Utilities|IsValid _gameinstance)
    (if (Variables|/Game/JuegoX/Blueprints/MyGameInstance.MyGameInstance_C|GetMapPuzzle_Completed _gameinstance)
      (Utilities|FlowControl|Sequence
        (:then_0
          (Utilities|FlowControl|DoOnce false
            (:Completed
              (Rendering|ToggleVisibility (Variables|Default|GetMesh) false))))
        (:then_1
          (Variables|/Game/JuegoX/Blueprints/Objects/Interactable.Interactable_C|SetinteractionActivated (Variables|Default|GetInteractuable) true)
          (if (Variables|/Game/JuegoX/Blueprints/Objects/Interactable.Interactable_C|GetisInspectingIt (Variables|Default|GetInteractuable))
            (Input|EnableInput _returnvalue :!label _label)
            (Rendering|SetVisibility _widget true false)
            (Transformation|SetWorldRotation (Variables|Default|GetTextRender) (Math|Rotator|FindLookatRotation (Transformation|GetActorLocation) (Transformation|GetActorLocation (Variables|Default|Getplayer))) false false)
            (elif (Variables|/Game/JuegoX/Blueprints/Objects/Interactable.Interactable_C|GetisFocused? (Variables|Default|GetInteractuable))
              (goto _label)
              (else
                (Input|DisableInput _returnvalue :!label _label_2)
                (Rendering|SetVisibility _widget false false))))))
      (else
        (goto _label_2)))))

(event EventBeginPlay
  (bind _asfirst_person_character (Utilities|Casting|CastToFirstPersonCharacter (Game|GetPlayerCharacter 0)))
  (Variables|Default|Setplayer _asfirst_person_character)
  (bind _asmy_game_instance (Utilities|Casting|CastToMyGameInstance (Game|GetGameInstance)))
  (Variables|Default|SetgameInstance _asmy_game_instance)
  (if (Actor|ActorHasTag "Polaroid")
    (Variables|Default|Setinit%20scale (Transformation|GetActorScale3D))))

(event Input|ActionEvents|InputActionInteract
  (params (Key :type Key%20Structure :default "None"))
  (:Pressed
    (if (Variables|/Game/JuegoX/Blueprints/Objects/Interactable.Interactable_C|GetisInspectingIt (Variables|Default|GetInteractuable))
      (CallFunction|Interact))))

(event Input|ActionEvents|InputActionInspect
  (params (Key :type Key%20Structure :default "None"))
  (bind _interactuable (Variables|Default|GetInteractuable))
  (bind _player (Variables|Default|Getplayer))
  (bind _interactuable_2 (Variables|Default|GetInteractuable))
  (:Pressed
    (if (Variables|/Game/JuegoX/Blueprints/Objects/Interactable.Interactable_C|GetisInspectingIt _interactuable)
      (CallFunction|EndInspection)
      (else
        (Utilities|FlowControl|Sequence
          (:then_0
            (CallFunction|ShowControlsMando))
          (:then_1
            (if (Actor|ActorHasTag "Big")
              (Variables|/Game/JuegoX/Blueprints/Objects/Interactable.Interactable_C|SetinspectionPoint _interactuable (Transformation|GetWorldLocation (Variables|/Game/FirstPersonBP/Blueprints/FirstPersonCharacter.FirstPersonCharacter_C|GetInpectionViewBig _player)))
              (else
                (Variables|/Game/JuegoX/Blueprints/Objects/Interactable.Interactable_C|SetinspectionPoint _interactuable (Transformation|GetWorldLocation (Variables|/Game/FirstPersonBP/Blueprints/FirstPersonCharacter.FirstPersonCharacter_C|GetInpectionView _player)))))
            (Variables|/Game/JuegoX/Blueprints/Objects/Interactable.Interactable_C|SetisInspectingIt _interactuable true)
            (Variables|/Game/FirstPersonBP/Blueprints/FirstPersonCharacter.FirstPersonCharacter_C|SetplayerInspectingObject (Variables|Default|Getplayer) true)
            (bind _move_object (Timeline|Inspect Play)
              (:Update
                (bind _output_get (Variables|Default|SetMovedObject _move_object))
                (Transformation|SetActorLocationAndRotation (Math|Vector|Lerp(Vector) (Variables|/Game/JuegoX/Blueprints/Objects/Interactable.Interactable_C|GetinitialPos _interactuable_2) (Variables|/Game/JuegoX/Blueprints/Objects/Interactable.Interactable_C|GetinspectionPoint _interactuable_2) _output_get) (Math|Rotator|Lerp(Rotator) (Variables|/Game/JuegoX/Blueprints/Objects/Interactable.Interactable_C|GetinitialRot _interactuable_2) (Transformation|GetActorRotation) _output_get))))))))))

(fn ConstructionScript)

(fn Interact
  (bind _avion (Variables|Default|GetAvion))
  (bind _outactors (Actor|GetAllActorswithTag "InvisiblePared"))
  (for _array_element _outactors
    (bind _astrigger_box (Utilities|Casting|CastToTriggerBox _array_element))
    (Collision|SetCollisionProfileName (Variables|/Script/Engine.TriggerBase|GetCollisionComponent _astrigger_box) "BlockAllDynamic" :!class /Script/Engine.PrimitiveComponent))
  (if (Utilities|IsValid _avion)
    (CallFunction|HideControlsMando)
    (CallFunction|ShowControlsPlane)
    (Pawn|Possess (Game|GetPlayerController 0) _avion)))

(fn ShowControlsMando
  (bind _player (Variables|Default|Getplayer))
  (if (Utilities|IsValid (Variables|/Game/FirstPersonBP/Blueprints/FirstPersonCharacter.FirstPersonCharacter_C|GetWB_Mando _player))
    _
    (else
      (bind _returnvalue (UserInterface|CreateWidget "/Game/JuegoX/UI/HUD/WB_Mando_Plane.WB_Mando_Plane_C" (Game|GetPlayerController 0)))
      (Variables|/Game/FirstPersonBP/Blueprints/FirstPersonCharacter.FirstPersonCharacter_C|SetWB_Mando _player _returnvalue)))
  (UserInterface|Viewport|AddtoViewport (Variables|/Game/FirstPersonBP/Blueprints/FirstPersonCharacter.FirstPersonCharacter_C|GetWB_Mando _player) 0))

(fn ShowControlsPlane
  (bind _player (Variables|Default|Getplayer))
  (if (Utilities|IsValid (Variables|/Game/FirstPersonBP/Blueprints/FirstPersonCharacter.FirstPersonCharacter_C|GetWB_DrivePlane _player))
    _
    (else
      (bind _returnvalue (UserInterface|CreateWidget "/Game/JuegoX/UI/HUD/WB_Drive_Plane.WB_Drive_Plane_C" (Game|GetPlayerController 0)))
      (Variables|/Game/FirstPersonBP/Blueprints/FirstPersonCharacter.FirstPersonCharacter_C|SetWB_DrivePlane _player _returnvalue)))
  (UserInterface|Viewport|AddtoViewport (Variables|/Game/FirstPersonBP/Blueprints/FirstPersonCharacter.FirstPersonCharacter_C|GetWB_DrivePlane _player) 0))

(fn HideControlsMando
  (Widget|RemovefromParent (Variables|/Game/FirstPersonBP/Blueprints/FirstPersonCharacter.FirstPersonCharacter_C|GetWB_Mando (Variables|Default|Getplayer))))