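; OBJ_Plane is the held paper plane the first-person player charges and throws.
; Every tick it follows the player's inspection point and camera rotation; holding the button runs a timeline that pulls the mesh back and tracks its launch location.
; On release it restores the default HUD hints, spawns a FirstPersonProjectile using the player's SpeedProjectile, then destroys itself.
; BeginPlay caches the player and shows throw controls on the shared WB_HUD.
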(event Custom|ThrowPlane
  (Utilities|FlowControl|Sequence
    (:then_0
      (bind _returnvalue (Game|SpawnActorfromClass "/Game/FirstPersonBP/Blueprints/FirstPersonProjectile.FirstPersonProjectile_C" (Math|Transform|MakeTransform (Variables|Default|GetprojectileLocation) (Transformation|GetActorRotation)) "AdjustIfPossibleButAlwaysSpawn" 0 0))
      (Variables|Default|SetTemporary_FPProjectile _returnvalue)
      (Variables|/Script/Engine.ProjectileMovementComponent|SetInitialSpeed (Variables|/Game/FirstPersonBP/Blueprints/FirstPersonProjectile.FirstPersonProjectile_C|GetProjectile (Variables|Default|GetTemporary_FPProjectile)) (Variables|/Game/FirstPersonBP/Blueprints/FirstPersonCharacter.FirstPersonCharacter_C|GetspeedProjectile (Variables|Default|Getplayer)))
      (Variables|/Script/Engine.MovementComponent|SetVelocity (Variables|/Game/FirstPersonBP/Blueprints/FirstPersonProjectile.FirstPersonProjectile_C|GetProjectile (Variables|Default|GetTemporary_FPProjectile)) (* (Variables|/Script/Engine.MovementComponent|GetVelocity (Variables|/Game/FirstPersonBP/Blueprints/FirstPersonProjectile.FirstPersonProjectile_C|GetProjectile (Variables|Default|GetTemporary_FPProjectile))) (Variables|/Game/FirstPersonBP/Blueprints/FirstPersonCharacter.FirstPersonCharacter_C|GetspeedProjectile (Variables|Default|Getplayer))))
      (Variables|/Game/FirstPersonBP/Blueprints/FirstPersonCharacter.FirstPersonCharacter_C|SetspeedProjectile (Variables|Default|Getplayer) 0.0))
    (:then_1
      (Actor|DestroyActor))))

(event Custom|End
  (Utilities|FlowControl|Sequence
    (:then_0
      (CallFunction|HideControls))
    (:then_1
      (Variables|/Game/FirstPersonBP/Blueprints/FirstPersonCharacter.FirstPersonCharacter_C|SetthrowingPaperPlane (Variables|Default|Getplayer) false)
      (Variables|/Game/FirstPersonBP/Blueprints/FirstPersonCharacter.FirstPersonCharacter_C|SethacerAvionDePapel? (Variables|Default|Getplayer) false)
      (bind _backwards (Timeline|BackWards Stop)
        (:Update
          (Transformation|SetRelativeLocation (Variables|Default|GetMesh) (Math|Vector|Lerp(Vector) (Variables|/Script/Engine.SceneComponent|GetRelativeLocation (Variables|Default|GetMesh)) (- (* (Variables|/Script/Engine.SceneComponent|GetRelativeLocation (Variables|Default|GetMesh)) (Class|KismetMathLibrary|VectorForward)) 1.0) _backwards) false false)
          (CallFunction|UpdateProjectileLocation))
        (:Finished
          (CallFunction|UpdateProjectileLocation))))
    (:then_2
      (Components|DestroyComponent (Variables|Default|GetMesh)))))

(event Custom|UpdateProjectileLocation
  (Variables|Default|SetprojectileLocation (Transformation|GetWorldLocation (Variables|Default|GetMesh))))

(event EventTick
  (params (DeltaSeconds :type Float%20%28single-precision%29))
  (bind _player (Variables|Default|Getplayer))
  (Transformation|SetActorLocationAndRotation (Transformation|GetWorldLocation (Variables|/Game/FirstPersonBP/Blueprints/FirstPersonCharacter.FirstPersonCharacter_C|GetInpectionAvion _player)) (Transformation|GetWorldRotation (Variables|/Game/FirstPersonBP/Blueprints/FirstPersonCharacter.FirstPersonCharacter_C|GetFirstPersonCamera _player)))
  (Utilities|FlowControl|Delay 0.2)
  (if (Variables|/Game/FirstPersonBP/Blueprints/FirstPersonCharacter.FirstPersonCharacter_C|GetholdButton (Variables|Default|Getplayer))
    (if (> (.X (Math|Vector|BreakVector (Variables|/Script/Engine.SceneComponent|GetRelativeLocation (Variables|Default|GetMesh)))) -2e+01)
      (bind _backwards (Timeline|BackWards Play)
        (:Update
          (Transformation|SetRelativeLocation (Variables|Default|GetMesh) (Math|Vector|Lerp(Vector) (Variables|/Script/Engine.SceneComponent|GetRelativeLocation (Variables|Default|GetMesh)) (- (* (Variables|/Script/Engine.SceneComponent|GetRelativeLocation (Variables|Default|GetMesh)) (Class|KismetMathLibrary|VectorForward)) 1.0) _backwards) false false)
          (CallFunction|UpdateProjectileLocation))
        (:Finished
          (CallFunction|UpdateProjectileLocation))))
    (elif (Variables|/Game/FirstPersonBP/Blueprints/FirstPersonCharacter.FirstPersonCharacter_C|GetthrowingPaperPlane (Variables|Default|Getplayer))
      (CallFunction|End)
      (CallFunction|ThrowPlane))))

(event EventBeginPlay
  (Utilities|IsValid (Variables|Default|GetMesh)
    (:Is%20Valid
      (bind _asfirst_person_character (Utilities|Casting|CastToFirstPersonCharacter (Game|GetPlayerCharacter 0)))
      (Variables|Default|Setplayer _asfirst_person_character)
      (Variables|/Game/FirstPersonBP/Blueprints/FirstPersonCharacter.FirstPersonCharacter_C|SetavionPapelRotation (Variables|Default|Getplayer) (Transformation|GetActorRotation))
      (CallFunction|ShowControls))))

(fn ConstructionScript)

(fn ShowControls
  (if (Utilities|IsValid (Variables|/Game/FirstPersonBP/Blueprints/FirstPersonCharacter.FirstPersonCharacter_C|GetHUD (Variables|Default|Getplayer)))
    _
    (else
      (bind _returnvalue (UserInterface|CreateWidget "/Game/JuegoX/UI/HUD/WB_HUD.WB_HUD_C" (Game|GetPlayerController 0)))
      (Variables|/Game/FirstPersonBP/Blueprints/FirstPersonCharacter.FirstPersonCharacter_C|SetHUD (Variables|Default|Getplayer) _returnvalue)))
  (CallFunction|SetVariables)
  (if (UserInterface|Viewport|IsinViewport (Variables|/Game/FirstPersonBP/Blueprints/FirstPersonCharacter.FirstPersonCharacter_C|GetHUD (Variables|Default|Getplayer)))
    _
    (else
      (UserInterface|Viewport|AddtoViewport (Variables|/Game/FirstPersonBP/Blueprints/FirstPersonCharacter.FirstPersonCharacter_C|GetHUD (Variables|Default|Getplayer)) 0)))
  (Class|UserWidget|PlayAnimationForward (Variables|/Game/FirstPersonBP/Blueprints/FirstPersonCharacter.FirstPersonCharacter_C|GetHUD (Variables|Default|Getplayer)) (Variables|Default|Getwidget_Anim) 4.0))

(fn HideControls
  (bind _player (Variables|Default|Getplayer))
  (bind _hud (Variables|/Game/FirstPersonBP/Blueprints/FirstPersonCharacter.FirstPersonCharacter_C|GetHUD _player))
  ;[1 1 1] Set to default controls
  (Rendering|Components|TextRender|SetText (Variables|/Game/JuegoX/UI/HUD/WB_HUD.WB_HUD_C|GetIcon_Drop (Variables|/Game/FirstPersonBP/Blueprints/FirstPersonCharacter.FirstPersonCharacter_C|GetHUD (Variables|Default|Getplayer))) "E")
  (Rendering|Components|TextRender|SetText (Variables|/Game/JuegoX/UI/HUD/WB_HUD.WB_HUD_C|GetIcon_Action (Variables|/Game/FirstPersonBP/Blueprints/FirstPersonCharacter.FirstPersonCharacter_C|GetHUD (Variables|Default|Getplayer))) "Left Click")
  (Rendering|Components|TextRender|SetText (Variables|/Game/JuegoX/UI/HUD/WB_HUD.WB_HUD_C|GetT_Drop _hud) "to drop")
  (Rendering|Components|TextRender|SetText (Variables|/Game/JuegoX/UI/HUD/WB_HUD.WB_HUD_C|GetT_Action _hud) "to make plane")
  (Class|UserWidget|PlayAnimationForward (Variables|/Game/FirstPersonBP/Blueprints/FirstPersonCharacter.FirstPersonCharacter_C|GetHUD (Variables|Default|Getplayer)) (Variables|Default|Getwidget_Anim) 4.0))

(fn SetVariables
  (Rendering|Components|TextRender|SetText (Variables|/Game/JuegoX/UI/HUD/WB_HUD.WB_HUD_C|GetIcon_Drop (Variables|/Game/FirstPersonBP/Blueprints/FirstPersonCharacter.FirstPersonCharacter_C|GetHUD (Variables|Default|Getplayer))) "Hold Left Click")
  (Rendering|Components|TextRender|SetText (Variables|/Game/JuegoX/UI/HUD/WB_HUD.WB_HUD_C|GetT_Drop (Variables|/Game/FirstPersonBP/Blueprints/FirstPersonCharacter.FirstPersonCharacter_C|GetHUD (Variables|Default|Getplayer))) "to set acceleration")
  (Rendering|Components|TextRender|SetText (Variables|/Game/JuegoX/UI/HUD/WB_HUD.WB_HUD_C|GetIcon_Action (Variables|/Game/FirstPersonBP/Blueprints/FirstPersonCharacter.FirstPersonCharacter_C|GetHUD (Variables|Default|Getplayer))) "Realase")
  (Rendering|Components|TextRender|SetText (Variables|/Game/JuegoX/UI/HUD/WB_HUD.WB_HUD_C|GetT_Action (Variables|/Game/FirstPersonBP/Blueprints/FirstPersonCharacter.FirstPersonCharacter_C|GetHUD (Variables|Default|Getplayer))) "to throw")
  (Variables|Default|Setwidget_Anim (Variables|/Game/JuegoX/UI/HUD/WB_HUD.WB_HUD_C|GetControls_2_Anim (Variables|/Game/FirstPersonBP/Blueprints/FirstPersonCharacter.FirstPersonCharacter_C|GetHUD (Variables|Default|Getplayer)))))