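; Collectible mannequin body piece (head, arm or leg) that the player can pick up.
; The construction script uses the Piece enum to choose mesh, texture and item type, applies the mesh to the main and optional duplicate components, and activates interaction.
; The HasItemtoTrue event records the piece type and the actor itself in two GameInstance inventories.
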(event EventBeginPlay
  (|CallParentFunction) ; This node is disabled and will not be called.\nDrag off pins to build functionality.
)

(event Collision|EventActorBeginOverlap
  (params (OtherActor :type Actor%20Object%20Reference)))

(event EventTick
  (params (DeltaSeconds :type Float%20%28single-precision%29))
  (|CallParentFunction DeltaSeconds) ; This node is disabled and will not be called.\nDrag off pins to build functionality.
)

(event EventHasItemtoTrue
  (bind _gameinstance (Variables|Default|GetGameInstance))
  (Utilities|Set|Add (Variables|/Game/JuegoX/Blueprints/MyGameInstance.MyGameInstance_C|Getmaniquis_pieces_Inventory _gameinstance) (Variables|Default|GetPiece))
  (Utilities|Array|Add (Variables|/Game/JuegoX/Blueprints/MyGameInstance.MyGameInstance_C|GetPieces_collected_inventory _gameinstance) self))

(fn ConstructionScript
  (bind _duplicate (Variables|Default|GetDuplicate))
  (|CallParentFunction)
  (switch string (Variables|Default|GetPiece)
    (:Head
      (Variables|Default|Setinitial_mesh "/Game/3D_Models/Zeus/Maniquí/Zeus_Maniquí_Cabeza.Zeus_Maniquí_Cabeza")
      (Variables|Default|Settexture "/Game/JuegoX/Sprites/inventario/cabeza.cabeza")
      (Variables|Default|Settype "NewEnumerator5"))
    (:Left_Arm
      (Variables|Default|Setinitial_mesh "/Game/3D_Models/Zeus/Maniquí/Zeus_Maniquí_BrazoIzquierdo.Zeus_Maniquí_BrazoIzquierdo")
      (Variables|Default|Settexture "/Game/JuegoX/Sprites/inventario/brazo.brazo")
      (Variables|Default|Settype "NewEnumerator6"))
    (:Right_Arm
      (Variables|Default|Setinitial_mesh "/Game/3D_Models/Zeus/Maniquí/Zeus_Maniquí_BrazoDerecho.Zeus_Maniquí_BrazoDerecho")
      (Variables|Default|Settexture "/Game/JuegoX/Sprites/inventario/brazo.brazo")
      (Variables|Default|Settype "NewEnumerator7"))
    (:Left_Leg
      (Variables|Default|Setinitial_mesh "/Game/3D_Models/Zeus/Maniquí/Zeus_Maniquí_PiernaIzquierda.Zeus_Maniquí_PiernaIzquierda")
      (Variables|Default|Settexture "/Game/JuegoX/Sprites/inventario/Pierna.Pierna")
      (Variables|Default|Settype "NewEnumerator8"))
    (:Right_Leg
      (Variables|Default|Setinitial_mesh "/Game/3D_Models/Zeus/Maniquí/Zeus_Maniquí_PiernaDerecha.Zeus_Maniquí_PiernaDerecha")
      (Variables|Default|Settexture "/Game/JuegoX/Sprites/inventario/Pierna.Pierna")
      (Variables|Default|Settype "NewEnumerator9")))
  (Components|StaticMesh|SetStaticMesh (Variables|Character|GetMesh) (Variables|Default|Getinitial_mesh))
  (Utilities|IsValid _duplicate
    (:Is%20Valid
      (Components|StaticMesh|SetStaticMesh _duplicate (Variables|Default|Getinitial_mesh)))
    (:Is%20Not%20Valid
      _))
  (Variables|/Game/JuegoX/Blueprints/Objects/Interactable.Interactable_C|SetinteractionActivated (Variables|Default|GetInteractable) true))