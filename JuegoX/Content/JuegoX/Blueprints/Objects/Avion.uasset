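; Held paper plane actor that the first-person player pulls back and throws.
; Each tick it follows the player's InpectionAvion point and camera rotation; while HoldButton is set, a timeline slides the mesh backwards, recording the launch location.
; On throw, it spawns a FirstPersonProjectile scaled by the player's SpeedProjectile, then destroys itself.
; It also swaps the throw-controls widget for the diary widget, caching both on the player.
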(event Custom|End
  (bind _mesh (Variables|Default|GetMesh))
  (bind _relativelocation (Variables|/Script/Engine.SceneComponent|GetRelativeLocation _mesh))
  (CallFunction|HideControls)
  (Components|DestroyComponent (Variables|Default|GetMesh))
  (Variables|/Game/FirstPersonBP/Blueprints/FirstPersonCharacter.FirstPersonCharacter_C|SetthrowingPaperPlane (Variables|Default|Getplayer) false)
  (bind _backwards (Timeline|BackWards Stop)
    (:Update
      (bind _output_get (Variables|Default|SetBack _backwards))
      (Transformation|SetRelativeLocation (Variables|Default|GetMesh) (Math|Vector|Lerp(Vector) _relativelocation (- (* _relativelocation (Class|KismetMathLibrary|VectorForward)) 1.0) _output_get) false false))
    (:Finished
      _))
  (Variables|Default|SetprojectileLocation (Transformation|GetWorldLocation (Variables|Default|GetMesh))))

(event EventTick
  (params (DeltaSeconds :type Float%20%28single-precision%29))
  (bind _player (Variables|Default|Getplayer))
  (bind _player_2 (Variables|Default|Getplayer))
  (bind _player_3 (Variables|Default|Getplayer))
  (bind _mesh (Variables|Default|GetMesh))
  (bind _relativelocation (Variables|/Script/Engine.SceneComponent|GetRelativeLocation _mesh))
  (Transformation|SetActorLocationAndRotation (Transformation|GetWorldLocation (Variables|/Game/FirstPersonBP/Blueprints/FirstPersonCharacter.FirstPersonCharacter_C|GetInpectionAvion _player_2)) (Transformation|GetWorldRotation (Variables|/Game/FirstPersonBP/Blueprints/FirstPersonCharacter.FirstPersonCharacter_C|GetFirstPersonCamera _player_2)))
  (Utilities|FlowControl|Delay 0.2)
  (if (Variables|/Game/FirstPersonBP/Blueprints/FirstPersonCharacter.FirstPersonCharacter_C|GetholdButton _player)
    (if (> (.X (Math|Vector|BreakVector _relativelocation)) -2e+01)
      (bind _backwards (Timeline|BackWards Play)
        (:Update
          (bind _output_get (Variables|Default|SetBack _backwards))
          (Transformation|SetRelativeLocation (Variables|Default|GetMesh) (Math|Vector|Lerp(Vector) _relativelocation (- (* _relativelocation (Class|KismetMathLibrary|VectorForward)) 1.0) _output_get) false false))
        (:Finished
          _))
      (Variables|Default|SetprojectileLocation (Transformation|GetWorldLocation (Variables|Default|GetMesh))))
    (elif (Variables|/Game/FirstPersonBP/Blueprints/FirstPersonCharacter.FirstPersonCharacter_C|GetthrowingPaperPlane _player)
      (CallFunction|End)
      (bind _returnvalue (Game|SpawnActorfromClass "/Game/FirstPersonBP/Blueprints/FirstPersonProjectile.FirstPersonProjectile_C" (Math|Transform|MakeTransform (Variables|Default|GetprojectileLocation) (Transformation|GetActorRotation)) "AdjustIfPossibleButAlwaysSpawn" 0 0))
      (Variables|/Script/Engine.ProjectileMovementComponent|SetInitialSpeed (Variables|/Game/FirstPersonBP/Blueprints/FirstPersonProjectile.FirstPersonProjectile_C|GetProjectile _returnvalue) (Variables|/Game/FirstPersonBP/Blueprints/FirstPersonCharacter.FirstPersonCharacter_C|GetspeedProjectile _player_3))
      (Variables|/Script/Engine.MovementComponent|SetVelocity (Variables|/Game/FirstPersonBP/Blueprints/FirstPersonProjectile.FirstPersonProjectile_C|GetProjectile _returnvalue) (* (Variables|/Script/Engine.MovementComponent|GetVelocity (Variables|/Game/FirstPersonBP/Blueprints/FirstPersonProjectile.FirstPersonProjectile_C|GetProjectile _returnvalue)) (Variables|/Game/FirstPersonBP/Blueprints/FirstPersonCharacter.FirstPersonCharacter_C|GetspeedProjectile _player_3)))
      (Variables|/Game/FirstPersonBP/Blueprints/FirstPersonCharacter.FirstPersonCharacter_C|SetspeedProjectile _player_3 0.0)
      (CallFunction|ShowDiaryControls)
      (Actor|DestroyActor))))

(event EventBeginPlay
  (if (Utilities|IsValid (Variables|Default|GetMesh))
    (bind _asfirst_person_character (Utilities|Casting|CastToFirstPersonCharacter (Game|GetPlayerCharacter 0)))
    (Variables|Default|Setplayer _asfirst_person_character)
    (Variables|/Game/FirstPersonBP/Blueprints/FirstPersonCharacter.FirstPersonCharacter_C|SetavionPapelRotation _asfirst_person_character (Transformation|GetActorRotation))
    (CallFunction|ShowControls)))

(fn ConstructionScript)

(fn ShowControls
  (bind _player (Variables|Default|Getplayer))
  (if (Utilities|IsValid (Variables|/Game/FirstPersonBP/Blueprints/FirstPersonCharacter.FirstPersonCharacter_C|GetWB_ThrowPlane _player))
    (if (not (Variables|/Game/FirstPersonBP/Blueprints/FirstPersonCharacter.FirstPersonCharacter_C|GetaddedAlreadyToViewport_ThrowPlane _player))
      (Variables|/Game/FirstPersonBP/Blueprints/FirstPersonCharacter.FirstPersonCharacter_C|SetaddedAlreadyToViewport_ThrowPlane _player true :!label _label)
      (UserInterface|Viewport|AddtoViewport (Variables|/Game/FirstPersonBP/Blueprints/FirstPersonCharacter.FirstPersonCharacter_C|GetWB_ThrowPlane _player) 0))
    (else
      (bind _returnvalue (UserInterface|CreateWidget "/Game/JuegoX/UI/HUD/WB_Throw_Paper_Plane.WB_Throw_Paper_Plane_C" (Game|GetPlayerController 0)))
      (Variables|/Game/FirstPersonBP/Blueprints/FirstPersonCharacter.FirstPersonCharacter_C|SetWB_ThrowPlane _player _returnvalue)
      (goto _label))))

(fn HideControls
  (bind _player (Variables|Default|Getplayer))
  (Variables|/Game/FirstPersonBP/Blueprints/FirstPersonCharacter.FirstPersonCharacter_C|SetaddedAlreadyToViewport_ThrowPlane _player false)
  (Widget|RemovefromParent (Variables|/Game/FirstPersonBP/Blueprints/FirstPersonCharacter.FirstPersonCharacter_C|GetWB_ThrowPlane _player)))

(fn ShowDiaryControls
  (bind _player (Variables|Default|Getplayer))
  (if (Utilities|IsValid (Variables|/Game/FirstPersonBP/Blueprints/FirstPersonCharacter.FirstPersonCharacter_C|GetWB_Diary _player))
    _
    (else
      (bind _returnvalue (UserInterface|CreateWidget "/Game/JuegoX/UI/HUD/WB_Diary.WB_Diary_C" (Game|GetPlayerController 0)))
      (Variables|/Game/FirstPersonBP/Blueprints/FirstPersonCharacter.FirstPersonCharacter_C|SetWB_Diary _player _returnvalue)))
  (UserInterface|Viewport|AddtoViewport (Variables|/Game/FirstPersonBP/Blueprints/FirstPersonCharacter.FirstPersonCharacter_C|GetWB_Diary _player) 0))