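; Interactable armchair the player sits in and stands up from with the Inspect input, which it receives only while focused or occupied.
; The Sofa timeline lerps the player between Stand and Sit points while turning toward PaperCan, and plays in reverse to stand.
; Sitting activates Diario's interaction, lights a point light, shows the stand prompt and makes the chair pawn-overlap.
; Standing undoes these, restoring blocking collision when the timeline finishes.
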(event Custom|EndSofa
  (Variables|Default|Setend true)
  (Variables|/Game/JuegoX/Blueprints/Objects/Interactable.Interactable_C|SetisFocused? (Variables|Default|GetInteractuable) false)
  (Variables|/Game/FirstPersonBP/Blueprints/FirstPersonCharacter.FirstPersonCharacter_C|SetplayerIsSitting? (Variables|Default|GetPlayer) false)
  (CallFunction|HideControls)
  (Variables|Default|SetSentado false)
  (CallFunction|ActivateInteraction (Variables|Default|GetDiario) false)
  (Rendering|Components|Light|SetIntensity (Variables|Default|GetPointLight) 0.0)
  (bind _sofa_sit (Timeline|Sofa Reverse)
    (:Update
      (Utilities|IsValid (Variables|Default|GetpaperCan)
        (:Is%20Valid
          (bind (_location _rotation) (CallFunction|CharacterLocationRotation _sofa_sit))
          (Transformation|SetActorLocationAndRotation (Variables|Default|GetPlayer) _location _rotation)
          (Variables|/Game/JuegoX/Blueprints/Objects/Interactable.Interactable_C|SetisFocused? (Variables|Default|GetInteractuable) false))))
    (:Finished
      (if (Variables|Default|Getend)
        (Collision|SetCollisionProfileName (Variables|Default|GetMesh) "BlockAll" :!class /Script/Engine.PrimitiveComponent)
        (Variables|Default|Setend false)))))

(event EventTick
  (params (DeltaSeconds :type Float%20%28single-precision%29))
  (bind _returnvalue (Game|GetPlayerController 0))
  (if (Variables|/Game/JuegoX/Blueprints/Objects/Interactable.Interactable_C|GetisFocused? (Variables|Default|GetInteractuable))
    (Input|EnableInput _returnvalue :!label _label)
    (elif (Variables|Default|GetSentado)
      (goto _label)
      (else
        (Input|DisableInput _returnvalue)))))

(event EventBeginPlay
  (bind _asfirst_person_character (Utilities|Casting|CastToFirstPersonCharacter (Game|GetPlayerCharacter 0)))
  (bind _output_get (Variables|Default|Setplayer _asfirst_person_character))
  (Variables|/Game/JuegoX/Blueprints/Objects/Interactable.Interactable_C|Setplayer (Variables|Default|GetInteractuable) _output_get)
  (Variables|/Game/JuegoX/Blueprints/Objects/Interactable.Interactable_C|SetMesh (Variables|Default|GetInteractuable) (Variables|Default|GetMesh))
  (Variables|/Game/JuegoX/Blueprints/Objects/Interactable.Interactable_C|SetText (Variables|Default|GetInteractuable) (Variables|Default|GetTextRender))
  (Variables|/Game/JuegoX/Blueprints/Objects/Interactable.Interactable_C|Setis%20a%20nonInspectionable%20Object? (Variables|Default|GetInteractuable) true))

(event Input|ActionEvents|InputActionInspect
  (params (Key :type Key%20Structure :default "None"))
  (:Pressed
    (if (Variables|/Game/JuegoX/Blueprints/Objects/Interactable.Interactable_C|GetisFocused? (Variables|Default|GetInteractuable))
      (if (Variables|Default|GetSentado)
        (CallFunction|EndSofa :!label _label)
        (else
          (Variables|Default|SetSentado true)
          (CallFunction|ActivateInteraction (Variables|Default|GetDiario) true)
          (Rendering|Components|Light|SetIntensity (Variables|Default|GetPointLight) 1e+02)
          (Collision|SetCollisionProfileName (Variables|Default|GetMesh) "OverlapOnlyPawn" :!class /Script/Engine.PrimitiveComponent)
          (Variables|/Game/FirstPersonBP/Blueprints/FirstPersonCharacter.FirstPersonCharacter_C|SetplayerIsSitting? (Variables|Default|GetPlayer) true)
          (CallFunction|ShowControls)
          (bind _sofa_sit (Timeline|Sofa Play)
            (:Update
              (Utilities|IsValid (Variables|Default|GetpaperCan)
                (:Is%20Valid
                  (bind (_location _rotation) (CallFunction|CharacterLocationRotation _sofa_sit))
                  (Transformation|SetActorLocationAndRotation (Variables|Default|GetPlayer) _location _rotation)
                  (Variables|/Game/JuegoX/Blueprints/Objects/Interactable.Interactable_C|SetisFocused? (Variables|Default|GetInteractuable) false))))
            (:Finished
              (if (Variables|Default|Getend)
                (Collision|SetCollisionProfileName (Variables|Default|GetMesh) "BlockAll" :!class /Script/Engine.PrimitiveComponent)
                (Variables|Default|Setend false))))))
      (elif (and (Variables|Default|GetSentado) (not (Variables|/Game/JuegoX/Blueprints/Objects/Interactable.Interactable_C|GetisFocused? (Variables|/Game/JuegoX/Blueprints/Objects/OBJ_ClosedDiary_DiaryParent.OBJ_ClosedDiary_DiaryParent_C|GetInteractuable (Variables|Default|GetDiario)))))
        (goto _label)))))

(fn ConstructionScript)

(fn ActivateInteraction
  (params (Mesh :type Actor%20Object%20Reference) (Activate? :type Boolean))
  (Utilities|IsValid Mesh
    (:Is%20Valid
      (Variables|/Game/JuegoX/Blueprints/Objects/Interactable.Interactable_C|SetinteractionActivated (Actor|GetComponentbyClass Mesh "/Game/JuegoX/Blueprints/Objects/Interactable.Interactable_C") Activate?))))

(fn CharacterLocationRotation
  (params (Alpha :type Float%20%28single-precision%29))
  (bind _stand (Variables|Default|GetStand))
  (bind _sit (Variables|Default|GetSit))
  (bind _player (Variables|Default|GetPlayer))
  (bind _returnvalue (Transformation|GetWorldLocation _sit))
  (bind _returnvalue_2 (Transformation|GetWorldLocation _stand))
  (bind _returnvalue_3 (Transformation|GetActorLocation _player))
  (bind _z (Math|Vector|BreakVector _returnvalue_3))
  (bind (_x _y) (Math|Vector|BreakVector _returnvalue))
  (bind (_x_2 _y_2) (Math|Vector|BreakVector _returnvalue_2))
  (bind _returnvalue_4 (Math|Vector|MakeVector _x _y _z))
  ;[1 1 1] Hacer una animacion con la camaara como la del mapa o la d levantarse
  (return (Math|Vector|Lerp(Vector) (Math|Vector|MakeVector _x_2 _y_2 _z) _returnvalue_4 Alpha) (Math|Rotator|Lerp(Rotator) (Transformation|GetActorRotation (Variables|Default|GetPlayer)) (Math|Rotator|FindLookatRotation _returnvalue_4 (Transformation|GetActorLocation (Variables|Default|GetpaperCan))) Alpha)))

(fn ShowControls
  (if (Utilities|IsValid (Variables|/Game/FirstPersonBP/Blueprints/FirstPersonCharacter.FirstPersonCharacter_C|GetInventoryHUD (Variables|Default|Getplayer)))
    _
    (else
      (bind _returnvalue (UserInterface|CreateWidget "/Game/JuegoX/UI/HUD/WB_Inventory.WB_Inventory_C" (Game|GetPlayerController 0)))
      (Variables|/Game/FirstPersonBP/Blueprints/FirstPersonCharacter.FirstPersonCharacter_C|SetInventoryHUD (Variables|Default|Getplayer) _returnvalue)))
  (Rendering|Components|TextRender|SetText (Variables|/Game/JuegoX/UI/HUD/WB_Inventory.WB_Inventory_C|GetAction_One (Variables|/Game/FirstPersonBP/Blueprints/FirstPersonCharacter.FirstPersonCharacter_C|GetInventoryHUD (Variables|Default|Getplayer))) "to stand")
  (Variables|Default|Setwidget_Anim (Variables|/Game/JuegoX/UI/HUD/WB_Inventory.WB_Inventory_C|GetControls_1_Anim (Variables|/Game/FirstPersonBP/Blueprints/FirstPersonCharacter.FirstPersonCharacter_C|GetInventoryHUD (Variables|Default|Getplayer))))
  (if (UserInterface|Viewport|IsinViewport (Variables|/Game/FirstPersonBP/Blueprints/FirstPersonCharacter.FirstPersonCharacter_C|GetInventoryHUD (Variables|Default|Getplayer)))
    _
    (else
      (UserInterface|Viewport|AddtoViewport (Variables|/Game/FirstPersonBP/Blueprints/FirstPersonCharacter.FirstPersonCharacter_C|GetInventoryHUD (Variables|Default|Getplayer)) 0)))
  (Class|UserWidget|PlayAnimationForward (Variables|/Game/FirstPersonBP/Blueprints/FirstPersonCharacter.FirstPersonCharacter_C|GetInventoryHUD (Variables|Default|Getplayer)) (Variables|Default|Getwidget_Anim) 4.0))

(fn HideControls
  (Class|UserWidget|PlayAnimationReverse (Variables|/Game/FirstPersonBP/Blueprints/FirstPersonCharacter.FirstPersonCharacter_C|GetInventoryHUD (Variables|Default|Getplayer)) (Variables|Default|Getwidget_Anim) 4.0))