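; Parent interactable object, named for cigarettes, that the player picks up to inspect and drops back in place.
; Tick enables input while the Interactable is focused or inspected.
; Inspect toggles a timeline that lerps the actor to the player's inspection point or back, showing HUD controls and gating the E prompt fade.
; Interact and ConnectWithCable are empty hooks, the latter reached when GameInstance holds an unconnected cable and this object accepts it.
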(event Custom|Inspection
  (if (Variables|/Game/JuegoX/Blueprints/Objects/Interactable.Interactable_C|GetisInspectingIt (Variables|Default|GetInteractable))
    (CallFunction|EndInspection)
    (else
      (Utilities|FlowControl|Sequence
        (:then_0
          (Audio|PlaySound2D (Variables|Default|GetSound) 1.0 1.0 0.0 0 0))
        (:then_1
          (CallFunction|BeginInspection))))))

(event Custom|EndInspection
  ;[1 1 1] lo de la E
  (if (Variables|Default|GetableToFadeE)
    _
    (else
      (Variables|Default|SetableToFadeE true)))
  (Variables|/Game/JuegoX/Blueprints/Objects/Interactable.Interactable_C|SetisInspectingIt (Variables|Default|GetInteractable) false)
  (CallFunction|HideControls)
  (bind _move_object (Timeline|inpection%20Timeline Reverse)
    (:Update
      (CallFunction|UpdateLocation _move_object))
    (:Finished
      (if (Variables|Default|GetableToFadeE) ; E appears when the animation finishes
        (Variables|/Game/JuegoX/Blueprints/Objects/Interactable.Interactable_C|SetfadeE (Variables|Default|GetInteractable) true)
        (Variables|/Game/FirstPersonBP/Blueprints/FirstPersonCharacter.FirstPersonCharacter_C|SetplayerInspectingObject (Variables|Default|Getplayer) false)))))

(event Custom|BeginInspection
  (Utilities|FlowControl|Sequence
    (:then_0
      (CallFunction|ShowControls))
    (:then_1
      (CallFunction|InspectionView)
      (Variables|/Game/JuegoX/Blueprints/Objects/Interactable.Interactable_C|SetisInspectingIt (Variables|Default|GetInteractable) true)
      (Variables|/Game/FirstPersonBP/Blueprints/FirstPersonCharacter.FirstPersonCharacter_C|SetplayerInspectingObject (Variables|Default|Getplayer) true)
      ;[1 1 1] lo de la E
      (Variables|Default|SetableToFadeE false)
      (Variables|/Game/JuegoX/Blueprints/Objects/Interactable.Interactable_C|SetfadeE (Variables|Default|GetInteractable) false)
      (Variables|/Game/JuegoX/Blueprints/Objects/Interactable.Interactable_C|SetinitialRot (Variables|Default|GetInteractable) (Transformation|GetActorRotation))
      (Variables|/Game/JuegoX/Blueprints/Objects/Interactable.Interactable_C|SetinitialPos (Variables|Default|GetInteractable) (Transformation|GetActorLocation))
      (bind _move_object (Timeline|inpection%20Timeline Play)
        (:Update
          (CallFunction|UpdateLocation _move_object))
        (:Finished
          (if (Variables|Default|GetableToFadeE) ; E appears when the animation finishes
            (Variables|/Game/JuegoX/Blueprints/Objects/Interactable.Interactable_C|SetfadeE (Variables|Default|GetInteractable) true)
            (Variables|/Game/FirstPersonBP/Blueprints/FirstPersonCharacter.FirstPersonCharacter_C|SetplayerInspectingObject (Variables|Default|Getplayer) false)))))))

(event EventBeginPlay
  (Variables|/Game/JuegoX/Blueprints/Objects/Interactable.Interactable_C|SetfadeE (Variables|Default|GetInteractable) true)
  (bind _asfirst_person_character (Utilities|Casting|CastToFirstPersonCharacter (Game|GetPlayerCharacter 0)))
  (bind _output_get (Variables|Default|Setplayer _asfirst_person_character))
  (Variables|/Game/JuegoX/Blueprints/Objects/Interactable.Interactable_C|Setplayer (Variables|Default|GetInteractable) _output_get)
  (bind _asmy_game_instance (Utilities|Casting|CastToMyGameInstance (Game|GetGameInstance)))
  (Variables|Default|SetGameInstance _asmy_game_instance))

(event EventTick
  (params (DeltaSeconds :type Float%20%28single-precision%29))
  (bind _returnvalue (Game|GetPlayerController 0))
  (if true
    (if (Variables|/Game/JuegoX/Blueprints/Objects/Interactable.Interactable_C|GetisInspectingIt (Variables|Default|GetInteractable))
      (Input|EnableInput _returnvalue :!label _label)
      (elif (Variables|/Game/JuegoX/Blueprints/Objects/Interactable.Interactable_C|GetisFocused? (Variables|Default|GetInteractable))
        (goto _label)
        (else
          (Input|DisableInput _returnvalue))))))

(event Input|ActionEvents|InputActionInteract
  (params (Key :type Key%20Structure :default "None"))
  (:Pressed
    (if true
      (if (Variables|/Game/JuegoX/Blueprints/Objects/Interactable.Interactable_C|GetisInspectingIt (Variables|Default|GetInteractable))
        (CallFunction|Interact) ; Aqui esta empty pq no tiene interaccion
      ))))

(event Input|ActionEvents|InputActionInspect
  (params (Key :type Key%20Structure :default "None"))
  (:Pressed
    (if (Variables|/Game/JuegoX/Blueprints/Objects/Interactable.Interactable_C|GetinteractionActivated (Variables|Default|GetInteractable))
      (if (Variables|/Game/JuegoX/Blueprints/MyGameInstance.MyGameInstance_C|GetCable_Connected? (Variables|Default|GetGameInstance))
        (CallFunction|Inspection)
        (elif (Variables|/Game/JuegoX/Blueprints/MyGameInstance.MyGameInstance_C|GetHas_Cable? (Variables|Default|GetGameInstance))
          (if (Variables|Default|GetCableCanConnect)
            (CallFunction|ConnectwithCable)
            (else
              (CallFunction|Inspection)))
          (else
            (CallFunction|Inspection)))))))

(fn ConstructionScript
  (Variables|Default|SetSound 0)
  (Variables|/Game/JuegoX/Blueprints/Objects/Interactable.Interactable_C|SetMesh (Variables|Default|GetInteractable) (Variables|Default|GetMesh))
  (Variables|/Game/JuegoX/Blueprints/Objects/Interactable.Interactable_C|SetText (Variables|Default|GetInteractable) (Variables|Default|GetTextRender)))

(fn ShowControls
  (if (Utilities|IsValid (Variables|/Game/FirstPersonBP/Blueprints/FirstPersonCharacter.FirstPersonCharacter_C|GetHUD (Variables|Default|Getplayer)))
    _
    (else
      (bind _returnvalue (UserInterface|CreateWidget "/Game/JuegoX/UI/HUD/WB_HUD.WB_HUD_C" (Game|GetPlayerController 0)))
      (Variables|/Game/FirstPersonBP/Blueprints/FirstPersonCharacter.FirstPersonCharacter_C|SetHUD (Variables|Default|Getplayer) _returnvalue)))
  (CallFunction|SetVariables)
  (if (UserInterface|Viewport|IsinViewport (Variables|/Game/FirstPersonBP/Blueprints/FirstPersonCharacter.FirstPersonCharacter_C|GetHUD (Variables|Default|Getplayer)))
    _
    (else
      (UserInterface|Viewport|AddtoViewport (Variables|/Game/FirstPersonBP/Blueprints/FirstPersonCharacter.FirstPersonCharacter_C|GetHUD (Variables|Default|Getplayer)) 0)))
  (Class|UserWidget|PlayAnimationForward (Variables|/Game/FirstPersonBP/Blueprints/FirstPersonCharacter.FirstPersonCharacter_C|GetHUD (Variables|Default|Getplayer)) (Variables|Default|Getwidget_Anim) 4.0))

(fn HideControls
  (Class|UserWidget|PlayAnimationReverse (Variables|/Game/FirstPersonBP/Blueprints/FirstPersonCharacter.FirstPersonCharacter_C|GetHUD (Variables|Default|Getplayer)) (Variables|Default|Getwidget_Anim) 4.0))

(fn Interact)

(fn UpdateLocation
  (params (timeline%20Value :type Float%20%28single-precision%29))
  (bind _interactable (Variables|Default|GetInteractable))
  (Transformation|SetActorLocationAndRotation (Math|Vector|Lerp(Vector) (Variables|/Game/JuegoX/Blueprints/Objects/Interactable.Interactable_C|GetinitialPos _interactable) (Variables|/Game/JuegoX/Blueprints/Objects/Interactable.Interactable_C|GetinspectionPoint _interactable) timeline%20Value) (Math|Rotator|Lerp(Rotator) (Variables|/Game/JuegoX/Blueprints/Objects/Interactable.Interactable_C|GetinitialRot _interactable) (Transformation|GetActorRotation) timeline%20Value) true))

(fn InspectionView
  (Variables|/Game/JuegoX/Blueprints/Objects/Interactable.Interactable_C|SetinspectionPoint (Variables|Default|GetInteractable) (Transformation|GetWorldLocation (Variables|/Game/FirstPersonBP/Blueprints/FirstPersonCharacter.FirstPersonCharacter_C|GetInpectionView (Variables|Default|Getplayer)))))

(fn SetVariables
  (Rendering|Components|TextRender|SetText (Variables|/Game/JuegoX/UI/HUD/WB_HUD.WB_HUD_C|GetAction_One (Variables|/Game/FirstPersonBP/Blueprints/FirstPersonCharacter.FirstPersonCharacter_C|GetHUD (Variables|Default|Getplayer))) "to drop")
  (Variables|Default|Setwidget_Anim (Variables|/Game/JuegoX/UI/HUD/WB_HUD.WB_HUD_C|GetControls_1_Anim (Variables|/Game/FirstPersonBP/Blueprints/FirstPersonCharacter.FirstPersonCharacter_C|GetHUD (Variables|Default|Getplayer)))))

(fn ConnectwithCable)