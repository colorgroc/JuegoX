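; Interactable remote controller object, child of an interactable base, that hands the player control of a remote-controlled plane once the map puzzle is completed.
; Tick waits for the GameInstance puzzle flag, toggles mesh visibility once, activates interaction and enables input only while focused or inspected.
; Interacting during inspection sets "InvisiblePared" trigger boxes to block, swaps HUD control hints, possesses the plane and destroys the controller.
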(event EventTick
  (params (DeltaSeconds :type Float%20%28single-precision%29))
  (bind _returnvalue (Game|GetPlayerController 0))
  (if (Utilities|IsValid (Variables|Default|GetGameInstance))
    (if (Variables|/Game/JuegoX/Blueprints/MyGameInstance.MyGameInstance_C|GetMapPuzzle_Completed (Variables|Default|GetGameInstance))
      (Utilities|FlowControl|Sequence
        (:then_0
          (Utilities|FlowControl|DoOnce false
            (:Completed
              (Rendering|ToggleVisibility (Variables|Character|GetMesh) false))))
        (:then_1
          (Variables|/Game/JuegoX/Blueprints/Objects/Interactable.Interactable_C|SetinteractionActivated (Variables|Default|GetInteractable) true)
          (if (Variables|/Game/JuegoX/Blueprints/Objects/Interactable.Interactable_C|GetisInspectingIt (Variables|Default|GetInteractable))
            (Input|EnableInput _returnvalue :!label _label)
            (elif (Variables|/Game/JuegoX/Blueprints/Objects/Interactable.Interactable_C|GetisFocused? (Variables|Default|GetInteractable))
              (goto _label)
              (else
                (Input|DisableInput _returnvalue :!label _label_2))))))
      (else
        (goto _label_2)))))

(event EventInteract
  (if (Variables|/Game/JuegoX/Blueprints/Objects/Interactable.Interactable_C|GetisInspectingIt (Variables|Default|GetInteractable))
    (Variables|/Game/JuegoX/Blueprints/Objects/Interactable.Interactable_C|SetisInspectingIt (Variables|Default|GetInteractable) false)
    (CallFunction|PlaneControl)))

(event EventSetVariables
  (bind _player (Variables|Default|Getplayer))
  (bind _hud (Variables|/Game/FirstPersonBP/Blueprints/FirstPersonCharacter.FirstPersonCharacter_C|GetHUD _player))
  (Rendering|Components|TextRender|SetText (Variables|/Game/JuegoX/UI/HUD/WB_HUD.WB_HUD_C|GetT_Drop _hud) "to drop")
  (Rendering|Components|TextRender|SetText (Variables|/Game/JuegoX/UI/HUD/WB_HUD.WB_HUD_C|GetT_Action _hud) "to pilot remote control plane")
  (Variables|Default|Setwidget_Anim (Variables|/Game/JuegoX/UI/HUD/WB_HUD.WB_HUD_C|GetControls_2_Anim _hud)))

(fn ConstructionScript)

(fn ShowControlsPlane
  (Variables|Default|Setwidget_Anim (Variables|/Game/JuegoX/UI/HUD/WB_HUD.WB_HUD_C|GetControls_4_Anim (Variables|/Game/FirstPersonBP/Blueprints/FirstPersonCharacter.FirstPersonCharacter_C|GetHUD (Variables|Default|Getplayer))))
  (if (UserInterface|Viewport|IsinViewport (Variables|/Game/FirstPersonBP/Blueprints/FirstPersonCharacter.FirstPersonCharacter_C|GetHUD (Variables|Default|Getplayer)))
    _
    (else
      (UserInterface|Viewport|AddtoViewport (Variables|/Game/FirstPersonBP/Blueprints/FirstPersonCharacter.FirstPersonCharacter_C|GetHUD (Variables|Default|Getplayer)) 0)))
  (Class|UserWidget|PlayAnimationForward (Variables|/Game/FirstPersonBP/Blueprints/FirstPersonCharacter.FirstPersonCharacter_C|GetHUD (Variables|Default|Getplayer)) (Variables|Default|Getwidget_Anim) 4.0))

(fn PlaneControl
  (bind _outactors (Actor|GetAllActorswithTag "InvisiblePared"))
  (for _array_element _outactors
    (bind _astrigger_box (Utilities|Casting|CastToTriggerBox _array_element))
    (Collision|SetCollisionProfileName (Variables|/Script/Engine.TriggerBase|GetCollisionComponent _astrigger_box) "BlockAllDynamic" :!class /Script/Engine.PrimitiveComponent))
  (if (Utilities|IsValid (Variables|Default|GetAvion))
    (CallFunction|HideControls) ; Hide controller widget
    (CallFunction|ShowControlsPlane)
    (Components|DestroyComponent (Variables|Character|GetMesh))
    (Pawn|Possess (Game|GetPlayerController 0) (Variables|Default|GetAvion))
    (Actor|DestroyActor)))