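; TapaBaul is an interactable chest lid that the player can open and close once the game instance flags the chest as interactable.
; While focused or inspected, it enables input, shows its widget and turns its text toward the player; otherwise it disables both input and widget.
; The Inspect action toggles a timeline that lerps the lid's position and rotation, reversing it to close, or prints a blocked message when locked.
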(event Custom|EndInspection
  (bind _interactuable (Variables|Default|GetInteractuable))
  (bind _initialpos (Variables|/Game/JuegoX/Blueprints/Objects/Interactable.Interactable_C|GetinitialPos _interactuable))
  (bind (_x _y) (Math|Vector|BreakVector _initialpos))
  (Variables|/Game/JuegoX/Blueprints/Objects/Interactable.Interactable_C|SetisInspectingIt (Variables|Default|GetInteractuable) false)
  (Variables|/Game/FirstPersonBP/Blueprints/FirstPersonCharacter.FirstPersonCharacter_C|SetplayerInspectingObject (Variables|Default|Getplayer) false)
  (bind _move_object (Timeline|Inspect Reverse)
    (:Update
      (bind _output_get (Variables|Default|SetMovedObject _move_object))
      (Transformation|SetActorLocationAndRotation (Math|Vector|Lerp(Vector) _initialpos (Math|Vector|MakeVector _x _y -233.0) _output_get) (Math|Rotator|Lerp(Rotator) (Variables|/Game/JuegoX/Blueprints/Objects/Interactable.Interactable_C|GetinitialRot _interactuable) "30.000000,30.000000, 0" _output_get true)))))

(event EventTick
  (params (DeltaSeconds :type Float%20%28single-precision%29))
  (bind _returnvalue (Game|GetPlayerController 0))
  (bind _widget (Variables|Default|GetWidget))
  (if (Variables|/Game/JuegoX/Blueprints/Objects/Interactable.Interactable_C|GetisInspectingIt (Variables|Default|GetInteractuable))
    (Input|EnableInput _returnvalue :!label _label)
    (Rendering|SetVisibility _widget true false)
    (Transformation|SetWorldRotation (Variables|Default|GetTextRender) (Math|Rotator|FindLookatRotation (Transformation|GetActorLocation) (Transformation|GetActorLocation (Variables|Default|Getplayer))) false false)
    (elif (Variables|/Game/JuegoX/Blueprints/Objects/Interactable.Interactable_C|GetisFocused? (Variables|Default|GetInteractuable))
      (goto _label)
      (else
        (Input|DisableInput _returnvalue)
        (Rendering|SetVisibility _widget false false)))))

(event EventBeginPlay
  (bind _asfirst_person_character (Utilities|Casting|CastToFirstPersonCharacter (Game|GetPlayerCharacter 0)))
  (Variables|Default|Setplayer _asfirst_person_character)
  (bind _asmy_game_instance (Utilities|Casting|CastToMyGameInstance (Game|GetGameInstance)))
  (Variables|Default|SetgameInstance _asmy_game_instance))

(event Input|ActionEvents|InputActionInspect
  (params (Key :type Key%20Structure :default "None"))
  (bind _interactuable (Variables|Default|GetInteractuable))
  (bind _initialpos (Variables|/Game/JuegoX/Blueprints/Objects/Interactable.Interactable_C|GetinitialPos _interactuable))
  (bind (_x _y) (Math|Vector|BreakVector _initialpos))
  (:Pressed
    (if (Variables|/Game/JuegoX/Blueprints/MyGameInstance.MyGameInstance_C|GetbaulInteractuable (Variables|Default|GetgameInstance))
      (if (Variables|/Game/JuegoX/Blueprints/Objects/Interactable.Interactable_C|GetisFocused? (Variables|Default|GetInteractuable))
        (if (Variables|Default|Getopened)
          (Variables|Default|Setopened false)
          (CallFunction|EndInspection)
          (else
            (Variables|Default|Setopened true)
            (bind _move_object (Timeline|Inspect Play)
              (:Update
                (bind _output_get (Variables|Default|SetMovedObject _move_object))
                (Transformation|SetActorLocationAndRotation (Math|Vector|Lerp(Vector) _initialpos (Math|Vector|MakeVector _x _y -233.0) _output_get) (Math|Rotator|Lerp(Rotator) (Variables|/Game/JuegoX/Blueprints/Objects/Interactable.Interactable_C|GetinitialRot _interactuable) "30.000000,30.000000, 0" _output_get true)))))))
      (else
        (Development|PrintString "It's blocked!" true true "(R=1.000000,G=0.016751,B=0.000000,A=1.000000)")))))

(fn ConstructionScript)