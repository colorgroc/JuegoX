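; Interactable table drawer that the player opens and closes.
; Each Tick, the Interactuable focus flag toggles input and the prompt widget, and rotates the text render toward the first-person player.
; While focused, Inspect plays the Anim sequence forward or in reverse with a drawer sound, flips IsOpen and clears focus.
; A separate Interact function performs the same toggle without sound or focus check.
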(event EventTick
  (params (DeltaSeconds :type Float%20%28single-precision%29))
  (bind _returnvalue (Game|GetPlayerController 0))
  (if (Variables|/Game/JuegoX/Blueprints/Objects/Interactable.Interactable_C|GetisFocused? (Variables|Default|GetInteractuable))
    (Input|EnableInput _returnvalue)
    (Rendering|SetVisibility (Variables|Default|GetWidget) true false)
    (Transformation|SetWorldRotation (Variables|Default|GetTextRender) (Math|Rotator|FindLookatRotation (Transformation|GetActorLocation) (Transformation|GetActorLocation (Variables|Default|Getplayer))) false false)
    (else
      (Input|DisableInput _returnvalue)
      (Rendering|SetVisibility (Variables|Default|GetWidget) false false))))

(event EventBeginPlay
  (bind _asfirst_person_character (Utilities|Casting|CastToFirstPersonCharacter (Game|GetPlayerCharacter 0)))
  (Variables|Default|Setplayer _asfirst_person_character))

(event Input|ActionEvents|InputActionInspect
  (params (Key :type Key%20Structure :default "None"))
  (bind _anim (Variables|Default|GetAnim))
  (bind _sequenceplayer (Variables|/Script/ActorSequence.ActorSequenceComponent|GetSequencePlayer _anim))
  (:Pressed
    (if (Variables|/Game/JuegoX/Blueprints/Objects/Interactable.Interactable_C|GetisFocused? (Variables|Default|GetInteractuable))
      (if (Variables|Default|GetisOpen?)
        (Audio|PlaySound2D "/Game/Soniditos/392770__danialarcon0698__abre-cajon.392770__danialarcon0698__abre-cajon" 1.0 1.0 0.0 0 0)
        (Class|MovieSceneSequencePlayer|PlayReverse _sequenceplayer)
        (Variables|Default|SetisOpen? false)
        (else
          (Audio|PlaySound2D "/Game/Soniditos/237379__squareal__cutlery-drawer-closing-01.237379__squareal__cutlery-drawer-closing-01" 1.0 1.0 0.0 0 0)
          (Sequencer|Player|Play _sequenceplayer :!class /Script/MovieScene.MovieSceneSequencePlayer)
          (Variables|Default|SetisOpen? true)))
      (Variables|/Game/JuegoX/Blueprints/Objects/Interactable.Interactable_C|SetisFocused? (Variables|Default|GetInteractuable) false))))

(fn ConstructionScript)

(fn Interact
  (bind _anim (Variables|Default|GetAnim))
  (bind _sequenceplayer (Variables|/Script/ActorSequence.ActorSequenceComponent|GetSequencePlayer _anim))
  (if (Variables|Default|GetisOpen?)
    (Class|MovieSceneSequencePlayer|PlayReverse _sequenceplayer)
    (Variables|Default|SetisOpen? false)
    (else
      (Sequencer|Player|Play _sequenceplayer :!class /Script/MovieScene.MovieSceneSequencePlayer)
      (Variables|Default|SetisOpen? true))))