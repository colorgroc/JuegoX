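; Actor component that marks its owner's Interactable as important and makes the mesh's highlight blink when the player is near.
; A looping timer runs SetHighlight, which does nothing while the Interactable is focused.
; Within DistanceToGlow, a counter keeps custom depth on for two calls and off for one; beyond it, the highlight turns off.
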(event EventBeginPlay
  (bind _returnvalue (Components|GetOwner))
  (Variables|Default|SetMesh (Actor|GetComponentbyClass _returnvalue "/Script/Engine.StaticMeshComponent"))
  (Variables|/Game/JuegoX/Blueprints/Objects/Interactable.Interactable_C|SetisImportant? (Actor|GetComponentbyClass _returnvalue "/Game/JuegoX/Blueprints/Objects/Interactable.Interactable_C") true)
  (Utilities|Time|SetTimerbyFunctionName 0 "SetHighlight" 0.3 true))

(event EventTick
  (params (DeltaSeconds :type Float%20%28single-precision%29)))

(fn SetHighlight
  (bind _returnvalue (Components|GetOwner))
  (bind _mesh (Variables|Default|GetMesh))
  (if (not (Variables|/Game/JuegoX/Blueprints/Objects/Interactable.Interactable_C|GetisFocused? (Actor|GetComponentbyClass _returnvalue "/Game/JuegoX/Blueprints/Objects/Interactable.Interactable_C")))
    (Math|Float|CompareFloat (Transformation|GetDistanceTo _returnvalue (Game|GetPlayerCharacter 0)) (Variables|Default|GetDistance%20to%20Glow)
      (:>
        (Rendering|SetRenderCustomDepth _mesh false :!label _label)
        (Rendering|SetCustomDepthStencilValue _mesh 1)
        (Variables|Default|Settimer 0))
      (:==
        (if (> (Variables|Default|Gettimer) 1) :!label _label_2
          (goto _label)
          (else
            (Rendering|SetRenderCustomDepth _mesh true)
            (Rendering|SetCustomDepthStencilValue _mesh 1)
            (Math|Integer|IncrementInt (Variables|Default|Gettimer)))))
      (:<
        (goto _label_2)))))