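; Actor component that highlights its owner's static mesh as an interactable through custom depth while the player's PlayerInpectingMapa flag is on.
; Each Tick, if InteractionActivated and that flag are true, it enables custom depth and sets one of two stencil values based on IsFocused; otherwise it disables custom depth.
; BoolCheck looks up the FirstPersonCharacter on every call instead of using the Player reference cached at BeginPlay.
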(event EventBeginPlay
  (Variables|Default|SetisFocused? false)
  (Variables|Default|SetMesh (Actor|GetComponentbyClass (Components|GetOwner) "/Script/Engine.StaticMeshComponent"))
  (bind _returnvalue (Actor|GetActorOfClass "/Game/FirstPersonBP/Blueprints/FirstPersonCharacter.FirstPersonCharacter_C"))
  (Variables|Default|Setplayer _returnvalue))

(event EventTick
  (params (DeltaSeconds :type Float%20%28single-precision%29))
  (bind _mesh (Variables|Default|GetMesh))
  (if (Variables|Default|GetinteractionActivated)
    (bind _bool (CallFunction|BoolCheck))
    (if _bool
      (Rendering|SetRenderCustomDepth (Variables|Default|GetMesh) true)
      (if (Variables|Default|GetisFocused?)
        (Rendering|SetCustomDepthStencilValue _mesh 2)
        (else
          (Rendering|SetCustomDepthStencilValue _mesh 1)))
      (else
        (Rendering|SetRenderCustomDepth (Variables|Default|GetMesh) false :!label _label)))
    (else
      (goto _label))))

(fn BoolCheck
  (bind _returnvalue (Actor|GetActorOfClass "/Game/FirstPersonBP/Blueprints/FirstPersonCharacter.FirstPersonCharacter_C"))
  (return (Variables|/Game/FirstPersonBP/Blueprints/FirstPersonCharacter.FirstPersonCharacter_C|GetplayerInpectingMapa _returnvalue)))