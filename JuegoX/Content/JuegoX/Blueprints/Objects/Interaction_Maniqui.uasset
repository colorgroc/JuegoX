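; Interaction_Maniqui is an interactable mannequin object that highlights itself while the player character's PlayerInteractinWithManiqui flag is set.
; Every Tick polls that flag and branches on Initial.
; When Initial is true, a dynamic transparent material fades in, red when focused and white otherwise.
; When false, custom depth with a focus-dependent stencil value marks the mesh until Changed is set.
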(event EventBeginPlay
  (Variables|Default|SetisFocused? false)
  (bind _returnvalue (Rendering|Material|CreateDynamicMaterialInstance (Variables|Default|GetMesh) 0 "/Game/JuegoX/Materials/MAT_Transparent_Inst.MAT_Transparent_Inst" "None" :!class /Script/Engine.PrimitiveComponent))
  (Variables|Default|SetMaterial _returnvalue))

(event EventTick
  (params (DeltaSeconds :type Float%20%28single-precision%29))
  (bind _mesh (Variables|Default|GetMesh))
  (bind _material (Variables|Default|GetMaterial))
  (bind _material_2 (Variables|Default|GetMaterial))
  (bind _material_3 (Variables|Default|GetMaterial))
  (if (Variables|Default|Getinitial)
    (bind _bool (CallFunction|BoolCheck))
    (if _bool
      (Utilities|IsValid _material_2
        (:Is%20Valid
          (Rendering|Material|SetScalarParameterValue _material_2 "Opacity" 0.3 :!class /Script/Engine.MaterialInstanceDynamic)
          (if (Variables|Default|GetisFocused?)
            (Rendering|Material|SetVectorParameterValue _material_3 "Color" "(R=1.000000,G=0.000000,B=0.000000,A=1.000000)" :!class /Script/Engine.MaterialInstanceDynamic)
            (else
              (Rendering|Material|SetVectorParameterValue _material_3 "Color" "(R=1.000000,G=1.000000,B=1.000000,A=1.000000)" :!class /Script/Engine.MaterialInstanceDynamic)))))
      (else
        (Utilities|IsValid _material
          (:Is%20Valid
            (Rendering|Material|SetScalarParameterValue _material "Opacity" 0.0 :!class /Script/Engine.MaterialInstanceDynamic)))))
    (else
      (bind _bool_2 (CallFunction|BoolCheck))
      (if _bool_2
        (if (Variables|Default|Getchanged)
          (Rendering|SetRenderCustomDepth (Variables|Default|GetMesh) false :!label _label)
          (else
            (Rendering|SetRenderCustomDepth (Variables|Default|GetMesh) true)
            (if (Variables|Default|GetisFocused?)
              (Rendering|SetCustomDepthStencilValue _mesh 2)
              (else
                (Rendering|SetCustomDepthStencilValue _mesh 1)))))
        (else
          (goto _label))))))

(fn BoolCheck
  (bind _asfirst_person_character (Utilities|Casting|CastToFirstPersonCharacter (Game|GetPlayerCharacter 0)))
  (return (Variables|/Game/FirstPersonBP/Blueprints/FirstPersonCharacter.FirstPersonCharacter_C|GetPlayer%20Interactin%20with%20Maniqui _asfirst_person_character)))