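; Interactable object the first-person player picks up to inspect in front of the camera and puts back, with an empty Interact hook.
; Tick enables input only while its Interactable state is activated and either focused or inspected.
; Inspect toggles a timeline that lerps the actor between its initial transform and the inspection point, animating the HUD controls.
; Button icons follow keyboard or gamepad, rechecked during inspection via GameInstance flags.
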(event Custom|Set_Initial_grab%20spot)

(event Custom|Inspection
  (if (Variables|/Game/JuegoX/Blueprints/Objects/Interactable.Interactable_C|GetisInspectingIt (Variables|Default|GetInteractable))
    (CallFunction|EndInspection)
    (else
      (Utilities|FlowControl|Sequence
        (:then_0
          (Audio|PlaySound2D (Variables|Default|GetSound) 1.0 1.0 0.0 0 0))
        (:then_1
          (CallFunction|BeginInspection))))))

(event Custom|EndInspection
  ;[1 1 1] lo de la E
  (if (Variables|Default|GetableToFadeE)
    _
    (else
      (Variables|Default|SetableToFadeE true)))
  (Variables|/Game/JuegoX/Blueprints/Objects/Interactable.Interactable_C|SetisInspectingIt (Variables|Default|GetInteractable) false)
  (Variables|/Game/FirstPersonBP/Blueprints/FirstPersonCharacter.FirstPersonCharacter_C|SetplayerInspectingObject (Variables|Default|Getplayer) false)
  (CallFunction|HideControls)
  (bind _move_object (Timeline|inpection%20Timeline Reverse)
    (:Update
      (CallFunction|UpdateLocation _move_object))
    (:Finished
      (if (Variables|Default|GetableToFadeE) ; E appears when the animation finishes
        (Variables|/Game/JuegoX/Blueprints/Objects/Interactable.Interactable_C|SetfadeE (Variables|Default|GetInteractable) true)
        (Variables|/Game/FirstPersonBP/Blueprints/FirstPersonCharacter.FirstPersonCharacter_C|SetplayerInspectingObject (Variables|Default|Getplayer) false)))))

(event Custom|BeginInspection
  (Utilities|FlowControl|Sequence
    (:then_0
      (CallFunction|ShowControls))
    (:then_1
      (CallFunction|InspectionView)
      (Variables|/Game/JuegoX/Blueprints/Objects/Interactable.Interactable_C|SetisInspectingIt (Variables|Default|GetInteractable) true)
      (Variables|/Game/FirstPersonBP/Blueprints/FirstPersonCharacter.FirstPersonCharacter_C|SetplayerInspectingObject (Variables|Default|Getplayer) true)
      ;[1 1 1] lo de la E
      (Variables|Default|SetableToFadeE false)
      (Variables|/Game/JuegoX/Blueprints/Objects/Interactable.Interactable_C|SetfadeE (Variables|Default|GetInteractable) false)
      (CallFunction|SetInitialGrabSpot)
      (bind _move_object (Timeline|inpection%20Timeline Play)
        (:Update
          (CallFunction|UpdateLocation _move_object))
        (:Finished
          (if (Variables|Default|GetableToFadeE) ; E appears when the animation finishes
            (Variables|/Game/JuegoX/Blueprints/Objects/Interactable.Interactable_C|SetfadeE (Variables|Default|GetInteractable) true)
            (Variables|/Game/FirstPersonBP/Blueprints/FirstPersonCharacter.FirstPersonCharacter_C|SetplayerInspectingObject (Variables|Default|Getplayer) false)))))))

(event EventBeginPlay
  (Variables|/Game/JuegoX/Blueprints/Objects/Interactable.Interactable_C|SetfadeE (Variables|Default|GetInteractable) true)
  (bind _returnvalue (Actor|GetActorOfClass "/Game/FirstPersonBP/Blueprints/FirstPersonCharacter.FirstPersonCharacter_C"))
  (bind _output_get (Variables|Default|Setplayer _returnvalue))
  (Variables|/Game/JuegoX/Blueprints/Objects/Interactable.Interactable_C|Setplayer (Variables|Default|GetInteractable) _output_get)
  (bind _asmy_game_instance (Utilities|Casting|CastToMyGameInstance (Game|GetGameInstance)))
  (Variables|Default|SetGameInstance _asmy_game_instance)
  (Utilities|FlowControl|Sequence
    (:then_0
      (if (Variables|/Game/JuegoX/Blueprints/MyGameInstance.MyGameInstance_C|GetusingGamepad? (Variables|Default|GetGameInstance))
        (Variables|Default|SetTexture_E "/Game/JuegoX/UI/Sprites/Gamepad/redondaizquierda.redondaizquierda")
        (Variables|Default|SetTexture_LClick "/Game/JuegoX/UI/Sprites/Gamepad/redondabajo.redondabajo")
        (Variables|Default|SetTexture_RClick "/Game/JuegoX/UI/Sprites/Gamepad/redondaarriba.redondaarriba")
        (else
          (Variables|Default|SetTexture_E "/Game/JuegoX/UI/Sprites/Keyboard/E.E")
          (Variables|Default|SetTexture_LClick "/Game/JuegoX/UI/Sprites/Keyboard/botonizquierda.botonizquierda")
          (Variables|Default|SetTexture_RClick "/Game/JuegoX/UI/Sprites/Keyboard/botonderecho.botonderecho"))))
    (:then_1
      (CallFunction|UpdateIcons)
      (Variables|/Game/JuegoX/Blueprints/Objects/Interactable.Interactable_C|SetinitialRot (Variables|Default|GetInteractable) (Transformation|GetActorRotation))
      (Variables|/Game/JuegoX/Blueprints/Objects/Interactable.Interactable_C|SetinitialPos (Variables|Default|GetInteractable) (Transformation|GetActorLocation)))))

(event EventTick
  (params (DeltaSeconds :type Float%20%28single-precision%29))
  (bind _returnvalue (Game|GetPlayerController 0))
  (if (Variables|/Game/JuegoX/Blueprints/Objects/Interactable.Interactable_C|GetinteractionActivated (Variables|Default|GetInteractable))
    (if (Variables|/Game/JuegoX/Blueprints/Objects/Interactable.Interactable_C|GetisInspectingIt (Variables|Default|GetInteractable))
      (CallFunction|CheckGamepatInput)
      (Input|EnableInput _returnvalue :!label _label)
      (elif (Variables|/Game/JuegoX/Blueprints/Objects/Interactable.Interactable_C|GetisFocused? (Variables|Default|GetInteractable))
        (goto _label)
        (else
          (Input|DisableInput _returnvalue :!label _label_2))))
    (else
      (goto _label_2))))

(event Input|ActionEvents|InputActionInteract
  (params (Key :type Key%20Structure :default "None"))
  (:Pressed
    (if (Variables|/Game/JuegoX/Blueprints/Objects/Interactable.Interactable_C|GetisInspectingIt (Variables|Default|GetInteractable))
      (CallFunction|Interact) ; Aqui esta empty pq no tiene interaccion
    )))

(event Input|ActionEvents|InputActionInspect
  (params (Key :type Key%20Structure :default "None"))
  (:Pressed
    (CallFunction|Inspection)))

(event Input|KeyboardEvents|Q
  (params (Key :type Key%20Structure :default "None"))
  (:Pressed
    (if (Variables|/Game/JuegoX/Blueprints/Objects/Interactable.Interactable_C|GetisInspectingIt (Variables|Default|GetInteractable))
      _)))

(fn ConstructionScript
  (Variables|Default|SetSound 0)
  (Variables|/Game/JuegoX/Blueprints/Objects/Interactable.Interactable_C|SetMesh (Variables|Default|GetInteractable) (Variables|Default|GetMesh))
  (Variables|/Game/JuegoX/Blueprints/Objects/Interactable.Interactable_C|SetBillboard (Variables|Default|GetInteractable) (Variables|Default|GetBillboard))
  (Variables|Default|SetinspectionDistance 4e+01)
  (Variables|/Game/JuegoX/Blueprints/Objects/Interactable.Interactable_C|SetAperture_Focus (Variables|Default|GetInteractable) 1.0)
  (Variables|Default|SetFMOD_Sound 0))

(fn ShowControls
  (if (Utilities|IsValid (Variables|/Game/FirstPersonBP/Blueprints/FirstPersonCharacter.FirstPersonCharacter_C|GetHUD (Variables|Default|Getplayer)))
    _
    (else
      (bind _returnvalue (UserInterface|CreateWidget "/Game/JuegoX/UI/HUD/WB_HUD.WB_HUD_C" (Game|GetPlayerController 0)))
      (Variables|/Game/FirstPersonBP/Blueprints/FirstPersonCharacter.FirstPersonCharacter_C|SetHUD (Variables|Default|Getplayer) _returnvalue)))
  (CallFunction|SetVariables)
  (if (UserInterface|Viewport|IsinViewport (Variables|/Game/FirstPersonBP/Blueprints/FirstPersonCharacter.FirstPersonCharacter_C|GetHUD (Variables|Default|Getplayer)))
    _
    (else
      (UserInterface|Viewport|AddtoViewport (Variables|/Game/FirstPersonBP/Blueprints/FirstPersonCharacter.FirstPersonCharacter_C|GetHUD (Variables|Default|Getplayer)) 0)))
  (Class|UserWidget|PlayAnimationForward (Variables|/Game/FirstPersonBP/Blueprints/FirstPersonCharacter.FirstPersonCharacter_C|GetHUD (Variables|Default|Getplayer)) (Variables|Default|Getwidget_Anim) 6.0))

(fn HideControls
  (Class|UserWidget|PlayAnimationReverse (Variables|/Game/FirstPersonBP/Blueprints/FirstPersonCharacter.FirstPersonCharacter_C|GetHUD (Variables|Default|Getplayer)) (Variables|Default|Getwidget_Anim) 6.0))

(fn Interact)

(fn UpdateLocation
  (params (timeline%20Value :type Float%20%28single-precision%29))
  (bind _interactable (Variables|Default|GetInteractable))
  (Transformation|SetActorLocationAndRotation (Math|Vector|Lerp(Vector) (Variables|/Game/JuegoX/Blueprints/Objects/Interactable.Interactable_C|GetinitialPos _interactable) (Variables|/Game/JuegoX/Blueprints/Objects/Interactable.Interactable_C|GetinspectionPoint _interactable) timeline%20Value) (Math|Rotator|Lerp(Rotator) (Variables|/Game/JuegoX/Blueprints/Objects/Interactable.Interactable_C|GetinitialRot _interactable) (Transformation|GetActorRotation) timeline%20Value true) true))

(fn InspectionView
  (bind _player (Variables|Default|Getplayer))
  (bind _firstpersoncamera (Variables|/Game/FirstPersonBP/Blueprints/FirstPersonCharacter.FirstPersonCharacter_C|GetFirstPersonCamera _player))
  (Variables|/Game/JuegoX/Blueprints/Objects/Interactable.Interactable_C|SetinspectionPoint (Variables|Default|GetInteractable) (+ (Transformation|GetWorldLocation _firstpersoncamera) (* (Math|Vector|GetForwardVector (Transformation|GetWorldRotation _firstpersoncamera)) (Variables|Default|GetinspectionDistance)))))

(fn SetVariables
  (Appearance|SetBrushfromTexture (Variables|/Game/JuegoX/UI/HUD/WB_HUD.WB_HUD_C|GetE_One (Variables|/Game/FirstPersonBP/Blueprints/FirstPersonCharacter.FirstPersonCharacter_C|GetHUD (Variables|Default|Getplayer))) (Variables|Default|GetTexture_E) false)
  (Rendering|Components|TextRender|SetText (Variables|/Game/JuegoX/UI/HUD/WB_HUD.WB_HUD_C|GetAction_One (Variables|/Game/FirstPersonBP/Blueprints/FirstPersonCharacter.FirstPersonCharacter_C|GetHUD (Variables|Default|Getplayer))) "to drop")
  (Variables|Default|Setwidget_Anim (Variables|/Game/JuegoX/UI/HUD/WB_HUD.WB_HUD_C|GetControls_1_Anim (Variables|/Game/FirstPersonBP/Blueprints/FirstPersonCharacter.FirstPersonCharacter_C|GetHUD (Variables|Default|Getplayer)))))

(fn UpdateIcons
  (if (Utilities|IsValid (Variables|/Game/FirstPersonBP/Blueprints/FirstPersonCharacter.FirstPersonCharacter_C|GetHUD (Variables|Default|Getplayer)))
    (Utilities|FlowControl|Sequence
      (:then_0
        (Appearance|SetBrushfromTexture (Variables|/Game/JuegoX/UI/HUD/WB_HUD.WB_HUD_C|GetE_One (Variables|/Game/FirstPersonBP/Blueprints/FirstPersonCharacter.FirstPersonCharacter_C|GetHUD (Variables|Default|Getplayer))) (Variables|Default|GetTexture_E) false))
      (:then_1
        (Appearance|SetBrushfromTexture (Variables|/Game/JuegoX/UI/HUD/WB_HUD.WB_HUD_C|GetE_Two (Variables|/Game/FirstPersonBP/Blueprints/FirstPersonCharacter.FirstPersonCharacter_C|GetHUD (Variables|Default|Getplayer))) (Variables|Default|GetTexture_E) false)
        (Appearance|SetBrushfromTexture (Variables|/Game/JuegoX/UI/HUD/WB_HUD.WB_HUD_C|GetLClick_Two (Variables|/Game/FirstPersonBP/Blueprints/FirstPersonCharacter.FirstPersonCharacter_C|GetHUD (Variables|Default|Getplayer))) (Variables|Default|GetTexture_LClick) false))
      (:then_2
        (Appearance|SetBrushfromTexture (Variables|/Game/JuegoX/UI/HUD/WB_HUD.WB_HUD_C|GetE_Three (Variables|/Game/FirstPersonBP/Blueprints/FirstPersonCharacter.FirstPersonCharacter_C|GetHUD (Variables|Default|Getplayer))) (Variables|Default|GetTexture_E) false)
        (Appearance|SetBrushfromTexture (Variables|/Game/JuegoX/UI/HUD/WB_HUD.WB_HUD_C|GetLClick_Three (Variables|/Game/FirstPersonBP/Blueprints/FirstPersonCharacter.FirstPersonCharacter_C|GetHUD (Variables|Default|Getplayer))) (Variables|Default|GetTexture_LClick) false)
        (Appearance|SetBrushfromTexture (Variables|/Game/JuegoX/UI/HUD/WB_HUD.WB_HUD_C|GetRClick_Three (Variables|/Game/FirstPersonBP/Blueprints/FirstPersonCharacter.FirstPersonCharacter_C|GetHUD (Variables|Default|Getplayer))) (Variables|Default|GetTexture_RClick) false))
      (:then_3
        (Appearance|SetBrushfromTexture (Variables|/Game/JuegoX/UI/HUD/WB_HUD.WB_HUD_C|GetLeft_Click (Variables|/Game/FirstPersonBP/Blueprints/FirstPersonCharacter.FirstPersonCharacter_C|GetHUD (Variables|Default|Getplayer))) (Variables|Default|GetTexture_LClick) false)
        (Appearance|SetBrushfromTexture (Variables|/Game/JuegoX/UI/HUD/WB_HUD.WB_HUD_C|GetRightClick (Variables|/Game/FirstPersonBP/Blueprints/FirstPersonCharacter.FirstPersonCharacter_C|GetHUD (Variables|Default|Getplayer))) (Variables|Default|GetTexture_RClick) false)
        (Appearance|SetBrushfromTexture (Variables|/Game/JuegoX/UI/HUD/WB_HUD.WB_HUD_C|GetQE (Variables|/Game/FirstPersonBP/Blueprints/FirstPersonCharacter.FirstPersonCharacter_C|GetHUD (Variables|Default|Getplayer))) (Variables|Default|GetTexture_Roll) false)
        (Appearance|SetBrushfromTexture (Variables|/Game/JuegoX/UI/HUD/WB_HUD.WB_HUD_C|GetMouse (Variables|/Game/FirstPersonBP/Blueprints/FirstPersonCharacter.FirstPersonCharacter_C|GetHUD (Variables|Default|Getplayer))) (Variables|Default|GetTexture_Mouse) false)))))

(fn CheckGamepatInput
  (if (Variables|/Game/JuegoX/Blueprints/MyGameInstance.MyGameInstance_C|GetcontrolChanged? (Variables|Default|GetGameInstance))
    (Utilities|FlowControl|Sequence
      (:then_0
        (if (Variables|/Game/JuegoX/Blueprints/MyGameInstance.MyGameInstance_C|GetusingGamepad? (Variables|Default|GetGameInstance))
          (Variables|Default|SetTexture_E "/Game/JuegoX/UI/Sprites/Gamepad/redondaizquierda.redondaizquierda")
          (Variables|Default|SetTexture_LClick "/Game/JuegoX/UI/Sprites/Gamepad/redondabajo.redondabajo")
          (Variables|Default|SetTexture_RClick "/Game/JuegoX/UI/Sprites/Gamepad/redondaarriba.redondaarriba")
          (Variables|Default|SetTexture_Roll "/Game/JuegoX/UI/Sprites/Gamepad/JoystickRHorizontal.JoystickRHorizontal")
          (Variables|Default|SetTexture_Mouse "/Game/JuegoX/UI/Sprites/Gamepad/joystickLVertical.joystickLVertical")
          (else
            (Variables|Default|SetTexture_E "/Game/JuegoX/UI/Sprites/Keyboard/E.E")
            (Variables|Default|SetTexture_LClick "/Game/JuegoX/UI/Sprites/Keyboard/botonizquierda.botonizquierda")
            (Variables|Default|SetTexture_RClick "/Game/JuegoX/UI/Sprites/Keyboard/botonderecho.botonderecho")
            (Variables|Default|SetTexture_Roll "/Game/JuegoX/UI/Sprites/Keyboard/QE.QE")
            (Variables|Default|SetTexture_Mouse "/Game/JuegoX/UI/Sprites/Keyboard/moverRatonAdelanteatras.moverRatonAdelanteatras"))))
      (:then_1
        (CallFunction|UpdateIcons))
      (:then_2
        (Variables|/Game/JuegoX/Blueprints/MyGameInstance.MyGameInstance_C|SetcontrolChanged? (Variables|Default|GetGameInstance) false))
      (:then_3
        (return)))
    (else
      (return))))