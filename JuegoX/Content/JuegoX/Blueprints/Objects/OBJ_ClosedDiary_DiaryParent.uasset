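; Closed diary parent actor that the player picks up to read at an armchair (Sillon), configuring its Interactuable component as a diary.
; Tick enables input only while the active diary is focused or being inspected.
; Inspect runs a timeline moving it to the chair's book point, then shows control prompts and swaps itself for a spawned opened diary tilted along the chair's direction.
; Interact is an empty stub.
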(event Custom|Inspect
  (bind _interactuable (Variables|Default|GetInteractuable))
  (bind _interactuable_2 (Variables|Default|GetInteractuable))
  (if (Variables|/Game/JuegoX/Blueprints/Objects/Interactable.Interactable_C|GetinteractionActivated (Variables|Default|GetInteractuable))
    (if (not (Variables|/Game/JuegoX/Blueprints/Objects/Interactable.Interactable_C|GetisInspectingIt (Variables|Default|GetInteractuable)))
      (Utilities|FlowControl|Sequence
        (:then_0
          (Audio|PlaySound2D (Variables|Default|Getsound) 1.0 1.0 0.0 0 0))
        (:then_1
          (Default|HideControls (Variables|DondeSeGuarda|GetSillon)))
        (:then_2
          (Variables|/Game/JuegoX/Blueprints/Objects/Interactable.Interactable_C|SetinspectionPoint _interactuable (Transformation|GetWorldLocation (Variables|/Game/JuegoX/Blueprints/Objects/OBJ_Armchair.OBJ_Armchair_C|GetBook (Variables|DondeSeGuarda|GetSillon))))
          (Variables|/Game/JuegoX/Blueprints/Objects/Interactable.Interactable_C|SetisInspectingIt _interactuable true)
          (bind _move_object (Timeline|Inspect_Timeline Play)
            (:Update
              (Transformation|SetActorLocationAndRotation (Math|Vector|Lerp(Vector) (Variables|/Game/JuegoX/Blueprints/Objects/Interactable.Interactable_C|GetinitialPos _interactuable_2) (Variables|/Game/JuegoX/Blueprints/Objects/Interactable.Interactable_C|GetinspectionPoint _interactuable_2) _move_object) (Math|Rotator|Lerp(Rotator) (Variables|/Game/JuegoX/Blueprints/Objects/Interactable.Interactable_C|GetinitialRot _interactuable_2) (Transformation|GetActorRotation) _move_object)))
            (:Finished
              (CallFunction|ShowControls)
              (CallFunction|OpenBook))))))))

(event EventTick
  (params (DeltaSeconds :type Float%20%28single-precision%29))
  (bind _returnvalue (Game|GetPlayerController 0))
  (if (Variables|/Game/JuegoX/Blueprints/Objects/Interactable.Interactable_C|GetinteractionActivated (Variables|Default|GetInteractuable))
    (if (Variables|/Game/JuegoX/Blueprints/Objects/Interactable.Interactable_C|GetisInspectingIt (Variables|Default|GetInteractuable))
      (Input|EnableInput _returnvalue :!label _label)
      (elif (Variables|/Game/JuegoX/Blueprints/Objects/Interactable.Interactable_C|GetisFocused? (Variables|Default|GetInteractuable))
        (goto _label)
        (else
          (Input|DisableInput _returnvalue))))))

(event EventBeginPlay
  (bind _asfirst_person_character (Utilities|Casting|CastToFirstPersonCharacter (Game|GetPlayerCharacter 0)))
  (bind _output_get (Variables|Default|Setplayer _asfirst_person_character))
  (Variables|/Game/JuegoX/Blueprints/Objects/Interactable.Interactable_C|Setplayer (Variables|Default|GetInteractuable) _output_get)
  (Variables|/Game/JuegoX/Blueprints/Objects/Interactable.Interactable_C|SetMesh (Variables|Default|GetInteractuable) (Variables|Default|GetMesh))
  (Variables|/Game/JuegoX/Blueprints/Objects/Interactable.Interactable_C|SetText (Variables|Default|GetInteractuable) (Variables|Default|GetTextRender))
  (Variables|/Game/JuegoX/Blueprints/Objects/Interactable.Interactable_C|Setis%20a%20diary? (Variables|Default|GetInteractuable) true))

(event Input|ActionEvents|InputActionInteract
  (params (Key :type Key%20Structure :default "None"))
  (:Pressed
    (CallFunction|Interact)))

(event Input|ActionEvents|InputActionInspect
  (params (Key :type Key%20Structure :default "None"))
  (:Pressed
    (CallFunction|Inspect)))

(fn ConstructionScript
  (Variables|Default|Setsound 0))

(fn OpenBook
  (Variables|/Game/JuegoX/Blueprints/Objects/Interactable.Interactable_C|SetisInspectingIt (Variables|Default|GetInteractuable) false)
  (bind _returnvalue (Game|SpawnActorfromClass "/Game/JuegoX/Blueprints/Objects/OBJ_OpenedDiary_DiaryChild.OBJ_OpenedDiary_DiaryChild_C" (Math|Transform|MakeTransform (Transformation|GetActorLocation) (Math|Rotator|MakeRotator (.Roll (Math|Rotator|BreakRotator (Math|Rotator|FindLookatRotation (Transformation|GetActorLocation) (Transformation|GetActorLocation (Variables|DondeSeGuarda|GetSillon))))) -3e+01 (.Yaw (Math|Rotator|BreakRotator (Math|Rotator|FindLookatRotation (Transformation|GetActorLocation) (Transformation|GetActorLocation (Variables|DondeSeGuarda|GetSillon)))))) (LocalVariables|GetdiaryScale)) "AlwaysSpawn" 0 0))
  (Variables|Default|SetopenedDiary _returnvalue)
  (Variables|/Game/JuegoX/Blueprints/Objects/OBJ_OpenedDiary_DiaryChild.OBJ_OpenedDiary_DiaryChild_C|SetinitialPoint (Variables|Default|GetopenedDiary) (Variables|/Game/JuegoX/Blueprints/Objects/Interactable.Interactable_C|GetinitialPos (Variables|Default|GetInteractuable)))
  (Variables|/Game/JuegoX/Blueprints/Objects/OBJ_OpenedDiary_DiaryChild.OBJ_OpenedDiary_DiaryChild_C|SetinitialRot (Variables|Default|GetopenedDiary) (Variables|/Game/JuegoX/Blueprints/Objects/Interactable.Interactable_C|GetinitialRot (Variables|Default|GetInteractuable)))
  (Variables|/Game/JuegoX/Blueprints/Objects/OBJ_OpenedDiary_DiaryChild.OBJ_OpenedDiary_DiaryChild_C|SetSillon (Variables|Default|GetopenedDiary) (Variables|DondeSeGuarda|GetSillon))
  (Variables|/Game/JuegoX/Blueprints/Objects/Interactable.Interactable_C|SetinteractionActivated (Variables|/Game/JuegoX/Blueprints/Objects/OBJ_Armchair.OBJ_Armchair_C|GetInteractuable (Variables|DondeSeGuarda|GetSillon)) false)
  (Variables|/Game/FirstPersonBP/Blueprints/FirstPersonCharacter.FirstPersonCharacter_C|SetplayerIsReading? (Variables|Default|Getplayer) true)
  (Actor|DestroyActor))

(fn ShowControls
  (if (Utilities|IsValid (Variables|/Game/FirstPersonBP/Blueprints/FirstPersonCharacter.FirstPersonCharacter_C|GetInventoryHUD (Variables|Default|Getplayer)))
    _
    (else
      (bind _returnvalue (UserInterface|CreateWidget "/Game/JuegoX/UI/HUD/WB_Inventory.WB_Inventory_C" (Game|GetPlayerController 0)))
      (Variables|/Game/FirstPersonBP/Blueprints/FirstPersonCharacter.FirstPersonCharacter_C|SetInventoryHUD (Variables|Default|Getplayer) _returnvalue)))
  (CallFunction|SetVariables)
  (if (UserInterface|Viewport|IsinViewport (Variables|/Game/FirstPersonBP/Blueprints/FirstPersonCharacter.FirstPersonCharacter_C|GetInventoryHUD (Variables|Default|Getplayer)))
    _
    (else
      (UserInterface|Viewport|AddtoViewport (Variables|/Game/FirstPersonBP/Blueprints/FirstPersonCharacter.FirstPersonCharacter_C|GetInventoryHUD (Variables|Default|Getplayer)) 0)))
  (Class|UserWidget|PlayAnimationForward (Variables|/Game/FirstPersonBP/Blueprints/FirstPersonCharacter.FirstPersonCharacter_C|GetInventoryHUD (Variables|Default|Getplayer)) (Variables|Default|GetWidget_Anim) 3.0))

(fn HideControls
  (UserInterface|Animation|PlayAnimation (Variables|/Game/FirstPersonBP/Blueprints/FirstPersonCharacter.FirstPersonCharacter_C|GetInventoryHUD (Variables|Default|Getplayer)) (Variables|Default|GetWidget_Anim) 0.0 1 "Reverse" 6.0))

(fn SetVariables
  (bind _player (Variables|Default|Getplayer))
  (bind _inventoryhud (Variables|/Game/FirstPersonBP/Blueprints/FirstPersonCharacter.FirstPersonCharacter_C|GetInventoryHUD _player))
  (Rendering|Components|TextRender|SetText (Variables|/Game/JuegoX/UI/HUD/WB_Inventory.WB_Inventory_C|GetT_Drop _inventoryhud) "to drop")
  (Rendering|Components|TextRender|SetText (Variables|/Game/JuegoX/UI/HUD/WB_Inventory.WB_Inventory_C|GetT_Action _inventoryhud) "to read")
  (Variables|Default|SetWidget_Anim (Variables|/Game/JuegoX/UI/HUD/WB_Inventory.WB_Inventory_C|GetControls_2_Anim _inventoryhud)))

(fn Interact)