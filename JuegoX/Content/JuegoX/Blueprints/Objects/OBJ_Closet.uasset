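; OBJ_Closet is an interactable closet that the player can open and close with the Inspect input while focusing on it.
; Its Interactable component receives the player, mesh and text render, and is flagged as a non-inspectable object.
; Tick enables or disables the actor's input according to focus.
; Inspect plays a sound and runs the Anim sequence forward or in reverse based on IsOpen, which this graph never sets.
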(event EventTick
  (params (DeltaSeconds :type Float%20%28single-precision%29))
  (bind _returnvalue (Game|GetPlayerController 0))
  (if (Variables|/Game/JuegoX/Blueprints/Objects/Interactable.Interactable_C|GetisFocused? (Variables|Default|GetInteractable))
    (Input|EnableInput _returnvalue)
    (else
      (Input|DisableInput _returnvalue))))

(event EventBeginPlay
  (bind _asfirst_person_character (Utilities|Casting|CastToFirstPersonCharacter (Game|GetPlayerCharacter 0)))
  (bind _output_get (Variables|Default|Setplayer _asfirst_person_character))
  (Variables|/Game/JuegoX/Blueprints/Objects/Interactable.Interactable_C|Setplayer (Variables|Default|GetInteractable) _output_get))

(event Collision|EventActorBeginOverlap
  (params (OtherActor :type Actor%20Object%20Reference)))

(event Input|ActionEvents|InputActionInspect
  (params (Key :type Key%20Structure :default "None"))
  (bind _anim (Variables|Default|GetAnim))
  (bind _sequenceplayer (Variables|/Script/ActorSequence.ActorSequenceComponent|GetSequencePlayer _anim))
  (:Pressed
    (if (Variables|/Game/JuegoX/Blueprints/Objects/Interactable.Interactable_C|GetisFocused? (Variables|Default|GetInteractable))
      (if (Variables|Default|GetisOpen?)
        (Audio|PlaySound2D "/Game/Soniditos/392770__danialarcon0698__abre-cajon.392770__danialarcon0698__abre-cajon" 1.0 1.0 0.0 0 0)
        (Class|MovieSceneSequencePlayer|PlayReverse _sequenceplayer)
        (else
          (Audio|PlaySound2D "/Game/Soniditos/237379__squareal__cutlery-drawer-closing-01.237379__squareal__cutlery-drawer-closing-01" 1.0 1.0 0.0 0 0)
          (Sequencer|Player|Play _sequenceplayer :!class /Script/MovieScene.MovieSceneSequencePlayer))))))

(fn ConstructionScript
  (bind _interactable (Variables|Default|GetInteractable))
  (Variables|/Game/JuegoX/Blueprints/Objects/Interactable.Interactable_C|SetMesh (Variables|Default|GetInteractable) (Variables|Character|GetMesh))
  (Variables|/Game/JuegoX/Blueprints/Objects/Interactable.Interactable_C|SetText _interactable (Variables|Default|GetTextRender))
  (Variables|/Game/JuegoX/Blueprints/Objects/Interactable.Interactable_C|Setis%20a%20nonInspectionable%20Object? _interactable true))