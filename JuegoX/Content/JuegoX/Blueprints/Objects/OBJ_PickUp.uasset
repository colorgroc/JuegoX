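; Collectible object that the player inspects and picks up, setting the GameInstance key flag and showing it in a four-slot HUD inventory.
; When saved inside another object, it attaches to that container and drives an outline on a duplicate mesh by focus, inspection and distance.
; Tick also toggles input and swaps gamepad or keyboard prompt icons.
; Interacting hides the mesh and animates its slot; HideInventory reverses this and shifts remaining icons.
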(event Custom|End_Of_interaction
  (CallFunction|ShowInventory))

(event EventTick
  (params (DeltaSeconds :type Float%20%28single-precision%29))
  (bind _returnvalue (Game|GetPlayerController 0))
  (bind _materialhighlight (Variables|Default|GetmaterialHighlight))
  (bind _materialhighlight_2 (Variables|Default|GetmaterialHighlight))
  (if (Variables|Savedinaclosed|GetitsSaved?)
    (if (Variables|/Game/JuegoX/Blueprints/Objects/Interactable.Interactable_C|GetinteractionActivated (Variables|Default|GetInteractable))
      (if (Variables|/Game/JuegoX/Blueprints/Objects/Interactable.Interactable_C|GetisInspectingIt (Variables|Default|GetInteractable))
        (Rendering|Material|SetScalarParameterValue _materialhighlight_2 "Scale" 0.0 :!class /Script/Engine.MaterialInstanceDynamic)
        (if (Variables|/Game/JuegoX/Blueprints/MyGameInstance.MyGameInstance_C|GetcontrolChanged? (Variables|Default|GetGameInstance))
          (Utilities|FlowControl|Sequence
            (:then_0
              (if (Variables|/Game/JuegoX/Blueprints/MyGameInstance.MyGameInstance_C|GetusingGamepad? (Variables|Default|GetGameInstance))
                (Variables|Default|SetTexture_E "/Game/JuegoX/UI/Sprites/Gamepad/redondaizquierda.redondaizquierda")
                (Variables|Default|SetTexture_LClick "/Game/JuegoX/UI/Sprites/Gamepad/redondabajo.redondabajo")
                (Variables|Default|SetTexture_RClick "/Game/JuegoX/UI/Sprites/Gamepad/redondaarriba.redondaarriba")
                (Variables|Default|SetTexture_Roll 0)
                (Variables|Default|SetTexture_Mouse 0)
                (else
                  (Variables|Default|SetTexture_E "/Game/JuegoX/UI/Sprites/Keyboard/E.E")
                  (Variables|Default|SetTexture_LClick "/Game/JuegoX/UI/Sprites/Keyboard/botonizquierda.botonizquierda")
                  (Variables|Default|SetTexture_RClick "/Game/JuegoX/UI/Sprites/Keyboard/botonderecho.botonderecho")
                  (Variables|Default|SetTexture_Roll 0)
                  (Variables|Default|SetTexture_Mouse 0))))
            (:then_1
              (CallFunction|UpdateIcons))
            (:then_2
              (Variables|/Game/JuegoX/Blueprints/MyGameInstance.MyGameInstance_C|SetcontrolChanged? (Variables|Default|GetGameInstance) false))
            (:then_3
              (Input|EnableInput _returnvalue :!label _label)))
          (else
            (goto _label)))
        (elif (Variables|/Game/JuegoX/Blueprints/Objects/Interactable.Interactable_C|GetisFocused? (Variables|Default|GetInteractable))
          (Rendering|Material|SetScalarParameterValue _materialhighlight_2 "Scale" 0.5 :!class /Script/Engine.MaterialInstanceDynamic)
          (Rendering|Material|SetVectorParameterValue _materialhighlight_2 "Color" "(R=1.000000,G=0.000000,B=0.000000,A=1.000000)" :!class /Script/Engine.MaterialInstanceDynamic)
          (goto _label)
          (else
            (Input|DisableInput _returnvalue)
            (Math|Float|CompareFloat (Transformation|GetDistanceTo (Variables|Default|Getplayer)) (Variables|/Game/JuegoX/Blueprints/Objects/Interactable.Interactable_C|GetDistance%20to%20Glow (Variables|Default|GetInteractable))
              (:>
                (Rendering|Material|SetScalarParameterValue _materialhighlight "Scale" 0.0 :!class /Script/Engine.MaterialInstanceDynamic))
              (:==
                (Rendering|Material|SetScalarParameterValue _materialhighlight "Scale" 0.5 :!class /Script/Engine.MaterialInstanceDynamic :!label _label_2))
              (:<
                (goto _label_2)))
            (Rendering|Material|SetVectorParameterValue _materialhighlight "Color" "(R=1.000000,G=1.000000,B=1.000000,A=1.000000)" :!class /Script/Engine.MaterialInstanceDynamic))))
      (else
        (Input|DisableInput (Game|GetPlayerController 0))
        (Rendering|Material|SetScalarParameterValue (Variables|Default|GetmaterialHighlight) "Scale" 0.0 :!class /Script/Engine.MaterialInstanceDynamic)))
    (else
      (|CallParentFunction 0.0))))

(event EventSetVariables
  (bind _player (Variables|Default|Getplayer))
  (bind _hud (Variables|/Game/FirstPersonBP/Blueprints/FirstPersonCharacter.FirstPersonCharacter_C|GetHUD _player))
  (Appearance|SetBrushfromTexture (Variables|/Game/JuegoX/UI/HUD/WB_HUD.WB_HUD_C|GetE_Two (Variables|/Game/FirstPersonBP/Blueprints/FirstPersonCharacter.FirstPersonCharacter_C|GetHUD (Variables|Default|Getplayer))) (Variables|Default|GetTexture_E) false)
  (Appearance|SetBrushfromTexture (Variables|/Game/JuegoX/UI/HUD/WB_HUD.WB_HUD_C|GetLClick_Two (Variables|/Game/FirstPersonBP/Blueprints/FirstPersonCharacter.FirstPersonCharacter_C|GetHUD (Variables|Default|Getplayer))) (Variables|Default|GetTexture_LClick) false)
  (Rendering|Components|TextRender|SetText (Variables|/Game/JuegoX/UI/HUD/WB_HUD.WB_HUD_C|GetT_Drop _hud) "to drop")
  (Rendering|Components|TextRender|SetText (Variables|/Game/JuegoX/UI/HUD/WB_HUD.WB_HUD_C|GetT_Action _hud) "to collect")
  (Variables|Default|Setwidget_Anim (Variables|/Game/JuegoX/UI/HUD/WB_HUD.WB_HUD_C|GetControls_2_Anim _hud)))

(event EventInteract
  (CallFunction|HideControls)
  (CallFunction|GameInstanceControl false)
  (Variables|/Game/JuegoX/Blueprints/Objects/Interactable.Interactable_C|SetisInspectingIt (Variables|Default|GetInteractable) false)
  (Variables|/Game/FirstPersonBP/Blueprints/FirstPersonCharacter.FirstPersonCharacter_C|SetplayerInspectingObject (Variables|Default|Getplayer) false)
  (Rendering|SetVisibility (Variables|Character|GetMesh) false true)
  (Variables|/Game/JuegoX/Blueprints/Objects/Interactable.Interactable_C|SetinteractionActivated (Variables|Default|GetInteractable) false)
  (CallFunction|EndOfInteraction))

(event EventBeginPlay
  (bind _lugardondeestaguardada (Variables|Savedinaclosed|GetlugarDondeEstaGuardada))
  (|CallParentFunction)
  (if (Variables|Savedinaclosed|GetitsSaved?)
    (bind _returnvalue (Rendering|Material|CreateDynamicMaterialInstance (Variables|Default|GetDuplicate) 0 "/Game/JuegoX/Materials/Outline_ObjectsHided.Outline_ObjectsHided" "None" :!class /Script/Engine.PrimitiveComponent))
    (Variables|Default|SetmaterialHighlight _returnvalue)
    (Utilities|IsValid _lugardondeestaguardada
      (:Is%20Valid
        (Transformation|AttachComponentToComponent (Variables|/Game/JuegoX/Blueprints/Objects/Interactable_Static/Dressers/OBJ_Furniture.OBJ_Furniture_C|GetMesh _lugardondeestaguardada) "None" "KeepWorld" "KeepWorld" "KeepWorld" true)))))

(event EventSetInitialGrabSpot
  (if (Variables|Savedinaclosed|GetitsSaved?)
    (Variables|/Game/JuegoX/Blueprints/Objects/Interactable.Interactable_C|SetinitialRot (Variables|Default|GetInteractable) (Transformation|GetActorRotation))
    (Variables|/Game/JuegoX/Blueprints/Objects/Interactable.Interactable_C|SetinitialPos (Variables|Default|GetInteractable) (Transformation|GetActorLocation))))

(fn ConstructionScript
  (|CallParentFunction)
  (Variables|Default|SetSound 0)
  (if (Variables|Savedinaclosed|GetitsSaved?)
    (Utilities|IsValid (Variables|Default|GetDuplicate)
      (:Is%20Valid
        (Components|StaticMesh|SetStaticMesh (Variables|Default|GetDuplicate) (Variables|/Script/Engine.StaticMeshComponent|GetStaticMesh (Variables|Character|GetMesh)))))
    (else
      (Utilities|IsValid (Variables|Default|GetDuplicate)
        (:Is%20Valid
          (Components|DestroyComponent (Variables|Default|GetDuplicate)))))))

(fn DestroyActor
  (bind _player (Variables|Default|Getplayer))
  (bind _player_2 (Variables|Default|Getplayer))
  (bind _hud (Variables|/Game/FirstPersonBP/Blueprints/FirstPersonCharacter.FirstPersonCharacter_C|GetHUD _player))
  (bind _hud_2 (Variables|/Game/FirstPersonBP/Blueprints/FirstPersonCharacter.FirstPersonCharacter_C|GetHUD _player_2))
  (Class|UserWidget|PlayAnimationReverse _hud_2 (Variables|/Game/JuegoX/UI/HUD/WB_HUD.WB_HUD_C|GetControls_2_Anim _hud_2) 6.0)
  (Class|UserWidget|BindtoAnimationFinished _hud (Variables|/Game/JuegoX/UI/HUD/WB_HUD.WB_HUD_C|GetControls_2_Anim _hud) (EventDispatchers|CreateEvent :!event K2DestroyActor)))

(fn ShowInventory
  (bind _player (Variables|Default|Getplayer))
  (bind _gameinstance (Variables|Default|GetGameInstance))
  (bind _inventorycounter (Variables|/Game/JuegoX/Blueprints/MyGameInstance.MyGameInstance_C|GetInventoryCounter _gameinstance))
  (bind _hud (Variables|/Game/FirstPersonBP/Blueprints/FirstPersonCharacter.FirstPersonCharacter_C|GetHUD _player))
  (Math|Integer|IncrementInt _inventorycounter
    (:%20%20
      (Variables|Default|SetinventorySlot _inventorycounter)
      (switch int _inventorycounter
        (:1
          (LocalVariables|SetItem (Variables|/Game/JuegoX/UI/HUD/WB_HUD.WB_HUD_C|GetItem_1 _hud))
          (LocalVariables|SetAnim (Variables|/Game/JuegoX/UI/HUD/WB_HUD.WB_HUD_C|GetInventory_Anim_Item_1 _hud)))
        (:2
          (LocalVariables|SetItem (Variables|/Game/JuegoX/UI/HUD/WB_HUD.WB_HUD_C|GetItem_2 _hud))
          (LocalVariables|SetAnim (Variables|/Game/JuegoX/UI/HUD/WB_HUD.WB_HUD_C|GetInventory_Anim_Item_2 _hud)))
        (:3
          (LocalVariables|SetItem (Variables|/Game/JuegoX/UI/HUD/WB_HUD.WB_HUD_C|GetItem_3 _hud))
          (LocalVariables|SetAnim (Variables|/Game/JuegoX/UI/HUD/WB_HUD.WB_HUD_C|GetInventory_Anim_Item_3 _hud)))
        (:4
          (LocalVariables|SetItem (Variables|/Game/JuegoX/UI/HUD/WB_HUD.WB_HUD_C|GetItem_4 _hud))
          (LocalVariables|SetAnim (Variables|/Game/JuegoX/UI/HUD/WB_HUD.WB_HUD_C|GetInventory_Anim_Item_4 _hud))))
      (Appearance|SetBrushfromTexture (LocalVariables|GetItem) (Variables|Default|Gettexture) true)
      (if (UserInterface|Viewport|IsinViewport (Variables|/Game/FirstPersonBP/Blueprints/FirstPersonCharacter.FirstPersonCharacter_C|GetHUD (Variables|Default|Getplayer)))
        _
        (else
          (UserInterface|Viewport|AddtoViewport (Variables|/Game/FirstPersonBP/Blueprints/FirstPersonCharacter.FirstPersonCharacter_C|GetHUD (Variables|Default|Getplayer)) 0)))
      (Class|UserWidget|PlayAnimationForward (Variables|/Game/FirstPersonBP/Blueprints/FirstPersonCharacter.FirstPersonCharacter_C|GetHUD (Variables|Default|Getplayer)) (LocalVariables|GetAnim) 1.0))))

(fn GameInstanceControl
  (params (OUT :type Boolean))
  (if OUT
    (Variables|/Game/JuegoX/Blueprints/MyGameInstance.MyGameInstance_C|SetHas_Key? (Variables|Default|GetGameInstance) false)
    (Development|PrintString "no key")
    (else
      (Variables|/Game/JuegoX/Blueprints/MyGameInstance.MyGameInstance_C|SetHas_Key? (Variables|Default|GetGameInstance) true))))

(fn HideInventory
  (bind _player (Variables|Default|GetPlayer))
  (bind _gameinstance (Variables|Default|GetGameInstance))
  (bind _gameinstance_2 (Variables|Default|GetGameInstance))
  (bind _player_2 (Variables|Default|GetPlayer))
  (bind _inventorycounter (Variables|/Game/JuegoX/Blueprints/MyGameInstance.MyGameInstance_C|GetInventoryCounter _gameinstance_2))
  (bind _hud (Variables|/Game/FirstPersonBP/Blueprints/FirstPersonCharacter.FirstPersonCharacter_C|GetHUD _player))
  (bind _inventorycounter_2 (Variables|/Game/JuegoX/Blueprints/MyGameInstance.MyGameInstance_C|GetInventoryCounter _gameinstance))
  (bind _hud_2 (Variables|/Game/FirstPersonBP/Blueprints/FirstPersonCharacter.FirstPersonCharacter_C|GetHUD _player_2))
  (bind _grid (Variables|/Game/JuegoX/UI/HUD/WB_HUD.WB_HUD_C|GetGrid _hud_2))
  (switch int (Variables|Default|GetinventorySlot)
    (:1
      (LocalVariables|SetinvAnim (Variables|/Game/JuegoX/UI/HUD/WB_HUD.WB_HUD_C|GetInventory_Anim_Item_1 _hud)))
    (:2
      (LocalVariables|SetinvAnim (Variables|/Game/JuegoX/UI/HUD/WB_HUD.WB_HUD_C|GetInventory_Anim_Item_2 _hud)))
    (:3
      (LocalVariables|SetinvAnim (Variables|/Game/JuegoX/UI/HUD/WB_HUD.WB_HUD_C|GetInventory_Anim_Item_3 _hud)))
    (:4
      (LocalVariables|SetinvAnim (Variables|/Game/JuegoX/UI/HUD/WB_HUD.WB_HUD_C|GetInventory_Anim_Item_4 _hud))))
  (Class|UserWidget|PlayAnimationReverse (Variables|/Game/FirstPersonBP/Blueprints/FirstPersonCharacter.FirstPersonCharacter_C|GetHUD (Variables|Default|GetPlayer)) (LocalVariables|GetinvAnim) 1.0)
  (Math|Integer|DecrementInt _inventorycounter
    (:%20%20
      (if (not (<= _inventorycounter 0))
        (for _index (range (Utilities|Array|Length (Class|PanelWidget|GetAllChildren (Variables|/Game/JuegoX/UI/HUD/WB_HUD.WB_HUD_C|GetGrid (Variables|/Game/FirstPersonBP/Blueprints/FirstPersonCharacter.FirstPersonCharacter_C|GetHUD (Variables|Default|GetPlayer))))) _inventorycounter_2)
          (if (not (<= (- _index 1) _inventorycounter_2))
            (bind _asimage (Utilities|Casting|CastToImage (Class|PanelWidget|GetChildat _grid _index)))
            (Widget|SetRenderOpacity (Class|PanelWidget|GetChildat _grid _index) 0.0)
            (bind _asimage_2 (Utilities|Casting|CastToImage (Class|PanelWidget|GetChildat _grid (- _index 1))))
            (Class|Image|SetBrush _asimage_2 (Variables|/Script/UMG.Image|GetBrush _asimage))
            (Widget|SetRenderOpacity (Class|PanelWidget|GetChildat _grid (- _index 1)) 1.0)))))))