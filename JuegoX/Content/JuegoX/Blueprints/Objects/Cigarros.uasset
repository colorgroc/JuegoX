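; Cigarettes prop (Cigarros) that the first-person player can pick up to inspect and put back with the Inspect input.
; Tick enables input only while the Interactuable component is focused or inspected.
; Inspection sets player and component flags, shows HUD controls and lerps the actor to the player's view point by timeline, restoring the E prompt after it reverses.
; Uncalled custom events and disconnected nodes retain an older variant with Polaroid outline, scaling and tag-specific handling.
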(event Custom|CustomEvent_1
  (bind _interactuable (Variables|Default|GetInteractuable))
  (bind _init_scale (Variables|Default|Getinit%20scale))
  ;[1 1 1] memoria antes y despues
  ;;[1 1 1] lo de la E
  (if (Variables|Default|GetableToFadeE)
    _
    (else
      (Variables|Default|SetableToFadeE true)))
  (CallFunction|HideControls)
  (Variables|/Game/JuegoX/Blueprints/Objects/Interactable.Interactable_C|SetisInspectingIt (Variables|Default|GetInteractuable) false)
  (Variables|/Game/FirstPersonBP/Blueprints/FirstPersonCharacter.FirstPersonCharacter_C|SetplayerInspectingObject (Variables|Default|Getplayer) false)
  (bind _move_object (Timeline|Timeline_0 Reverse)
    (:Update
      (bind _output_get (Variables|Default|SetMovedObject _move_object))
      ;;[1 1 1] Si es una Polaroid
      (if (Actor|ActorHasTag "Polaroid")
        (Variables|Default|Setrotation "0, 0, 0") ; Rotacion pa que mire enfrente bien
        (Transformation|SetActorLocation (Math|Vector|Lerp(Vector) (Variables|/Game/JuegoX/Blueprints/Objects/Interactable.Interactable_C|GetinitialPos _interactuable) (Variables|/Game/JuegoX/Blueprints/Objects/Interactable.Interactable_C|GetinspectionPoint _interactuable) _output_get) false false)
        (Transformation|SetActorRotation (Math|Rotator|Lerp(Rotator) (Variables|/Game/JuegoX/Blueprints/Objects/Interactable.Interactable_C|GetinitialRot _interactuable) (Variables|Default|Getrotation) _output_get))
        (Transformation|SetActorScale3D (Math|Vector|Lerp(Vector) _init_scale (* _init_scale 2.0) _output_get))
        (else
          (Variables|Default|Setrotation (Transformation|GetActorRotation))
          (Transformation|SetActorLocationAndRotation (Math|Vector|Lerp(Vector) (Variables|/Game/JuegoX/Blueprints/Objects/Interactable.Interactable_C|GetinitialPos _interactuable) (Variables|/Game/JuegoX/Blueprints/Objects/Interactable.Interactable_C|GetinspectionPoint _interactuable) _output_get) (Math|Rotator|Lerp(Rotator) (Variables|/Game/JuegoX/Blueprints/Objects/Interactable.Interactable_C|GetinitialRot _interactuable) (Variables|Default|Getrotation) _output_get) true))))
    (:Finished
      ;;[1 1 1] la E aparece cuando acaba la animacion
      (if (Variables|Default|GetableToFadeE)
        (Variables|/Game/JuegoX/Blueprints/Objects/Interactable.Interactable_C|SetfadeE (Variables|Default|GetInteractuable) true)))))

(event Custom|Inspection
  (if (Variables|/Game/JuegoX/Blueprints/Objects/Interactable.Interactable_C|GetisInspectingIt (Variables|Default|GetInteractuable))
    (CallFunction|EndInspection)
    (bind _move_object (Timeline|Timeline_1 Reverse)
      (:Update
        (CallFunction|UpdateLocation _move_object))
      (:Finished
        (if (Variables|Default|GetableToFadeE) ; E appears when the animation finishes
          (Variables|/Game/JuegoX/Blueprints/Objects/Interactable.Interactable_C|SetfadeE (Variables|Default|GetInteractuable) true))))
    (else
      (Utilities|FlowControl|Sequence
        (:then_0
          (Variables|/Game/JuegoX/Blueprints/Objects/Interactable.Interactable_C|SetinspectionPoint (Variables|Default|GetInteractuable) (Transformation|GetWorldLocation (Variables|/Game/FirstPersonBP/Blueprints/FirstPersonCharacter.FirstPersonCharacter_C|GetInpectionView (Variables|Default|Getplayer)))))
        (:then_1
          (CallFunction|BeginInspection)
          (Timeline|Timeline_1 Play))))))

(event Custom|EndInspection
  ;[1 1 1] lo de la E
  (if (Variables|Default|GetableToFadeE)
    _
    (else
      (Variables|Default|SetableToFadeE true)))
  (CallFunction|HideControls)
  (Variables|/Game/JuegoX/Blueprints/Objects/Interactable.Interactable_C|SetisInspectingIt (Variables|Default|GetInteractuable) false)
  (Variables|/Game/FirstPersonBP/Blueprints/FirstPersonCharacter.FirstPersonCharacter_C|SetplayerInspectingObject (Variables|Default|Getplayer) false))

(event Custom|BeginInspection
  (Utilities|FlowControl|Sequence
    (:then_0
      (CallFunction|ShowControls))
    (:then_1
      (Variables|/Game/JuegoX/Blueprints/Objects/Interactable.Interactable_C|SetisInspectingIt (Variables|Default|GetInteractuable) true)
      (Variables|/Game/FirstPersonBP/Blueprints/FirstPersonCharacter.FirstPersonCharacter_C|SetplayerInspectingObject (Variables|Default|Getplayer) true)
      ;[1 1 1] lo de la E
      (Variables|Default|SetableToFadeE false)
      (Variables|/Game/JuegoX/Blueprints/Objects/Interactable.Interactable_C|SetfadeE (Variables|Default|GetInteractuable) false))))

(event Custom|CustomEvent_2
  (params (DeltaSeconds :type Float%20%28single-precision%29))
  (bind _returnvalue (Actor|ActorHasTag "Polaroid"))
  (bind _returnvalue_2 (Game|GetPlayerController 0))
  (bind _materialhighlight (Variables|Default|GetMaterialHighlight))
  (bind _materialhighlight_2 (Variables|Default|GetMaterialHighlight))
  ;[1 1 1] memoria antes y despues
  ;;[1 1 1] event tick
  (if (Variables|/Game/JuegoX/Blueprints/Objects/Interactable.Interactable_C|GetisInspectingIt (Variables|Default|GetInteractuable))
    (if _returnvalue
      (Rendering|Material|SetScalarParameterValue _materialhighlight_2 "Scale" 0.0 :!class /Script/Engine.MaterialInstanceDynamic))
    (Input|EnableInput _returnvalue_2 :!label _label)
    (elif (Variables|/Game/JuegoX/Blueprints/Objects/Interactable.Interactable_C|GetisFocused? (Variables|Default|GetInteractuable))
      (if _returnvalue
        (Rendering|Material|SetScalarParameterValue _materialhighlight_2 "Scale" 0.5 :!class /Script/Engine.MaterialInstanceDynamic)
        (Rendering|Material|SetVectorParameterValue _materialhighlight_2 "Color" "(R=1.000000,G=0.000000,B=0.000000,A=1.000000)" :!class /Script/Engine.MaterialInstanceDynamic)
        (goto _label)
        (else
          (goto _label)))
      (elif _returnvalue
        (Input|DisableInput _returnvalue_2)
        (Math|Float|CompareFloat (Transformation|GetDistanceTo (Variables|Default|Getplayer)) (Variables|/Game/JuegoX/Blueprints/Objects/Interactable.Interactable_C|GetDistance%20to%20Glow (Variables|Default|GetInteractuable))
          (:>
            (Rendering|Material|SetScalarParameterValue _materialhighlight "Scale" 0.0 :!class /Script/Engine.MaterialInstanceDynamic))
          (:==
            (Rendering|Material|SetScalarParameterValue _materialhighlight "Scale" 0.5 :!class /Script/Engine.MaterialInstanceDynamic :!label _label_2))
          (:<
            (goto _label_2)))
        (Rendering|Material|SetVectorParameterValue _materialhighlight "Color" "(R=1.000000,G=1.000000,B=1.000000,A=1.000000)" :!class /Script/Engine.MaterialInstanceDynamic)
        (else
          (Input|DisableInput _returnvalue_2))))))

(event Custom|CustomEvent
  (bind _mesh (Variables|Default|GetMesh))
  ;[1 1 1] memoria antes y despues
  ;;[1 1 1] begin play
  (Variables|/Game/JuegoX/Blueprints/Objects/Interactable.Interactable_C|SetfadeE (Variables|Default|GetInteractuable) true)
  ;;[1 1 1] control de duplicado de mesh para el outline - solo duplicar mesh cuando es una polaroid
  (if (Actor|ActorHasTag "Polaroid")
    (bind _returnvalue (AddComponent|AddStaticMeshComponent true (Transformation|GetWorldTransform _mesh)))
    (Transformation|AttachComponentToComponent _returnvalue _mesh "None" "KeepRelative" "KeepRelative" "KeepRelative" true)
    (Components|StaticMesh|SetStaticMesh _returnvalue (Variables|/Script/Engine.StaticMeshComponent|GetStaticMesh _mesh))
    (Rendering|Material|SetMaterial _returnvalue 0 (Rendering|Material|GetMaterial _mesh 0))
    (bind _returnvalue_2 (Rendering|Material|CreateDynamicMaterialInstance _returnvalue 0 "/Game/JuegoX/Materials/Outline_ObjectsHided.Outline_ObjectsHided" "None" :!class /Script/Engine.PrimitiveComponent))
    (Variables|Default|SetMaterialHighlight _returnvalue_2))
  (bind _asfirst_person_character (Utilities|Casting|CastToFirstPersonCharacter (Game|GetPlayerCharacter 0)))
  (Variables|Default|Setplayer _asfirst_person_character)
  (if (Actor|ActorHasTag "Polaroid")
    (Variables|Default|Setinit%20scale (Transformation|GetActorScale3D))))

(event EventBeginPlay
  (Variables|/Game/JuegoX/Blueprints/Objects/Interactable.Interactable_C|SetfadeE (Variables|Default|GetInteractuable) true)
  (bind _asfirst_person_character (Utilities|Casting|CastToFirstPersonCharacter (Game|GetPlayerCharacter 0)))
  (Variables|Default|Setplayer _asfirst_person_character))

(event EventTick
  (params (DeltaSeconds :type Float%20%28single-precision%29))
  (bind _returnvalue (Game|GetPlayerController 0))
  (if (Variables|/Game/JuegoX/Blueprints/Objects/Interactable.Interactable_C|GetisInspectingIt (Variables|Default|GetInteractuable))
    (Input|EnableInput _returnvalue :!label _label)
    (elif (Variables|/Game/JuegoX/Blueprints/Objects/Interactable.Interactable_C|GetisFocused? (Variables|Default|GetInteractuable))
      (goto _label)
      (else
        (Input|DisableInput _returnvalue)))))

(event Input|ActionEvents|InputActionInspect
  (params (Key :type Key%20Structure :default "None"))
  ;[1 1 1] memoria antes y despues
)

(event Input|ActionEvents|InputActionInspect
  (params (Key :type Key%20Structure :default "None"))
  (:Pressed
    (CallFunction|Inspection)))

(fn ConstructionScript)

(fn ShowControls
  (bind _player (Variables|Default|Getplayer))
  (if (Utilities|IsValid (Variables|/Game/FirstPersonBP/Blueprints/FirstPersonCharacter.FirstPersonCharacter_C|GetInventoryHUD _player))
    _
    (else
      (bind _returnvalue (UserInterface|CreateWidget "/Game/JuegoX/UI/HUD/WB_Inventory.WB_Inventory_C" (Game|GetPlayerController 0)))
      (Variables|/Game/FirstPersonBP/Blueprints/FirstPersonCharacter.FirstPersonCharacter_C|SetInventoryHUD _player _returnvalue)))
  (Rendering|Components|TextRender|SetText (Variables|/Game/JuegoX/UI/HUD/WB_Inventory.WB_Inventory_C|GetAction_One (Variables|/Game/FirstPersonBP/Blueprints/FirstPersonCharacter.FirstPersonCharacter_C|GetInventoryHUD _player)) "to drop")
  (if (UserInterface|Viewport|IsinViewport (Variables|/Game/FirstPersonBP/Blueprints/FirstPersonCharacter.FirstPersonCharacter_C|GetInventoryHUD _player))
    _
    (else
      (UserInterface|Viewport|AddtoViewport (Variables|/Game/FirstPersonBP/Blueprints/FirstPersonCharacter.FirstPersonCharacter_C|GetInventoryHUD _player) 0)))
  (Class|UserWidget|PlayAnimationForward (Variables|/Game/FirstPersonBP/Blueprints/FirstPersonCharacter.FirstPersonCharacter_C|GetInventoryHUD _player) (Variables|/Game/JuegoX/UI/HUD/WB_Inventory.WB_Inventory_C|GetControls_1_Anim (Variables|/Game/FirstPersonBP/Blueprints/FirstPersonCharacter.FirstPersonCharacter_C|GetInventoryHUD _player)) 4.0))

(fn HideControls
  (bind _player (Variables|Default|Getplayer))
  (bind _inventoryhud (Variables|/Game/FirstPersonBP/Blueprints/FirstPersonCharacter.FirstPersonCharacter_C|GetInventoryHUD _player))
  (Class|UserWidget|PlayAnimationReverse _inventoryhud (Variables|/Game/JuegoX/UI/HUD/WB_Inventory.WB_Inventory_C|GetControls_1_Anim _inventoryhud) 5.0))

(fn SetVisibility
  (Widget|SetVisibility (Variables|/Game/JuegoX/UI/HUD/WB_Inventory.WB_Inventory_C|GetLegend_One (Variables|/Game/FirstPersonBP/Blueprints/FirstPersonCharacter.FirstPersonCharacter_C|GetInventoryHUD (Variables|Default|Getplayer))) "Hidden"))

(fn UpdateLocation
  (params (timeline%20Value :type Float%20%28single-precision%29%20%28by%20ref%29))
  (bind _interactuable (Variables|Default|GetInteractuable))
  (Variables|Default|Setrotation (Transformation|GetActorRotation))
  (Transformation|SetActorLocationAndRotation (Math|Vector|Lerp(Vector) (Variables|/Game/JuegoX/Blueprints/Objects/Interactable.Interactable_C|GetinitialPos _interactuable) (Variables|/Game/JuegoX/Blueprints/Objects/Interactable.Interactable_C|GetinspectionPoint _interactuable) timeline%20Value) (Math|Rotator|Lerp(Rotator) (Variables|/Game/JuegoX/Blueprints/Objects/Interactable.Interactable_C|GetinitialRot _interactuable) (Variables|Default|Getrotation) timeline%20Value) true))

(fn Update
  (params (NewParam :type Float%20%28single-precision%29%20%28by%20ref%29)))