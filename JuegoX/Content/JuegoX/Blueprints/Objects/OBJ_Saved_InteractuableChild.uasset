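; Interactable object stored inside another actor, snapped to that container's inside point and attached to its mesh so it moves with it.
; A duplicated mesh with a dynamic outline material glows white when the player is near, red when focused and hides during inspection.
; Input is enabled only while focused or inspected.
; Overrides supply the inspection point, lerped movement and "to drop" HUD prompt, leaving Interact and ConnectWithCable empty.
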(event EventTick
  (params (DeltaSeconds :type Float%20%28single-precision%29))
  (bind _returnvalue (Game|GetPlayerController 0))
  (bind _materialhighlight (Variables|Default|GetmaterialHighlight))
  (bind _materialhighlight_2 (Variables|Default|GetmaterialHighlight))
  (if (Variables|/Game/JuegoX/Blueprints/Objects/Interactable.Interactable_C|GetisInspectingIt (Variables|Default|GetInteractable))
    (Rendering|Material|SetScalarParameterValue _materialhighlight "Scale" 0.0 :!class /Script/Engine.MaterialInstanceDynamic)
    (Input|EnableInput _returnvalue :!label _label)
    (elif (Variables|/Game/JuegoX/Blueprints/Objects/Interactable.Interactable_C|GetisFocused? (Variables|Default|GetInteractable))
      (Rendering|Material|SetScalarParameterValue _materialhighlight "Scale" 0.5 :!class /Script/Engine.MaterialInstanceDynamic)
      (Rendering|Material|SetVectorParameterValue _materialhighlight "Color" "(R=1.000000,G=0.000000,B=0.000000,A=1.000000)" :!class /Script/Engine.MaterialInstanceDynamic)
      (goto _label)
      (else
        (Input|DisableInput _returnvalue)
        (Math|Float|CompareFloat (Transformation|GetDistanceTo (Variables|Default|Getplayer)) (Variables|/Game/JuegoX/Blueprints/Objects/Interactable.Interactable_C|GetDistance%20to%20Glow (Variables|Default|GetInteractable))
          (:>
            (Rendering|Material|SetScalarParameterValue _materialhighlight_2 "Scale" 0.0 :!class /Script/Engine.MaterialInstanceDynamic))
          (:==
            (Rendering|Material|SetScalarParameterValue _materialhighlight_2 "Scale" 0.5 :!class /Script/Engine.MaterialInstanceDynamic :!label _label_2))
          (:<
            (goto _label_2)))
        (Rendering|Material|SetVectorParameterValue _materialhighlight_2 "Color" "(R=1.000000,G=1.000000,B=1.000000,A=1.000000)" :!class /Script/Engine.MaterialInstanceDynamic)))))

(event EventBeginPlay
  (|CallParentFunction)
  (bind _returnvalue (Rendering|Material|CreateDynamicMaterialInstance (Variables|Default|GetDuplicated) 0 "/Game/JuegoX/Materials/Outline_ObjectsHided.Outline_ObjectsHided" "None" :!class /Script/Engine.PrimitiveComponent))
  (Variables|Default|SetmaterialHighlight _returnvalue)
  (if (Utilities|IsValid (Variables|Default|GetWhatToFollow))
    ;[1 1 1] si se coloca bien, esto no hace falta
    (Transformation|SetActorLocation (Transformation|GetWorldLocation (Variables|Default|GetWhatToFollow)) false false))
  (Transformation|AttachComponentToComponent (Variables|/Game/JuegoX/Blueprints/Objects/OBJ_Dresser_DrawerParent.OBJ_Dresser_DrawerParent_C|GetMesh (Variables|Default|GetlugarDondeEstaGuardada)) "None" "KeepWorld" "KeepWorld" "KeepWorld" true))

(fn ConstructionScript
  (bind _lugardondeestaguardada (Variables|Default|GetlugarDondeEstaGuardada))
  (|CallParentFunction)
  (Variables|Default|SetSound 0)
  (Components|StaticMesh|SetStaticMesh (Variables|Default|GetDuplicated) (Variables|/Script/Engine.StaticMeshComponent|GetStaticMesh (Variables|Default|GetMesh)))
  (if (Utilities|IsValid _lugardondeestaguardada)
    (Variables|Default|SetWhatToFollow (Variables|/Game/JuegoX/Blueprints/Objects/OBJ_Dresser_DrawerParent.OBJ_Dresser_DrawerParent_C|GetObjectInside _lugardondeestaguardada))))

(fn ShowControls
  (if (Utilities|IsValid (Variables|/Game/FirstPersonBP/Blueprints/FirstPersonCharacter.FirstPersonCharacter_C|GetHUD (Variables|Default|Getplayer)))
    _
    (else
      (bind _returnvalue (UserInterface|CreateWidget "/Game/JuegoX/UI/HUD/WB_HUD.WB_HUD_C" (Game|GetPlayerController 0)))
      (Variables|/Game/FirstPersonBP/Blueprints/FirstPersonCharacter.FirstPersonCharacter_C|SetHUD (Variables|Default|Getplayer) _returnvalue)))
  (CallFunction|SetVariables)
  (if (UserInterface|Viewport|IsinViewport (Variables|/Game/FirstPersonBP/Blueprints/FirstPersonCharacter.FirstPersonCharacter_C|GetHUD (Variables|Default|Getplayer)))
    _
    (else
      (UserInterface|Viewport|AddtoViewport (Variables|/Game/FirstPersonBP/Blueprints/FirstPersonCharacter.FirstPersonCharacter_C|GetHUD (Variables|Default|Getplayer)) 0)))
  (Class|UserWidget|PlayAnimationForward (Variables|/Game/FirstPersonBP/Blueprints/FirstPersonCharacter.FirstPersonCharacter_C|GetHUD (Variables|Default|Getplayer)) (Variables|Default|Getwidget_Anim) 4.0))

(fn HideControls
  (Class|UserWidget|PlayAnimationReverse (Variables|/Game/FirstPersonBP/Blueprints/FirstPersonCharacter.FirstPersonCharacter_C|GetHUD (Variables|Default|Getplayer)) (Variables|Default|Getwidget_Anim) 4.0))

(fn Interact)

(fn UpdateLocation
  (params (timeline%20Value :type Float%20%28single-precision%29))
  (bind _interactable (Variables|Default|GetInteractable))
  (Transformation|SetActorLocationAndRotation (Math|Vector|Lerp(Vector) (Variables|/Game/JuegoX/Blueprints/Objects/Interactable.Interactable_C|GetinitialPos _interactable) (Variables|/Game/JuegoX/Blueprints/Objects/Interactable.Interactable_C|GetinspectionPoint _interactable) timeline%20Value) (Math|Rotator|Lerp(Rotator) (Variables|/Game/JuegoX/Blueprints/Objects/Interactable.Interactable_C|GetinitialRot _interactable) (Transformation|GetActorRotation) timeline%20Value) true))

(fn InspectionView
  (Variables|/Game/JuegoX/Blueprints/Objects/Interactable.Interactable_C|SetinspectionPoint (Variables|Default|GetInteractable) (Transformation|GetWorldLocation (Variables|/Game/FirstPersonBP/Blueprints/FirstPersonCharacter.FirstPersonCharacter_C|GetInpectionView (Variables|Default|Getplayer)))))

(fn SetVariables
  (Rendering|Components|TextRender|SetText (Variables|/Game/JuegoX/UI/HUD/WB_HUD.WB_HUD_C|GetAction_One (Variables|/Game/FirstPersonBP/Blueprints/FirstPersonCharacter.FirstPersonCharacter_C|GetHUD (Variables|Default|Getplayer))) "to drop")
  (Variables|Default|Setwidget_Anim (Variables|/Game/JuegoX/UI/HUD/WB_HUD.WB_HUD_C|GetControls_1_Anim (Variables|/Game/FirstPersonBP/Blueprints/FirstPersonCharacter.FirstPersonCharacter_C|GetHUD (Variables|Default|Getplayer)))))

(fn ConnectwithCable)