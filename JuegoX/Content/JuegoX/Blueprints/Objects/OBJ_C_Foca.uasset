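; OBJ_C_Foca is an inspectable seal object built on a parent interactable class.
; Its construction script assigns a loud male scream as the object's Sound after running the parent setup.
; On InspectionView, it sets the Interactuable inspection point to the location of the player's big inspection view anchor.
; BeginPlay and Tick only defer to the parent.
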(event EventBeginPlay
  (|CallParentFunction))

(event Collision|EventActorBeginOverlap
  (params (OtherActor :type Actor%20Object%20Reference)))

(event EventTick
  (params (DeltaSeconds :type Float%20%28single-precision%29))
  (|CallParentFunction DeltaSeconds))

(event EventInspectionView
  (Variables|/Game/JuegoX/Blueprints/Objects/Interactable.Interactable_C|SetinspectionPoint (Variables|Default|GetInteractuable) (Transformation|GetWorldLocation (Variables|/Game/FirstPersonBP/Blueprints/FirstPersonCharacter.FirstPersonCharacter_C|GetInpectionViewBig (Variables|Default|Getplayer)))))

(fn ConstructionScript
  (|CallParentFunction)
  (Variables|Default|SetSound "/Game/Soniditos/435851__dersuperanton__hello-scream-male-loud.435851__dersuperanton__hello-scream-male-loud"))