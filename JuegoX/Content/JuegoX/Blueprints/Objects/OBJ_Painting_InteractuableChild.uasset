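; Interactable painting child Blueprint that the player inspects and uses to travel between past and present.
; Interacting teleports the player to the connected mesh's Teleport point at the player's current height, turns them toward that mesh, toggles InThePast on the GameInstance and ends inspection.
; Inspection uses the player's big view point and sets "to travel"/"to drop" HUD prompts.
; Tick activates interaction on "Baul"-tagged instances once the GameInstance's BaulInteractuable flag is set.
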(event EventBeginPlay
  (|CallParentFunction) ; This node is disabled and will not be called.\nDrag off pins to build functionality.
)

(event Collision|EventActorBeginOverlap
  (params (OtherActor :type Actor%20Object%20Reference)))

(event EventSetVariables
  (bind _player (Variables|Default|Getplayer))
  (bind _inventoryhud (Variables|/Game/FirstPersonBP/Blueprints/FirstPersonCharacter.FirstPersonCharacter_C|GetInventoryHUD _player))
  (Rendering|Components|TextRender|SetText (Variables|/Game/JuegoX/UI/HUD/WB_Inventory.WB_Inventory_C|GetT_Drop _inventoryhud) "to drop")
  (Rendering|Components|TextRender|SetText (Variables|/Game/JuegoX/UI/HUD/WB_Inventory.WB_Inventory_C|GetT_Action _inventoryhud) "to travel")
  (Variables|Default|Setwidget_Anim (Variables|/Game/JuegoX/UI/HUD/WB_Inventory.WB_Inventory_C|GetControls_2_Anim _inventoryhud)))

(event EventTick
  (params (DeltaSeconds :type Float%20%28single-precision%29))
  (if (Variables|/Game/JuegoX/Blueprints/Objects/Interactable.Interactable_C|GetinteractionActivated (Variables|Default|GetInteractuable))
    _
    (elif (and (Actor|ActorHasTag "Baul") (Variables|/Game/JuegoX/Blueprints/MyGameInstance.MyGameInstance_C|GetbaulInteractuable (Variables|Default|GetGameInstance)))
      (Variables|/Game/JuegoX/Blueprints/Objects/Interactable.Interactable_C|SetinteractionActivated (Variables|Default|GetInteractuable) true)))
  (|CallParentFunction DeltaSeconds))

(event EventInspectionView
  (Variables|/Game/JuegoX/Blueprints/Objects/Interactable.Interactable_C|SetinspectionPoint (Variables|Default|GetInteractuable) (Transformation|GetWorldLocation (Variables|/Game/FirstPersonBP/Blueprints/FirstPersonCharacter.FirstPersonCharacter_C|GetInpectionViewBig (Variables|Default|Getplayer)))))

(event EventInteract
  (bind _player (Variables|Default|Getplayer))
  (bind _meshconnectedto (Variables|Default|GetMeshConnectedTo))
  (bind _gameinstance (Variables|Default|GetgameInstance))
  (bind _returnvalue (Transformation|GetActorLocation _player))
  (bind _teleport (Variables|OBJ_Painting_InteractuableChild_C|GetTeleport _meshconnectedto))
  (bind _returnvalue_2 (Transformation|GetWorldLocation _teleport))
  (bind (_x _y) (Math|Vector|BreakVector _returnvalue_2))
  (Transformation|SetActorLocationAndRotation (Variables|Default|Getplayer) (Math|Vector|MakeVector _x _y (.Z (Math|Vector|BreakVector _returnvalue))) (Math|Rotator|FindLookatRotation _returnvalue (Transformation|GetActorLocation (Variables|Default|GetMeshConnectedTo))))
  (if (Variables|/Game/JuegoX/Blueprints/MyGameInstance.MyGameInstance_C|GetinThePast _gameinstance)
    (Variables|/Game/JuegoX/Blueprints/MyGameInstance.MyGameInstance_C|SetinThePast _gameinstance false)
    (else
      (Variables|/Game/JuegoX/Blueprints/MyGameInstance.MyGameInstance_C|SetinThePast _gameinstance true)))
  (CallFunction|EndInspection))

(fn ConstructionScript)