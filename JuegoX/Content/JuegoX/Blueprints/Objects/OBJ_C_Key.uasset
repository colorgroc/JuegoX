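; Collectible key that the player can inspect and pick up, recording possession in the GameInstance.
; Tick drives an outline material on a duplicate mesh (white when nearby, red when focused) and enables input only while focused or inspected.
; When saved inside another object, the key follows that object's inner component.
; Interact sets HasKey, removes both meshes, shows the inventory icon and reverses the HUD controls animation.
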(event EventTick
  (params (DeltaSeconds :type Float%20%28single-precision%29))
  (bind _returnvalue (Game|GetPlayerController 0))
  (bind _materialhighlight (Variables|Default|GetmaterialHighlight))
  (bind _materialhighlight_2 (Variables|Default|GetmaterialHighlight))
  (if (Variables|/Game/JuegoX/Blueprints/Objects/Interactable.Interactable_C|GetisInspectingIt (Variables|Default|GetInteractuable))
    (Rendering|Material|SetScalarParameterValue _materialhighlight "Scale" 0.0 :!class /Script/Engine.MaterialInstanceDynamic)
    (Input|EnableInput _returnvalue :!label _label)
    (else
      (if (Variables|Default|GetitsSaved?)
        (Transformation|SetActorLocation (Transformation|GetWorldLocation (Variables|Default|GetWhatToFollow)) false false))
      (Variables|/Game/JuegoX/Blueprints/Objects/Interactable.Interactable_C|SetinitialPos (Variables|Default|GetInteractuable) (Transformation|GetActorLocation))
      (if (Variables|/Game/JuegoX/Blueprints/Objects/Interactable.Interactable_C|GetisFocused? (Variables|Default|GetInteractuable))
        (Rendering|Material|SetScalarParameterValue _materialhighlight "Scale" 0.5 :!class /Script/Engine.MaterialInstanceDynamic)
        (Rendering|Material|SetVectorParameterValue _materialhighlight "Color" "(R=1.000000,G=0.000000,B=0.000000,A=1.000000)" :!class /Script/Engine.MaterialInstanceDynamic)
        (goto _label)
        (else
          (Input|DisableInput _returnvalue)
          (Math|Float|CompareFloat (Transformation|GetDistanceTo (Variables|Default|Getplayer)) (Variables|/Game/JuegoX/Blueprints/Objects/Interactable.Interactable_C|GetDistance%20to%20Glow (Variables|Default|GetInteractuable))
            (:>
              (Rendering|Material|SetScalarParameterValue _materialhighlight_2 "Scale" 0.0 :!class /Script/Engine.MaterialInstanceDynamic))
            (:==
              (Rendering|Material|SetScalarParameterValue _materialhighlight_2 "Scale" 0.5 :!class /Script/Engine.MaterialInstanceDynamic :!label _label_2))
            (:<
              (goto _label_2)))
          (Rendering|Material|SetVectorParameterValue _materialhighlight_2 "Color" "(R=1.000000,G=1.000000,B=1.000000,A=1.000000)" :!class /Script/Engine.MaterialInstanceDynamic))))))

(event EventInteract
  (CallFunction|GameInstanceControl)
  (Variables|/Game/JuegoX/Blueprints/Objects/Interactable.Interactable_C|SetisInspectingIt (Variables|Default|GetInteractuable) false)
  (Variables|/Game/FirstPersonBP/Blueprints/FirstPersonCharacter.FirstPersonCharacter_C|SetplayerInspectingObject (Variables|Default|Getplayer) false)
  (Components|DestroyComponent (Variables|Default|GetDuplicate))
  (Components|DestroyComponent (Variables|Character|GetMesh))
  (CallFunction|ShowInventory)
  (CallFunction|DestroyKey))

(event EventBeginPlay
  (|CallParentFunction)
  (bind _returnvalue (Rendering|Material|CreateDynamicMaterialInstance (Variables|Default|GetDuplicate) 0 "/Game/JuegoX/Materials/Outline_ObjectsHided.Outline_ObjectsHided" "None" :!class /Script/Engine.PrimitiveComponent))
  (Variables|Default|SetmaterialHighlight _returnvalue))

(event EventSetvariables
  (bind _player (Variables|Default|Getplayer))
  (bind _inventoryhud (Variables|/Game/FirstPersonBP/Blueprints/FirstPersonCharacter.FirstPersonCharacter_C|GetInventoryHUD _player))
  (Rendering|Components|TextRender|SetText (Variables|/Game/JuegoX/UI/HUD/WB_Inventory.WB_Inventory_C|GetT_Drop _inventoryhud) "to drop")
  (Rendering|Components|TextRender|SetText (Variables|/Game/JuegoX/UI/HUD/WB_Inventory.WB_Inventory_C|GetT_Action _inventoryhud) "to pick")
  (Variables|Default|Setwidget_Anim (Variables|/Game/JuegoX/UI/HUD/WB_Inventory.WB_Inventory_C|GetControls_2_Anim _inventoryhud)))

(fn ConstructionScript
  (bind _lugardondeestaguardada (Variables|Default|GetlugarDondeEstaGuardada))
  (|CallParentFunction)
  (Variables|Default|Settexture "/Game/JuegoX/Sprites/inventario/llave.llave")
  (if (Variables|Default|GetitsSaved?)
    (if (Utilities|IsValid _lugardondeestaguardada)
      (Variables|Default|SetWhatToFollow (Variables|/Game/JuegoX/Blueprints/Objects/Cajon_Comoda.Cajon_Comoda_C|GetObjectInside _lugardondeestaguardada)))))

(fn DestroyKey
  (bind _player (Variables|Default|Getplayer))
  (bind _inventoryhud (Variables|/Game/FirstPersonBP/Blueprints/FirstPersonCharacter.FirstPersonCharacter_C|GetInventoryHUD _player))
  (bind _controls_2_anim (Variables|/Game/JuegoX/UI/HUD/WB_Inventory.WB_Inventory_C|GetControls_2_Anim _inventoryhud))
  (Class|UserWidget|PlayAnimationReverse _inventoryhud _controls_2_anim 6.0)
  (Class|UserWidget|BindtoAnimationFinished _inventoryhud _controls_2_anim (EventDispatchers|CreateEvent :!event K2DestroyActor)))

(fn ShowInventory
  (bind _player (Variables|Default|Getplayer))
  (bind _inventoryhud (Variables|/Game/FirstPersonBP/Blueprints/FirstPersonCharacter.FirstPersonCharacter_C|GetInventoryHUD _player))
  (Appearance|SetBrushfromTexture (Variables|/Game/JuegoX/UI/HUD/WB_Inventory.WB_Inventory_C|GetItem (Variables|/Game/FirstPersonBP/Blueprints/FirstPersonCharacter.FirstPersonCharacter_C|GetInventoryHUD (Variables|Default|Getplayer))) (Variables|Default|Gettexture) true)
  (Class|UserWidget|PlayAnimationForward _inventoryhud (Variables|/Game/JuegoX/UI/HUD/WB_Inventory.WB_Inventory_C|GetInventory_Anim _inventoryhud) 1.0))

(fn GameInstanceControl
  (Variables|/Game/JuegoX/Blueprints/MyGameInstance.MyGameInstance_C|SetHas_Key? (Variables|Default|GetGameInstance) true))