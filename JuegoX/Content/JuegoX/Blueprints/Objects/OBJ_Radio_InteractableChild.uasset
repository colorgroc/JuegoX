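; Interactable radio that the player inspects to plug in a cable, insert a cassette and toggle playback.
; SetVariables picks HUD control prompts from GameInstance and local state, while Interact and an extra input action route to cable, cassette or playback logic.
; PlugCable attaches the OBJ_Plug cable to the radio or spawns and removes a player-attached cable component.
; Play and Stop only set IsPlaying, with values inverted from their names.
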(event EventBeginPlay
  (|CallParentFunction) ; This node is disabled and will not be called.\nDrag off pins to build functionality.
)

(event Collision|EventActorBeginOverlap
  (params (OtherActor :type Actor%20Object%20Reference)))

(event EventTick
  (params (DeltaSeconds :type Float%20%28single-precision%29))
  (|CallParentFunction DeltaSeconds) ; This node is disabled and will not be called.\nDrag off pins to build functionality.
)

(event EventSetVariables
  (bind _player (Variables|Default|Getplayer))
  (bind _player_2 (Variables|Default|Getplayer))
  (bind _player_3 (Variables|Default|Getplayer))
  (bind _player_4 (Variables|Default|Getplayer))
  (bind _player_5 (Variables|Default|Getplayer))
  (bind _player_6 (Variables|Default|Getplayer))
  (bind _player_7 (Variables|Default|Getplayer))
  (bind _hud (Variables|/Game/FirstPersonBP/Blueprints/FirstPersonCharacter.FirstPersonCharacter_C|GetHUD _player))
  (bind _hud_2 (Variables|/Game/FirstPersonBP/Blueprints/FirstPersonCharacter.FirstPersonCharacter_C|GetHUD _player_6))
  (bind _hud_3 (Variables|/Game/FirstPersonBP/Blueprints/FirstPersonCharacter.FirstPersonCharacter_C|GetHUD _player_2))
  (bind _hud_4 (Variables|/Game/FirstPersonBP/Blueprints/FirstPersonCharacter.FirstPersonCharacter_C|GetHUD _player_3))
  (bind _hud_5 (Variables|/Game/FirstPersonBP/Blueprints/FirstPersonCharacter.FirstPersonCharacter_C|GetHUD _player_4))
  (bind _hud_6 (Variables|/Game/FirstPersonBP/Blueprints/FirstPersonCharacter.FirstPersonCharacter_C|GetHUD _player_5))
  (bind _hud_7 (Variables|/Game/FirstPersonBP/Blueprints/FirstPersonCharacter.FirstPersonCharacter_C|GetHUD _player_7))
  (if (Variables|/Game/JuegoX/Blueprints/MyGameInstance.MyGameInstance_C|GetHas_Cable? (Variables|Default|GetGameInstance))
    (if (Variables|Default|GetCableConnected)
      (if (Variables|/Game/JuegoX/Blueprints/MyGameInstance.MyGameInstance_C|GetCable_Connected? (Variables|Default|GetGameInstance))
        (if (Variables|/Game/JuegoX/Blueprints/MyGameInstance.MyGameInstance_C|GetCaseteInsideRadio? (Variables|Default|GetGameInstance))
          (if (Variables|Default|GetisPlaying?)
            (Rendering|Components|TextRender|SetText (Variables|/Game/JuegoX/UI/HUD/WB_HUD.WB_HUD_C|GetT_Drop _hud_2) "to drop")
            (Rendering|Components|TextRender|SetText (Variables|/Game/JuegoX/UI/HUD/WB_HUD.WB_HUD_C|GetT_Action _hud_2) "to stop")
            (Variables|Default|Setwidget_Anim (Variables|/Game/JuegoX/UI/HUD/WB_HUD.WB_HUD_C|GetControls_2_Anim _hud_2))
            (else
              (Rendering|Components|TextRender|SetText (Variables|/Game/JuegoX/UI/HUD/WB_HUD.WB_HUD_C|GetT_Drop _hud_4) "to drop")
              (Rendering|Components|TextRender|SetText (Variables|/Game/JuegoX/UI/HUD/WB_HUD.WB_HUD_C|GetT_Action _hud_4) "to play")
              (Variables|Default|Setwidget_Anim (Variables|/Game/JuegoX/UI/HUD/WB_HUD.WB_HUD_C|GetControls_2_Anim _hud_4))))
          (else
            (Rendering|Components|TextRender|SetText (Variables|/Game/JuegoX/UI/HUD/WB_HUD.WB_HUD_C|GetT_Drop _hud_6) "to drop")
            (Rendering|Components|TextRender|SetText (Variables|/Game/JuegoX/UI/HUD/WB_HUD.WB_HUD_C|GetT_Action _hud_6) "to insert cassette")
            (Variables|Default|Setwidget_Anim (Variables|/Game/JuegoX/UI/HUD/WB_HUD.WB_HUD_C|GetControls_2_Anim _hud_6))))
        (else
          (Rendering|Components|TextRender|SetText (Variables|/Game/JuegoX/UI/HUD/WB_HUD.WB_HUD_C|GetT_Drop _hud) "to drop")
          (Rendering|Components|TextRender|SetText (Variables|/Game/JuegoX/UI/HUD/WB_HUD.WB_HUD_C|GetT_Action _hud) "to unplug cable")
          (Variables|Default|Setwidget_Anim (Variables|/Game/JuegoX/UI/HUD/WB_HUD.WB_HUD_C|GetControls_2_Anim _hud))))
      (elif (Variables|/Game/JuegoX/Blueprints/MyGameInstance.MyGameInstance_C|GetHas_Cassette? (Variables|Default|GetGameInstance))
        (Rendering|Components|TextRender|SetText (Variables|/Game/JuegoX/UI/HUD/WB_HUD.WB_HUD_C|GetDrop _hud_5) "to drop")
        (Rendering|Components|TextRender|SetText (Variables|/Game/JuegoX/UI/HUD/WB_HUD.WB_HUD_C|GetActionOne _hud_5) "to plug cable")
        (Rendering|Components|TextRender|SetText (Variables|/Game/JuegoX/UI/HUD/WB_HUD.WB_HUD_C|GetActionTwo _hud_5) "to insert cassette")
        (Variables|Default|Setwidget_Anim (Variables|/Game/JuegoX/UI/HUD/WB_HUD.WB_HUD_C|GetControls_3_Anim _hud_5))
        (else
          (Rendering|Components|TextRender|SetText (Variables|/Game/JuegoX/UI/HUD/WB_HUD.WB_HUD_C|GetT_Drop _hud_7) "to drop")
          (Rendering|Components|TextRender|SetText (Variables|/Game/JuegoX/UI/HUD/WB_HUD.WB_HUD_C|GetT_Action _hud_7) "to plug cable")
          (Variables|Default|Setwidget_Anim (Variables|/Game/JuegoX/UI/HUD/WB_HUD.WB_HUD_C|GetControls_2_Anim _hud_7)))))
    (elif (Variables|/Game/JuegoX/Blueprints/MyGameInstance.MyGameInstance_C|GetHas_Cassette? (Variables|Default|GetGameInstance))
      (Rendering|Components|TextRender|SetText (Variables|/Game/JuegoX/UI/HUD/WB_HUD.WB_HUD_C|GetT_Drop _hud_3) "to drop")
      (Rendering|Components|TextRender|SetText (Variables|/Game/JuegoX/UI/HUD/WB_HUD.WB_HUD_C|GetT_Action _hud_3) "to insert cassete")
      (Variables|Default|Setwidget_Anim (Variables|/Game/JuegoX/UI/HUD/WB_HUD.WB_HUD_C|GetControls_2_Anim _hud_3))
      (else
        (Rendering|Components|TextRender|SetText (Variables|/Game/JuegoX/UI/HUD/WB_HUD.WB_HUD_C|GetAction_One (Variables|/Game/FirstPersonBP/Blueprints/FirstPersonCharacter.FirstPersonCharacter_C|GetHUD (Variables|Default|Getplayer))) "to drop")
        (Variables|Default|Setwidget_Anim (Variables|/Game/JuegoX/UI/HUD/WB_HUD.WB_HUD_C|GetControls_1_Anim (Variables|/Game/FirstPersonBP/Blueprints/FirstPersonCharacter.FirstPersonCharacter_C|GetHUD (Variables|Default|Getplayer))))))))

(event EventInteract
  (if (not (Variables|/Game/JuegoX/Blueprints/MyGameInstance.MyGameInstance_C|GetCable_Connected? (Variables|Default|GetGameInstance)))
    (if (Variables|/Game/JuegoX/Blueprints/MyGameInstance.MyGameInstance_C|GetHas_Cable? (Variables|Default|GetGameInstance))
      (CallFunction|PlugCable)
      (elif (Variables|/Game/JuegoX/Blueprints/MyGameInstance.MyGameInstance_C|GetHas_Cassette? (Variables|Default|GetGameInstance))
        (if (Variables|/Game/JuegoX/Blueprints/MyGameInstance.MyGameInstance_C|GetCaseteInsideRadio? (Variables|Default|GetGameInstance))
          (if (Variables|Default|GetisPlaying?)
            (CallFunction|StopCassette)
            (else
              (CallFunction|PlayCassette)))
          (else
            (Variables|/Game/JuegoX/Blueprints/MyGameInstance.MyGameInstance_C|SetCaseteInsideRadio? (Variables|Default|GetGameInstance) true)
            (bind _returnvalue (Actor|GetActorOfClass "/Game/JuegoX/Blueprints/Objects/OBJ_Cassete.OBJ_Cassete_C"))
            (Default|HideInventory _returnvalue)))))))

(event EventInspectionView
  (Variables|/Game/JuegoX/Blueprints/Objects/Interactable.Interactable_C|SetinspectionPoint (Variables|Default|GetInteractable) (Transformation|GetWorldLocation (Variables|/Game/FirstPersonBP/Blueprints/FirstPersonCharacter.FirstPersonCharacter_C|GetInpectionViewBig (Variables|Default|Getplayer)))))

(event Input|ActionEvents|InputActionAction2
  (params (Key :type Key%20Structure :default "None"))
  (bind _gameinstance (Variables|Default|GetGameInstance))
  (:Pressed
    ;[1 1 1] INput extra
    (if (Variables|/Game/JuegoX/Blueprints/Objects/Interactable.Interactable_C|GetinteractionActivated (Variables|Default|GetInteractable))
      (if (Variables|/Game/JuegoX/Blueprints/Objects/Interactable.Interactable_C|GetisInspectingIt (Variables|Default|GetInteractable))
        (if (not (Variables|/Game/JuegoX/Blueprints/MyGameInstance.MyGameInstance_C|GetCable_Connected? _gameinstance))
          (if (Math|Boolean|ANDBoolean (Variables|/Game/JuegoX/Blueprints/MyGameInstance.MyGameInstance_C|GetHas_Cable? _gameinstance) (Variables|/Game/JuegoX/Blueprints/MyGameInstance.MyGameInstance_C|GetHas_Cassette? _gameinstance) (not (Variables|Default|GetCableConnected)))
            (if (Variables|Default|GetisPlaying?)
              ;[1 1 1] Stop Music
              (CallFunction|StopCassette)
              (else
                ;[1 1 1] PLay Music
                (CallFunction|PlayCassette)))))))))

(fn ConstructionScript
  (|CallParentFunction)
  (Variables|Default|SetSound 0)
  (bind _returnvalue (Actor|GetActorOfClass "/Game/JuegoX/Blueprints/Objects/OBJ_Plug.OBJ_Plug_C"))
  (Variables|Default|SetObject _returnvalue))

(fn PlugCable
  (if (Variables|/Game/JuegoX/Blueprints/Objects/OBJ_Plug.OBJ_Plug_C|GetCableConnected (Variables|Default|GetObject))
    (Variables|/Script/CableComponent.CableComponent|SetbAttachEnd (Variables|/Game/JuegoX/Blueprints/Objects/OBJ_Plug.OBJ_Plug_C|GetCable (Variables|Default|GetObject)) true)
    (Class|CableComponent|SetAttachEndto (Variables|/Game/JuegoX/Blueprints/Objects/OBJ_Plug.OBJ_Plug_C|GetCable (Variables|Default|GetObject)) self "None" "None")
    (Variables|/Script/CableComponent.CableComponent|SetEndLocation (Variables|/Game/JuegoX/Blueprints/Objects/OBJ_Plug.OBJ_Plug_C|GetCable (Variables|Default|GetObject)) "0, 0, 0")
    (Variables|Default|SetCableConnected true)
    (Variables|/Game/JuegoX/Blueprints/MyGameInstance.MyGameInstance_C|SetCable_Connected? (Variables|Default|GetGameInstance) true)
    (bind _returnvalue (Actor|GetActorOfClass "/Game/JuegoX/Blueprints/Objects/OBJ_Cable_KeyChild.OBJ_Cable_KeyChild_C"))
    (Default|HideInventory _returnvalue)
    (elif (Variables|Default|GetCableConnected)
      (Utilities|IsValid (Variables|Default|GetCable)
        (:Is%20Valid
          (Components|DestroyComponent (Variables|Default|GetCable))
          (Variables|Default|SetCableConnected false))
        (:Is%20Not%20Valid
          (CallFunction|Interact)))
      (else
        (bind _returnvalue_2 (AddComponent|AddCableComponent false (Variables|Default|GetTransform)))
        (Variables|Default|SetCable _returnvalue_2)
        (Variables|/Script/CableComponent.CableComponent|SetbAttachEnd (Variables|Default|GetCable) true)
        (Class|CableComponent|SetAttachEndto (Variables|Default|GetCable) (Variables|Default|Getplayer) "None" "None")
        (Variables|/Script/CableComponent.CableComponent|SetCableWidth (Variables|Default|GetCable) 3.0)
        (Variables|/Script/CableComponent.CableComponent|SetbEnableCollision (Variables|Default|GetCable) true)
        (Variables|Default|SetCableConnected true)))))

(fn PlayCassette
  (Variables|Default|SetisPlaying? false))

(fn StopCassette
  (Variables|Default|SetisPlaying? true))