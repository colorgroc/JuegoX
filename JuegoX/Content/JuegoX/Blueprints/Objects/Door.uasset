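; Interactive door that opens and closes on the Inspect input, optionally requiring a key.
; Tick enables player input only while its Interactuable is focused.
; If NeedKey is set, it checks HasKey on MyGameInstance, otherwise printing a message and playing a locked sound.
; A FlipFlop alternates open/close sounds and sets IsOpen, which Interact uses to play the Anim sequence forward or in reverse.
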(event EventTick
  (params (DeltaSeconds :type Float%20%28single-precision%29))
  (bind _returnvalue (Game|GetPlayerController 0))
  (if (Variables|/Game/JuegoX/Blueprints/Objects/Interactable.Interactable_C|GetisFocused? (Variables|Default|GetInteractuable))
    (Input|EnableInput _returnvalue)
    (else
      (Input|DisableInput _returnvalue))))

(event EventBeginPlay
  (Variables|Default|SetisOpen? false))

(event Input|ActionEvents|InputActionInspect
  (params (Key :type Key%20Structure :default "None"))
  (:Pressed
    (if (Variables|/Game/JuegoX/Blueprints/Objects/Interactable.Interactable_C|GetisFocused? (Variables|Default|GetInteractuable))
      (if (Variables|Default|GetneedKey?)
        (bind _asmy_game_instance (Utilities|Casting|CastToMyGameInstance (Game|GetGameInstance)))
        (if (Variables|/Game/JuegoX/Blueprints/MyGameInstance.MyGameInstance_C|GetHas_Key? _asmy_game_instance)
          (Utilities|FlowControl|FlipFlop :!label _label
            (:A
              (Variables|Default|SetisOpen? false)
              (Audio|PlaySound2D "/Game/Soniditos/398750__anthousai__door-open-01.398750__anthousai__door-open-01" 1.0 1.0 0.0 0 0))
            (:B
              (Variables|Default|SetisOpen? true)
              (Audio|PlaySound2D "/Game/Soniditos/411791__inspectorj__door-wooden-close-a-h1.411791__inspectorj__door-wooden-close-a-h1" 1.0 1.0 0.0 0 0)))
          (CallFunction|Interact)
          (else
            (Development|PrintString "Need a Key to open it" true true "(R=1.000000,G=0.016184,B=0.000000,A=1.000000)")
            (Audio|PlaySound2D "/Game/Soniditos/12739__leady__locked-door.12739__leady__locked-door" 1.0 1.0 0.0 0 0)))
        (else
          (goto _label))))))

(fn ConstructionScript)

(fn Interact
  (bind _anim (Variables|Default|GetAnim))
  (bind _sequenceplayer (Variables|/Script/ActorSequence.ActorSequenceComponent|GetSequencePlayer _anim))
  (if (Variables|Default|GetisOpen?)
    (Class|MovieSceneSequencePlayer|PlayReverse _sequenceplayer)
    (Variables|Default|SetisOpen? false)
    (else
      (Sequencer|Player|Play _sequenceplayer :!class /Script/MovieScene.MovieSceneSequencePlayer)
      (Variables|Default|SetisOpen? true))))