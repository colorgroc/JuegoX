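; OBJ_C_Taker is a placeable object Blueprint for the Taker item, extending a parent object class.
; Its construction script sets the Taker texture and, when saved inside a valid storage location, follows that location's internal object.
; On the GameInstanceControl event it flags HasTaker on the GameInstance, presumably recording that the player owns it.
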(event EventBeginPlay
  (|CallParentFunction))

(event EventGameInstanceControl
  (Variables|/Game/JuegoX/Blueprints/MyGameInstance.MyGameInstance_C|SetHas_Taker? (Variables|Default|GetGameInstance) true))

(fn ConstructionScript
  (bind _lugardondeestaguardado (Variables|Default|GetlugarDondeEstaGuardado))
  (|CallParentFunction)
  (Variables|Default|Settexture "/Game/JuegoX/Sprites/inventario/taker.taker")
  (if (Variables|Default|GetitsSaved?)
    (if (Utilities|IsValid _lugardondeestaguardado)
      (Variables|Default|SetWhatToFollow (Variables|/Game/JuegoX/Blueprints/Objects/Cajon_Mesa.Cajon_Mesa_C|GetObjetoInterno _lugardondeestaguardado)))))