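; Interactable child Blueprint for a glasses item that the player can inspect, then pick up and put on immediately.
; Interacting flags the glasses as owned and worn in the GameInstance, ends inspection, hides the mesh and calls ShowInventory.
; It then triggers the player's GlassesAction, notifies the glasses cable actor found at BeginPlay, and destroys itself.
; SetVariables supplies the HUD's drop and pick-and-use prompts and controls animation.
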(event EventBeginPlay
  (|CallParentFunction)
  (bind _returnvalue (Actor|GetActorOfClass "/Game/JuegoX/Blueprints/Objects/OBJ_Glasses_Cable.OBJ_Glasses_Cable_C"))
  (Variables|Default|SetCable_0 _returnvalue))

(event Collision|EventActorBeginOverlap
  (params (OtherActor :type Actor%20Object%20Reference)))

(event EventTick
  (params (DeltaSeconds :type Float%20%28single-precision%29)))

(event EventInteract
  (CallFunction|GameInstanceControl)
  (Variables|/Game/JuegoX/Blueprints/Objects/Interactable.Interactable_C|SetisInspectingIt (Variables|Default|GetInteractable) false)
  (Variables|/Game/FirstPersonBP/Blueprints/FirstPersonCharacter.FirstPersonCharacter_C|SetplayerInspectingObject (Variables|Default|Getplayer) false)
  (Rendering|SetVisibility (Variables|Character|GetMesh) false true)
  (Variables|/Game/JuegoX/Blueprints/Objects/Interactable.Interactable_C|SetinteractionActivated (Variables|Default|GetInteractable) false)
  ;[1 1 1] si inicialment no es poses les ulleres
  (CallFunction|ShowInventory)
  ;[1 1 1] Hacer Fade
  (Default|GlassesAction (Variables|Default|Getplayer) true)
  (Default|Glasseson (Variables|Default|GetCable_0))
  (CallFunction|DestroyActor))

(event EventSetVariables
  (bind _player (Variables|Default|Getplayer))
  (bind _hud (Variables|/Game/FirstPersonBP/Blueprints/FirstPersonCharacter.FirstPersonCharacter_C|GetHUD _player))
  (Rendering|Components|TextRender|SetText (Variables|/Game/JuegoX/UI/HUD/WB_HUD.WB_HUD_C|GetT_Drop _hud) "to drop")
  (Rendering|Components|TextRender|SetText (Variables|/Game/JuegoX/UI/HUD/WB_HUD.WB_HUD_C|GetT_Action _hud) "to pick and use")
  (Variables|Default|Setwidget_Anim (Variables|/Game/JuegoX/UI/HUD/WB_HUD.WB_HUD_C|GetControls_2_Anim _hud)))

(event EventGameInstanceControl
  (Variables|/Game/JuegoX/Blueprints/MyGameInstance.MyGameInstance_C|SetHas_Glasses? (Variables|Default|GetGameInstance) true)
  (Variables|/Game/JuegoX/Blueprints/MyGameInstance.MyGameInstance_C|SetHas_GlassesOn? (Variables|Default|GetGameInstance) true))

(fn ConstructionScript
  (|CallParentFunction)
  ;[1 1 1] Glasses
  (Variables|Default|Settexture 0))