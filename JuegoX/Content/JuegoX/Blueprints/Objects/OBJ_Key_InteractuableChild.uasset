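; Key pickup, a child of an interactable parent, that can be inspected and collected, and can start stored inside another object.
; Tick drives an outline material on the duplicate mesh: red when focused, white within glow range, hidden when inspected or out of range, enabling input only while focused or inspected.
; Interact sets HasKey on the game instance, destroys both meshes, shows the key in the inventory HUD and reverses the controls animation.
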(event EventTick
  (params (DeltaSeconds :type Float%20%28single-precision%29))
  (bind _returnvalue (Game|GetPlayerController 0))
  (bind _materialhighlight (Variables|Default|GetmaterialHighlight))
  (bind _materialhighlight_2 (Variables|Default|GetmaterialHighlight))
  (if (Variables|/Game/JuegoX/Blueprints/Objects/Interactable.Interactable_C|GetisInspectingIt (Variables|Default|GetInteractuable))
    (Rendering|Material|SetScalarParameterValue _materialhighlight "Scale" 0.0 :!class /Script/Engine.MaterialInstanceDynamic)
    (Input|EnableInput _returnvalue :!label _label)
    (elif (Variables|/Game/JuegoX/Blueprints/Objects/Interactable.Interactable_C|GetisFocused? (Variables|Default|GetInteractuable))
      (Rendering|Material|SetScalarParameterValue _materialhighlight "Scale" 0.5 :!class /Script/Engine.MaterialInstanceDynamic)
      (Rendering|Material|SetVectorParameterValue _materialhighlight "Color" "(R=1.000000,G=0.000000,B=0.000000,A=1.000000)" :!class /Script/Engine.MaterialInstanceDynamic)
      (goto _label)
      (else
        (Input|DisableInput _returnvalue)
        (Math|Float|CompareFloat (Transformation|GetDistanceTo (Variables|Default|Getplayer)) (Variables|/Game/JuegoX/Blueprints/Objects/Interactable.Interactable_C|GetDistance%20to%20Glow (Variables|Default|GetInteractuable))
          (:>
            (Rendering|Material|SetScalarParameterValue _materialhighlight_2 "Scale" 0.0 :!class /Script/Engine.MaterialInstanceDynamic))
          (:==
            (Rendering|Material|SetScalarParameterValue _materialhighlight_2 "Scale" 0.5 :!class /Script/Engine.MaterialInstanceDynamic :!label _label_2))
          (:<
            (goto _label_2)))
        (Rendering|Material|SetVectorParameterValue _materialhighlight_2 "Color" "(R=1.000000,G=1.000000,B=1.000000,A=1.000000)" :!class /Script/Engine.MaterialInstanceDynamic)))))

(event EventInspection
  (if (Variables|/Game/JuegoX/Blueprints/Objects/Interactable.Interactable_C|GetisInspectingIt (Variables|Default|GetInteractuable))
    (CallFunction|EndInspection)
    (else
      (Utilities|FlowControl|Sequence
        (:then_0
          (Audio|PlaySound2D (Variables|Default|GetSound) 1.0 1.0 0.0 0 0))
        (:then_1
          (CallFunction|BeginInspection))))))

(event EventInteract
  (CallFunction|GameInstanceControl)
  (Variables|/Game/JuegoX/Blueprints/Objects/Interactable.Interactable_C|SetisInspectingIt (Variables|Default|GetInteractuable) false)
  (Variables|/Game/FirstPersonBP/Blueprints/FirstPersonCharacter.FirstPersonCharacter_C|SetplayerInspectingObject (Variables|Default|Getplayer) false)
  (Components|DestroyComponent (Variables|Default|GetDuplicate))
  (Components|DestroyComponent (Variables|Character|GetMesh))
  (CallFunction|ShowInventory)
  (CallFunction|DestroyKey))

(event EventBeginPlay
  (|CallParentFunction)
  (bind _returnvalue (Rendering|Material|CreateDynamicMaterialInstance (Variables|Default|GetDuplicate) 0 "/Game/JuegoX/Materials/Outline_ObjectsHided.Outline_ObjectsHided" "None" :!class /Script/Engine.PrimitiveComponent))
  (Variables|Default|SetmaterialHighlight _returnvalue)
  ;[1 1 1] si se coloca bien, esto no hace falta
  (if (and (Variables|Default|GetitsSaved?) (Utilities|IsValid (Variables|Default|GetWhatToFollow)))
    (Transformation|SetActorLocation (Transformation|GetWorldLocation (Variables|Default|GetWhatToFollow)) false false)
    (Transformation|AttachComponentToComponent (Variables|/Game/JuegoX/Blueprints/Objects/OBJ_Dresser_DrawerParent.OBJ_Dresser_DrawerParent_C|GetMesh (Variables|Default|GetlugarDondeEstaGuardada)) "None" "KeepWorld" "KeepWorld" "KeepWorld" true)))

(event EventSetvariables
  (bind _player (Variables|Default|Getplayer))
  (bind _inventoryhud (Variables|/Game/FirstPersonBP/Blueprints/FirstPersonCharacter.FirstPersonCharacter_C|GetInventoryHUD _player))
  (Rendering|Components|TextRender|SetText (Variables|/Game/JuegoX/UI/HUD/WB_HUD.WB_HUD_C|GetT_Drop _inventoryhud) "to drop")
  (Rendering|Components|TextRender|SetText (Variables|/Game/JuegoX/UI/HUD/WB_HUD.WB_HUD_C|GetT_Action _inventoryhud) "to pick")
  (Variables|Default|Setwidget_Anim (Variables|/Game/JuegoX/UI/HUD/WB_HUD.WB_HUD_C|GetControls_2_Anim _inventoryhud)))

(fn ConstructionScript
  (bind _lugardondeestaguardada (Variables|Default|GetlugarDondeEstaGuardada))
  (Variables|Default|Settexture "/Game/JuegoX/Sprites/inventario/llave.llave")
  (if (Variables|Default|GetitsSaved?)
    (if (Utilities|IsValid _lugardondeestaguardada)
      (Variables|Default|SetWhatToFollow (Variables|/Game/JuegoX/Blueprints/Objects/OBJ_Dresser_DrawerParent.OBJ_Dresser_DrawerParent_C|GetObjectInside _lugardondeestaguardada))
      (|CallParentFunction))))

(fn DestroyKey
  (bind _player (Variables|Default|Getplayer))
  (bind _player_2 (Variables|Default|Getplayer))
  (bind _inventoryhud (Variables|/Game/FirstPersonBP/Blueprints/FirstPersonCharacter.FirstPersonCharacter_C|GetInventoryHUD _player))
  (bind _inventoryhud_2 (Variables|/Game/FirstPersonBP/Blueprints/FirstPersonCharacter.FirstPersonCharacter_C|GetInventoryHUD _player_2))
  (Class|UserWidget|PlayAnimationReverse _inventoryhud_2 (Variables|/Game/JuegoX/UI/HUD/WB_HUD.WB_HUD_C|GetControls_2_Anim _inventoryhud_2) 6.0)
  (Class|UserWidget|BindtoAnimationFinished _inventoryhud (Variables|/Game/JuegoX/UI/HUD/WB_HUD.WB_HUD_C|GetControls_2_Anim _inventoryhud) (EventDispatchers|CreateEvent :!event K2DestroyActor)))

(fn ShowInventory
  (bind _player (Variables|Default|Getplayer))
  (bind _inventoryhud (Variables|/Game/FirstPersonBP/Blueprints/FirstPersonCharacter.FirstPersonCharacter_C|GetInventoryHUD _player))
  (Appearance|SetBrushfromTexture (Variables|/Game/JuegoX/UI/HUD/WB_HUD.WB_HUD_C|GetItem (Variables|/Game/FirstPersonBP/Blueprints/FirstPersonCharacter.FirstPersonCharacter_C|GetInventoryHUD (Variables|Default|Getplayer))) (Variables|Default|Gettexture) true)
  (if (UserInterface|Viewport|IsinViewport (Variables|/Game/FirstPersonBP/Blueprints/FirstPersonCharacter.FirstPersonCharacter_C|GetInventoryHUD (Variables|Default|Getplayer)))
    _
    (else
      (UserInterface|Viewport|AddtoViewport (Variables|/Game/FirstPersonBP/Blueprints/FirstPersonCharacter.FirstPersonCharacter_C|GetInventoryHUD (Variables|Default|Getplayer)) 0)))
  (Class|UserWidget|PlayAnimationForward _inventoryhud (Variables|/Game/JuegoX/UI/HUD/WB_HUD.WB_HUD_C|GetInventory_Anim _inventoryhud) 1.0))

(fn GameInstanceControl
  (Variables|/Game/JuegoX/Blueprints/MyGameInstance.MyGameInstance_C|SetHas_Key? (Variables|Default|GetGameInstance) true))