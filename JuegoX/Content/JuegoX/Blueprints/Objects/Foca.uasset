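; Foca is an inspectable object that plays a scream sound when the player starts examining it.
; Its Inspection event toggles on the Interactuable state: starting sets the inspection point from the player's big inspection view and plays the Inspect_Deco timeline.
; Ending reverses that timeline, whose MoveObject track updates the location, then re-enables the E fade on finish if allowed.
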(event EventBeginPlay
  (|CallParentFunction))

(event Collision|EventActorBeginOverlap
  (params (OtherActor :type Actor%20Object%20Reference)))

(event EventTick
  (params (DeltaSeconds :type Float%20%28single-precision%29))
  (|CallParentFunction DeltaSeconds))

(event EventInspection
  (if (Variables|/Game/JuegoX/Blueprints/Objects/Interactable.Interactable_C|GetisInspectingIt (Variables|Default|GetInteractuable))
    (CallFunction|EndInspection)
    (bind _move_object (Timeline|Inspect_Deco Reverse)
      (:Update
        (CallFunction|UpdateLocation _move_object))
      (:Finished
        (if (Variables|Default|GetableToFadeE) ; E appears when the animation finishes
          (Variables|/Game/JuegoX/Blueprints/Objects/Interactable.Interactable_C|SetfadeE (Variables|Default|GetInteractuable) true))))
    (else
      (Utilities|FlowControl|Sequence
        (:then_0
          (Variables|/Game/JuegoX/Blueprints/Objects/Interactable.Interactable_C|SetinspectionPoint (Variables|Default|GetInteractuable) (Transformation|GetWorldLocation (Variables|/Game/FirstPersonBP/Blueprints/FirstPersonCharacter.FirstPersonCharacter_C|GetInpectionViewBig (Variables|Default|Getplayer)))))
        (:then_1
          (Audio|PlaySound2D "/Game/Soniditos/435851__dersuperanton__hello-scream-male-loud.435851__dersuperanton__hello-scream-male-loud" 1.0 1.0 0.0 0 0))
        (:then_2
          (CallFunction|BeginInspection)
          (Timeline|Inspect_Deco Play))))))

(fn ConstructionScript
  (|CallParentFunction))