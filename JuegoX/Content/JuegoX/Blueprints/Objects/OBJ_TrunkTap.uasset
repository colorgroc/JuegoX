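; Trunk lid object (OBJ_TrunkTap) that the player opens and closes with the Inspect input, unlocked by the game instance's BaulInteractuable flag.
; Its Interactuable component is set up as non-inspectable, and Tick enables input only while it is focused or being inspected.
; Inspect plays the Anim sequence forward or in reverse, or shows a blocked hint through the player's inventory HUD.
; The timeline-driven EndInspection event is marked deprecated.
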(event Custom|EndInspection
  (bind _interactuable (Variables|Default|GetInteractuable))
  (bind _initialrot (Variables|/Game/JuegoX/Blueprints/Objects/Interactable.Interactable_C|GetinitialRot _interactuable))
  (bind _initialpos (Variables|/Game/JuegoX/Blueprints/Objects/Interactable.Interactable_C|GetinitialPos _interactuable))
  (bind (_roll _pitch _yaw) (Math|Rotator|BreakRotator _initialrot))
  (bind (_x _y) (Math|Vector|BreakVector _initialpos))
  ;[1 1 1] Deprecated
  (Variables|/Game/JuegoX/Blueprints/Objects/Interactable.Interactable_C|SetisInspectingIt (Variables|Default|GetInteractuable) false)
  (Variables|/Game/FirstPersonBP/Blueprints/FirstPersonCharacter.FirstPersonCharacter_C|SetplayerInspectingObject (Variables|Default|Getplayer) false)
  (bind _move_object (Timeline|Inspect Reverse)
    (:Update
      (bind _output_get (Variables|Default|SetMovedObject _move_object))
      (Transformation|SetActorLocationAndRotation (Math|Vector|Lerp(Vector) _initialpos (Math|Vector|MakeVector _x _y -1.9e+02) _output_get) (Math|Rotator|Lerp(Rotator) _initialrot (Math|Rotator|MakeRotator _roll -3e+01 _yaw) _output_get true)))))

(event EventTick
  (params (DeltaSeconds :type Float%20%28single-precision%29))
  (bind _returnvalue (Game|GetPlayerController 0))
  (if (Variables|/Game/JuegoX/Blueprints/Objects/Interactable.Interactable_C|GetisInspectingIt (Variables|Default|GetInteractuable))
    (Input|EnableInput _returnvalue :!label _label)
    (elif (Variables|/Game/JuegoX/Blueprints/Objects/Interactable.Interactable_C|GetisFocused? (Variables|Default|GetInteractuable))
      (goto _label)
      (else
        (Input|DisableInput _returnvalue)))))

(event EventBeginPlay
  (bind _asfirst_person_character (Utilities|Casting|CastToFirstPersonCharacter (Game|GetPlayerCharacter 0)))
  (bind _output_get (Variables|Default|Setplayer _asfirst_person_character))
  (Variables|/Game/JuegoX/Blueprints/Objects/Interactable.Interactable_C|Setplayer (Variables|Default|GetInteractuable) _output_get)
  (bind _asmy_game_instance (Utilities|Casting|CastToMyGameInstance (Game|GetGameInstance)))
  (Variables|Default|SetgameInstance _asmy_game_instance)
  (Variables|/Game/JuegoX/Blueprints/Objects/Interactable.Interactable_C|SetText (Variables|Default|GetInteractuable) (Variables|Default|GetTextRender))
  (Variables|/Game/JuegoX/Blueprints/Objects/Interactable.Interactable_C|SetMesh (Variables|Default|GetInteractuable) (Variables|Default|GetMesh))
  (Variables|/Game/JuegoX/Blueprints/Objects/Interactable.Interactable_C|Setis%20a%20nonInspectionable%20Object? (Variables|Default|GetInteractuable) true))

(event Input|ActionEvents|InputActionInspect
  (params (Key :type Key%20Structure :default "None"))
  (bind _anim (Variables|Default|GetAnim))
  (bind _sequenceplayer (Variables|/Script/ActorSequence.ActorSequenceComponent|GetSequencePlayer _anim))
  (:Pressed
    (if (Variables|/Game/JuegoX/Blueprints/MyGameInstance.MyGameInstance_C|GetbaulInteractuable (Variables|Default|GetgameInstance))
      (if (Variables|/Game/JuegoX/Blueprints/Objects/Interactable.Interactable_C|GetisFocused? (Variables|Default|GetInteractuable))
        (if (Variables|Default|Getopened)
          (Variables|Default|Setopened false)
          (Class|MovieSceneSequencePlayer|PlayReverse _sequenceplayer)
          (else
            (Variables|Default|Setopened true)
            (Sequencer|Player|Play _sequenceplayer :!class /Script/MovieScene.MovieSceneSequencePlayer))))
      (else
        (CallFunction|ShowHint "It's blocked!")))))

(fn ConstructionScript)

(fn ShowHint
  (params (hint :type Text))
  (if (Utilities|IsValid (Variables|/Game/FirstPersonBP/Blueprints/FirstPersonCharacter.FirstPersonCharacter_C|GetInventoryHUD (Variables|Default|Getplayer)))
    _
    (else
      (bind _returnvalue (UserInterface|CreateWidget "/Game/JuegoX/UI/HUD/WB_Inventory.WB_Inventory_C" (Game|GetPlayerController 0)))
      (Variables|/Game/FirstPersonBP/Blueprints/FirstPersonCharacter.FirstPersonCharacter_C|SetInventoryHUD (Variables|Default|Getplayer) _returnvalue)))
  (Rendering|Components|TextRender|SetText (Variables|/Game/JuegoX/UI/HUD/WB_Inventory.WB_Inventory_C|GetHInt_Text (Variables|/Game/FirstPersonBP/Blueprints/FirstPersonCharacter.FirstPersonCharacter_C|GetInventoryHUD (Variables|Default|Getplayer))) hint)
  (if (UserInterface|Viewport|IsinViewport (Variables|/Game/FirstPersonBP/Blueprints/FirstPersonCharacter.FirstPersonCharacter_C|GetInventoryHUD (Variables|Default|Getplayer)))
    _
    (else
      (UserInterface|Viewport|AddtoViewport (Variables|/Game/FirstPersonBP/Blueprints/FirstPersonCharacter.FirstPersonCharacter_C|GetInventoryHUD (Variables|Default|Getplayer)) 0)))
  (Class|UserWidget|PlayAnimationForward (Variables|/Game/FirstPersonBP/Blueprints/FirstPersonCharacter.FirstPersonCharacter_C|GetInventoryHUD (Variables|Default|Getplayer)) (Variables|/Game/JuegoX/UI/HUD/WB_Inventory.WB_Inventory_C|GetHint_Anim (Variables|/Game/FirstPersonBP/Blueprints/FirstPersonCharacter.FirstPersonCharacter_C|GetInventoryHUD (Variables|Default|Getplayer))) 4.0))