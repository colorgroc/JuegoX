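; Interactable armchair actor that lets the player sit down and stand up with the Inspect input while it is focused.
; Focus toggles input and a widget, and turns a text label toward the player.
; A timeline, reversed on standing, lerps the character between Stand and Sit points, turning them toward PaperCan.
; Sitting relaxes mesh collision and sets PlayerIsReading; light and diary-interaction toggles are disconnected.
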(event Custom|EndSofa
  (bind _returnvalue (Game|GetPlayerCharacter 0))
  (bind _stand (Variables|Default|GetStand))
  (bind _sit (Variables|Default|GetSit))
  (bind _papercan (Variables|Default|GetpaperCan))
  (bind _returnvalue_2 (Transformation|GetWorldLocation _sit))
  (bind _returnvalue_3 (Transformation|GetWorldLocation _stand))
  (bind _returnvalue_4 (Transformation|GetActorLocation _returnvalue))
  (bind _z (Math|Vector|BreakVector _returnvalue_4))
  (bind (_x _y) (Math|Vector|BreakVector _returnvalue_2))
  (bind (_x_2 _y_2) (Math|Vector|BreakVector _returnvalue_3))
  (bind _returnvalue_5 (Math|Vector|MakeVector _x _y _z))
  (Variables|Default|Setend true)
  (Variables|/Game/JuegoX/Blueprints/Objects/Interactable.Interactable_C|SetisFocused? (Variables|Default|GetInteractuable) false)
  (Variables|/Game/FirstPersonBP/Blueprints/FirstPersonCharacter.FirstPersonCharacter_C|SetplayerIsReading? (stale Input|ActionEvents|InputActionInspect _asfirst_person_character) false)
  (bind _sofa_sit (Timeline|Sofa Reverse)
    (:Update
      (bind _output_get (Variables|Default|Setsit_sofa _sofa_sit))
      (if (Utilities|IsValid _papercan)
        (Transformation|SetActorLocationAndRotation _returnvalue (Math|Vector|Lerp(Vector) (Math|Vector|MakeVector _x_2 _y_2 _z) _returnvalue_5 _output_get) (Math|Rotator|Lerp(Rotator) (Transformation|GetActorRotation _returnvalue) (Math|Rotator|FindLookatRotation _returnvalue_5 (Transformation|GetActorLocation _papercan)) _output_get))
        (Variables|/Game/JuegoX/Blueprints/Objects/Interactable.Interactable_C|SetisFocused? (Variables|Default|GetInteractuable) false)))
    (:Finished
      (if (Variables|Default|Getend)
        (Collision|SetCollisionProfileName (Variables|Default|GetMesh) "BlockAll" :!class /Script/Engine.PrimitiveComponent)
        (Variables|Default|Setend false)))))

(event EventTick
  (params (DeltaSeconds :type Float%20%28single-precision%29))
  (bind _returnvalue (Game|GetPlayerController 0))
  (bind _widget (Variables|Default|GetWidget))
  (if (Variables|/Game/JuegoX/Blueprints/Objects/Interactable.Interactable_C|GetisFocused? (Variables|Default|GetInteractuable))
    (Input|EnableInput _returnvalue)
    (Rendering|SetVisibility _widget true false)
    (Transformation|SetWorldRotation (Variables|Default|GetTextRender) (Math|Rotator|FindLookatRotation (Transformation|GetActorLocation) (Transformation|GetActorLocation (Variables|Default|GetPlayer))) false false)
    (else
      (Input|DisableInput _returnvalue)
      (Rendering|SetVisibility _widget false false))))

(event EventBeginPlay
  (bind _asfirst_person_character (Utilities|Casting|CastToFirstPersonCharacter (Game|GetPlayerCharacter 0)))
  (Variables|Default|Setplayer _asfirst_person_character))

(event Input|ActionEvents|InputActionInspect
  (params (Key :type Key%20Structure :default "None"))
  (bind _returnvalue (Game|GetPlayerCharacter 0))
  (bind _stand (Variables|Default|GetStand))
  (bind _sit (Variables|Default|GetSit))
  (bind _papercan (Variables|Default|GetpaperCan))
  (bind _interactuable (Variables|Default|GetInteractuable))
  (bind _diario (Variables|Default|GetDiario))
  (bind _returnvalue_2 (Transformation|GetWorldLocation _sit))
  (bind _returnvalue_3 (Transformation|GetWorldLocation _stand))
  (bind _returnvalue_4 (Transformation|GetActorLocation _returnvalue))
  (bind _z (Math|Vector|BreakVector _returnvalue_4))
  (bind (_x _y) (Math|Vector|BreakVector _returnvalue_2))
  (bind (_x_2 _y_2) (Math|Vector|BreakVector _returnvalue_3))
  (bind _returnvalue_5 (Math|Vector|MakeVector _x _y _z))
  (:Pressed
    (if (Variables|/Game/JuegoX/Blueprints/Objects/Interactable.Interactable_C|GetisFocused? (Variables|Default|GetInteractuable))
      (if (Variables|Default|GetSentado)
        (Variables|Default|SetSentado false)
        (if (Utilities|IsValid _diario)
          (CallFunction|EndSofa))
        (else
          (Variables|Default|SetSentado true)
          (Variables|Default|SetDiario_Transfrom (Transformation|GetActorTransform _diario))
          (Collision|SetCollisionProfileName (Variables|Default|GetMesh) "OverlapOnlyPawn" :!class /Script/Engine.PrimitiveComponent)
          (bind _asfirst_person_character (Utilities|Casting|CastToFirstPersonCharacter _returnvalue))
          (Variables|/Game/FirstPersonBP/Blueprints/FirstPersonCharacter.FirstPersonCharacter_C|SetplayerIsReading? _asfirst_person_character true)
          (if (Variables|/Game/JuegoX/Blueprints/Objects/Interactable.Interactable_C|GetisFocused? _interactuable)
            (bind _sofa_sit (Timeline|Sofa Play)
              (:Update
                (bind _output_get (Variables|Default|Setsit_sofa _sofa_sit))
                (if (Utilities|IsValid _papercan)
                  (Transformation|SetActorLocationAndRotation _returnvalue (Math|Vector|Lerp(Vector) (Math|Vector|MakeVector _x_2 _y_2 _z) _returnvalue_5 _output_get) (Math|Rotator|Lerp(Rotator) (Transformation|GetActorRotation _returnvalue) (Math|Rotator|FindLookatRotation _returnvalue_5 (Transformation|GetActorLocation _papercan)) _output_get))
                  (Variables|/Game/JuegoX/Blueprints/Objects/Interactable.Interactable_C|SetisFocused? _interactuable false)))
              (:Finished
                (if (Variables|Default|Getend)
                  (Collision|SetCollisionProfileName (Variables|Default|GetMesh) "BlockAll" :!class /Script/Engine.PrimitiveComponent)
                  (Variables|Default|Setend false))))))))))

(fn ConstructionScript)

(fn Interact)