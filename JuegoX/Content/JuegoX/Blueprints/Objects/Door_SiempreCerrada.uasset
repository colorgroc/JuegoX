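; Door actor that stays locked and plays a locked-door sound when the player inspects it.
; Tick enables or disables its input based on whether the Interactuable is focused, and the Inspect action plays the sound only while focused.
; An Interact function toggles IsOpen and plays the door animation forward or in reverse, but nothing in this graph calls it.
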(event EventTick
  (params (DeltaSeconds :type Float%20%28single-precision%29))
  (bind _returnvalue (Game|GetPlayerController 0))
  (if (Variables|/Game/JuegoX/Blueprints/Objects/Interactable.Interactable_C|GetisFocused? (Variables|Default|GetInteractuable))
    (Input|EnableInput _returnvalue)
    (else
      (Input|DisableInput _returnvalue))))

(event EventBeginPlay
  (Variables|Default|SetisOpen? false))

(event Input|ActionEvents|InputActionInspect
  (params (Key :type Key%20Structure :default "None"))
  (:Pressed
    (if (Variables|/Game/JuegoX/Blueprints/Objects/Interactable.Interactable_C|GetisFocused? (Variables|Default|GetInteractuable))
      (Audio|PlaySound2D "/Game/Soniditos/12739__leady__locked-door.12739__leady__locked-door" 1.0 1.0 0.0 0 0))))

(fn ConstructionScript)

(fn Interact
  (bind _anim (Variables|Default|GetAnim))
  (bind _sequenceplayer (Variables|/Script/ActorSequence.ActorSequenceComponent|GetSequencePlayer _anim))
  (if (Variables|Default|GetisOpen?)
    (Class|MovieSceneSequencePlayer|PlayReverse _sequenceplayer)
    (Variables|Default|SetisOpen? false)
    (else
      (Sequencer|Player|Play _sequenceplayer :!class /Script/MovieScene.MovieSceneSequencePlayer)
      (Variables|Default|SetisOpen? true))))