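; Map puzzle pin representing a city, which the player toggles while inspecting the map, provided they have the "taker".
; Tick enables input and shows the city name on the HUD only while the pin is focused and the puzzle is unsolved.
; Interact switches the marker and a dynamic glow material between white and a random default color, updating GameInstance's marked and correct city counts against its city list.
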(event EventTick
  (params (DeltaSeconds :type Float%20%28single-precision%29))
  (bind _returnvalue (Game|GetPlayerController 0))
  (bind _city_name (Variables|Ciudad|GetCity%20Name))
  (bind _returnvalue_2 (Utilities|Text|ToText(Name) _city_name))
  (if (Variables|/Game/JuegoX/Blueprints/MyGameInstance.MyGameInstance_C|GetMapPuzzle_Completed (Variables|Default|GetgameInstance))
    (Input|DisableInput _returnvalue :!label _label)
    (CallFunction|HideCityName _returnvalue_2)
    (elif (Variables|/Game/FirstPersonBP/Blueprints/FirstPersonCharacter.FirstPersonCharacter_C|GetplayerInpectingMapa (Variables|Default|GetPlayer))
      (if (Variables|/Game/JuegoX/Blueprints/Objects/InteraccionLugaresMapa.InteraccionLugaresMapa_C|GetisFocused? (Variables|Default|GetInteraccionLugaresMapa))
        (Input|EnableInput _returnvalue)
        (CallFunction|ShowCityName _returnvalue_2)
        (else
          (goto _label)))
      (else
        (Input|DisableInput (Game|GetPlayerController 0))))))

(event EventBeginPlay
  (bind _asmy_game_instance (Utilities|Casting|CastToMyGameInstance (Game|GetGameInstance)))
  (Variables|Default|SetgameInstance _asmy_game_instance)
  (bind _asfirst_person_character (Utilities|Casting|CastToFirstPersonCharacter (Game|GetPlayerCharacter 0)))
  (Variables|Default|SetPlayer _asfirst_person_character)
  (Rendering|SetVisibility (Variables|Default|GetName) false false)
  (Rendering|SetVisibility (Variables|Default|GetMarker) false false)
  (Rendering|Material|SetScalarParameterValue (Variables|Default|GetGlow_Mat) "Glow" 0.1 :!class /Script/Engine.MaterialInstanceDynamic))

(event Input|ActionEvents|InputActionInteract
  (params (Key :type Key%20Structure :default "None"))
  (bind _gameinstance (Variables|Default|GetgameInstance))
  (:Pressed
    (if (Variables|/Game/FirstPersonBP/Blueprints/FirstPersonCharacter.FirstPersonCharacter_C|GetplayerInpectingMapa (Variables|Default|GetPlayer))
      (if (not (Variables|/Game/JuegoX/Blueprints/MyGameInstance.MyGameInstance_C|GetMapPuzzle_Completed (Variables|Default|GetgameInstance)))
        (if (Variables|/Game/JuegoX/Blueprints/Objects/InteraccionLugaresMapa.InteraccionLugaresMapa_C|GetisFocused? (Variables|Default|GetInteraccionLugaresMapa))
          (if (Variables|/Game/JuegoX/Blueprints/MyGameInstance.MyGameInstance_C|GetHas_Taker? (Variables|Default|GetgameInstance))
            (if (Variables|Default|Getclicked)
              ;[1 1 1] Control de xinxetes activades
              (Variables|Default|Setclicked false)
              (CallFunction|Interact)
              (Math|Integer|DecrementInt (Variables|/Game/JuegoX/Blueprints/MyGameInstance.MyGameInstance_C|GetMarkedCities (Variables|Default|GetgameInstance))
                (:%20%20
                  (bind _inthelist (CallFunction|CheckCity (Variables|Ciudad|GetCity%20Name)))
                  (if _inthelist
                    (Math|Integer|DecrementInt (Variables|/Game/JuegoX/Blueprints/MyGameInstance.MyGameInstance_C|GetOkayCities (Variables|Default|GetgameInstance))))))
              (else
                (Variables|Default|Setclicked true)
                (CallFunction|Interact)
                (if (< (Variables|/Game/JuegoX/Blueprints/MyGameInstance.MyGameInstance_C|GetMarkedCities _gameinstance) (Utilities|Array|Length (Variables|/Game/JuegoX/Blueprints/MyGameInstance.MyGameInstance_C|GetListOfCities _gameinstance)))
                  (Math|Integer|IncrementInt (Variables|/Game/JuegoX/Blueprints/MyGameInstance.MyGameInstance_C|GetMarkedCities (Variables|Default|GetgameInstance))
                    (:%20%20
                      (bind _inthelist_2 (CallFunction|CheckCity (Variables|Ciudad|GetCity%20Name)))
                      (if _inthelist_2
                        (Math|Integer|IncrementInt (Variables|/Game/JuegoX/Blueprints/MyGameInstance.MyGameInstance_C|GetOkayCities (Variables|Default|GetgameInstance)))))))))
            (else
              (CallFunction|ShowHint "A taker is needed!"))))))))

(fn ConstructionScript
  (Rendering|Components|TextRender|SetText (Variables|Default|GetName) (Utilities|Text|ToText(Name) (Variables|Ciudad|GetCity%20Name)))
  (Rendering|SetVisibility (Variables|Default|GetMarker) true false)
  (bind _returnvalue (Rendering|Material|CreateDynamicMaterialInstance (Variables|Default|GetMesh) 0 "/Game/Materiales/Map/Mat_Instance_Glow_Pin.Mat_Instance_Glow_Pin" "None" :!class /Script/Engine.PrimitiveComponent))
  (Variables|Default|SetGlow_Mat _returnvalue)
  (Variables|Default|SetDefault%20Color (Math|Color|MakeColor (Math|Random|RandomFloatinRange 0.0 1.0) (Math|Random|RandomFloatinRange 0.0 1.0) (Math|Random|RandomFloatinRange 0.0 1.0)))
  (Rendering|Material|SetVectorParameterValue (Variables|Default|GetGlow_Mat) "Color" (Variables|Default|GetDefault%20Color) :!class /Script/Engine.MaterialInstanceDynamic)
  (Rendering|Material|SetScalarParameterValue (Variables|Default|GetGlow_Mat) "Glow" 0.0 :!class /Script/Engine.MaterialInstanceDynamic))

(fn Interact
  (bind _marker (Variables|Default|GetMarker))
  (if (Variables|Default|Getclicked)
    (Rendering|SetVisibility _marker true false)
    (Rendering|Material|SetScalarParameterValue (Variables|Default|GetGlow_Mat) "Glow" 1.0 :!class /Script/Engine.MaterialInstanceDynamic)
    (Rendering|Material|SetVectorParameterValue (Variables|Default|GetGlow_Mat) "Color" (Class|KismetMathLibrary|LinearColorWhite) :!class /Script/Engine.MaterialInstanceDynamic)
    (else
      (Rendering|SetVisibility _marker false false)
      (Rendering|Material|SetScalarParameterValue (Variables|Default|GetGlow_Mat) "Glow" 0.1 :!class /Script/Engine.MaterialInstanceDynamic)
      (Rendering|Material|SetVectorParameterValue (Variables|Default|GetGlow_Mat) "Color" (Variables|Default|GetDefault%20Color) :!class /Script/Engine.MaterialInstanceDynamic))))

(fn CheckCity
  (params (City :type Name%20%28by%20ref%29))
  (if (== (Utilities|Array|FindItem (Variables|/Game/JuegoX/Blueprints/MyGameInstance.MyGameInstance_C|GetListOfCities (Variables|Default|GetgameInstance)) City) -1)
    (return false)
    (else
      (return true))))

(fn ShowHint
  (params (hint :type Text))
  (if (Utilities|IsValid (Variables|/Game/FirstPersonBP/Blueprints/FirstPersonCharacter.FirstPersonCharacter_C|GetHUD (Variables|Default|Getplayer)))
    _
    (else
      (bind _returnvalue (UserInterface|CreateWidget "/Game/JuegoX/UI/HUD/WB_HUD.WB_HUD_C" (Game|GetPlayerController 0)))
      (Variables|/Game/FirstPersonBP/Blueprints/FirstPersonCharacter.FirstPersonCharacter_C|SetHUD (Variables|Default|Getplayer) _returnvalue)))
  (Rendering|Components|TextRender|SetText (Variables|/Game/JuegoX/UI/HUD/WB_HUD.WB_HUD_C|GetHInt_Text (Variables|/Game/FirstPersonBP/Blueprints/FirstPersonCharacter.FirstPersonCharacter_C|GetHUD (Variables|Default|Getplayer))) hint)
  (if (UserInterface|Viewport|IsinViewport (Variables|/Game/FirstPersonBP/Blueprints/FirstPersonCharacter.FirstPersonCharacter_C|GetHUD (Variables|Default|Getplayer)))
    _
    (else
      (UserInterface|Viewport|AddtoViewport (Variables|/Game/FirstPersonBP/Blueprints/FirstPersonCharacter.FirstPersonCharacter_C|GetHUD (Variables|Default|Getplayer)) 0)))
  (Class|UserWidget|PlayAnimationForward (Variables|/Game/FirstPersonBP/Blueprints/FirstPersonCharacter.FirstPersonCharacter_C|GetHUD (Variables|Default|Getplayer)) (Variables|/Game/JuegoX/UI/HUD/WB_HUD.WB_HUD_C|GetHint_Anim (Variables|/Game/FirstPersonBP/Blueprints/FirstPersonCharacter.FirstPersonCharacter_C|GetHUD (Variables|Default|Getplayer))) 4.0))

(fn ShowCityName
  (params (Name :type Text))
  (if (Utilities|IsValid (Variables|/Game/FirstPersonBP/Blueprints/FirstPersonCharacter.FirstPersonCharacter_C|GetHUD (Variables|Default|Getplayer)))
    (if (not (Utilities|Enum|Equal(Enum) (Class|EditableText|GetText (Variables|/Game/JuegoX/UI/HUD/WB_HUD.WB_HUD_C|GetCity_Name (Variables|/Game/FirstPersonBP/Blueprints/FirstPersonCharacter.FirstPersonCharacter_C|GetHUD (Variables|Default|Getplayer)))) Name))
      (Rendering|Components|TextRender|SetText (Variables|/Game/JuegoX/UI/HUD/WB_HUD.WB_HUD_C|GetCity_Name (Variables|/Game/FirstPersonBP/Blueprints/FirstPersonCharacter.FirstPersonCharacter_C|GetHUD (Variables|Default|Getplayer))) Name :!label _label)
      (if (UserInterface|Viewport|IsinViewport (Variables|/Game/FirstPersonBP/Blueprints/FirstPersonCharacter.FirstPersonCharacter_C|GetHUD (Variables|Default|Getplayer)))
        _
        (else
          (UserInterface|Viewport|AddtoViewport (Variables|/Game/FirstPersonBP/Blueprints/FirstPersonCharacter.FirstPersonCharacter_C|GetHUD (Variables|Default|Getplayer)) 0)))
      (Class|UserWidget|PlayAnimationForward (Variables|/Game/FirstPersonBP/Blueprints/FirstPersonCharacter.FirstPersonCharacter_C|GetHUD (Variables|Default|Getplayer)) (Variables|/Game/JuegoX/UI/HUD/WB_HUD.WB_HUD_C|GetCity_Anim (Variables|/Game/FirstPersonBP/Blueprints/FirstPersonCharacter.FirstPersonCharacter_C|GetHUD (Variables|Default|Getplayer))) 4.0))
    (else
      (bind _returnvalue (UserInterface|CreateWidget "/Game/JuegoX/UI/HUD/WB_HUD.WB_HUD_C" (Game|GetPlayerController 0)))
      (Variables|/Game/FirstPersonBP/Blueprints/FirstPersonCharacter.FirstPersonCharacter_C|SetHUD (Variables|Default|Getplayer) _returnvalue)
      (goto _label))))

(fn HideCityName
  (params (Name :type Text))
  (bind _player (Variables|Default|Getplayer))
  (bind _hud (Variables|/Game/FirstPersonBP/Blueprints/FirstPersonCharacter.FirstPersonCharacter_C|GetHUD _player))
  (if (Utilities|Enum|Equal(Enum) Name (Class|EditableText|GetText (Variables|/Game/JuegoX/UI/HUD/WB_HUD.WB_HUD_C|GetCity_Name (Variables|/Game/FirstPersonBP/Blueprints/FirstPersonCharacter.FirstPersonCharacter_C|GetHUD (Variables|Default|Getplayer)))))
    (Class|UserWidget|PlayAnimationReverse _hud (Variables|/Game/JuegoX/UI/HUD/WB_HUD.WB_HUD_C|GetCity_Anim _hud) 1.0)
    (Rendering|Components|TextRender|SetText (Variables|/Game/JuegoX/UI/HUD/WB_HUD.WB_HUD_C|GetCity_Name (Variables|/Game/FirstPersonBP/Blueprints/FirstPersonCharacter.FirstPersonCharacter_C|GetHUD (Variables|Default|Getplayer))) "")))