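; Inspectable cigarettes prop that the player can bring up for a closer look and put back, with no extra interaction.
; Input is enabled only while the Interactuable component is focused or inspecting.
; Inspect toggles a timeline that lerps the actor between its initial transform and the player's inspection point, playing a sound on pickup.
; Inspection also flags the player, animates inventory HUD controls, and hides the E prompt until the return finishes.
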(event Custom|Inspection
  (if (Variables|/Game/JuegoX/Blueprints/Objects/Interactable.Interactable_C|GetisInspectingIt (Variables|Default|GetInteractuable))
    (CallFunction|EndInspection)
    (bind _move_object (Timeline|inpection%20Timeline Reverse)
      (:Update
        (CallFunction|UpdateLocation _move_object))
      (:Finished
        (if (Variables|Default|GetableToFadeE) ; E appears when the animation finishes
          (Variables|/Game/JuegoX/Blueprints/Objects/Interactable.Interactable_C|SetfadeE (Variables|Default|GetInteractuable) true))))
    (else
      (Utilities|FlowControl|Sequence
        (:then_0
          (CallFunction|InspectionView))
        (:then_1
          (Audio|PlaySound2D (Variables|Default|GetSound) 1.0 1.0 0.0 0 0))
        (:then_2
          (CallFunction|BeginInspection)
          (Timeline|inpection%20Timeline Play))))))

(event Custom|EndInspection
  ;[1 1 1] lo de la E
  (if (Variables|Default|GetableToFadeE)
    _
    (else
      (Variables|Default|SetableToFadeE true)))
  (Variables|/Game/JuegoX/Blueprints/Objects/Interactable.Interactable_C|SetisInspectingIt (Variables|Default|GetInteractuable) false)
  (Variables|/Game/FirstPersonBP/Blueprints/FirstPersonCharacter.FirstPersonCharacter_C|SetplayerInspectingObject (Variables|Default|Getplayer) false)
  (CallFunction|HideControls))

(event Custom|BeginInspection
  (Utilities|FlowControl|Sequence
    (:then_0
      (CallFunction|ShowControls))
    (:then_1
      (Variables|/Game/JuegoX/Blueprints/Objects/Interactable.Interactable_C|SetisInspectingIt (Variables|Default|GetInteractuable) true)
      (Variables|/Game/FirstPersonBP/Blueprints/FirstPersonCharacter.FirstPersonCharacter_C|SetplayerInspectingObject (Variables|Default|Getplayer) true)
      ;[1 1 1] lo de la E
      (Variables|Default|SetableToFadeE false)
      (Variables|/Game/JuegoX/Blueprints/Objects/Interactable.Interactable_C|SetfadeE (Variables|Default|GetInteractuable) false))))

(event EventBeginPlay
  (Variables|/Game/JuegoX/Blueprints/Objects/Interactable.Interactable_C|SetfadeE (Variables|Default|GetInteractuable) true)
  (bind _asfirst_person_character (Utilities|Casting|CastToFirstPersonCharacter (Game|GetPlayerCharacter 0)))
  (Variables|Default|Setplayer _asfirst_person_character)
  (bind _asmy_game_instance (Utilities|Casting|CastToMyGameInstance (Game|GetGameInstance)))
  (Variables|Default|SetGameInstance _asmy_game_instance))

(event EventTick
  (params (DeltaSeconds :type Float%20%28single-precision%29))
  (bind _returnvalue (Game|GetPlayerController 0))
  (if (Variables|/Game/JuegoX/Blueprints/Objects/Interactable.Interactable_C|GetisInspectingIt (Variables|Default|GetInteractuable))
    (Input|EnableInput _returnvalue :!label _label)
    (elif (Variables|/Game/JuegoX/Blueprints/Objects/Interactable.Interactable_C|GetisFocused? (Variables|Default|GetInteractuable))
      (goto _label)
      (else
        (Input|DisableInput _returnvalue)))))

(event Input|ActionEvents|InputActionInteract
  (params (Key :type Key%20Structure :default "None"))
  (:Pressed
    (if (Variables|/Game/JuegoX/Blueprints/Objects/Interactable.Interactable_C|GetisInspectingIt (Variables|Default|GetInteractuable))
      (CallFunction|Interact) ; Aqui esta empty pq no tiene interaccion
    )))

(event Input|ActionEvents|InputActionInspect
  (params (Key :type Key%20Structure :default "None"))
  (:Pressed
    (if (Variables|/Game/JuegoX/Blueprints/Objects/Interactable.Interactable_C|GetinteractionActivated (Variables|Default|GetInteractuable))
      (CallFunction|Inspection))))

(fn ConstructionScript)

(fn ShowControls
  (if (Utilities|IsValid (Variables|/Game/FirstPersonBP/Blueprints/FirstPersonCharacter.FirstPersonCharacter_C|GetInventoryHUD (Variables|Default|Getplayer)))
    _
    (else
      (bind _returnvalue (UserInterface|CreateWidget "/Game/JuegoX/UI/HUD/WB_Inventory.WB_Inventory_C" (Game|GetPlayerController 0)))
      (Variables|/Game/FirstPersonBP/Blueprints/FirstPersonCharacter.FirstPersonCharacter_C|SetInventoryHUD (Variables|Default|Getplayer) _returnvalue)))
  (CallFunction|SetVariables)
  (if (UserInterface|Viewport|IsinViewport (Variables|/Game/FirstPersonBP/Blueprints/FirstPersonCharacter.FirstPersonCharacter_C|GetInventoryHUD (Variables|Default|Getplayer)))
    (Development|PrintString (Utilities|String|Append (Utilities|GetObjectName (Variables|Default|GetMesh)) "_True") true true "(R=0.000000,G=1.000000,B=0.078817,A=1.000000)")
    (else
      (Development|PrintString (Utilities|String|Append (Utilities|GetObjectName (Variables|Default|GetMesh)) "_False") true true "(R=1.000000,G=0.000000,B=0.065548,A=1.000000)")
      (UserInterface|Viewport|AddtoViewport (Variables|/Game/FirstPersonBP/Blueprints/FirstPersonCharacter.FirstPersonCharacter_C|GetInventoryHUD (Variables|Default|Getplayer)) 0)))
  (Class|UserWidget|PlayAnimationForward (Variables|/Game/FirstPersonBP/Blueprints/FirstPersonCharacter.FirstPersonCharacter_C|GetInventoryHUD (Variables|Default|Getplayer)) (Variables|Default|Getwidget_Anim) 4.0))

(fn HideControls
  (Class|UserWidget|PlayAnimationReverse (Variables|/Game/FirstPersonBP/Blueprints/FirstPersonCharacter.FirstPersonCharacter_C|GetInventoryHUD (Variables|Default|Getplayer)) (Variables|Default|Getwidget_Anim) 4.0))

(fn Interact)

(fn UpdateLocation
  (params (timeline%20Value :type Float%20%28single-precision%29))
  (bind _interactuable (Variables|Default|GetInteractuable))
  (Variables|Default|Setrotation (Transformation|GetActorRotation))
  (Transformation|SetActorLocationAndRotation (Math|Vector|Lerp(Vector) (Variables|/Game/JuegoX/Blueprints/Objects/Interactable.Interactable_C|GetinitialPos _interactuable) (Variables|/Game/JuegoX/Blueprints/Objects/Interactable.Interactable_C|GetinspectionPoint _interactuable) timeline%20Value) (Math|Rotator|Lerp(Rotator) (Variables|/Game/JuegoX/Blueprints/Objects/Interactable.Interactable_C|GetinitialRot _interactuable) (Variables|Default|Getrotation) timeline%20Value) true))

(fn InspectionView
  (Variables|/Game/JuegoX/Blueprints/Objects/Interactable.Interactable_C|SetinspectionPoint (Variables|Default|GetInteractuable) (Transformation|GetWorldLocation (Variables|/Game/FirstPersonBP/Blueprints/FirstPersonCharacter.FirstPersonCharacter_C|GetInpectionView (Variables|Default|Getplayer)))))

(fn SetVariables
  (Rendering|Components|TextRender|SetText (Variables|/Game/JuegoX/UI/HUD/WB_Inventory.WB_Inventory_C|GetAction_One (Variables|/Game/FirstPersonBP/Blueprints/FirstPersonCharacter.FirstPersonCharacter_C|GetInventoryHUD (Variables|Default|Getplayer))) "to drop")
  (Variables|Default|Setwidget_Anim (Variables|/Game/JuegoX/UI/HUD/WB_Inventory.WB_Inventory_C|GetControls_1_Anim (Variables|/Game/FirstPersonBP/Blueprints/FirstPersonCharacter.FirstPersonCharacter_C|GetInventoryHUD (Variables|Default|Getplayer)))))