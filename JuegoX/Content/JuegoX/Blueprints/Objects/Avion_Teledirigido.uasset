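; Player-controlled remote-control plane that flies through physics forces on its Driver component.
; Input axes add pitch, yaw and roll torque scaled by AirControl, while Tick counters spin and applies constant downward acceleration.
; A looping timer steps a clamped throttle from held inputs, and CalculateSpeed blends velocity toward the resulting capped forward speed.
; On hit, the plane's rotation nudges toward the surface normal to deflect it.
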(event EventBeginPlay
  (Utilities|Time|SetTimerbyFunctionName 0 "ThrottleInput" 0.05 true))

(event Collision|EventHit
  (params (MyComp :type Primitive%20Component%20Object%20Reference) (Other :type Actor%20Object%20Reference) (OtherComp :type Primitive%20Component%20Object%20Reference) (bSelfMoved :type Boolean) (HitLocation :type Vector :default "0, 0, 0") (HitNormal :type Vector :default "0, 0, 0") (NormalImpulse :type Vector :default "0, 0, 0") (Hit :type Hit%20Result%20Structure%20%28by%20ref%29))
  (bind _driver (Variables|Default|GetDriver))
  ;[1 1 1] Deflect when colliding
  (Transformation|SetWorldRotation _driver (Math|Rotator|Lerp(Rotator) (Transformation|GetWorldRotation _driver) (Math|Conversions|RotationFromXVector HitNormal) 0.01 true) false false))

(event EventTick
  (params (DeltaSeconds :type Float%20%28single-precision%29))
  (bind _driver (Variables|Default|GetDriver))
  (Class|PrimitiveComponent|AddTorqueinDegrees _driver (/ (Math|Vector|NegateVector (Physics|GetPhysicsAngularVelocityinDegrees (Variables|Default|GetDriver) "None")) 0.5) "None" true)
  (Physics|AddForce _driver "0, 0,-50.000000" "None" true)
  (CallFunction|CalculateSpeed))

(event Input|ActionEvents|InputActionThrottleUp
  (params (Key :type Key%20Structure :default "None"))
  (:Pressed
    (Variables|Default|SetThrottleUp true)
    (Development|PrintString "up"))
  (:Released
    (Variables|Default|SetThrottleUp false)))

(event Input|ActionEvents|InputActionThrottleDown
  (params (Key :type Key%20Structure :default "None"))
  (:Pressed
    (Variables|Default|SetThrottleDown true)
    (Development|PrintString "Down"))
  (:Released
    (Variables|Default|SetThrottleDown false)))

(event Input|AxisEvents|InputAxisRoll
  (params (AxisValue :type Float%20%28single-precision%29))
  (Class|PrimitiveComponent|AddTorqueinDegrees (Variables|Default|GetDriver) (Math|Vector|Lerp(Vector) "0, 0, 0" (* (Math|Vector|GetForwardVector (Variables|Default|GetDriver)) (* AxisValue (Variables|Default|GetAirControl))) 0.1) "None" true))

(event Input|AxisEvents|InputAxisMoveRight
  (params (AxisValue :type Float%20%28single-precision%29))
  (Class|PrimitiveComponent|AddTorqueinDegrees (Variables|Default|GetDriver) (Math|Vector|Lerp(Vector) "0, 0, 0" (* (Math|Vector|GetUpVector (Variables|Default|GetDriver)) (* AxisValue (Variables|Default|GetAirControl))) 0.1) "None" true))

(event Input|AxisEvents|InputAxisMoveForward
  (params (AxisValue :type Float%20%28single-precision%29))
  (Class|PrimitiveComponent|AddTorqueinDegrees (Variables|Default|GetDriver) (Math|Vector|Lerp(Vector) "0, 0, 0" (* (Math|Vector|GetRightVector (Variables|Default|GetDriver)) (* AxisValue (Variables|Default|GetAirControl))) 0.1) "None" true))

(event Input|AxisEvents|InputAxisTurn
  (params (AxisValue :type Float%20%28single-precision%29))
  (Class|PrimitiveComponent|AddTorqueinDegrees (Variables|Default|GetDriver) (Math|Vector|Lerp(Vector) "0, 0, 0" (* (Math|Vector|GetUpVector (Variables|Default|GetDriver)) (* AxisValue (Variables|Default|GetAirControl))) 0.1) "None" true))

(event Input|AxisEvents|InputAxisTurnRate
  (params (AxisValue :type Float%20%28single-precision%29))
  (Class|PrimitiveComponent|AddTorqueinDegrees (Variables|Default|GetDriver) (Math|Vector|Lerp(Vector) "0, 0, 0" (* (Math|Vector|GetUpVector (Variables|Default|GetDriver)) (* (stale Input|AxisEvents|InputAxisMoveRight AxisValue) (Variables|Default|GetAirControl))) 0.1) "None" true))

(event Input|AxisEvents|InputAxisLookUp
  (params (AxisValue :type Float%20%28single-precision%29))
  (Class|PrimitiveComponent|AddTorqueinDegrees (Variables|Default|GetDriver) (Math|Vector|Lerp(Vector) "0, 0, 0" (* (Math|Vector|GetRightVector (Variables|Default|GetDriver)) (* AxisValue (Variables|Default|GetAirControl))) 0.1) "None" true))

(fn ConstructionScript)

(fn ThrottleInput
  (if (Variables|Default|GetThrottleUp)
    (bind _result (Math|Integer|IncrementInt (Variables|Default|GetThrottleAmount))
      (:%20%20
        (bind _output_get (Variables|Default|SetThrottleAmount (Math|Integer|Clamp(Integer) _result 0 8)))
        (Development|PrintString (Utilities|String|ToString(Integer) _output_get))))
    (elif (Variables|Default|GetThrottleDown)
      (bind _result_2 (Math|Integer|DecrementInt (Variables|Default|GetThrottleAmount))
        (:%20%20
          (bind _output_get_2 (Variables|Default|SetThrottleAmount (Math|Integer|Clamp(Integer) _result_2 0 8)))
          (Development|PrintString (Utilities|String|ToString(Integer) _output_get_2)))))))

(fn CalculateSpeed
  (bind _driver (Variables|Default|GetDriver))
  (bind _returnvalue (Physics|GetPhysicsLinearVelocity _driver "None"))
  (Physics|SetPhysicsLinearVelocity _driver (Math|Vector|Lerp(Vector) _returnvalue (* (Math|Vector|GetForwardVector _driver) (Math|Float|Clamp(Float) (* (Variables|Default|GetThrottleAmount) 5e+01) 0.0 2e+02)) 0.01) false "None"))