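; Blablacar is an interactable object Blueprint, with its interaction behavior still empty.
; Tick polls the Interactuable component's IsFocused flag, enabling input for player controller 0 while focused and calling DisableInput otherwise.
; The Interact input action calls the Interact function when focused, but that function is a stub.
; A disconnected SetControlRotation snippet never runs.
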(event EventTick
  (params (DeltaSeconds :type Float%20%28single-precision%29))
  (bind _returnvalue (Game|GetPlayerController 0))
  (if (Variables|/Game/JuegoX/Blueprints/Objects/Interactable.Interactable_C|GetisFocused? (Variables|Default|GetInteractuable))
    (Input|EnableInput _returnvalue)
    (else
      (Input|DisableInput _returnvalue 0))))

(event Input|ActionEvents|InputActionInteract
  (params (Key :type Key%20Structure :default "None"))
  (:Pressed
    (if (Variables|/Game/JuegoX/Blueprints/Objects/Interactable.Interactable_C|GetisFocused? (Variables|Default|GetInteractuable))
      (CallFunction|Interact))))

(event Input|ActionEvents|InputActionInteract
  (params (Key :type Key%20Structure :default "None")))

(fn ConstructionScript)

(fn Interact)