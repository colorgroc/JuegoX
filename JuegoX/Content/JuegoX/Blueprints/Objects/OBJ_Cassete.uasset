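; OBJ_Cassete is a cassette object that records in the GameInstance whether the cassette is held.
; Its Construction Script runs the parent's, then applies the cassette texture and flag, disables the Interactable's InteractionActivated and hides the text render.
; The GameInstanceControl event clears HasCassette when OUT is true and sets it otherwise.
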(event EventBeginPlay
  (|CallParentFunction) ; This node is disabled and will not be called.\nDrag off pins to build functionality.
)

(event Collision|EventActorBeginOverlap
  (params (OtherActor :type Actor%20Object%20Reference)))

(event EventTick
  (params (DeltaSeconds :type Float%20%28single-precision%29))
  (|CallParentFunction DeltaSeconds) ; This node is disabled and will not be called.\nDrag off pins to build functionality.
)

(event EventGameInstanceControl
  (params (OUT :type Boolean))
  (if OUT
    (Variables|/Game/JuegoX/Blueprints/MyGameInstance.MyGameInstance_C|SetHas_Cassette? (Variables|Default|GetGameInstance) false)
    (else
      (Variables|/Game/JuegoX/Blueprints/MyGameInstance.MyGameInstance_C|SetHas_Cassette? (Variables|Default|GetGameInstance) true))))

(fn ConstructionScript
  (|CallParentFunction)
  (Variables|Default|Settexture "/Game/JuegoX/Sprites/inventario/casette.casette")
  (Variables|/Game/JuegoX/Blueprints/Objects/Interactable.Interactable_C|SetinteractionActivated (Variables|Default|GetInteractable) false)
  (Variables|Default|SetCassette? true)
  (Rendering|SetVisibility (Variables|Default|GetTextRender) false false))