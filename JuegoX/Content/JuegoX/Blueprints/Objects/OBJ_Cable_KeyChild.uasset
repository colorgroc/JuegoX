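; OBJ_Cable_KeyChild is a child key-object Blueprint for the Cable item, setting its texture to Cable in the construction script.
; Its GameInstanceControl event sets the HasCable flag on the GameInstance according to the OUT boolean: false when OUT is true, true otherwise.
; The same event finds the OBJ_Plug actor by class and switches its interaction on or off to match the flag.
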(event EventBeginPlay
  (|CallParentFunction) ; This node is disabled and will not be called.\nDrag off pins to build functionality.
)

(event Collision|EventActorBeginOverlap
  (params (OtherActor :type Actor%20Object%20Reference)))

(event EventTick
  (params (DeltaSeconds :type Float%20%28single-precision%29))
  (|CallParentFunction DeltaSeconds) ; This node is disabled and will not be called.\nDrag off pins to build functionality.
)

(event EventGameInstanceControl
  (params (OUT :type Boolean))
  (if OUT
    (Variables|/Game/JuegoX/Blueprints/MyGameInstance.MyGameInstance_C|SetHas_Cable? (Variables|Default|GetGameInstance) false)
    (bind _returnvalue (Actor|GetActorOfClass "/Game/JuegoX/Blueprints/Objects/OBJ_Plug.OBJ_Plug_C"))
    (Variables|/Game/JuegoX/Blueprints/Objects/Interactable.Interactable_C|SetinteractionActivated (Variables|/Game/JuegoX/Blueprints/Objects/OBJ_Plug.OBJ_Plug_C|GetInteractable _returnvalue) false)
    (else
      (Variables|/Game/JuegoX/Blueprints/MyGameInstance.MyGameInstance_C|SetHas_Cable? (Variables|Default|GetGameInstance) true)
      (bind _returnvalue_2 (Actor|GetActorOfClass "/Game/JuegoX/Blueprints/Objects/OBJ_Plug.OBJ_Plug_C"))
      (Variables|/Game/JuegoX/Blueprints/Objects/Interactable.Interactable_C|SetinteractionActivated (Variables|/Game/JuegoX/Blueprints/Objects/OBJ_Plug.OBJ_Plug_C|GetInteractable _returnvalue_2) true))))

(fn ConstructionScript
  (|CallParentFunction)
  (Variables|Default|Settexture "/Game/JuegoX/Sprites/inventario/cable.cable"))