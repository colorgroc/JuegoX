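; Inspectable painting actor that the player can bring up close and use to teleport to a connected object.
; Tick enables input only while its Interactuable is focused or being inspected.
; Inspect toggles a timeline that moves the painting between its initial position and the player's inspection point.
; Interact during inspection moves the player to the connected mesh's Teleport point, keeping height, sets a look-at rotation, then ends inspection.
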(event Custom|EndInspection
  (bind _interactuable (Variables|Default|GetInteractuable))
  (Variables|/Game/JuegoX/Blueprints/Objects/Interactable.Interactable_C|SetisInspectingIt (Variables|Default|GetInteractuable) false)
  (Variables|/Game/FirstPersonBP/Blueprints/FirstPersonCharacter.FirstPersonCharacter_C|SetplayerInspectingObject (Variables|Default|Getplayer) false)
  (bind _move_object (Timeline|Inspection Reverse)
    (:Update
      (bind _output_get (Variables|Default|SetMovedObject _move_object))
      (Transformation|SetActorLocationAndRotation (Math|Vector|Lerp(Vector) (Variables|/Game/JuegoX/Blueprints/Objects/Interactable.Interactable_C|GetinitialPos _interactuable) (Variables|/Game/JuegoX/Blueprints/Objects/Interactable.Interactable_C|GetinspectionPoint _interactuable) _output_get) (Math|Rotator|Lerp(Rotator) (Variables|/Game/JuegoX/Blueprints/Objects/Interactable.Interactable_C|GetinitialRot _interactuable) (Transformation|GetActorRotation) _output_get)))))

(event EventTick
  (params (DeltaSeconds :type Float%20%28single-precision%29))
  (bind _returnvalue (Game|GetPlayerController 0))
  (if (Variables|/Game/JuegoX/Blueprints/Objects/Interactable.Interactable_C|GetisInspectingIt (Variables|Default|GetInteractuable))
    (Input|EnableInput _returnvalue :!label _label)
    (elif (Variables|/Game/JuegoX/Blueprints/Objects/Interactable.Interactable_C|GetisFocused? (Variables|Default|GetInteractuable))
      (goto _label)
      (else
        (Input|DisableInput _returnvalue)))))

(event EventBeginPlay
  (bind _asfirst_person_character (Utilities|Casting|CastToFirstPersonCharacter (Game|GetPlayerCharacter 0)))
  (Variables|Default|Setplayer _asfirst_person_character))

(event Input|ActionEvents|InputActionInteract
  (params (Key :type Key%20Structure :default "None"))
  (:Pressed
    (if (Variables|/Game/JuegoX/Blueprints/Objects/Interactable.Interactable_C|GetisInspectingIt (Variables|Default|GetInteractuable))
      (CallFunction|Interact))))

(event Input|ActionEvents|InputActionInspect
  (params (Key :type Key%20Structure :default "None"))
  (bind _interactuable (Variables|Default|GetInteractuable))
  (bind _interactuable_2 (Variables|Default|GetInteractuable))
  (:Pressed
    (if (Variables|/Game/JuegoX/Blueprints/Objects/Interactable.Interactable_C|GetisInspectingIt _interactuable)
      (CallFunction|EndInspection)
      (else
        (Variables|/Game/JuegoX/Blueprints/Objects/Interactable.Interactable_C|SetinspectionPoint _interactuable (Transformation|GetWorldLocation (Variables|/Game/FirstPersonBP/Blueprints/FirstPersonCharacter.FirstPersonCharacter_C|GetInpectionViewBig (Variables|Default|Getplayer))))
        (Variables|/Game/JuegoX/Blueprints/Objects/Interactable.Interactable_C|SetisInspectingIt _interactuable true)
        (Variables|/Game/FirstPersonBP/Blueprints/FirstPersonCharacter.FirstPersonCharacter_C|SetplayerInspectingObject (Variables|Default|Getplayer) true)
        (bind _move_object (Timeline|Inspection Play)
          (:Update
            (bind _output_get (Variables|Default|SetMovedObject _move_object))
            (Transformation|SetActorLocationAndRotation (Math|Vector|Lerp(Vector) (Variables|/Game/JuegoX/Blueprints/Objects/Interactable.Interactable_C|GetinitialPos _interactuable_2) (Variables|/Game/JuegoX/Blueprints/Objects/Interactable.Interactable_C|GetinspectionPoint _interactuable_2) _output_get) (Math|Rotator|Lerp(Rotator) (Variables|/Game/JuegoX/Blueprints/Objects/Interactable.Interactable_C|GetinitialRot _interactuable_2) (Transformation|GetActorRotation) _output_get))))))))

(fn ConstructionScript)

(fn Interact
  (bind _returnvalue (Game|GetPlayerCharacter 0))
  (bind _meshconnectedto (Variables|ConnectedPainting|GetMeshConnectedTo))
  (bind _returnvalue_2 (Transformation|GetActorLocation _returnvalue))
  (bind _teleport (Variables|Painting_C|GetTeleport _meshconnectedto))
  (bind _returnvalue_3 (Transformation|GetWorldLocation _teleport))
  (bind (_x _y) (Math|Vector|BreakVector _returnvalue_3))
  (Transformation|SetActorLocationAndRotation _returnvalue (Math|Vector|MakeVector _x _y (.Z (Math|Vector|BreakVector _returnvalue_2))) (Math|Rotator|FindLookatRotation _returnvalue_2 (Transformation|GetActorLocation (Variables|ConnectedPainting|GetMeshConnectedTo))))
  (CallFunction|EndInspection))