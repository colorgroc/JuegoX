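; Interactable piano puzzle actor that unlocks a linked Door when the played melody matches the target stored in MyGameInstance.
; While focused it accepts Inspect input, which, if the player has the key, toggles play mode with a forward or reversed sequence animation.
; CheckMelody, not called within this Blueprint, compares the melody arrays, clears wrong attempts and shows HUD hints.
; Helper functions animate control prompts on the shared HUD.
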(event Custom|Begin
  (Variables|/Game/FirstPersonBP/Blueprints/FirstPersonCharacter.FirstPersonCharacter_C|SetPlayer%20Playing%20Piano (Variables|Default|GetPlayer) true)
  (Sequencer|Player|Play (Variables|/Script/ActorSequence.ActorSequenceComponent|GetSequencePlayer (Variables|Default|GetAnim)) :!class /Script/MovieScene.MovieSceneSequencePlayer)
  (Variables|/Game/JuegoX/Blueprints/Objects/Interactable.Interactable_C|SetinteractionActivated (Variables|Default|GetInteractable) false)
  (Rendering|SetVisibility (Variables|Default|GetTextRender) false false))

(event Custom|End
  (Variables|/Game/FirstPersonBP/Blueprints/FirstPersonCharacter.FirstPersonCharacter_C|SetPlayer%20Playing%20Piano (Variables|Default|GetPlayer) false)
  (CallFunction|HideControls)
  (Class|MovieSceneSequencePlayer|PlayReverse (Variables|/Script/ActorSequence.ActorSequenceComponent|GetSequencePlayer (Variables|Default|GetAnim)))
  (Utilities|FlowControl|Delay 0.2)
  (Variables|/Game/JuegoX/Blueprints/Objects/Interactable.Interactable_C|SetinteractionActivated (Variables|Default|GetInteractable) true)
  (Rendering|SetVisibility (Variables|Default|GetTextRender) true false))

(event EventBeginPlay
  (Variables|/Game/JuegoX/Blueprints/Objects/Interactable.Interactable_C|SetinteractionActivated (Variables|Default|GetInteractable) true)
  (bind _asmy_game_instance (Utilities|Casting|CastToMyGameInstance (Game|GetGameInstance)))
  (Variables|Default|SetgameInstance _asmy_game_instance)
  (bind _asfirst_person_character (Utilities|Casting|CastToFirstPersonCharacter (Game|GetPlayerCharacter 0)))
  (bind _output_get (Variables|Default|Setplayer _asfirst_person_character))
  (Variables|/Game/JuegoX/Blueprints/Objects/Interactable.Interactable_C|Setplayer (Variables|Default|GetInteractable) _output_get)
  (Variables|/Game/JuegoX/Blueprints/Objects/Interactable.Interactable_C|SetMesh (Variables|Default|GetInteractable) (Variables|Default|GetMesh))
  (Variables|/Game/JuegoX/Blueprints/Objects/Interactable.Interactable_C|SetText (Variables|Default|GetInteractable) (Variables|Default|GetTextRender))
  (Variables|/Game/JuegoX/Blueprints/Objects/Interactable.Interactable_C|Setis%20a%20nonInspectionable%20Object? (Variables|Default|GetInteractable) true))

(event Collision|EventActorBeginOverlap
  (params (OtherActor :type Actor%20Object%20Reference)))

(event EventTick
  (params (DeltaSeconds :type Float%20%28single-precision%29))
  (bind _returnvalue (Game|GetPlayerController 0))
  (if (Variables|/Game/JuegoX/Blueprints/Objects/Interactable.Interactable_C|GetisFocused? (Variables|Default|GetInteractable))
    (Input|EnableInput _returnvalue)
    (else
      (Input|DisableInput _returnvalue))))

(event Input|ActionEvents|InputActionInspect
  (params (Key :type Key%20Structure :default "None"))
  (:Pressed
    (if (Variables|/Game/JuegoX/Blueprints/MyGameInstance.MyGameInstance_C|GetHas_Key? (Variables|Default|GetGameInstance))
      (Default|HideInventory (Variables|Default|Getkey))
      (if (Variables|/Game/JuegoX/Blueprints/Objects/Interactable.Interactable_C|GetisFocused? (Variables|Default|GetInteractable))
        (if (Variables|/Game/FirstPersonBP/Blueprints/FirstPersonCharacter.FirstPersonCharacter_C|GetPlayer%20Playing%20Piano (Variables|Default|GetPlayer))
          (CallFunction|End :!label _label)
          (else
            (CallFunction|Begin)))
        (elif (Variables|/Game/FirstPersonBP/Blueprints/FirstPersonCharacter.FirstPersonCharacter_C|GetPlayer%20Playing%20Piano (Variables|Default|GetPlayer))
          (goto _label))))))

(fn ConstructionScript)

(fn ShowHint
  (params (Hint :type Text))
  (if (Utilities|IsValid (Variables|/Game/FirstPersonBP/Blueprints/FirstPersonCharacter.FirstPersonCharacter_C|GetHUD (Variables|Default|Getplayer)))
    _
    (else
      (bind _returnvalue (UserInterface|CreateWidget "/Game/JuegoX/UI/HUD/WB_HUD.WB_HUD_C" (Game|GetPlayerController 0)))
      (Variables|/Game/FirstPersonBP/Blueprints/FirstPersonCharacter.FirstPersonCharacter_C|SetHUD (Variables|Default|Getplayer) _returnvalue)))
  (Rendering|Components|TextRender|SetText (Variables|/Game/JuegoX/UI/HUD/WB_HUD.WB_HUD_C|GetHInt_Text (Variables|/Game/FirstPersonBP/Blueprints/FirstPersonCharacter.FirstPersonCharacter_C|GetHUD (Variables|Default|Getplayer))) Hint)
  (if (UserInterface|Viewport|IsinViewport (Variables|/Game/FirstPersonBP/Blueprints/FirstPersonCharacter.FirstPersonCharacter_C|GetHUD (Variables|Default|Getplayer)))
    _
    (else
      (UserInterface|Viewport|AddtoViewport (Variables|/Game/FirstPersonBP/Blueprints/FirstPersonCharacter.FirstPersonCharacter_C|GetHUD (Variables|Default|Getplayer)) 0)))
  (Class|UserWidget|PlayAnimationForward (Variables|/Game/FirstPersonBP/Blueprints/FirstPersonCharacter.FirstPersonCharacter_C|GetHUD (Variables|Default|Getplayer)) (Variables|/Game/JuegoX/UI/HUD/WB_HUD.WB_HUD_C|GetHint_Anim (Variables|/Game/FirstPersonBP/Blueprints/FirstPersonCharacter.FirstPersonCharacter_C|GetHUD (Variables|Default|Getplayer))) 4.0))

(fn CheckMelody
  (bind _gameinstance (Variables|Default|GetGameInstance))
  (bind _door (Variables|Default|GetDoor))
  (bind _gameinstance_2 (Variables|Default|GetGameInstance))
  (if (not (Variables|/Game/JuegoX/Blueprints/MyGameInstance.MyGameInstance_C|GetPianoPuzzleCompleted (Variables|Default|GetGameInstance)))
    (if (== (Utilities|Array|Length (Variables|/Game/JuegoX/Blueprints/MyGameInstance.MyGameInstance_C|GetMelodyPlayed _gameinstance)) (Utilities|Array|Length (Variables|/Game/JuegoX/Blueprints/MyGameInstance.MyGameInstance_C|GetPianoMelody _gameinstance)))
      (if (Utilities|Array|Identical (Variables|/Game/JuegoX/Blueprints/MyGameInstance.MyGameInstance_C|GetMelodyPlayed _gameinstance_2) (Variables|/Game/JuegoX/Blueprints/MyGameInstance.MyGameInstance_C|GetPianoMelody _gameinstance_2))
        ;[1 1 1] Puzzle completed
        (CallFunction|ShowHint "You are an artist!")
        (Utilities|IsValid _door
          (:Is%20Valid
            (Variables|/Game/JuegoX/Blueprints/Objects/OBJ_KeyDoor_DoorParent.OBJ_KeyDoor_DoorParent_C|SetneedKey? _door false))
          (:Is%20Not%20Valid
            (Development|PrintString "Door not set")))
        (else
          ;[1 1 1] reset puzzle
          (Utilities|Array|Clear (Variables|/Game/JuegoX/Blueprints/MyGameInstance.MyGameInstance_C|GetMelodyPlayed (Variables|Default|GetGameInstance)))
          (CallFunction|ShowHint "Wrong melody! Try again"))))))

(fn ShowControls
  (if (Utilities|IsValid (Variables|/Game/FirstPersonBP/Blueprints/FirstPersonCharacter.FirstPersonCharacter_C|GetHUD (Variables|Default|Getplayer)))
    _
    (else
      (bind _returnvalue (UserInterface|CreateWidget "/Game/JuegoX/UI/HUD/WB_HUD.WB_HUD_C" (Game|GetPlayerController 0)))
      (Variables|/Game/FirstPersonBP/Blueprints/FirstPersonCharacter.FirstPersonCharacter_C|SetHUD (Variables|Default|Getplayer) _returnvalue)))
  (Rendering|Components|TextRender|SetText (Variables|/Game/JuegoX/UI/HUD/WB_HUD.WB_HUD_C|GetT_Drop (Variables|/Game/FirstPersonBP/Blueprints/FirstPersonCharacter.FirstPersonCharacter_C|GetHUD (Variables|Default|Getplayer))) "to exit")
  (Rendering|Components|TextRender|SetText (Variables|/Game/JuegoX/UI/HUD/WB_HUD.WB_HUD_C|GetT_Action (Variables|/Game/FirstPersonBP/Blueprints/FirstPersonCharacter.FirstPersonCharacter_C|GetHUD (Variables|Default|Getplayer))) "to play key")
  (Variables|Default|SetWidgetAnim (Variables|/Game/JuegoX/UI/HUD/WB_HUD.WB_HUD_C|GetControls_2_Anim (Variables|/Game/FirstPersonBP/Blueprints/FirstPersonCharacter.FirstPersonCharacter_C|GetHUD (Variables|Default|Getplayer))))
  (if (UserInterface|Viewport|IsinViewport (Variables|/Game/FirstPersonBP/Blueprints/FirstPersonCharacter.FirstPersonCharacter_C|GetHUD (Variables|Default|Getplayer)))
    _
    (else
      (UserInterface|Viewport|AddtoViewport (Variables|/Game/FirstPersonBP/Blueprints/FirstPersonCharacter.FirstPersonCharacter_C|GetHUD (Variables|Default|Getplayer)) 0)))
  (Class|UserWidget|PlayAnimationForward (Variables|/Game/FirstPersonBP/Blueprints/FirstPersonCharacter.FirstPersonCharacter_C|GetHUD (Variables|Default|Getplayer)) (Variables|Default|GetWidgetAnim) 4.0))

(fn HideControls
  (Class|UserWidget|PlayAnimationReverse (Variables|/Game/FirstPersonBP/Blueprints/FirstPersonCharacter.FirstPersonCharacter_C|GetHUD (Variables|Default|Getplayer)) (Variables|Default|GetWidgetAnim) 4.0))