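; Interactable wall-map puzzle where the player must mark the correct cities with OBJ_Pin markers.
; Inspect input toggles a timeline that snaps the player to an interaction point and lerps the camera toward the map, reversing on exit.
; Tick gates input by focus and polls GameInstance city counters: a wrong full selection resets all pins, while a correct one completes the puzzle and ends inspection.
; HUD animations show controls and result hints.
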(event Custom|CheckCities_Marked
  (bind _gameinstance (Variables|Default|GetgameInstance))
  (bind _listofcities (Variables|/Game/JuegoX/Blueprints/MyGameInstance.MyGameInstance_C|GetListOfCities _gameinstance))
  (bind _returnvalue (Utilities|Array|Length _listofcities))
  (if (== (Variables|/Game/JuegoX/Blueprints/MyGameInstance.MyGameInstance_C|GetMarkedCities (Variables|Default|GetgameInstance)) _returnvalue)
    (if (== _returnvalue (Variables|/Game/JuegoX/Blueprints/MyGameInstance.MyGameInstance_C|GetOkayCities (Variables|Default|GetgameInstance)))
      (Variables|/Game/JuegoX/Blueprints/MyGameInstance.MyGameInstance_C|SetMapPuzzle_Completed (Variables|Default|GetgameInstance) true)
      (CallFunction|ShowHint "Completed!")
      (Audio|PlaySound2D "/Game/Soniditos/252681__jomellejager__magic-sound-1.252681__jomellejager__magic-sound-1" 1.0 1.0 0.0 0 0)
      (CallFunction|HideControls)
      ;[1 1 1] No hace falta
      (Variables|/Game/JuegoX/Blueprints/Objects/Interactable.Interactable_C|SetinteractionActivated (Variables|Default|GetInteractuable) false)
      (else
        (Utilities|FlowControl|Delay 0.2)
        (Variables|/Game/JuegoX/Blueprints/MyGameInstance.MyGameInstance_C|SetResetCities? (Variables|Default|GetgameInstance) true)
        (CallFunction|ShowHint "Wrong!")
        (Audio|PlaySound2D "/Game/Soniditos/351563__bertrof__game-sound-incorrect-with-delay.351563__bertrof__game-sound-incorrect-with-delay" 1.0 1.0 0.0 0 0)))))

(event Custom|EndInspection
  (bind _player (Variables|Default|GetPlayer))
  (bind _interactpointactor (Variables|Default|GetInteractPointActor))
  (bind _returnvalue (Transformation|GetWorldLocation _interactpointactor))
  (bind _firstpersoncamera (Variables|/Game/FirstPersonBP/Blueprints/FirstPersonCharacter.FirstPersonCharacter_C|GetFirstPersonCamera _player))
  (bind _returnvalue_2 (Transformation|GetWorldLocation _firstpersoncamera))
  (bind (_x _y) (Math|Vector|BreakVector _returnvalue))
  (bind (_x_2 _y_2) (Math|Vector|BreakVector _returnvalue_2))
  (CallFunction|HideControls)
  (Variables|/Game/FirstPersonBP/Blueprints/FirstPersonCharacter.FirstPersonCharacter_C|SetplayerInpectingMapa (Variables|Default|GetPlayer) false)
  ;[1 1 1] Aqui es donde iria el zoom in/out -> branca de (SetCollision [BlockAllDynamic]) es el ZoomIn y la branca (SetCollision [NoCollision]) es el ZoomOut
  (Variables|/Game/JuegoX/Blueprints/Objects/Interactable.Interactable_C|SetisFocused? (Variables|Default|GetInteractuable) false)
  (Variables|/Game/JuegoX/Blueprints/Objects/Interactable.Interactable_C|SetinteractionActivated (Variables|Default|GetInteractuable) true)
  (bind _maptoplayer (Timeline|MapToPlayer Reverse)
    (:Update
      (Variables|Default|Setmap _maptoplayer)
      (Transformation|SetActorLocationAndRotation (Variables|Default|GetPlayer) (Math|Vector|MakeVector _x _y (.Z (Math|Vector|BreakVector (Transformation|GetActorLocation (Variables|Default|GetPlayer))))) (Math|Rotator|FindLookatRotation (Transformation|GetWorldLocation (Variables|Default|GetInteractPointActor)) (Transformation|GetWorldLocation (Variables|Default|GetMesh))) false true)
      (Transformation|SetWorldLocation (Variables|/Game/FirstPersonBP/Blueprints/FirstPersonCharacter.FirstPersonCharacter_C|GetFirstPersonCamera (Variables|Default|GetPlayer)) (Math|Vector|Lerp(Vector) (Math|Vector|MakeVector _x_2 _y_2 (.Z (Math|Vector|BreakVector (Variables|Default|GetcameraPos)))) (Transformation|GetWorldLocation (Variables|Default|GetInteractPointCamera)) (Variables|Default|Getmap)) false false)
      (Variables|/Game/JuegoX/Blueprints/Objects/Interactable.Interactable_C|SetisFocused? (Variables|Default|GetInteractuable) false))))

(event EventTick
  (params (DeltaSeconds :type Float%20%28single-precision%29))
  (CallFunction|CheckInput)
  (if (Variables|/Game/JuegoX/Blueprints/MyGameInstance.MyGameInstance_C|GetMapPuzzle_Completed (Variables|Default|GetgameInstance))
    ;[1 1 1] sortir del mapa al completar-lo
    (Utilities|FlowControl|DoOnce false
      (:Completed
        (CallFunction|EndInspection)
        (Variables|/Game/JuegoX/Blueprints/Objects/Interactable.Interactable_C|SetinteractionActivated (Variables|Default|GetInteractuable) false)
        (CallFunction|HideControls)
        (CallFunction|HideInventory)))
    (elif (Variables|/Game/JuegoX/Blueprints/MyGameInstance.MyGameInstance_C|GetResetCities? (Variables|Default|GetgameInstance))
      (for _array_element (Variables|Default|GetListaXinxetas)
        (Variables|/Game/JuegoX/Blueprints/Objects/OBJ_Pin.OBJ_Pin_C|Setclicked _array_element false)
        (Rendering|SetVisibility (Variables|/Game/JuegoX/Blueprints/Objects/OBJ_Pin.OBJ_Pin_C|GetMarker _array_element) false false)
        (Rendering|Material|SetVectorParameterValue (Variables|/Game/JuegoX/Blueprints/Objects/OBJ_Pin.OBJ_Pin_C|GetGlow_Mat _array_element) "Color" (Variables|/Game/JuegoX/Blueprints/Objects/OBJ_Pin.OBJ_Pin_C|GetDefault%20Color _array_element) :!class /Script/Engine.MaterialInstanceDynamic)
        (Rendering|Material|SetScalarParameterValue (Variables|/Game/JuegoX/Blueprints/Objects/OBJ_Pin.OBJ_Pin_C|GetGlow_Mat _array_element) "Glow" 0.1 :!class /Script/Engine.MaterialInstanceDynamic))
      (Variables|/Game/JuegoX/Blueprints/MyGameInstance.MyGameInstance_C|SetMarkedCities (Variables|Default|GetgameInstance) 0)
      (Variables|/Game/JuegoX/Blueprints/MyGameInstance.MyGameInstance_C|SetOkayCities (Variables|Default|GetgameInstance) 0)
      (Variables|/Game/JuegoX/Blueprints/MyGameInstance.MyGameInstance_C|SetResetCities? (Variables|Default|GetgameInstance) false)
      (else
        (CallFunction|CheckCitiesMarked)))))

(event EventBeginPlay
  (Variables|/Game/JuegoX/Blueprints/Objects/Interactable.Interactable_C|SetinteractionActivated (Variables|Default|GetInteractuable) true)
  (bind _outactors (Actor|GetAllActorsOfClass "/Game/JuegoX/Blueprints/Objects/OBJ_Pin.OBJ_Pin_C"))
  (Variables|Default|SetListaXinxetas _outactors)
  (bind _asmy_game_instance (Utilities|Casting|CastToMyGameInstance (Game|GetGameInstance)))
  (Variables|Default|SetgameInstance _asmy_game_instance)
  (bind _asfirst_person_character (Utilities|Casting|CastToFirstPersonCharacter (Game|GetPlayerCharacter 0)))
  (bind _output_get (Variables|Default|Setplayer _asfirst_person_character))
  (Variables|/Game/JuegoX/Blueprints/Objects/Interactable.Interactable_C|Setplayer (Variables|Default|GetInteractuable) _output_get)
  (Variables|/Game/JuegoX/Blueprints/Objects/Interactable.Interactable_C|SetMesh (Variables|Default|GetInteractuable) (Variables|Default|GetMesh))
  (Variables|/Game/JuegoX/Blueprints/Objects/Interactable.Interactable_C|SetText (Variables|Default|GetInteractuable) (Variables|Default|GetTextRender))
  (Variables|/Game/JuegoX/Blueprints/Objects/Interactable.Interactable_C|Setis%20a%20nonInspectionable%20Object? (Variables|Default|GetInteractuable) true))

(event Input|ActionEvents|InputActionInspect
  (params (Key :type Key%20Structure :default "None"))
  (bind _player (Variables|Default|GetPlayer))
  (bind _interactpointactor (Variables|Default|GetInteractPointActor))
  (bind _returnvalue (Transformation|GetWorldLocation _interactpointactor))
  (bind _firstpersoncamera (Variables|/Game/FirstPersonBP/Blueprints/FirstPersonCharacter.FirstPersonCharacter_C|GetFirstPersonCamera _player))
  (bind _returnvalue_2 (Transformation|GetWorldLocation _firstpersoncamera))
  (bind (_x _y) (Math|Vector|BreakVector _returnvalue))
  (bind (_x_2 _y_2) (Math|Vector|BreakVector _returnvalue_2))
  (:Pressed
    (if (not (Variables|/Game/JuegoX/Blueprints/MyGameInstance.MyGameInstance_C|GetMapPuzzle_Completed (Variables|Default|GetgameInstance)))
      (if (Variables|/Game/JuegoX/Blueprints/Objects/Interactable.Interactable_C|GetisFocused? (Variables|Default|GetInteractuable))
        (if (Variables|/Game/FirstPersonBP/Blueprints/FirstPersonCharacter.FirstPersonCharacter_C|GetplayerInpectingMapa (Variables|Default|GetPlayer))
          (CallFunction|EndInspection :!label _label)
          (else
            (CallFunction|ShowControls)
            (Variables|/Game/FirstPersonBP/Blueprints/FirstPersonCharacter.FirstPersonCharacter_C|SetplayerInpectingMapa (Variables|Default|GetPlayer) true)
            ;[1 1 1] Aqui es donde iria el zoom in/out -> branca de (SetCollision [BlockAllDynamic]) es el ZoomIn y la branca (SetCollision [NoCollision]) es el ZoomOut
            (Variables|Default|SetcameraPos (Transformation|GetWorldLocation (Variables|/Game/FirstPersonBP/Blueprints/FirstPersonCharacter.FirstPersonCharacter_C|GetFirstPersonCamera (Variables|Default|GetPlayer))))
            (bind _maptoplayer (Timeline|MapToPlayer Play)
              (:Update
                (Variables|Default|Setmap _maptoplayer)
                (Transformation|SetActorLocationAndRotation (Variables|Default|GetPlayer) (Math|Vector|MakeVector _x _y (.Z (Math|Vector|BreakVector (Transformation|GetActorLocation (Variables|Default|GetPlayer))))) (Math|Rotator|FindLookatRotation (Transformation|GetWorldLocation (Variables|Default|GetInteractPointActor)) (Transformation|GetWorldLocation (Variables|Default|GetMesh))) false true)
                (Transformation|SetWorldLocation (Variables|/Game/FirstPersonBP/Blueprints/FirstPersonCharacter.FirstPersonCharacter_C|GetFirstPersonCamera (Variables|Default|GetPlayer)) (Math|Vector|Lerp(Vector) (Math|Vector|MakeVector _x_2 _y_2 (.Z (Math|Vector|BreakVector (Variables|Default|GetcameraPos)))) (Transformation|GetWorldLocation (Variables|Default|GetInteractPointCamera)) (Variables|Default|Getmap)) false false)
                (Variables|/Game/JuegoX/Blueprints/Objects/Interactable.Interactable_C|SetisFocused? (Variables|Default|GetInteractuable) false)))))
        (elif (Variables|/Game/FirstPersonBP/Blueprints/FirstPersonCharacter.FirstPersonCharacter_C|GetplayerInpectingMapa (Variables|Default|GetPlayer))
          (goto _label))))))

(fn ConstructionScript)

(fn CheckInput
  (bind _returnvalue (Game|GetPlayerController 0))
  (if (Variables|/Game/JuegoX/Blueprints/Objects/Interactable.Interactable_C|GetisFocused? (Variables|Default|GetInteractuable))
    (Input|EnableInput (Game|GetPlayerController 0))
    (elif (Variables|/Game/FirstPersonBP/Blueprints/FirstPersonCharacter.FirstPersonCharacter_C|GetplayerInpectingMapa (Variables|Default|GetPlayer))
      (Input|EnableInput _returnvalue)
      (Variables|/Game/JuegoX/Blueprints/Objects/Interactable.Interactable_C|SetinteractionActivated (Variables|Default|GetInteractuable) false)
      (Rendering|SetVisibility (Variables|Default|GetTextRender) false false)
      (else
        (Input|DisableInput _returnvalue)))))

(fn ShowControls
  (if (Utilities|IsValid (Variables|/Game/FirstPersonBP/Blueprints/FirstPersonCharacter.FirstPersonCharacter_C|GetHUD (Variables|Default|Getplayer)))
    _
    (else
      (bind _returnvalue (UserInterface|CreateWidget "/Game/JuegoX/UI/HUD/WB_HUD.WB_HUD_C" (Game|GetPlayerController 0)))
      (Variables|/Game/FirstPersonBP/Blueprints/FirstPersonCharacter.FirstPersonCharacter_C|SetHUD (Variables|Default|Getplayer) _returnvalue)))
  (Rendering|Components|TextRender|SetText (Variables|/Game/JuegoX/UI/HUD/WB_HUD.WB_HUD_C|GetT_Drop (Variables|/Game/FirstPersonBP/Blueprints/FirstPersonCharacter.FirstPersonCharacter_C|GetHUD (Variables|Default|Getplayer))) "to exit")
  (Rendering|Components|TextRender|SetText (Variables|/Game/JuegoX/UI/HUD/WB_HUD.WB_HUD_C|GetT_Action (Variables|/Game/FirstPersonBP/Blueprints/FirstPersonCharacter.FirstPersonCharacter_C|GetHUD (Variables|Default|Getplayer))) "to circle location")
  (Variables|Default|Setwidget_Anim (Variables|/Game/JuegoX/UI/HUD/WB_HUD.WB_HUD_C|GetControls_2_Anim (Variables|/Game/FirstPersonBP/Blueprints/FirstPersonCharacter.FirstPersonCharacter_C|GetHUD (Variables|Default|Getplayer))))
  (if (UserInterface|Viewport|IsinViewport (Variables|/Game/FirstPersonBP/Blueprints/FirstPersonCharacter.FirstPersonCharacter_C|GetHUD (Variables|Default|Getplayer)))
    _
    (else
      (UserInterface|Viewport|AddtoViewport (Variables|/Game/FirstPersonBP/Blueprints/FirstPersonCharacter.FirstPersonCharacter_C|GetHUD (Variables|Default|Getplayer)) 0)))
  (Class|UserWidget|PlayAnimationForward (Variables|/Game/FirstPersonBP/Blueprints/FirstPersonCharacter.FirstPersonCharacter_C|GetHUD (Variables|Default|Getplayer)) (Variables|Default|Getwidget_Anim) 4.0))

(fn HideControls
  (Class|UserWidget|PlayAnimationReverse (Variables|/Game/FirstPersonBP/Blueprints/FirstPersonCharacter.FirstPersonCharacter_C|GetHUD (Variables|Default|Getplayer)) (Variables|Default|Getwidget_Anim) 4.0))

(fn ShowHint
  (params (hint :type Text))
  (if (Utilities|IsValid (Variables|/Game/FirstPersonBP/Blueprints/FirstPersonCharacter.FirstPersonCharacter_C|GetHUD (Variables|Default|Getplayer)))
    _
    (else
      (bind _returnvalue (UserInterface|CreateWidget "/Game/JuegoX/UI/HUD/WB_HUD.WB_HUD_C" (Game|GetPlayerController 0)))
      (Variables|/Game/FirstPersonBP/Blueprints/FirstPersonCharacter.FirstPersonCharacter_C|SetHUD (Variables|Default|Getplayer) _returnvalue)))
  (Rendering|Components|TextRender|SetText (Variables|/Game/JuegoX/UI/HUD/WB_HUD.WB_HUD_C|GetHInt_Text (Variables|/Game/FirstPersonBP/Blueprints/FirstPersonCharacter.FirstPersonCharacter_C|GetHUD (Variables|Default|Getplayer))) hint)
  (Variables|Default|Setwidget_Anim (Variables|/Game/JuegoX/UI/HUD/WB_HUD.WB_HUD_C|GetHint_Anim (Variables|/Game/FirstPersonBP/Blueprints/FirstPersonCharacter.FirstPersonCharacter_C|GetHUD (Variables|Default|Getplayer))))
  (if (UserInterface|Viewport|IsinViewport (Variables|/Game/FirstPersonBP/Blueprints/FirstPersonCharacter.FirstPersonCharacter_C|GetHUD (Variables|Default|Getplayer)))
    _
    (else
      (UserInterface|Viewport|AddtoViewport (Variables|/Game/FirstPersonBP/Blueprints/FirstPersonCharacter.FirstPersonCharacter_C|GetHUD (Variables|Default|Getplayer)) 0)))
  (Class|UserWidget|PlayAnimationForward (Variables|/Game/FirstPersonBP/Blueprints/FirstPersonCharacter.FirstPersonCharacter_C|GetHUD (Variables|Default|Getplayer)) (Variables|Default|Getwidget_Anim) 4.0))

(fn HideInventory
  (bind _returnvalue (Actor|GetActorOfClass "/Game/JuegoX/Blueprints/Objects/OBJ_Taker_KeyChild.OBJ_Taker_KeyChild_C"))
  (Default|HideInventory _returnvalue))