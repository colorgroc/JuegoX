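; Interactable map object that lets the player start and stop inspecting it as part of the map puzzle.
; Tick enables the actor's input only while its Interactuable is focused.
; Interact alternates through a FlipFlop: entering requires an unfinished map puzzle in MyGameInstance, flags the FirstPersonCharacter as inspecting and makes TriggerBox block all.
; Exiting clears that flag and disables TriggerBox collision; both transitions reset focus.
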(event EventTick
  (params (DeltaSeconds :type Float%20%28single-precision%29))
  (bind _returnvalue (Game|GetPlayerController 0))
  (if (Variables|/Game/JuegoX/Blueprints/Objects/Interactable.Interactable_C|GetisFocused? (Variables|Default|GetInteractuable))
    (Input|EnableInput _returnvalue)
    (else
      (Input|DisableInput _returnvalue))))

(event Input|ActionEvents|InputActionInteract
  (params (Key :type Key%20Structure :default "None"))
  (bind _triggerbox (Variables|Default|GettriggerBox))
  (bind _collisioncomponent (Variables|/Script/Engine.TriggerBase|GetCollisionComponent _triggerbox))
  (:Pressed
    (if (Variables|/Game/JuegoX/Blueprints/Objects/Interactable.Interactable_C|GetisFocused? (Variables|Default|GetInteractuable))
      (bind _asfirst_person_character (Utilities|Casting|CastToFirstPersonCharacter (Game|GetPlayerCharacter 0)))
      (Utilities|FlowControl|FlipFlop
        (:A
          (bind _asmy_game_instance (Utilities|Casting|CastToMyGameInstance (Game|GetGameInstance)))
          (if (not (Variables|/Game/JuegoX/Blueprints/MyGameInstance.MyGameInstance_C|GetMapPuzzle_Completed _asmy_game_instance))
            (Variables|/Game/FirstPersonBP/Blueprints/FirstPersonCharacter.FirstPersonCharacter_C|SetplayerInpectingMapa _asfirst_person_character true)
            (Collision|SetCollisionProfileName _collisioncomponent "BlockAll" :!class /Script/Engine.PrimitiveComponent)
            (Variables|/Game/JuegoX/Blueprints/Objects/Interactable.Interactable_C|SetisFocused? (Variables|Default|GetInteractuable) false :!label _label)))
        (:B
          (Variables|/Game/FirstPersonBP/Blueprints/FirstPersonCharacter.FirstPersonCharacter_C|SetplayerInpectingMapa _asfirst_person_character false)
          (Collision|SetCollisionProfileName _collisioncomponent "NoCollision" :!class /Script/Engine.PrimitiveComponent)
          (goto _label))))))

(fn ConstructionScript)