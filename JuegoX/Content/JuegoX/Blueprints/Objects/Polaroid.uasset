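; Polaroid actor that the player can focus and inspect up close, driven by its Interactuable state.
; At BeginPlay it adds a mesh copy with a dynamic outline material, which Tick shows white nearby, red when focused and hidden during inspection.
; Tick enables input only while focused or inspected.
; Inspection plays or reverses a timeline that lerps position, player-facing rotation and doubled scale, then can fade the E prompt when finished.
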(event EventBeginPlay
  (bind _mesh (Variables|Character|GetMesh))
  (|CallParentFunction)
  (bind _returnvalue (AddComponent|AddStaticMeshComponent true (Transformation|GetWorldTransform (Variables|Character|GetMesh))))
  (Transformation|AttachComponentToComponent _returnvalue (Variables|Character|GetMesh) "None" "KeepRelative" "KeepRelative" "KeepRelative" true)
  (Components|StaticMesh|SetStaticMesh _returnvalue (Variables|/Script/Engine.StaticMeshComponent|GetStaticMesh _mesh))
  (Rendering|Material|SetMaterial _returnvalue 0 (Rendering|Material|GetMaterial _mesh 0))
  (bind _returnvalue_2 (Rendering|Material|CreateDynamicMaterialInstance _returnvalue 0 "/Game/JuegoX/Materials/Outline_ObjectsHided.Outline_ObjectsHided" "None" :!class /Script/Engine.PrimitiveComponent))
  (Variables|Default|SetMaterialHighlight _returnvalue_2)
  (Variables|Default|Setinit%20scale (Transformation|GetActorScale3D)))

(event EventTick
  (params (DeltaSeconds :type Float%20%28single-precision%29))
  (bind _returnvalue (Game|GetPlayerController 0))
  (bind _materialhighlight (Variables|Default|GetMaterialHighlight))
  (bind _materialhighlight_2 (Variables|Default|GetMaterialHighlight))
  (if (Variables|/Game/JuegoX/Blueprints/Objects/Interactable.Interactable_C|GetisInspectingIt (Variables|Default|GetInteractuable))
    (Rendering|Material|SetScalarParameterValue _materialhighlight "Scale" 0.0 :!class /Script/Engine.MaterialInstanceDynamic)
    (Input|EnableInput _returnvalue :!label _label)
    (elif (Variables|/Game/JuegoX/Blueprints/Objects/Interactable.Interactable_C|GetisFocused? (Variables|Default|GetInteractuable))
      (Rendering|Material|SetScalarParameterValue _materialhighlight "Scale" 0.5 :!class /Script/Engine.MaterialInstanceDynamic)
      (Rendering|Material|SetVectorParameterValue _materialhighlight "Color" "(R=1.000000,G=0.000000,B=0.000000,A=1.000000)" :!class /Script/Engine.MaterialInstanceDynamic)
      (goto _label)
      (else
        (Input|DisableInput _returnvalue)
        (Math|Float|CompareFloat (Transformation|GetDistanceTo (Variables|Default|Getplayer)) (Variables|/Game/JuegoX/Blueprints/Objects/Interactable.Interactable_C|GetDistance%20to%20Glow (Variables|Default|GetInteractuable))
          (:>
            (Rendering|Material|SetScalarParameterValue _materialhighlight_2 "Scale" 0.0 :!class /Script/Engine.MaterialInstanceDynamic))
          (:==
            (Rendering|Material|SetScalarParameterValue _materialhighlight_2 "Scale" 0.5 :!class /Script/Engine.MaterialInstanceDynamic :!label _label_2))
          (:<
            (goto _label_2)))
        (Rendering|Material|SetVectorParameterValue _materialhighlight_2 "Color" "(R=1.000000,G=1.000000,B=1.000000,A=1.000000)" :!class /Script/Engine.MaterialInstanceDynamic)))))

(event EventInspection
  (if (Variables|/Game/JuegoX/Blueprints/Objects/Interactable.Interactable_C|GetisInspectingIt (Variables|Default|GetInteractuable))
    (CallFunction|EndInspection)
    (bind _object_moved (Timeline|Polaroid%20Inspect Reverse)
      (:Update
        (CallFunction|UpdateLocationPolaroid _object_moved))
      (:Finished
        (if (Variables|Default|GetableToFadeE) ; E appears when the animation finishes
          (Variables|/Game/JuegoX/Blueprints/Objects/Interactable.Interactable_C|SetfadeE (Variables|Default|GetInteractuable) true))))
    (else
      (CallFunction|BeginInspection)
      (Timeline|Polaroid%20Inspect Play))))

(fn ConstructionScript
  (|CallParentFunction))

(fn UpdateLocationPolaroid
  (params (Timeline%20Value :type Float%20%28single-precision%29%20%28by%20ref%29))
  (bind _init_scale (Variables|Default|Getinit%20scale))
  (bind _interactuable (Variables|Default|GetInteractuable))
  (Variables|Default|Setrotation "0, 0, 0") ; Rotacion pa que mire enfrente bien
  (Transformation|SetActorLocation (Math|Vector|Lerp(Vector) (Variables|/Game/JuegoX/Blueprints/Objects/Interactable.Interactable_C|GetinitialPos _interactuable) (Variables|/Game/JuegoX/Blueprints/Objects/Interactable.Interactable_C|GetinspectionPoint _interactuable) Timeline%20Value) false false)
  (Transformation|SetActorRotation (Math|Rotator|Lerp(Rotator) (Variables|/Game/JuegoX/Blueprints/Objects/Interactable.Interactable_C|GetinitialRot _interactuable) (Math|Rotator|FindLookatRotation (Transformation|GetActorLocation) (Transformation|GetActorLocation (Variables|Default|Getplayer))) Timeline%20Value))
  (Transformation|SetActorScale3D (Math|Vector|Lerp(Vector) _init_scale (* _init_scale 2.0) Timeline%20Value)))