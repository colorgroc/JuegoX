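; Interactable dresser drawer that opens and closes with sound when the player inspects it.
; Tick enables player input only while its Interactuable component is focused.
; The Inspect action alternates open and close sounds through a FlipFlop that also presets IsOpen, then clears focus after calling Interact.
; Interact reads IsOpen to play the Anim sequence forward or in reverse, then toggles the flag.
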(event EventTick
  (params (DeltaSeconds :type Float%20%28single-precision%29))
  (bind _returnvalue (Game|GetPlayerController 0))
  (if (Variables|/Game/JuegoX/Blueprints/Objects/Interactable.Interactable_C|GetisFocused? (Variables|Default|GetInteractuable))
    (Input|EnableInput _returnvalue)
    (else
      (Input|DisableInput _returnvalue))))

(event Input|ActionEvents|InputActionInspect
  (params (Key :type Key%20Structure))
  (:Pressed
    (if (Variables|/Game/JuegoX/Blueprints/Objects/Interactable.Interactable_C|GetisFocused? (Variables|Default|GetInteractuable))
      (Utilities|FlowControl|FlipFlop
        (:A
          (Variables|Default|SetisOpen? false)
          (Audio|PlaySound2D "/Game/Soniditos/392770__danialarcon0698__abre-cajon.392770__danialarcon0698__abre-cajon" 1.0 1.0 0.0 0 0))
        (:B
          (Variables|Default|SetisOpen? true)
          (Audio|PlaySound2D "/Game/Soniditos/237379__squareal__cutlery-drawer-closing-01.237379__squareal__cutlery-drawer-closing-01" 1.0 1.0 0.0 0 0)))
      (CallFunction|Interact)
      (Variables|/Game/JuegoX/Blueprints/Objects/Interactable.Interactable_C|SetisFocused? (Variables|Default|GetInteractuable) false))))

(fn ConstructionScript)

(fn Interact
  (bind _anim (Variables|Default|GetAnim))
  (bind _sequenceplayer (Variables|/Script/ActorSequence.ActorSequenceComponent|GetSequencePlayer _anim))
  (if (Variables|Default|GetisOpen?)
    (Class|MovieSceneSequencePlayer|PlayReverse _sequenceplayer)
    (Variables|Default|SetisOpen? false)
    (else
      (Sequencer|Player|Play _sequenceplayer :!class /Script/MovieScene.MovieSceneSequencePlayer)
      (Variables|Default|SetisOpen? true))))